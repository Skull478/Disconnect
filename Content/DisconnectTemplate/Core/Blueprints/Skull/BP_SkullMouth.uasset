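; Replicated skull mouth actor that periodically swings its mesh open and back while spawning falling gear particles.
; On BeginPlay the server slows both timelines and starts a looping timer for the mouth motion.
; The timelines interpolate a rotation variable, applied to the static mesh through its OnRep so clients follow.
; When the first swing finishes, an MC event spawns the gear Niagara effect at a marker component and the reverse timeline plays.
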(event `self.ReceiveBeginPlay`
  ; FIX POUR QUE CA MARCHE SERV ET CLIENT ET LE RETOUR ET BUG
  (`/Engine/EditorBlueprintResources/ActorMacros.Switch Has Authority`
    (:`Authority`
      (`TimelineComponent.SetPlayRate` (`self.T_MOUTH`) (/ 1.0 2.0))
      (`TimelineComponent.SetPlayRate` (`self.T_MouthReverse`) (/ 1.0 2.0))
      (`KismetSystemLibrary.K2_SetTimerDelegate` (delegate `MOUTH`) 10.0 true true))))

(event `MOUTH`
  ; FIX POUR QUE CA MARCHE SERV ET CLIENT ET LE RETOUR ET BUG
  (bind (_direction _alpha) (`Timeline|T_MOUTH` :!via `PlayFromStart`)
    (:`Update`
      (set `self.MouthRotation` (`KismetMathLibrary.RLerp` (struct :`Yaw` 180.0 :`Roll` 170.0) (struct :`Yaw` 180.0 :`Roll` 200.0) _alpha true)))
    (:`Finished`
      (`self.MC_SpawnNiagara` (`SceneComponent.K2_GetComponentLocation` (`self.NiagaraSpawnEffect`)))
      (bind (_direction_2 _alpha_2) (`Timeline|T_MouthReverse` :!via `PlayFromStart`)
        (:`Update`
          (set `self.MouthRotation` (`KismetMathLibrary.RLerp` (struct :`Yaw` 180.0 :`Roll` 200.0) (struct :`Yaw` 180.0 :`Roll` 170.0) _alpha_2 true)))))))

(event `MC_SpawnNiagara`
  (params (Location :type "Vector Structure"))
  ; FIX POUR QUE CA MARCHE SERV ET CLIENT ET LE RETOUR ET BUG
  (`NiagaraFunctionLibrary.SpawnSystemAtLocation` "/Game/DisconnectTemplate/VFX/Skull/NS_GearFalling.NS_GearFalling" Location))

(fn `OnRep_MouthRotation`
  (`SceneComponent.K2_SetRelativeRotation` (`self.StaticMesh`) (`self.MouthRotation`) false false))

(fn `UserConstructionScript`)