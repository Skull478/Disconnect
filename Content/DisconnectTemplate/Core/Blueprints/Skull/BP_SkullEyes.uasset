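; BP_SkullEyes is a skull-eyes actor whose Arrow component turns to face the Disconnect player character.
; After a startup delay, a fast looping timer computes a look-at rotation, which a RepNotify applies to the Arrow.
; If the player reference becomes invalid, it searches again, clears the timer and restarts it after a short wait.
; An optional Flicker flag swaps in a flickering emissive searchlight material at construction.
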(event `self.ReceiveBeginPlay`
  (`KismetSystemLibrary.Delay` 10.0)
  (bind _returnvalue (`GameplayStatics.GetActorOfClass` "/Game/DisconnectTemplate/Core/Blueprints/Character/Game/Player/BP_DisconnectPlayer_Character.BP_DisconnectPlayer_Character_C"))
  (bind _output_get (set `self.PLAYER CHARA` _returnvalue))
  (`/Engine/EditorBlueprintResources/StandardMacros.IsValid` _output_get
    (:`Is Valid`
      (bind _returnvalue_2 (`KismetSystemLibrary.K2_SetTimerDelegate` (delegate `LOOK_AT_PLAYER`) 0.1 true true :!label _label)))))

(event `LOOK_AT_PLAYER`
  (`self.PLAYER CHARA`
    (:`then`
      (set `self.RotationToLookAtPlayer` (`KismetMathLibrary.FindLookAtRotation` (`SceneComponent.K2_GetComponentLocation` (`self.Arrow`)) (`self.K2_GetActorLocation` (`self.PLAYER CHARA`)))))
    (:`else`
      (bind _returnvalue (`GameplayStatics.GetActorOfClass` "/Game/DisconnectTemplate/Core/Blueprints/Character/Game/Player/BP_DisconnectPlayer_Character.BP_DisconnectPlayer_Character_C"))
      (set `self.PLAYER CHARA` _returnvalue)
      (`KismetSystemLibrary.K2_ClearAndInvalidateTimerHandle` (stale `self.ReceiveBeginPlay` _returnvalue_2))
      (`KismetSystemLibrary.Delay` 1.0)
      (goto _label))))

(fn `OnRep_RotationToLookAtPlayer`
  (`SceneComponent.K2_SetWorldRotation` (`self.Arrow`) (`self.RotationToLookAtPlayer`) false false))

(fn `UserConstructionScript`
  (if (`self.bFlicker?`)
    (`PrimitiveComponent.SetMaterial` (`self.StaticMesh1`) 0 "/Game/DisconnectTemplate/MaterialLibrary/Instance/Emssive/MI_SearchLight_Ligh_EmissiveFlicker.MI_SearchLight_Ligh_EmissiveFlicker")))