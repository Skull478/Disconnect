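; Tool actor that scatters randomized stacks of tires as instanced static meshes within a radius.
; Generate_Stack checks stack count against packing area, then retries random shape-scaled positions until sphere traces find no overlap.
; Each tire drops by sphere trace onto the surface below, with random scale and rotation; only tires per stack uses the random stream.
; The actor temporarily moves to the world origin during generation, then its transform is restored.
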(event `Generate_Stack`
  (bind _spawnradius (`self.SpawnRadius`))
  (bind _tireradius (`self.TireRadius`))
  (bind (_tireposition_x _tireposition_y) (`KismetMathLibrary.BreakVector` (`self.TirePosition`)))
  (`KismetSystemLibrary.FlushPersistentDebugLines`)
  (if (< (`self.NumStack`) (* (/ (* _spawnradius _spawnradius (`KismetMathLibrary.GetPI`)) (* _tireradius _tireradius (`KismetMathLibrary.GetPI`))) (`self.PackingTolerence`)))
    (`InstancedStaticMeshComponent.ClearInstances` (`self.ISM_Tire`))
    ; Put Actor in Local Space
    (set `self.ActorTransform` (`self.GetTransform`))
    (`self.K2_SetActorRotation` (struct))
    (`self.K2_SetActorLocation` (0.0 0.0 0.0))
    (for _ (range 1 (+ (`self.NumStack`) 1))
      ; Loop until we find a stack location that doesn't overlap another
      (bind _collisiondetected (`self.GenerateRandomStackLocation`))
      (set `self.CollisionDetected` _collisiondetected)
      (while (`self.CollisionDetected`)
        (bind _collisiondetected_2 (`self.GenerateRandomStackLocation`))
        (set `self.CollisionDetected` _collisiondetected_2))
      (for _index (range 1 (+ (`KismetMathLibrary.RandomIntegerInRangeFromStream` (`self.Stream`) (`self.MinTirePerStack`) (`self.MaxTirePerStack`)) 1))
        ; Get Z Position
        (bind _outhit (`KismetSystemLibrary.SphereTraceSingle` (`KismetMathLibrary.MakeVector` _tireposition_x _tireposition_y (`self.TraceStartHeight`)) (`KismetMathLibrary.MakeVector` _tireposition_x _tireposition_y) (* (`self.TireRadius`) (`self.ClippingTolerance`)) "TraceTypeQuery1" false (`self.GetOverlappingActors` null) "None" false))
        (set `self.TirePosition` (`.ImpactPoint` (`GameplayStatics.BreakHitResult` _outhit)))
        (set `self.TireScale` (`KismetMathLibrary.Conv_DoubleToVector` (`KismetMathLibrary.RandomFloatInRange` (select `bool` (== _index 1) :`false` (`self.ScaleMin`) :`true` 1.0) (`self.ScaleMax`))))
        (set `self.TireRotation` (`KismetMathLibrary.MakeRotator` (`KismetMathLibrary.RandomFloatInRange` 0.0 (.roll (`self.RandomRotation`))) (`KismetMathLibrary.RandomFloatInRange` 0.0 (.pitch (`self.RandomRotation`))) (`KismetMathLibrary.RandomFloatInRange` 0.0 (.yaw (`self.RandomRotation`)))))
        (`InstancedStaticMeshComponent.AddInstance` (`self.ISM_Tire`) (`KismetMathLibrary.MakeTransform` (`self.TirePosition`) (`self.TireRotation`) (`self.TireScale`)) true)
        (`StaticMeshComponent.SetStaticMesh` (`self.ISM_Tire`) (`self.SM_StaticMesh`))))
    ; Restore Actor to World Space
    (`self.K2_SetActorLocation` (.location (`self.ActorTransform`)))
    (`self.K2_SetActorRotation` (.rotation (`self.ActorTransform`)))
    (`self.SetActorScale3D` (.scale (`self.ActorTransform`)))
    (else
      (`KismetSystemLibrary.PrintText` "ERROR - Radius too small to acomodate number of stacks" true true (struct :`R` 1.0 :`G` 0.241012 :`A` 1.0)))))

(fn `UserConstructionScript`
  (locals (L_ActorTransform :type "Transform Structure" :default "0.000000,0.000000,0.000000|0.000000,0.000000,0.000000|1.000000,1.000000,1.000000") (L_TirePosition :type "Vector Structure" :default (0.0 0.0 100.0))))