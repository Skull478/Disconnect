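; Test Blueprint that builds a physics-constrained chain of links in its construction script, using a spline and an EndPoint.
; Each spline point gets a HISM component holding one Maille1 instance, rotated toward EndPoint.
; For each point, static mesh links step from SMChainMaille along the EndPoint direction, spaced by its length over NumOfMaille.
; Left and right physics constraints join each link to the previous one.
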(fn `CreatePC`
  (params (Location :type "Vector Structure") (Rotation :type "Rotator Structure") (Scale :type "Vector Structure") (Component1 :type "StaticMeshComponent Object Reference") (Component2 :type "StaticMeshComponent Object Reference") (LeftPC :type Boolean))
  (bind _returnvalue (`KismetMathLibrary.GetRightVector` Rotation))
  (bind _returnvalue_2 (`AddComponent|NODE_AddPhysicsConstraintComponent-1` :`RelativeTransform` (`KismetMathLibrary.MakeTransform` (+ (* (`KismetMathLibrary.SelectVector` (* _returnvalue -1.0) _returnvalue LeftPC) 70.0) Location) Rotation Scale)))
  (`PhysicsConstraintComponent.SetConstrainedComponents` _returnvalue_2 Component1 "None" Component2 "None"))

(fn `CreateStaticMesh`
  (params (Location :type "Vector Structure") (Rotation :type "Rotator Structure") (Scale :type "Vector Structure"))
  (returns (ReturnValue :type "StaticMeshComponent Object Reference") (Transform :type "Transform Structure"))
  (bind _returnvalue (`KismetMathLibrary.MakeTransform` (+ Location (* (`KismetMathLibrary.GetDirectionUnitVector` (0.0 0.0 0.0) (`self.EndPoint`)) (/ (`KismetMathLibrary.VSize` (`self.EndPoint`)) (`self.NumOfMaille`)))) Rotation Scale))
  (bind _returnvalue_2 (`AddComponent|NODE_AddStaticMeshComponent-1` :`RelativeTransform` _returnvalue))
  (return _returnvalue_2 _returnvalue))

(fn `UserConstructionScript`
  (locals (L_Index :type Integer) (L_HISM_FirstLink :type "HierarchicalInstancedStaticMeshComponent Object Reference"))
  (bind _last_link (`self.Last_Link`))
  (for _index (range (`SplineComponent.GetNumberOfSplinePoints` (`self.Spline`)))
    (set `local.L_Index` _index)
    (bind _returnvalue (`AddComponent|NODE_AddHierarchicalInstancedStaticMeshComponent-0`))
    (bind _output_get (set `local.L_HISM_FirstLink` _returnvalue))
    (`StaticMeshComponent.SetStaticMesh` _output_get (`self.Maille_1`))
    (set `self.StartLocation` (`SplineComponent.GetLocationAndTangentAtSplinePoint` (`self.Spline`) (`local.L_Index`) "Local"))
    (`InstancedStaticMeshComponent.AddInstance` (`local.L_HISM_FirstLink`) (`KismetMathLibrary.MakeTransform` (`self.StartLocation`)) false)
    (`SceneComponent.K2_SetRelativeRotation` (`local.L_HISM_FirstLink`) (`KismetMathLibrary.FindLookAtRotation` (0.0 0.0 0.0) (`self.EndPoint`)) false false)
    (set `self.Last_Link` (`self.SM_ChainMaille`))
    (for _ (range (+ (`self.NumOfMaille`) 1))
      (bind (_returnvalue_2 _transform) (`self.CreateStaticMesh` (.location (`SceneComponent.GetRelativeTransform` _last_link)) (.rotation (`SceneComponent.GetRelativeTransform` _last_link)) (.scale (`SceneComponent.GetRelativeTransform` _last_link))))
      (bind _location (.location _transform))
      (bind _rotation (.rotation _transform))
      (bind _scale (.scale _transform))
      (`self.CreatePC` _location _rotation _scale _returnvalue_2 _last_link true)
      (`self.CreatePC` _location _rotation _scale _returnvalue_2 _last_link)
      (set `self.Last_Link` _returnvalue_2))))