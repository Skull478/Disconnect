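; Spline-driven mover that slides a row of repeated meshes along a spline, apparently for a garage door, given its opening sound.
; UpdateSpline calls MC_UPDATE and posts the Wwise sound; a timeline then drives Distance along the spline.
; Each update, and the construction script, rebuilds HISM instances spaced by mesh bounds on the chosen axis.
; Instance rotation comes from a per-spline-point array rather than the spline tangent.
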(event `MC_UPDATE`
  (set `self.Distance` 0.0)
  (`self.Update`))

(event `UpdateSpline`
  (`self.MC_UPDATE`)
  (`AkGameObject.PostAssociatedAkEvent` :`self` (`self.Play_OBJ_GarageDoor_open`)))

(event `Update`
  (bind (_direction _alpha) (`Timeline|Timeline` :!via `PlayFromStart`)
    (:`Update`
      (set `self.Distance` (`KismetMathLibrary.Lerp` 0.0 (`SplineComponent.GetSplineLength` (`self.Spline`)) _alpha))
      (`self.SPLINE_UPDATE`))))

(fn `OnRep_Distance`)

(fn `SPLINE_UPDATE`
  (locals (L_MeshSize :type "Vector Structure") (L_TotalDistance :type "Float (single-precision)") (L_DistanceForSplinePoint :type "Array of Float (double-precision)") (L_DistanceCurrentToDeterminePoint :type "Float (double-precision)") (L_IndexStop :type Integer))
  (bind (_returnvalue_min _returnvalue_max) (break `Box` (`StaticMesh.GetBoundingBox` (`self.Mesh`))))
  (bind _x (.x (* (`SplineComponent.GetNumberOfSplinePoints` (`self.Spline`)) (`local.L_MeshSize`))))
  (`InstancedStaticMeshComponent.ClearInstances` (`self.HISM_Mesh`))
  (`self.Mesh`
    (:`then`
      (set `local.L_MeshSize` (- _returnvalue_max _returnvalue_min))
      (`StaticMeshComponent.SetStaticMesh` (`self.HISM_Mesh`) (`self.Mesh`))
      (set `self.Distance` (`KismetMathLibrary.FClamp` (`self.Distance`) 0.0 (- (`SplineComponent.GetSplineLength` (`self.Spline`)) (* (select `EAxis` (`self.AxesSize`) :`None` _x :`X` _x :`Y` (.y (* (`SplineComponent.GetNumberOfSplinePoints` (`self.Spline`)) (`local.L_MeshSize`))) :`Z` (.z (* (`SplineComponent.GetNumberOfSplinePoints` (`self.Spline`)) (`local.L_MeshSize`)))) 5.0))))
      (set `local.L_TotalDistance` 0.0)
      (`KismetArrayLibrary.Array_Clear` (`local.L_DistanceForSplinePoint`))
      (for _index (range (`SplineComponent.GetNumberOfSplinePoints` (`self.Spline`)))
        (bind _output_get (set `local.L_TotalDistance` (+ (`SplineComponent.GetDistanceAlongSplineAtSplinePoint` (`self.Spline`) _index) (`local.L_TotalDistance`))))
        (`KismetArrayLibrary.Array_Add` (`local.L_DistanceForSplinePoint`) _output_get))
      (for _index_2 (range (`self.NumberOfMesh`))
        (set `local.L_IndexStop` 0)
        (for (_array_element _array_index) (`local.L_DistanceForSplinePoint`)
          (bind _x_2 (.x (* _index_2 (`local.L_MeshSize`))))
          (bind _returnvalue (+ (`self.Distance`) (select `EAxis` (`self.AxesSize`) :`None` _x_2 :`X` _x_2 :`Y` (.y (* _index_2 (`local.L_MeshSize`))) :`Z` (.z (* _index_2 (`local.L_MeshSize`))))))
          (set `local.L_DistanceCurrentToDeterminePoint` _returnvalue)
          (if (< _array_element (`local.L_DistanceCurrentToDeterminePoint`))
            (set `local.L_IndexStop` _array_index)))
        (`InstancedStaticMeshComponent.AddInstance` (`self.HISM_Mesh`) (`KismetMathLibrary.MakeTransform` (.location (`SplineComponent.GetTransformAtDistanceAlongSpline` (`self.Spline`) _returnvalue "Local" false)) (`|GetArrayItem` (`self.RotationForEachSplinePoint`) (`local.L_IndexStop`))) false))
      (return))
    (:`else`
      (return))))

(fn `UserConstructionScript`
  (locals (L_Length :type "Float (double-precision)") (L_MeshSize :type "Vector Structure") (L_TotalDistance :type "Float (single-precision)" :default 0.0) (L_DistanceForSplinePoint :type "Array of Float (double-precision)") (L_DistanceCurrentToDeterminePoint :type "Float (double-precision)") (L_IndexStop :type Integer))
  (`self.SPLINE_UPDATE`))