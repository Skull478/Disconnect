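; Scatter tool that drops physics-simulated static mesh actors at random points inside a box on BeginPlay, using no HISM components despite its name.
; It builds a spawn list from per-mesh amounts and seeded random rotation and scale, retrying trace-blocked points and offsetting height by index.
; The list is optionally shuffled, then spawned as movable actors with mass and damping overrides.
; Four wall components are destroyed after a short delay.
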(event `self.ReceiveBeginPlay`
  (bind _meshtospawn (`self.MeshToSpawn`))
  (bind (_spawnpoint_x _spawnpoint_y) (`KismetMathLibrary.BreakVector` (`self.SpawnPoint`)))
  (bind _spawnradius (`self.SpawnRadius`))
  (bind _spawnmeshes (`self.SpawnMeshes`))
  (bind _damping (`self.Damping`))
  (bind _collisiontracerange (`self.CollisionTraceRange`))
  (bind (_mesh _scale_min _scale_max _b_scalerandom_ _rotation_min _rotation_max) (break `/Game/DisconnectTemplate/Core/Blueprints/Tools/S_ScatterMeshes` (`self.Mesh`)))
  (bind (_returnvalue_x _returnvalue_y _returnvalue_z) (`KismetMathLibrary.BreakVector` (`SceneComponent.K2_GetComponentLocation` (`self.SpawnRadius`))))
  (bind _returnvalue (`KismetMathLibrary.Conv_IntToDouble` (`self.Index`)))
  (bind _returnvalue_2 (/ _collisiontracerange 5.0))
  (bind _returnvalue_3 (+ (`self.K2_GetActorLocation`) (`self.SpawnPoint`)))
  (bind _returnvalue_4 (`KismetMathLibrary.RandomFloatInRangeFromStream` (`self.RandomStream`) _scale_min _scale_max))
  (`|ExecutionSequence`
    (:`then_0`
      ; Initialisation
      (`KismetArrayLibrary.Array_Clear` (`self.SpawnMeshes`))
      (`KismetMathLibrary.SetRandomStreamSeed` (`self.RandomStream`) (`KismetMathLibrary.RandomIntegerInRange` 111111 999999))
      ; Loops
      (for _index (range (+ (`KismetArrayLibrary.Array_Length` _meshtospawn) 1))
        (bind _output (`|GetArrayItem` _meshtospawn _index))
        (set `self.Mesh` _output)
        (bind ((`Mesh_10_1BDBB79B4A7B612B086FCA98234465C1` _mesh_2) (`Amount_22_836F5B7D496B106EE697638EFC5C3F0A` _amount)) (break `/Game/DisconnectTemplate/Core/Blueprints/Tools/S_ScatterMeshes` _output))
        (set `self.StaticMeshActor` _mesh_2)
        (set `self.Index` _index)
        (for _ (range (+ _amount 1))
          (set `self.SpawnPoint` (`KismetMathLibrary.RandomPointInBoundingBoxFromStream` (`self.RandomStream`) (`SceneComponent.K2_GetComponentLocation` _spawnradius) (- (`BoxComponent.BoxExtent` _spawnradius) (`KismetMathLibrary.MakeVector` _returnvalue _returnvalue _returnvalue))) :!label _label)
          (bind (_outhit _returnvalue_5) (`KismetSystemLibrary.SphereTraceSingle` :`Start` (+ (`KismetMathLibrary.MakeVector` 0.0 0.0 _collisiontracerange) _returnvalue_3) :`End` (+ (`KismetMathLibrary.MakeVector` 0.0 0.0 (/ _returnvalue_2 1.0)) _returnvalue_3) :`Radius` _returnvalue_2 :`TraceChannel` "TraceTypeQuery1" :`bTraceComplex` true :`DrawDebugType` (select `bool` (`self.Collision_Debug`) :`true` "ForDuration" :!type "EDrawDebugTrace Enum")))
          (if _returnvalue_5
            (`/Engine/EditorBlueprintResources/StandardMacros.Do N` 0 :!label _label_2
              (:`Exit`
                (goto _label)))
            (else
              (`|ExecutionSequence`
                (:`then_0`
                  (goto _label_2 :!via `Reset`))
                (:`then_1`
                  (`KismetArrayLibrary.Array_Add` (`self.SpawnMeshes`) (make `/Game/DisconnectTemplate/Core/Blueprints/Tools/S_SpawnActor` (`self.StaticMeshActor`) (`KismetMathLibrary.MakeTransform` (`KismetMathLibrary.MakeVector` _spawnpoint_x _spawnpoint_y (+ _returnvalue_z (* (`self.Height`) (`self.Index`)))) (`KismetMathLibrary.MakeRotator` 0.0 0.0 (`KismetMathLibrary.RandomFloatInRangeFromStream` (`self.RandomStream`) _rotation_min _rotation_max)) (`KismetMathLibrary.MakeVector` _returnvalue_4 _returnvalue_4 _returnvalue_4))))))))))
      (if (`self.RandomOrder`)
        (`KismetArrayLibrary.Array_Shuffle` _spawnmeshes))
      (for _array_element _spawnmeshes
        (bind (_mesh_3 _mesh_transform) (break `/Game/DisconnectTemplate/Core/Blueprints/Tools/S_SpawnActor` _array_element))
        (bind _returnvalue_6 (`|SpawnActorFromClass` "/Script/Engine.StaticMeshActor" _mesh_transform "Undefined" "MultiplyWithRoot" null null))
        (`StaticMeshActor.SetMobility` _returnvalue_6 "Movable")
        (bind _staticmeshcomponent (`StaticMeshActor.StaticMeshComponent` _returnvalue_6))
        (`StaticMeshComponent.SetStaticMesh` _staticmeshcomponent _mesh_3)
        (`PrimitiveComponent.SetSimulatePhysics` _staticmeshcomponent true)
        (`PrimitiveComponent.SetEnableGravity` _staticmeshcomponent true)
        (`PrimitiveComponent.SetMassOverrideInKg` _staticmeshcomponent "None" (`self.Mass in Kg`) true)
        (bind _staticmeshcomponent_2 (`StaticMeshActor.StaticMeshComponent` _returnvalue_6))
        (`PrimitiveComponent.SetLinearDamping` _staticmeshcomponent_2 _damping)
        (`PrimitiveComponent.SetAngularDamping` _staticmeshcomponent_2 _damping)))
    (:`then_1`
      ; Delete Wall
      (`KismetSystemLibrary.Delay` 5.0)
      (`ActorComponent.K2_DestroyComponent` (`self.Wall`))
      (`ActorComponent.K2_DestroyComponent` (`self.Wall1`))
      (`ActorComponent.K2_DestroyComponent` (`self.Wall2`))
      (`ActorComponent.K2_DestroyComponent` (`self.Wall3`)))))

(fn `UserConstructionScript`)