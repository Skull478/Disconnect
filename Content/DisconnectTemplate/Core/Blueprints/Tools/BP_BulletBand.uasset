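; BP_BulletBand is a tool Blueprint that builds a row of repeated bullet band meshes in the construction script.
; The spline's segment count sets how many instances are added to two instanced static mesh components, one using SMBulletBand and the other NewMesh.
; Both are spaced along X by the SMBulletBand bounding-box width, so the row stays straight rather than following the spline's curve.
; The event graph has no active logic.
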(fn `UserConstructionScript`
  (bind _sm_bulletband (`self.SM_BulletBand`))
  (bind (_returnvalue_min _returnvalue_max) (break `Box` (`StaticMesh.GetBoundingBox` _sm_bulletband)))
  (for _index (range (`SplineComponent.GetNumberOfSplineSegments` (`self.Spline`)))
    (`StaticMeshComponent.SetStaticMesh` (`self.InstancedStaticMesh`) _sm_bulletband)
    (bind _returnvalue (* (.x (- _returnvalue_max _returnvalue_min)) _index))
    (`InstancedStaticMeshComponent.AddInstance` (`self.InstancedStaticMesh`) (`KismetMathLibrary.MakeTransform` (`KismetMathLibrary.MakeVector` _returnvalue)) false)
    (`StaticMeshComponent.SetStaticMesh` (`self.InstancedStaticMesh1`) (`self.New Mesh`))
    (`InstancedStaticMeshComponent.AddInstance` (`self.InstancedStaticMesh1`) (`KismetMathLibrary.MakeTransform` (`KismetMathLibrary.MakeVector` _returnvalue)) false)))