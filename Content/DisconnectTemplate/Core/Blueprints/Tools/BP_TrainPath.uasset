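; BP_TrainPath is a placeable spline actor that builds train rail geometry along its spline.
; The construction script divides the spline length by MeshSize and adds one collision-enabled spline mesh using the Rails mesh per whole segment.
; Segment positions and tangents are sampled in local space, with tangent length clamped to MeshSize.
; It has no runtime logic, and any remainder shorter than one segment stays uncovered.
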(fn `UserConstructionScript`
  (locals (L_SplineMeshComp :type "SplineMeshComponent Object Reference"))
  (bind _spline (`self.Spline`))
  (bind _meshsize (`self.MeshSize`))
  (bind _l_splinemeshcomp (`local.L_SplineMeshComp`))
  (for _index (range (`KismetMathLibrary.FTrunc` (/ (`SplineComponent.GetSplineLength` (`self.Spline`)) (`self.MeshSize`))))
    (bind _returnvalue (`AddComponent|NODE_AddSplineMeshComponent-0`))
    (bind _output_get (set `local.L_SplineMeshComp` _returnvalue))
    (bind _returnvalue_2 (* _index _meshsize))
    (bind _returnvalue_3 (+ _returnvalue_2 _meshsize))
    (`SplineMeshComponent.SetStartAndEnd` _output_get (`SplineComponent.GetLocationAtDistanceAlongSpline` _spline _returnvalue_2 "Local") (`KismetMathLibrary.ClampVectorSize` (`SplineComponent.GetTangentAtDistanceAlongSpline` _spline _returnvalue_2 "Local") 0.0 (`self.MeshSize`)) (`SplineComponent.GetLocationAtDistanceAlongSpline` _spline _returnvalue_3 "Local") (`KismetMathLibrary.ClampVectorSize` (`SplineComponent.GetTangentAtDistanceAlongSpline` _spline _returnvalue_3 "Local") 0.0 (`self.MeshSize`)) true)
    (`PrimitiveComponent.SetCollisionEnabled` _l_splinemeshcomp "QueryAndPhysics")
    (`StaticMeshComponent.SetStaticMesh` _l_splinemeshcomp (`self.Rails`))))