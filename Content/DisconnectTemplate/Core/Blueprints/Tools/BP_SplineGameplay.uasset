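; Spline tool actor that builds seeded-random meshes along a spline in the construction script, optionally visible only to Dev-role players.
; HISM mode makes points linear, fills segments with instances, stretches the last piece to fit and places optional elbows at interior points.
; Otherwise it bends spline mesh components along the curve.
; An optional glitch pass sets material, custom stencil and tag, while a server role event multicasts HISM visibility.
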(event `self.ReceiveBeginPlay`
  (`KismetSystemLibrary.DelayUntilNextTick`)
  (if (`self.bSplineOnlyVisibleByDev?`)
    (`/Engine/EditorBlueprintResources/ActorMacros.Switch Has Authority`
      (:`Authority`
        (bind _ref (message `/Game/DisconnectTemplate/Core/Library/BPI_Game_GameMode.GetGameModeRef` (`GameplayStatics.GetGameMode`)))
        (`/Engine/EditorBlueprintResources/StandardMacros.IsValid` _ref
          (:`Is Valid`
            (add `/Game/DisconnectTemplate/Core/Blueprints/Character/Game/BP_DisconnectGame_GameMode.OnRoleGived` _ref (delegate `TSRV_RoleGived`)))
          (:`Is Not Valid`
            (`KismetSystemLibrary.PrintString` "not valid ref game mode" true false (struct :`R` 0.066372 :`B` 1.0 :`A` 1.0) 10.0)))))))

(event `TSRV_RoleGived`
  (`self.MC_ShowOnlyForDev`)
  (`KismetSystemLibrary.PrintString` "trigger mc" true false (struct :`R` 0.066372 :`B` 1.0 :`A` 1.0) 10.0))

(event `MC_ShowOnlyForDev`
  (for _array_element (`SceneComponent.GetChildrenComponents` (`self.RootComponent`) false)
    (if (== (`GameplayStatics.GetObjectClass` _array_element) "/Script/Engine.HierarchicalInstancedStaticMeshComponent")
      (bind (_validpc_ _playerroles) (message `/Game/DisconnectTemplate/Core/Library/BPI_UpdateData.getPC_Role` (`GameplayStatics.GetPlayerController` 0)))
      (if _validpc_
        (`SceneComponent.SetVisibility` _array_element (select `/Game/DisconnectTemplate/Core/Blueprints/Character/Data/EPlayerRole` _playerroles :`NewEnumerator2` true) false)))))

(fn `getElbowOffset`
  (returns (ElbowOffset :type "Float (double-precision)"))
  (return (* (`self.ElbowOffset`) (`self.MeshScale`))))

(fn `getMeshSize`
  (params (mesh :type "StaticMesh Object Reference"))
  (returns (ReturnValue :type "Vector Structure"))
  (bind (_returnvalue_min _returnvalue_max) (break `Box` (`StaticMesh.GetBoundingBox` mesh)))
  (return (* (- _returnvalue_max _returnvalue_min) (`self.MeshScale`))))

(fn `SetupHISM_Glitch`
  (params (HISM :type "PrimitiveComponent Object Reference"))
  (`PrimitiveComponent.SetRenderCustomDepth` (`local.HISM`) true)
  (`PrimitiveComponent.SetCustomDepthStencilValue` (`local.HISM`) 4)
  (`PrimitiveComponent.SetMaterial` (`local.HISM`) 0 "/Game/DisconnectTemplate/MaterialLibrary/BasicMaterial/MI_UV_LikeMat.MI_UV_LikeMat")
  (set `ActorComponent.ComponentTags` (`|MakeArray` "Glitched" :!type "Name") (`local.HISM`)))

(fn `UserConstructionScript`
  (locals (L_RndIndex :type Integer) (L_YLength :type "Float (double-precision)" :default 0.0) (L_ZLength :type "Float (double-precision)" :default 0.0) (L_Scaling :type "Float (double-precision)") (L_Index :type Integer) (L_currentLength :type "Float (single-precision)" :default 0.0) (L_RndLength :type "Float (single-precision)" :default 0.0) (`Loop?` :type Boolean) (L_MeshForHISM :type "Map of StaticMesh Object Reference to HierarchicalInstancedStaticMeshComponent Object Reference") (L_Meshs :type "Array of StaticMesh Object Reference") (L_LoopLimiter :type Integer) (L_ShoulderHISM :type "HierarchicalInstancedStaticMeshComponent Object Reference") (L_SplineCurrentLength :type "Float (double-precision)") (L_DistanceLeft :type "Float (double-precision)") (L_MeshDistanceMoyenne :type "Float (double-precision)" :default 0.0) (L_NumberOfMeshToPlace :type Integer :default 0) (L_DistanceStart :type "Float (double-precision)") (L_DistanceEnd :type "Float (double-precision)") (L_IndexShoulders :type Integer))
  (bind _spline (`self.Spline`))
  (bind _spline_2 (`self.Spline`))
  (bind _meshscale (`self.MeshScale`))
  (bind _meshscale_2 (`self.MeshScale`))
  (bind _meshscale_3 (`self.MeshScale`))
  (bind _returnvalue (+ (`local.L_currentLength`) (`local.L_Scaling`)))
  (bind (_returnvalue_min _returnvalue_max) (break `Box` (`StaticMesh.GetBoundingBox` (`|GetArrayItem` (`self.Meshs`) (`local.L_RndIndex`)))))
  (bind _returnvalue_x (`KismetMathLibrary.BreakVector` (`self.getMeshSize` (`|GetArrayItem` (`self.Meshs`) (`local.L_RndIndex`)))))
  (bind _returnvalue_x_2 (`KismetMathLibrary.BreakVector` (`self.getMeshSize` (`|GetArrayItem` (`self.Meshs`) (`local.L_RndIndex`)))))
  (bind _returnvalue_x_3 (`KismetMathLibrary.BreakVector` (`self.getMeshSize` (`|GetArrayItem` (`self.Meshs`) (`local.L_RndIndex`)))))
  (bind _returnvalue_x_4 (`KismetMathLibrary.BreakVector` (`self.getMeshSize` (`|GetArrayItem` (`self.Meshs`) (`local.L_RndIndex`)))))
  (bind (_returnvalue_x_5 _returnvalue_y _returnvalue_z) (`KismetMathLibrary.BreakVector` (+ (`KismetMathLibrary.Vector_GetAbs` _returnvalue_min) (`KismetMathLibrary.Vector_GetAbs` _returnvalue_max))))
  (`|ExecutionSequence`
    (:`then_0`
      (if (> (`KismetArrayLibrary.Array_Length` (`self.Meshs`)) 0)
        (if (`self.bIsHISM?`)
          (for _index (range (`SplineComponent.GetNumberOfSplinePoints` (`self.Spline`)))
            (`SplineComponent.SetSplinePointType` (`self.Spline`) _index "Linear" true))
          (bind (_keypin _valuepin) (`|MapForEach` (`local.L_MeshForHISM`))
            (:`then`
              (`/Engine/EditorBlueprintResources/StandardMacros.IsValid` _valuepin
                (:`Is Valid`
                  (`InstancedStaticMeshComponent.ClearInstances` _valuepin))))
            (:`CompletedPin`
              (for _array_element (`self.Meshs`)
                (bind _returnvalue_2 (`AddComponent|NODE_AddHierarchicalInstancedStaticMeshComponent-1`))
                (`BlueprintMapLibrary.Map_Add` (`local.L_MeshForHISM`) _array_element _returnvalue_2)
                (`StaticMeshComponent.SetStaticMesh` _returnvalue_2 _array_element))
              (`|ExecutionSequence`
                (:`then_0`
                  (if (and (`self.bHaveElbow?`) (`KismetSystemLibrary.IsValid` (`self.ElbowMesh`)))
                    (bind _returnvalue_3 (`AddComponent|NODE_AddHierarchicalInstancedStaticMeshComponent-2`))
                    (bind _output_get (set `local.L_ShoulderHISM` _returnvalue_3))
                    (`StaticMeshComponent.SetStaticMesh` _output_get (`self.ElbowMesh`))))
                (:`then_1`
                  (set `local.L_MeshDistanceMoyenne` 0.0)
                  (for _array_element_2 (`self.Meshs`)
                    (bind _returnvalue_x_6 (`KismetMathLibrary.BreakVector` (`self.getMeshSize` _array_element_2)))
                    (set `local.L_MeshDistanceMoyenne` (+ _returnvalue_x_6 (`local.L_MeshDistanceMoyenne`))))
                  (set `local.L_MeshDistanceMoyenne` (/ (`local.L_MeshDistanceMoyenne`) (`KismetArrayLibrary.Array_Length` (`self.Meshs`))))
                  (set `local.L_SplineCurrentLength` 0.0)
                  (set `local.L_Index` 0)
                  (bind _keys (`BlueprintMapLibrary.Map_Keys` (`local.L_MeshForHISM`)))
                  (set `local.L_Meshs` _keys)
                  (for _index_2 (range (`SplineComponent.GetNumberOfSplinePoints` (`self.Spline`)))
                    (set `local.L_Index` _index_2)
                    (set `local.L_DistanceStart` (+ (`SplineComponent.GetDistanceAlongSplineAtSplinePoint` (`self.Spline`) (`local.L_Index`)) (`self.getElbowOffset`)))
                    (set `local.L_DistanceEnd` (- (`SplineComponent.GetDistanceAlongSplineAtSplinePoint` (`self.Spline`) (+ (`local.L_Index`) 1)) (`self.getElbowOffset`)))
                    (set `local.L_DistanceLeft` (- (`local.L_DistanceEnd`) (`local.L_DistanceStart`)))
                    (while (> (`local.L_DistanceLeft`) 0.0)
                      (set `local.L_RndIndex` (`.OutIndex` (`KismetArrayLibrary.Array_RandomFromStream` (`self.Meshs`) (`self.RandomStream`))))
                      (if (<= _returnvalue_x_3 (`local.L_DistanceLeft`))
                        (`InstancedStaticMeshComponent.AddInstance` (`BlueprintMapLibrary.Map_Find` (`local.L_MeshForHISM`) (`|GetArrayItem` (`self.Meshs`) (`local.L_RndIndex`))) (`KismetMathLibrary.MakeTransform` (`SplineComponent.GetLocationAtDistanceAlongSpline` (`self.Spline`) (`local.L_DistanceStart`) "Local") (`SplineComponent.GetRotationAtDistanceAlongSpline` (`self.Spline`) (`local.L_DistanceStart`) "Local") (`KismetMathLibrary.MakeVector` _meshscale_3 _meshscale_3 _meshscale_3)) false)
                        (set `local.L_DistanceStart` (+ (`local.L_DistanceStart`) _returnvalue_x_4))
                        (set `local.L_DistanceLeft` (- (`local.L_DistanceLeft`) _returnvalue_x_2))
                        (else
                          (`InstancedStaticMeshComponent.AddInstance` (`BlueprintMapLibrary.Map_Find` (`local.L_MeshForHISM`) (`|GetArrayItem` (`self.Meshs`) (`local.L_RndIndex`))) (`KismetMathLibrary.MakeTransform` (`SplineComponent.GetLocationAtDistanceAlongSpline` (`self.Spline`) (`local.L_DistanceStart`) "Local") (`SplineComponent.GetRotationAtDistanceAlongSpline` (`self.Spline`) (`local.L_DistanceStart`) "Local") (`KismetMathLibrary.MakeVector` (* (/ (`local.L_DistanceLeft`) _returnvalue_x) (`self.MeshScale`)) _meshscale_2 _meshscale_2)) false)
                          (set `local.L_DistanceLeft` 0.0))))))
                (:`then_2`
                  (if (`self.bHaveElbow?`)
                    (for _index_3 (range 1 (+ (- (`SplineComponent.GetNumberOfSplinePoints` (`self.Spline`)) 2) 1))
                      (set `local.L_IndexShoulders` _index_3)
                      (`InstancedStaticMeshComponent.AddInstance` (`local.L_ShoulderHISM`) (`KismetMathLibrary.MakeTransform` (`.Position` (break `SplinePoint` (`SplineComponent.GetSplinePointAt` (`self.Spline`) (`local.L_IndexShoulders`) "Local"))) (`KismetMathLibrary.ComposeRotators` (`KismetMathLibrary.MakeRotFromXZ` (`KismetMathLibrary.Normal` (- (`SplineComponent.GetLocationAtSplinePoint` (`self.Spline`) (+ (`local.L_IndexShoulders`) 1) "Local") (`SplineComponent.GetLocationAtSplinePoint` (`self.Spline`) (`local.L_IndexShoulders`) "Local"))) (`KismetMathLibrary.Normal` (- (`SplineComponent.GetLocationAtSplinePoint` (`self.Spline`) (+ (`local.L_IndexShoulders`) -1) "Local") (`SplineComponent.GetLocationAtSplinePoint` (`self.Spline`) (`local.L_IndexShoulders`) "Local")))) (`|GetArrayItem` (`self.AddElbowRotation`) (- (`local.L_IndexShoulders`) 1))) (`KismetMathLibrary.MakeVector` _meshscale _meshscale _meshscale)) false))))
                (:`then_3`
                  (set `self.HISM_ForMeshs` (`local.L_MeshForHISM`))))))
          (else
            (set `local.L_Scaling` 0.0)
            (set `local.L_currentLength` 0.0)
            (if (`self.bIsRandomizeLength?`)
              (set `self.Min` (`KismetMathLibrary.FClamp` (`self.Min`) 1.0 (`self.Max`)))
              (set `self.Max` (`KismetMathLibrary.FClamp` (`self.Max`) (`self.Min`) (`SplineComponent.GetSplineLength` (`self.Spline`))))
              (set `local.L_RndIndex` (`.OutIndex` (`KismetArrayLibrary.Array_RandomFromStream` (`self.Meshs`) (`self.RandomStream`))) :!label _label)
              (set `local.L_RndLength` (`KismetMathLibrary.RandomFloatInRangeFromStream` (`self.RandomStream`) (`self.Min`) (`self.Max`)))
              (if (or (> (`local.L_RndLength`) (`SplineComponent.GetSplineLength` (`self.Spline`))) (> (+ (`local.L_RndLength`) (`local.L_Scaling`)) (`SplineComponent.GetSplineLength` (`self.Spline`)))) :!label _label_2
                (set `local.L_Scaling` _returnvalue)
                (set `local.L_currentLength` (- (`SplineComponent.GetSplineLength` (`self.Spline`)) (`local.L_Scaling`)))
                (set `local.Loop?` false)
                (else
                  (set `local.L_Scaling` _returnvalue)
                  (set `local.L_currentLength` (`local.L_RndLength`))
                  (set `local.Loop?` true)))
              (bind _output_get_2 (set `self.Length` (select `ESplineMeshAxis` (`self.MeshForwardAxis`) :`X` _returnvalue_x_5 :`Y` _returnvalue_y :`Z` _returnvalue_z)))
              (for _index_4 (range (+ (`KismetMathLibrary.FFloor` (/ (`local.L_currentLength`) _output_get_2)) 1))
                (bind _returnvalue_4 (`AddComponent|NODE_AddSplineMeshComponent-0`))
                (`PrimitiveComponent.SetCollisionEnabled` _returnvalue_4 "QueryAndPhysics")
                (`SplineMeshComponent.SetForwardAxis` _returnvalue_4 (`self.MeshForwardAxis`) true)
                (`StaticMeshComponent.SetStaticMesh` _returnvalue_4 (`|GetArrayItem` (`self.Meshs`) (`local.L_RndIndex`)))
                (bind _returnvalue_5 (+ (* _index_4 (`self.Length`)) (`local.L_Scaling`)))
                (bind _returnvalue_6 (+ (* (+ _index_4 1) (`self.Length`)) (`local.L_Scaling`)))
                (`SplineMeshComponent.SetStartAndEnd` _returnvalue_4 (`SplineComponent.GetLocationAtDistanceAlongSpline` _spline_2 _returnvalue_5 "Local") (`KismetMathLibrary.ClampVectorSize` (`SplineComponent.GetTangentAtDistanceAlongSpline` _spline_2 _returnvalue_5 "Local") 0.0 (`self.Length`)) (`SplineComponent.GetLocationAtDistanceAlongSpline` _spline _returnvalue_6 "Local") (`KismetMathLibrary.ClampVectorSize` (`SplineComponent.GetTangentAtDistanceAlongSpline` _spline _returnvalue_6 "Local") 0.0 (`self.Length`)) true))
              (if (`local.Loop?`)
                (goto _label))
              (else
                (set `local.L_RndLength` (`SplineComponent.GetSplineLength` (`self.Spline`)))
                (goto _label_2)))))))
    (:`then_1`
      (if (`self.bGlitchMeshEffect`)
        (bind (_keypin_2 _valuepin_2) (`|MapForEach` (`self.HISM_ForMeshs`))
          (:`then`
            (`self.SetupHISM_Glitch` _valuepin_2))
          (:`CompletedPin`
            (`self.SetupHISM_Glitch` (`local.L_ShoulderHISM`))))))))