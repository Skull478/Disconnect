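; BP_Fences is a tool Blueprint that lays out a straight row of repeated meshes, named for fences.
; Its construction script adds NumOfMesh instances of Mesh to an InstancedStaticMesh component.
; Each instance is spaced along X by the mesh's bounding-box width, with XOffset shifting the whole row rather than widening gaps.
; The event graph holds only disabled default events, so it has no runtime logic.
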(fn `UserConstructionScript`
  (bind _mesh (`self.Mesh`))
  (bind (_returnvalue_min _returnvalue_max) (break `Box` (`StaticMesh.GetBoundingBox` _mesh)))
  (for _index (range (`self.NumOfMesh`))
    (`StaticMeshComponent.SetStaticMesh` (`self.InstancedStaticMesh`) _mesh)
    (`InstancedStaticMeshComponent.AddInstance` (`self.InstancedStaticMesh`) (`KismetMathLibrary.MakeTransform` (`KismetMathLibrary.MakeVector` (+ (* (.x (- _returnvalue_max _returnvalue_min)) _index) (`self.XOffset`)))) false)))