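; BP_Appartements is a procedural apartment building tool that builds a modular facade in the construction script, sized by WallCountX and WallCountZ.
; Nested loops place hierarchical instanced meshes for walls, end corners and pillars, spacing them from mesh bounding boxes plus hardcoded offsets.
; Pillars go in at every third interior column.
; Roof-wall pieces appear only at those columns, at ground height, because the IsLastZ test matches row zero.
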(fn `UserConstructionScript`
  (bind _index_x (`self.Index X`))
  (bind _index_x_2 (`self.Index X`))
  (bind _hism_angle (`self.HISM_Angle`))
  (bind _index_x_3 (`self.Index X`))
  (bind _returnvalue (+ (`self.Final X`) 200.0))
  (bind _returnvalue_2 (+ (`self.Final X`) 254.65))
  (bind (_returnvalue_min _returnvalue_max) (break `Box` (`StaticMesh.GetBoundingBox` (`StaticMeshComponent.StaticMesh` (`self.HISM_Pilier`)))))
  (bind (_returnvalue_min_2 _returnvalue_max_2) (break `Box` (`StaticMesh.GetBoundingBox` (`StaticMeshComponent.StaticMesh` (`self.HISM_Mur`)))))
  (bind _returnvalue_3 (+ (- (`self.Final X`) (/ (`self.WallSpacing`) 2.0)) 28.0))
  (bind _returnvalue_x (`KismetMathLibrary.BreakVector` (- _returnvalue_max _returnvalue_min)))
  (bind _returnvalue_x_2 (`KismetMathLibrary.BreakVector` (- _returnvalue_max_2 _returnvalue_min_2)))
  (`AddComponent|NODE_AddHierarchicalInstancedStaticMeshComponent-6` :`self` (`ActorComponent.GetOwner` (`self.HISM_ToitMur`)))
  (`AddComponent|NODE_AddHierarchicalInstancedStaticMeshComponent-5` :`self` (`ActorComponent.GetOwner` (`self.HISM_Angle`)))
  (`AddComponent|NODE_AddHierarchicalInstancedStaticMeshComponent-4` :`self` (`ActorComponent.GetOwner` (`self.HISM_Mur`)))
  (`AddComponent|NODE_AddHierarchicalInstancedStaticMeshComponent-3` :`self` (`ActorComponent.GetOwner` (`self.HISM_Pilier`)))
  (for _index (range (`self.WallCount X`))
    (set `self.Index X` _index)
    (bind _output_get (set `self.WallSpacing` _returnvalue_x_2))
    (bind _output_get_2 (set `self.PillierWidth` (- _returnvalue_x 21.0)))
    (set `self.Final X` (+ (* _output_get _index_x) (* _output_get_2 (- (/ _index_x 3) 1))))
    (set `self.IsFirst X` (== _index_x_3 0))
    (set `self.IsLast X` (== _index_x_3 (- (`self.WallCount X`) 1)))
    (if (or (`self.IsFirst X`) (`self.IsLast X`))
      (if (`self.IsLast X`)
        (`InstancedStaticMeshComponent.AddInstance` _hism_angle (`KismetMathLibrary.MakeTransform` (`KismetMathLibrary.MakeVector` _returnvalue -200.0) (struct :`Yaw` -90.0)) false)
        (for _index_2 (range (`self.WallCount Z`))
          (bind _output_get_3 (set `self.Index Z` _index_2))
          (`InstancedStaticMeshComponent.AddInstance` (`self.HISM_Angle`) (`KismetMathLibrary.MakeTransform` (`KismetMathLibrary.MakeVector` _returnvalue -200.0 (* _output_get_3 (`self.WallSpacing`))) (struct :`Yaw` -90.0)) false))
        (else
          (`InstancedStaticMeshComponent.AddInstance` _hism_angle (`KismetMathLibrary.MakeTransform` (`KismetMathLibrary.MakeVector` _returnvalue_2) (struct)) false)
          (for _index_3 (range (`self.WallCount Z`))
            (bind _output_get_4 (set `self.Index Z` _index_3))
            (`InstancedStaticMeshComponent.AddInstance` (`self.HISM_Angle`) (`KismetMathLibrary.MakeTransform` (`KismetMathLibrary.MakeVector` _returnvalue_2 0.0 (* _output_get_4 (`self.WallSpacing`))) (struct)) false))))
      (else
        (`InstancedStaticMeshComponent.AddInstance` (`self.HISM_Mur`) (`KismetMathLibrary.MakeTransform` (`KismetMathLibrary.MakeVector` (`self.Final X`))) false)
        (for _index_4 (range (`self.WallCount Z`))
          (bind _output_get_5 (set `self.Index Z` _index_4))
          (`InstancedStaticMeshComponent.AddInstance` (`self.HISM_Mur`) (`KismetMathLibrary.MakeTransform` (`KismetMathLibrary.MakeVector` (`self.Final X`) 0.0 (* _output_get_5 (`self.WallSpacing`)))) false)
          (if (and (== (mod _index_x_2 3) 0) (!= _index_x_2 0))
            (`InstancedStaticMeshComponent.AddInstance` (`self.HISM_Pilier`) (`KismetMathLibrary.MakeTransform` (`KismetMathLibrary.MakeVector` _returnvalue_3)) false)
            (`InstancedStaticMeshComponent.AddInstance` (`self.HISM_Pilier`) (`KismetMathLibrary.MakeTransform` (`KismetMathLibrary.MakeVector` _returnvalue_3 0.0 (* (`self.Index Z`) (`self.WallSpacing`)))) false)
            (set `self.IsLast Z` (== 0 (- 0 (`self.Index Z`))))
            (if (`self.IsLast Z`)
              (`InstancedStaticMeshComponent.AddInstance` (`self.HISM_ToitMur`) (`KismetMathLibrary.MakeTransform` (`KismetMathLibrary.MakeVector` (`self.Final X`))) false))))))))