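; BP_Usine is a procedural factory building, assembled in the Construction Script from modular meshes with no runtime logic.
; Nested loops over wall counts in X, Y and Z add HISM instances for walls, corners, pillars and roof pieces.
; First, last and top-level checks choose each piece, with pillars at every third index in X and Y.
; Spacing comes from mesh bounding boxes, corrected by hardcoded offsets.
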(fn `UserConstructionScript`
  (bind _wallspacing (`self.WallSpacing`))
  (bind _index_y (`self.Index Y`))
  (bind _hism_angle (`self.HISM_Angle`))
  (bind _wallspacing_2 (`self.WallSpacing`))
  (bind _index_x (`self.Index X`))
  (bind _index_y_2 (`self.Index Y`))
  (bind _index_x_2 (`self.Index X`))
  (bind _index_y_3 (`self.Index Y`))
  (bind _index_x_3 (`self.Index X`))
  (bind _final_y (`self.Final Y`))
  (bind _index_x_4 (`self.Index X`))
  (bind _index_y_4 (`self.Index Y`))
  (bind _returnvalue (+ (`self.Final X`) 254.65))
  (bind _returnvalue_2 (+ (`self.Final Y`) _wallspacing))
  (bind _returnvalue_3 (+ (`self.Final X`) 200.0))
  (bind _returnvalue_4 (* (`self.Index Z`) (`self.WallSpacing`)))
  (bind (_returnvalue_min _returnvalue_max) (break `Box` (`StaticMesh.GetBoundingBox` (`StaticMeshComponent.StaticMesh` (`self.HISM_Mur`)))))
  (bind (_returnvalue_min_2 _returnvalue_max_2) (break `Box` (`StaticMesh.GetBoundingBox` (`StaticMeshComponent.StaticMesh` (`self.HISM_Pilier`)))))
  (bind (_returnvalue_min_3 _returnvalue_max_3) (break `Box` (`StaticMesh.GetBoundingBox` (`StaticMeshComponent.StaticMesh` (`self.HISM_Angle`)))))
  (bind _returnvalue_5 (+ (+ _wallspacing (`self.Final X`)) -54.6))
  (bind _returnvalue_6 (+ (* (`self.Index Z`) (`self.WallSpacing`)) (`self.WallSpacing`)))
  (bind _returnvalue_7 (- (`self.Final Z`) (* (`self.WallSpacing`) 2.0)))
  (bind _returnvalue_8 (+ (- (`self.Final X`) (/ (`self.WallSpacing`) 2.0)) 28.0))
  (bind _returnvalue_x (`KismetMathLibrary.BreakVector` (- _returnvalue_max _returnvalue_min)))
  (bind _returnvalue_x_2 (`KismetMathLibrary.BreakVector` (- _returnvalue_max_2 _returnvalue_min_2)))
  (bind (_returnvalue_x_3 _returnvalue_y) (`KismetMathLibrary.BreakVector` (- _returnvalue_max_3 _returnvalue_min_3)))
  ; Add HISMs
  (`AddComponent|NODE_AddHierarchicalInstancedStaticMeshComponent-6` :`self` (`ActorComponent.GetOwner` (`self.HISM_ToitMur`)))
  (`AddComponent|NODE_AddHierarchicalInstancedStaticMeshComponent-5` :`self` (`ActorComponent.GetOwner` (`self.HISM_Angle`)))
  (`AddComponent|NODE_AddHierarchicalInstancedStaticMeshComponent-4` :`self` (`ActorComponent.GetOwner` (`self.HISM_Mur`)))
  (`AddComponent|NODE_AddHierarchicalInstancedStaticMeshComponent-3` :`self` (`ActorComponent.GetOwner` (`self.HISM_Pilier`)))
  ; Set Position X & Y
  (for _index (range (`self.WallCount X`))
    (set `self.Index X` _index)
    (bind _output_get (set `self.WallSpacing` _returnvalue_x))
    (bind _output_get_2 (set `self.PillierWidth` (- _returnvalue_x_2 21.0)))
    (set `self.Final X` (+ (* _output_get _index_x) (* _output_get_2 (- (/ _index_x 3) 1))))
    (for _index_2 (range (`self.WallCount Y`))
      (set `self.Index Y` _index_2)
      (bind _output_get_3 (set `self.Angle Width` (+ (* _returnvalue_y 2.0) 75.0)))
      (set `self.Final Y` (- 0.0 (+ _output_get_3 (+ (* (`self.WallSpacing`) _index_y_2) (* (`self.PillierWidth`) (- (/ _index_y_2 3) 1))))))
      ; Set Pos Z & Final X & Z
      (set `self.IsFirst X` (== _index_x_2 0))
      (set `self.IsLast X` (== _index_x_2 (- (`self.WallCount X`) 1)))
      (set `self.IsLast Y` (== (`self.Index Y`) (- (`self.WallCount Y`) 1)))
      (for _index_3 (range (`self.WallCount Z`))
        (bind _output_get_4 (set `self.Index Z` _index_3))
        (set `self.Final Z` (* _output_get_4 (`self.WallSpacing`)))
        (set `self.IsLast Z` (== (`self.Index Z`) (- (`self.WallCount Z`) 1)))
        (`|ExecutionSequence`
          (:`then_0`
            (if (or (`self.IsFirst X`) (`self.IsLast X`))
              (if (`self.IsLast X`)
                (`|ExecutionSequence`
                  (:`then_0`
                    ; Murs Angle Start X
                    (`InstancedStaticMeshComponent.AddInstance` _hism_angle (`KismetMathLibrary.MakeTransform` (`KismetMathLibrary.MakeVector` _returnvalue_3 -227.0) (struct :`Yaw` -90.0)) false)
                    (`InstancedStaticMeshComponent.AddInstance` (`self.HISM_Angle`) (`KismetMathLibrary.MakeTransform` (`KismetMathLibrary.MakeVector` _returnvalue_3 -227.0 _returnvalue_4) (struct :`Yaw` -90.0)) false)
                    (if (`self.IsLast Z`)
                      (`InstancedStaticMeshComponent.AddInstance` (`self.HISM_ToitAngle`) (`KismetMathLibrary.MakeTransform` (`KismetMathLibrary.MakeVector` _returnvalue_3 -200.0 (+ (`self.Final Z`) (`self.WallSpacing`))) (struct :`Yaw` -90.0)) false)))
                  (:`then_1`
                    ; Murs End X
                    (`InstancedStaticMeshComponent.AddInstance` (`self.HISM_Mur`) (`KismetMathLibrary.MakeTransform` (`KismetMathLibrary.MakeVector` _returnvalue_5 _returnvalue_2) (struct :`Yaw` -90.0)) false)
                    (`InstancedStaticMeshComponent.AddInstance` (`self.HISM_Mur`) (`KismetMathLibrary.MakeTransform` (`KismetMathLibrary.MakeVector` _returnvalue_5 _returnvalue_2 (`self.Final Z`)) (struct :`Yaw` -90.0)) false)
                    (if (and (== (mod _index_y_3 3) 0) (!= _index_y_3 0))
                      ; Pilliers End X
                      (`InstancedStaticMeshComponent.AddInstance` (`self.HISM_Pilier`) (`KismetMathLibrary.MakeTransform` (`KismetMathLibrary.MakeVector` (+ (+ (`self.WallSpacing`) (`self.Final X`)) -54.6) (+ (+ (`self.Final Y`) (`self.WallSpacing`)) (`self.PillierWidth`)) (`self.Final Z`)) (struct :`Yaw` -90.0)) false)
                      (if (`self.IsLast Z`)
                        ; Toit Pillier End X
                        (`InstancedStaticMeshComponent.AddInstance` (`self.HISM_ToitPilier`) (`KismetMathLibrary.MakeTransform` (`KismetMathLibrary.MakeVector` (+ (+ (`self.WallSpacing`) (`self.Final X`)) -54.6) (+ (+ (`self.Final Y`) (`self.WallSpacing`)) (`self.PillierWidth`)) (+ (* (`self.Index Z`) (`self.WallSpacing`)) (`self.WallSpacing`))) (struct :`Yaw` -90.0)) false))))
                  (:`then_2`
                    (if (`self.IsLast Y`)
                      ; Angle X Y
                      (`InstancedStaticMeshComponent.AddInstance` (`self.HISM_Angle`) (`KismetMathLibrary.MakeTransform` (`KismetMathLibrary.MakeVector` (`self.Final X`) (- (`self.Final Y`) 200.0) (`self.Final Z`)) (struct :`Yaw` 180.0)) false))))
                (else
                  (`InstancedStaticMeshComponent.AddInstance` _hism_angle (`KismetMathLibrary.MakeTransform` (`KismetMathLibrary.MakeVector` _returnvalue -27.0)) false)
                  (`InstancedStaticMeshComponent.AddInstance` (`self.HISM_Angle`) (`KismetMathLibrary.MakeTransform` (`KismetMathLibrary.MakeVector` _returnvalue -27.0 _returnvalue_4)) false)
                  (if (`self.IsLast Z`)
                    (`InstancedStaticMeshComponent.AddInstance` (`self.HISM_ToitAngle`) (`KismetMathLibrary.MakeTransform` (`KismetMathLibrary.MakeVector` _returnvalue -27.0 (+ (* (`self.Index Z`) (`self.WallSpacing`)) (`self.WallSpacing`)))) false))))
              (else
                ;[0.02999 0.15 0.03024 0.5] Murs Start Y
                (`InstancedStaticMeshComponent.AddInstance` (`self.HISM_Mur`) (`KismetMathLibrary.MakeTransform` (`KismetMathLibrary.MakeVector` (`self.Final X`) -27.0)) false)
                (`InstancedStaticMeshComponent.AddInstance` (`self.HISM_Mur`) (`KismetMathLibrary.MakeTransform` (`KismetMathLibrary.MakeVector` (`self.Final X`) -27.0 (`self.Final Z`))) false)
                (`|ExecutionSequence`
                  (:`then_0`
                    ; Piliers
                    (if (and (== (mod _index_x_4 3) 0) (!= _index_x_4 0))
                      (`InstancedStaticMeshComponent.AddInstance` (`self.HISM_Pilier`) (`KismetMathLibrary.MakeTransform` (`KismetMathLibrary.MakeVector` _returnvalue_8 -27.0 (`self.Final Z`))) false)
                      (if (`self.IsLast Y`)
                        (`InstancedStaticMeshComponent.AddInstance` (`self.HISM_Pilier`) (`KismetMathLibrary.MakeTransform` (`KismetMathLibrary.MakeVector` (`self.Final X`) (+ (- (`self.Final Y`) (`self.WallSpacing`)) 54.6) (`self.Final Z`)) (struct :`Yaw` 180.0)) false)
                        (if (`self.IsLast Z`)
                          (`InstancedStaticMeshComponent.AddInstance` (`self.HISM_ToitPilier`) (`KismetMathLibrary.MakeTransform` (`KismetMathLibrary.MakeVector` _returnvalue_8 -27.0 _returnvalue_6)) false)
                          (`InstancedStaticMeshComponent.AddInstance` (`self.HISM_ToitPilier`) (`KismetMathLibrary.MakeTransform` (`KismetMathLibrary.MakeVector` (`self.Final X`) (+ (- (`self.Final Y`) (`self.WallSpacing`)) 54.6) _returnvalue_6) (struct :`Yaw` 180.0)) false)))))
                  (:`then_1`
                    ; Toit Mur
                    (if (`self.IsLast Z`)
                      (`InstancedStaticMeshComponent.AddInstance` (`self.HISM_ToitMur`) (`KismetMathLibrary.MakeTransform` (`KismetMathLibrary.MakeVector` (`self.Final X`) -27.0 _returnvalue_7)) false)
                      (`InstancedStaticMeshComponent.AddInstance` (`self.HISM_ToitMur`) (`KismetMathLibrary.MakeTransform` (`KismetMathLibrary.MakeVector` -44.37 (`self.Final Y`) _returnvalue_7) (struct :`Yaw` 90.0)) false)
                      ; Toit Centre
                      (`InstancedStaticMeshComponent.AddInstance` (`self.HISM_ToitCentre`) (`KismetMathLibrary.MakeTransform` (`KismetMathLibrary.MakeVector` (`self.Final X`) (+ (`self.Final Y`) (`self.WallSpacing`)) (+ (`self.Final Z`) (`self.WallSpacing`)))) false)))
                  (:`then_2`
                    ; Murs Start X
                    (`InstancedStaticMeshComponent.AddInstance` (`self.HISM_Mur`) (`KismetMathLibrary.MakeTransform` (`KismetMathLibrary.MakeVector` -44.37 _final_y (`self.Final Z`)) (struct :`Yaw` 90.0)) false)
                    (`InstancedStaticMeshComponent.AddInstance` (`self.HISM_Mur`) (`KismetMathLibrary.MakeTransform` (`KismetMathLibrary.MakeVector` -44.37 _final_y (`self.Final Z`)) (struct :`Yaw` 90.0)) false)
                    (if (`self.IsLast Y`)
                      ; Murs End Y
                      (`InstancedStaticMeshComponent.AddInstance` (`self.HISM_Mur`) (`KismetMathLibrary.MakeTransform` (`KismetMathLibrary.MakeVector` (+ (`self.Final X`) _wallspacing_2) (+ (- (`self.Final Y`) _wallspacing_2) 54.6) (`self.Final Z`)) (struct :`Yaw` 180.0)) false)
                      ; Angle End Y
                      (`InstancedStaticMeshComponent.AddInstance` (`self.HISM_Angle`) (`KismetMathLibrary.MakeTransform` (`KismetMathLibrary.MakeVector` -44.37 (`self.Final Y`) (`self.Final Z`)) (struct :`Yaw` 90.0)) false)))
                  (:`then_3`
                    (if (and (== (mod _index_y_4 3) 0) (!= _index_y_4 0))
                      ; Pilliers Start X
                      (`InstancedStaticMeshComponent.AddInstance` (`self.HISM_Pilier`) (`KismetMathLibrary.MakeTransform` (`KismetMathLibrary.MakeVector` -44.37 (+ (`self.Final Y`) (`self.WallSpacing`)) (`self.Final Z`)) (struct :`Yaw` 90.0)) false)
                      (if (`self.IsLast Z`)
                        ; Toit Pillier Start X
                        (`InstancedStaticMeshComponent.AddInstance` (`self.HISM_ToitPilier`) (`KismetMathLibrary.MakeTransform` (`KismetMathLibrary.MakeVector` -44.37 (+ (`self.Final Y`) (`self.WallSpacing`)) (+ (* (`self.Index Z`) (`self.WallSpacing`)) (`self.WallSpacing`))) (struct :`Yaw` 90.0)) false))))))))
          (:`then_1`
            ; Toit Angle End X Y
            (if (`self.IsLast Z`)
              (if (`self.IsLast X`)
                (if (`self.IsLast Y`)
                  (`InstancedStaticMeshComponent.AddInstance` (`self.HISM_ToitAngle`) (`KismetMathLibrary.MakeTransform` (`KismetMathLibrary.MakeVector` (`self.Final X`) (+ (`self.Final Y`) -200.0) (+ (* (`self.Index Z`) (`self.WallSpacing`)) (`self.WallSpacing`))) (struct :`Yaw` 180.0)) false)
                  ; Toit Angle End Y
                  (`InstancedStaticMeshComponent.AddInstance` (`self.HISM_ToitAngle`) (`KismetMathLibrary.MakeTransform` (`KismetMathLibrary.MakeVector` -44.37 (+ (`self.Final Y`) 0.0) (+ (* (`self.Index Z`) (`self.WallSpacing`)) (`self.WallSpacing`))) (struct :`Yaw` 90.0)) false)))))
          (:`then_2`
            (if (`self.IsLast Z`)
              (if (`self.IsLast X`)
                ; Toit Mur End X
                (`InstancedStaticMeshComponent.AddInstance` (`self.HISM_ToitMur`) (`KismetMathLibrary.MakeTransform` (`KismetMathLibrary.MakeVector` (+ (+ (+ 0.0 (`self.Final X`)) -54.6) (`self.WallSpacing`)) (+ (`self.Final Y`) (`self.WallSpacing`)) (- (`self.Final Z`) (* (`self.WallSpacing`) 2.0))) (struct :`Yaw` -90.0)) false))))
          (:`then_3`
            (if (`self.IsFirst X`)
              _
              (elif (`self.IsLast X`)
                _
                (elif (`self.IsLast Z`)
                  (if (`self.IsLast Y`)
                    ; Toit Mur End X
                    (`InstancedStaticMeshComponent.AddInstance` (`self.HISM_ToitMur`) (`KismetMathLibrary.MakeTransform` (`KismetMathLibrary.MakeVector` (+ (+ 0.0 (`self.Final X`)) (`self.WallSpacing`)) (+ (- (`self.Final Y`) (`self.WallSpacing`)) 54.6) (- (`self.Final Z`) (* (`self.WallSpacing`) 2.0))) (struct :`Yaw` 180.0)) false))))))
          (:`then_4`
            ; Toit Centre Pilier X
            (if (`self.IsLast Z`)
              (if (and (== (mod _index_x_3 3) 0) (!= _index_x_3 0))
                (`InstancedStaticMeshComponent.AddInstance` (`self.HISM_ToitCentrePilier`) (`KismetMathLibrary.MakeTransform` (`KismetMathLibrary.MakeVector` (- (`self.Final X`) (`self.PillierWidth`)) (+ (+ (`self.Final Y`) (* (`self.PillierWidth`) 2.0)) 56.567) (+ (`self.Final Z`) (`self.WallSpacing`)))) false))))
          (:`then_5`
            ; Toit Centre Pilier Y
            (if (`self.IsFirst X`)
              _
              (elif (`self.IsLast X`)
                _
                (elif (`self.IsLast Z`)
                  (if (and (== (mod _index_y 3) 0) (!= _index_y 0))
                    (`InstancedStaticMeshComponent.AddInstance` (`self.HISM_ToitCentrePilier`) (`KismetMathLibrary.MakeTransform` (`KismetMathLibrary.MakeVector` (`self.Final X`) (+ (`self.Final Y`) (`self.WallSpacing`)) (+ (`self.Final Z`) (`self.WallSpacing`))) (struct :`Yaw` 90.0)) false)))))))))))