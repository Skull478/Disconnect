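; Construction-script scatter tool that fills a box area with random instances of several meshes.
; It creates one HISM component per MeshToSpawn entry, mapped to that entry's scatter data.
; Seeded random points are sphere-traced on Visibility, with blocked points re-rolled through a DoN retry limit.
; Clear points become instances at a shared AltitudeZ with random yaw and per-axis scale from each entry's ranges.
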(fn `UserConstructionScript`
  (locals (L_InstancedMesh :type "InstancedStaticMeshComponent Object Reference") (L_ScatterData :type "/Game/DisconnectTemplate/Core/Blueprints/Tools/S_ScatterMeshes Structure"))
  (bind _collisiontracerange (`self.CollisionTraceRange`))
  (bind (_spawnpoint_x _spawnpoint_y) (`KismetMathLibrary.BreakVector` (`self.SpawnPoint`)))
  (bind _meshtospawn (`self.MeshToSpawn`))
  (bind _spawnradius (`self.SpawnRadius`))
  (bind ((`Mesh_10_1BDBB79B4A7B612B086FCA98234465C1` _mesh) (`Scale_Min_12_4AC9CC5B48261765FB73AF8FB67370B8` _scale_min) (`Scale_Max_14_08C503D34C2D04540DBB7482EB0078B4` _scale_max) (`Rotation_Min_17_BA8CD56342BB95B916920EAC524FBC56` _rotation_min) (`Rotation_Max_19_5672626349D0850C340B309D739507A3` _rotation_max)) (break `/Game/DisconnectTemplate/Core/Blueprints/Tools/S_ScatterMeshes` (`local.L_ScatterData`)))
  (bind _returnvalue (/ _collisiontracerange 5.0))
  (bind _returnvalue_2 (+ (`self.K2_GetActorLocation`) (`self.SpawnPoint`)))
  (bind _returnvalue_3 (`KismetMathLibrary.RandomFloatInRangeFromStream` (`self.RandomStream`) _scale_min _scale_max))
  (`BoxComponent.SetBoxExtent` (`self.SpawnRadius`) (`KismetMathLibrary.MakeVector` (`self.Size_X`) (`self.Size_Y`) (`self.Size_Z`)) true)
  (`BlueprintMapLibrary.Map_Clear` (`self.InstancedMeshes`))
  (for _index (range (+ (`KismetArrayLibrary.Array_Length` _meshtospawn) 1))
    (bind _returnvalue_4 (`AddComponent|NODE_AddHierarchicalInstancedStaticMeshComponent-0`))
    (bind _output (`|GetArrayItem` _meshtospawn _index))
    (`StaticMeshComponent.SetStaticMesh` _returnvalue_4 (`.Mesh_10_1BDBB79B4A7B612B086FCA98234465C1` (break `/Game/DisconnectTemplate/Core/Blueprints/Tools/S_ScatterMeshes` _output)))
    (`BlueprintMapLibrary.Map_Add` (`self.InstancedMeshes`) _returnvalue_4 _output))
  (bind _keys (`BlueprintMapLibrary.Map_Keys` (`self.InstancedMeshes`)))
  (for _array_element _keys
    (set `local.L_InstancedMesh` _array_element)
    (bind _value (`BlueprintMapLibrary.Map_Find` (`self.InstancedMeshes`) _array_element))
    (set `local.L_ScatterData` _value)
    (for _ (range (+ (`.Amount_22_836F5B7D496B106EE697638EFC5C3F0A` (break `/Game/DisconnectTemplate/Core/Blueprints/Tools/S_ScatterMeshes` _value)) 1))
      (set `self.SpawnPoint` (`KismetMathLibrary.RandomPointInBoundingBoxFromStream` (`self.RandomStream`) (`SceneComponent.RelativeLocation` _spawnradius) (`BoxComponent.BoxExtent` _spawnradius)) :!label _label)
      (bind (_outhit _returnvalue_5) (`KismetSystemLibrary.SphereTraceSingle` :`Start` (+ (`KismetMathLibrary.MakeVector` 0.0 0.0 _collisiontracerange) _returnvalue_2) :`End` (+ (`KismetMathLibrary.MakeVector` 0.0 0.0 (/ _returnvalue 1.0)) _returnvalue_2) :`Radius` _returnvalue :`TraceChannel` "TraceTypeQuery1" :`bTraceComplex` true :`DrawDebugType` (select `bool` (`self.b_CollisionDebug?`) :`true` "ForDuration" :!type "EDrawDebugTrace Enum") :`bIgnoreSelf` false))
      (if _returnvalue_5
        (`/Engine/EditorBlueprintResources/StandardMacros.Do N` 0 :!label _label_2
          (:`Exit`
            (goto _label)))
        (else
          (`|ExecutionSequence`
            (:`then_0`
              (goto _label_2 :!via `Reset`))
            (:`then_1`
              (`InstancedStaticMeshComponent.AddInstance` (`local.L_InstancedMesh`) (`KismetMathLibrary.MakeTransform` (`KismetMathLibrary.MakeVector` _spawnpoint_x _spawnpoint_y (`self.Altitude_Z`)) (`KismetMathLibrary.MakeRotator` 0.0 0.0 (`KismetMathLibrary.RandomFloatInRangeFromStream` (`self.RandomStream`) _rotation_min _rotation_max)) (`KismetMathLibrary.MakeVector` _returnvalue_3 _returnvalue_3 _returnvalue_3)) false))))))))