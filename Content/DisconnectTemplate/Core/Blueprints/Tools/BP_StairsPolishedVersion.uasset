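; Procedural staircase tool that builds start, middle and end sections from hierarchical instanced static meshes in the construction script.
; NumberSteps drives a loop that places middle sections at a fixed offset, then positions the end section after them.
; Each section adds small steps scaled by StairsWidth, a width-offset border and, when UseFence is on, ramps on both sides.
; Older bounding-box and spline-based layouts remain as disconnected nodes.
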(fn `AddAllSmallSteps`
  (params (TransformLocation :type "Vector Structure") (numbers :type Integer :default 2))
  (locals (L_Index :type Integer))
  (for _index (range numbers)
    (set `local.L_Index` _index)
    (`self.AddSmallStepsInstance` (+ (`local.TransformLocation`) (* (`self.OffsetSmallStep`) (`local.L_Index`))))))

(fn `AddSmallStepsInstance`
  (params (InstanceTransform_Location :type "Vector Structure"))
  (`InstancedStaticMeshComponent.AddInstance` (`self.HISM_SmallSteps`) (`KismetMathLibrary.MakeTransform` InstanceTransform_Location (struct) (`KismetMathLibrary.MakeVector` (/ (`self.StairsWidth`) 100.0) 1.0 1.0)) false))

(fn `getCustomScale`
  (returns (ReturnValue :type "Vector Structure"))
  (return (`KismetMathLibrary.MakeVector` (+ (/ (`self.StairsWidth`) 100.0) 1.0) 1.0 1.0)))

(fn `getMeshSizes`
  (params (StaticMesh :type "StaticMesh Object Reference"))
  (returns (Size :type "Vector Structure") (HalfSize :type "Vector Structure"))
  (bind (_returnvalue_min _returnvalue_max) (break `Box` (`StaticMesh.GetBoundingBox` StaticMesh)))
  (bind _returnvalue (- _returnvalue_max _returnvalue_min))
  (return _returnvalue (/ _returnvalue 2.0)))

(fn `LocCalculatedForBorder`
  (returns (ReturnValue :type "Vector Structure"))
  (return (`KismetMathLibrary.MakeVector` (/ (`self.StairsWidth`) 2.0))))

(fn `MeshRampOtherSideOffset`
  (returns (ReturnValue :type "Vector Structure"))
  (return (`KismetMathLibrary.MakeVector` (+ (.x (`self.getMeshSizes` (`self.MeshStartSteps`))) (/ (`self.StairsWidth`) 2.0)))))

(fn `UserConstructionScript`
  (locals (L_Index :type Integer) (L_TransformLocation :type "Vector Structure") (L_EndTransformLocation :type "Vector Structure"))
  (`|ExecutionSequence`
    (:`then_0`
      ; Start Steps
      (`InstancedStaticMeshComponent.AddInstance` (`self.HISM_StartSteps`) (`KismetMathLibrary.MakeTransform` (0.0 0.0 0.0)) false)
      (`self.AddAllSmallSteps` (0.0 0.0 0.0))
      (`InstancedStaticMeshComponent.AddInstance` (`self.HISM_StartBorder`) (`KismetMathLibrary.MakeTransform` (`self.LocCalculatedForBorder`)) false)
      (`self.UseFence?`
        (:`True`
          (`InstancedStaticMeshComponent.AddInstance` (`self.HISM_StartRamp`) (`KismetMathLibrary.MakeTransform` (0.0 0.0 0.0)) false)
          (`InstancedStaticMeshComponent.AddInstance` (`self.HISM_StartRamp`) (`KismetMathLibrary.MakeTransform` (`self.MeshRampOtherSideOffset`)) false))))
    (:`then_1`
      ; Middle Steps
      (for _index (range 1 (`self.NumberSteps`))
        (set `local.L_Index` _index)
        (set `local.L_TransformLocation` (* (`local.L_Index`) (`self.OffsetMiddleSteps`)))
        (`InstancedStaticMeshComponent.AddInstance` (`self.HISM_MiddleSteps`) (`KismetMathLibrary.MakeTransform` (`local.L_TransformLocation`)) false)
        (`self.AddAllSmallSteps` (`local.L_TransformLocation`) 3)
        (`InstancedStaticMeshComponent.AddInstance` (`self.HISM_MiddleBorder`) (`KismetMathLibrary.MakeTransform` (+ (`local.L_TransformLocation`) (`self.LocCalculatedForBorder`))) false)
        (`self.UseFence?`
          (:`True`
            (`InstancedStaticMeshComponent.AddInstance` (`self.HISM_MiddleRamp`) (`KismetMathLibrary.MakeTransform` (`local.L_TransformLocation`)) false)
            (`InstancedStaticMeshComponent.AddInstance` (`self.HISM_MiddleRamp`) (`KismetMathLibrary.MakeTransform` (+ (`local.L_TransformLocation`) (`self.MeshRampOtherSideOffset`))) false))))
      ; End Steps
      (set `local.L_EndTransformLocation` (+ (* (- (`local.L_Index`) 1) (`self.OffsetMiddleSteps`)) (`self.OffsetEndStep`)))
      (`InstancedStaticMeshComponent.AddInstance` (`self.HISM_EndSteps`) (`KismetMathLibrary.MakeTransform` (`local.L_EndTransformLocation`)) false)
      (`self.AddAllSmallSteps` (`local.L_EndTransformLocation`))
      (`InstancedStaticMeshComponent.AddInstance` (`self.HISM_EndBorder`) (`KismetMathLibrary.MakeTransform` (+ (`local.L_EndTransformLocation`) (`self.LocCalculatedForBorder`))) false)
      (`self.UseFence?`
        (:`True`
          (`InstancedStaticMeshComponent.AddInstance` (`self.HISM_EndRamp`) (`KismetMathLibrary.MakeTransform` (`local.L_EndTransformLocation`)) false)
          (`InstancedStaticMeshComponent.AddInstance` (`self.HISM_EndRamp`) (`KismetMathLibrary.MakeTransform` (+ (`local.L_EndTransformLocation`) (`self.MeshRampOtherSideOffset`))) false))))))