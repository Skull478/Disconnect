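; BP_Grids is a construction-time tool actor that lays out a 2D grid of static mesh instances on HISMGrid.
; Nested loops over NbX and NBY space instances by mesh bounding-box size plus OffsetX and OffsetY, with a fixed 90-degree rotation.
; The outer loop also adds an instance per column, duplicating the first row.
; The script also adds an unused HISM component; the event graph is empty.
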(fn `UserConstructionScript`
  (bind (_returnvalue_min _returnvalue_max) (break `Box` (`StaticMesh.GetBoundingBox` (`StaticMeshComponent.StaticMesh` (`self.HISM_Grid`)))))
  (bind (_returnvalue_min_2 _returnvalue_max_2) (break `Box` (`StaticMesh.GetBoundingBox` (`StaticMeshComponent.StaticMesh` (`self.HISM_Grid`)))))
  (bind (_returnvalue_x _returnvalue_y) (`KismetMathLibrary.BreakVector` (- _returnvalue_max _returnvalue_min)))
  (bind _returnvalue_x_2 (`KismetMathLibrary.BreakVector` (- _returnvalue_max_2 _returnvalue_min_2)))
  (`AddComponent|NODE_AddHierarchicalInstancedStaticMeshComponent-0` :`self` (`ActorComponent.GetOwner` (`self.HISM_Grid`)))
  (for _index (range (`self.Nb X`))
    (bind _returnvalue (* _index (+ _returnvalue_x_2 (`self.Offset X`))))
    (`InstancedStaticMeshComponent.AddInstance` (`self.HISM_Grid`) (`KismetMathLibrary.MakeTransform` (`KismetMathLibrary.MakeVector` _returnvalue) (struct :`Yaw` 90.0)) false)
    (for _index_2 (range (`self.NB Y`))
      (`InstancedStaticMeshComponent.AddInstance` (`self.HISM_Grid`) (`KismetMathLibrary.MakeTransform` (`KismetMathLibrary.MakeVector` _returnvalue (* _index_2 (+ _returnvalue_y (`self.Offset Y`)))) (struct :`Yaw` 90.0)) false))))