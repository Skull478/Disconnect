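; BP_Train is a train pawn that drives itself along the spline of an assigned ActivePath using movement input.
; Each Tick it moves forward at Speed with audio on, then GetPath turns it toward the spline point nearest a short look-ahead along the closest tangent.
; Nearing the spline's end point, read in local space, sets Stop, which mutes audio and halts input.
; The construction script adds one train mesh instance.
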(event `self.ReceiveTick`
  (params (DeltaSeconds :type "Float (single-precision)"))
  (if (`self.Stop`)
    (`AudioComponent.SetVolumeMultiplier` (`self.Audio`) 0.0)
    (else
      (`AudioComponent.SetVolumeMultiplier` (`self.Audio`) 4.0)
      (`self.AddMovementInput` (`self.GetActorForwardVector`) (`self.Speed`))
      (`self.GetPath`))))

(fn `GetPath`
  (locals (L_Spline :type "SplineComponent Object Reference"))
  (bind _returnvalue (`self.K2_GetActorLocation`))
  (bind _l_spline (`local.L_Spline`))
  (set `local.L_Spline` (`/Game/DisconnectTemplate/Core/Blueprints/Tools/BP_TrainPath.Spline` (`self.ActivePath`)))
  (`/Engine/EditorBlueprintResources/StandardMacros.IsValid` (`self.ActivePath`)
    (:`Is Valid`
      (if (== (`SplineComponent.GetLocationAtSplinePoint` _l_spline (`SplineComponent.GetNumberOfSplinePoints` (`local.L_Spline`)) "Local") _returnvalue :`ErrorTolerance` 50.0)
        (set `self.Stop` true)
        (else
          (`self.K2_SetActorRotation` (`KismetMathLibrary.FindLookAtRotation` _returnvalue (`SplineComponent.FindLocationClosestToWorldLocation` (`local.L_Spline`) (+ (* (`KismetMathLibrary.Normal` (`SplineComponent.FindTangentClosestToWorldLocation` _l_spline _returnvalue "World")) 50.0) _returnvalue) "World"))))))))

(fn `UserConstructionScript`
  (`InstancedStaticMeshComponent.AddInstance` (`self.ISM_Train`) (`KismetMathLibrary.MakeTransform` (0.0 0.0 0.0)) false))