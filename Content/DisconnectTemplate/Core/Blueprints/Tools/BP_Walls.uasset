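; BP_Walls is a level-building tool that assembles a modular wall along X in its construction script.
; HISMWall02 instances form bottom and top rows, with two slightly offset HISMWall01 rows stacked between them.
; Mesh bounds set spacing and heights, WallsX sets the length, and RemoveWall01 shortens the middle rows.
; UseGlitchedWalls toggles custom depth on both instanced components, with Depth as the stencil value.
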(fn `UserConstructionScript`
  (bind _hism_wall_01 (`self.HISM_Wall_01`))
  (bind (_returnvalue_min _returnvalue_max) (break `Box` (`StaticMesh.GetBoundingBox` (`StaticMeshComponent.StaticMesh` (`self.HISM_Wall_02`)))))
  (bind (_returnvalue_min_2 _returnvalue_max_2) (break `Box` (`StaticMesh.GetBoundingBox` (`StaticMeshComponent.StaticMesh` (`self.HISM_Wall_01`)))))
  (bind (_returnvalue_x _returnvalue_y _returnvalue_z) (`KismetMathLibrary.BreakVector` (- _returnvalue_max _returnvalue_min)))
  (bind (_returnvalue_x_2 _returnvalue_y_2 _returnvalue_z_2) (`KismetMathLibrary.BreakVector` (- _returnvalue_max_2 _returnvalue_min_2)))
  (bind _returnvalue (- (+ _returnvalue_z _returnvalue_z_2) 2.5))
  (`|ExecutionSequence`
    (:`then_0`
      (`AddComponent|NODE_AddHierarchicalInstancedStaticMeshComponent-0` :`self` (`ActorComponent.GetOwner` (`self.HISM_Wall_02`)))
      (for _index (range (`self.Walls X`))
        (bind _returnvalue_2 (* _index _returnvalue_x))
        (`InstancedStaticMeshComponent.AddInstance` (`self.HISM_Wall_02`) (`KismetMathLibrary.MakeTransform` (`KismetMathLibrary.MakeVector` _returnvalue_2)) false)
        (`InstancedStaticMeshComponent.AddInstance` (`self.HISM_Wall_02`) (`KismetMathLibrary.MakeTransform` (`KismetMathLibrary.MakeVector` _returnvalue_2 0.0 (- (+ _returnvalue _returnvalue_z_2) 2.5))) false)))
    (:`then_1`
      (`AddComponent|NODE_AddHierarchicalInstancedStaticMeshComponent-1` :`self` (`ActorComponent.GetOwner` (`self.HISM_Wall_01`)))
      (for _index_2 (range (- (`self.Walls X`) (`self.Remove Wall 01`)))
        (bind _returnvalue_3 (* _index_2 (- _returnvalue_x_2 2.5)))
        (`InstancedStaticMeshComponent.AddInstance` (`self.HISM_Wall_01`) (`KismetMathLibrary.MakeTransform` (`KismetMathLibrary.MakeVector` _returnvalue_3 -5.0 _returnvalue_z)) false)
        (`InstancedStaticMeshComponent.AddInstance` (`self.HISM_Wall_01`) (`KismetMathLibrary.MakeTransform` (`KismetMathLibrary.MakeVector` _returnvalue_3 -5.0 _returnvalue)) false)))
    (:`then_2`
      (`PrimitiveComponent.SetRenderCustomDepth` _hism_wall_01 (`self.bUseGlitchedWalls`))
      (`PrimitiveComponent.SetRenderCustomDepth` (`self.HISM_Wall_02`) (`self.bUseGlitchedWalls`))
      (`PrimitiveComponent.SetCustomDepthStencilValue` _hism_wall_01 (`self.Depth`))
      (`PrimitiveComponent.SetCustomDepthStencilValue` (`self.HISM_Wall_02`) (`self.Depth`)))))