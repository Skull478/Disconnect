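; BP_Stairs is an editor tool that procedurally builds a modular staircase in its Construction Script.
; HISM start, middle and end pieces form steps, two railings and a border, with NumberSteps repeating middles at bounding-box spacing minus hard-coded offsets.
; Width scales the small steps and a spline, whose world-space point X plus fixed offsets positions the second railing and border.
; Barrières toggles railing visibility.
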(fn `UserConstructionScript`
  (bind _hism_md_ramp02 (`self.HISM_Md_Ramp02`))
  (bind _hism_end_ramp02 (`self.HISM_End_Ramp02`))
  (bind _hism_md_steps (`self.HISM_Md_Steps`))
  (bind _hism_end_steps (`self.HISM_End_Steps`))
  (bind _hism_mdborder (`self.HISM_MdBorder`))
  (bind _hism_endborder (`self.HISM_EndBorder`))
  (bind `_barrières__` (`self.Barrières ?`))
  (bind _hism_md_ramp01 (`self.HISM_Md_Ramp01`))
  (bind _hism_end_ramp01 (`self.HISM_End_Ramp01`))
  (bind _returnvalue_x (`KismetMathLibrary.BreakVector` (`SplineComponent.GetLocationAtSplineInputKey` (`self.Spline`) 1.0 "World")))
  (bind (_returnvalue_min _returnvalue_max) (break `Box` (`StaticMesh.GetBoundingBox` (`StaticMeshComponent.StaticMesh` (`self.HISM_Md_Steps`)))))
  (bind (_returnvalue_min_2 _returnvalue_max_2) (break `Box` (`StaticMesh.GetBoundingBox` (`StaticMeshComponent.StaticMesh` (`self.HISM_StartBorder`)))))
  (bind (_returnvalue_min_3 _returnvalue_max_3) (break `Box` (`StaticMesh.GetBoundingBox` (`StaticMeshComponent.StaticMesh` _hism_md_steps))))
  (bind (_returnvalue_min_4 _returnvalue_max_4) (break `Box` (`StaticMesh.GetBoundingBox` (`StaticMeshComponent.StaticMesh` (`self.HISM_St_Steps`)))))
  (bind (_returnvalue_min_5 _returnvalue_max_5) (break `Box` (`StaticMesh.GetBoundingBox` (`StaticMeshComponent.StaticMesh` _hism_mdborder))))
  (bind (_returnvalue_min_6 _returnvalue_max_6) (break `Box` (`StaticMesh.GetBoundingBox` (`StaticMeshComponent.StaticMesh` (`self.HISM_St_Ramp01`)))))
  (bind (_returnvalue_min_7 _returnvalue_max_7) (break `Box` (`StaticMesh.GetBoundingBox` (`StaticMeshComponent.StaticMesh` _hism_md_ramp01))))
  (bind (_returnvalue_min_8 _returnvalue_max_8) (break `Box` (`StaticMesh.GetBoundingBox` (`StaticMeshComponent.StaticMesh` (`self.HISM_St_Ramp02`)))))
  (bind (_returnvalue_min_9 _returnvalue_max_9) (break `Box` (`StaticMesh.GetBoundingBox` (`StaticMeshComponent.StaticMesh` _hism_md_ramp02))))
  (bind _returnvalue (+ _returnvalue_x 3196.5))
  (bind _returnvalue_2 (- _returnvalue 2.7))
  (bind _returnvalue_3 (- _returnvalue 105.87))
  (bind _returnvalue_4 (- (- _returnvalue_max_9 _returnvalue_min_9) (0.0 92.375 75.06)))
  (bind (_returnvalue_x_2 _returnvalue_y _returnvalue_z) (`KismetMathLibrary.BreakVector` (- (- _returnvalue_max_4 _returnvalue_min_4) (0.0 70.32 17.8))))
  (bind _returnvalue_5 (- (- _returnvalue_max_3 _returnvalue_min_3) (0.0 99.97 31.74)))
  (bind (_returnvalue_x_3 _returnvalue_y_2 _returnvalue_z_2) (`KismetMathLibrary.BreakVector` (- (- _returnvalue_max_8 _returnvalue_min_8) (0.0 81.0 93.5))))
  (bind (_returnvalue_x_4 _returnvalue_y_3 _returnvalue_z_3) (`KismetMathLibrary.BreakVector` (- (- _returnvalue_max_2 _returnvalue_min_2) (0.0 70.08 17.81))))
  (bind _returnvalue_6 (- (- _returnvalue_max_5 _returnvalue_min_5) (0.0 99.1 31.78)))
  (bind (_returnvalue_x_5 _returnvalue_y_4 _returnvalue_z_4) (`KismetMathLibrary.BreakVector` (- (- _returnvalue_max_6 _returnvalue_min_6) (0.0 81.0 93.5))))
  (bind _returnvalue_7 (- (- _returnvalue_max_7 _returnvalue_min_7) (0.0 92.375 75.06)))
  (bind (_returnvalue_x_6 _returnvalue_y_5 _returnvalue_z_5) (`KismetMathLibrary.BreakVector` (* (+ (`self.FinalStep`) 1) _returnvalue_5)))
  (bind (_returnvalue_x_7 _returnvalue_y_6 _returnvalue_z_6) (`KismetMathLibrary.BreakVector` (* (+ (`self.FinalStep`) 1) _returnvalue_6)))
  (bind (_returnvalue_x_8 _returnvalue_y_7 _returnvalue_z_7) (`KismetMathLibrary.BreakVector` (* (+ (`self.FinalStep`) 1) _returnvalue_7)))
  (bind (_returnvalue_x_9 _returnvalue_y_8 _returnvalue_z_8) (`KismetMathLibrary.BreakVector` (* (+ (`self.FinalStep`) 1) _returnvalue_4)))
  (`|ExecutionSequence`
    (:`then_0`
      (`|ExecutionSequence`
        (:`then_0`
          (`SceneComponent.SetVisibility` (`self.HISM_St_Ramp01`) `_barrières__` false))
        (:`then_1`
          (`SceneComponent.SetVisibility` (`self.HISM_Md_Ramp01`) `_barrières__` false))
        (:`then_2`
          (`SceneComponent.SetVisibility` (`self.HISM_End_Ramp01`) `_barrières__` false))
        (:`then_3`
          (`SceneComponent.SetVisibility` (`self.HISM_St_Ramp02`) `_barrières__` false))
        (:`then_4`
          (`SceneComponent.SetVisibility` (`self.HISM_Md_Ramp02`) `_barrières__` false))
        (:`then_5`
          (`SceneComponent.SetVisibility` (`self.HISM_End_Ramp02`) `_barrières__` false)
          (`AddComponent|NODE_AddHierarchicalInstancedStaticMeshComponent-1` :`self` (`ActorComponent.GetOwner` (`self.HISM_St_Steps`)))
          (`InstancedStaticMeshComponent.AddInstance` (`self.HISM_St_Steps`) (`KismetMathLibrary.MakeTransform` (0.0 0.0 0.0)) false)
          (`AddComponent|NODE_AddHierarchicalInstancedStaticMeshComponent-2` :`self` (`ActorComponent.GetOwner` (`self.HISM_End_Steps`)))
          (`InstancedStaticMeshComponent.AddInstance` (`self.HISM_End_Steps`) (`KismetMathLibrary.MakeTransform` (0.0 -30.75 35.87)) false)
          (`AddComponent|NODE_AddHierarchicalInstancedStaticMeshComponent-0` :`self` (`ActorComponent.GetOwner` (`self.HISM_Md_Steps`)))
          (`SceneComponent.K2_AddLocalTransform` (`self.HISM_Md_Steps`) (`KismetMathLibrary.MakeTransform` (`KismetMathLibrary.MakeVector` 0.0 _returnvalue_y _returnvalue_z)) false false)
          (for _index (range (`self.Number Steps`))
            (bind _output_get (set `self.FinalStep` _index))
            (bind (_returnvalue_x_10 _returnvalue_y_9 _returnvalue_z_9) (`KismetMathLibrary.BreakVector` (* _output_get _returnvalue_5)))
            (`InstancedStaticMeshComponent.AddInstance` _hism_md_steps (`KismetMathLibrary.MakeTransform` (`KismetMathLibrary.MakeVector` 0.0 _returnvalue_y_9 _returnvalue_z_9)) false)
            (`SceneComponent.K2_SetRelativeLocation` _hism_end_steps (0.0 0.0 0.0) false false)
            (`SceneComponent.K2_AddLocalTransform` _hism_end_steps (`KismetMathLibrary.MakeTransform` (`KismetMathLibrary.MakeVector` 0.0 _returnvalue_y_5 _returnvalue_z_5)) false false)))))
    (:`then_1`
      (`AddComponent|NODE_AddHierarchicalInstancedStaticMeshComponent-4` :`self` (`ActorComponent.GetOwner` (`self.HISM_St_Ramp01`)))
      (`InstancedStaticMeshComponent.AddInstance` (`self.HISM_St_Ramp01`) (`KismetMathLibrary.MakeTransform` (0.0 0.0 0.0)) false)
      (`AddComponent|NODE_AddHierarchicalInstancedStaticMeshComponent-5` :`self` (`ActorComponent.GetOwner` (`self.HISM_End_Ramp01`)))
      (`InstancedStaticMeshComponent.AddInstance` (`self.HISM_End_Ramp01`) (`KismetMathLibrary.MakeTransform` (0.0 -30.75 35.85)) false)
      (`AddComponent|NODE_AddHierarchicalInstancedStaticMeshComponent-3` :`self` (`ActorComponent.GetOwner` (`self.HISM_Md_Ramp01`)))
      (`SceneComponent.K2_AddLocalTransform` (`self.HISM_Md_Ramp01`) (`KismetMathLibrary.MakeTransform` (`KismetMathLibrary.MakeVector` 0.0 _returnvalue_y_4 _returnvalue_z_4)) false false)
      (for _index_2 (range (`self.Number Steps`))
        (bind _output_get_2 (set `self.FinalStep` _index_2))
        (bind (_returnvalue_x_11 _returnvalue_y_10 _returnvalue_z_10) (`KismetMathLibrary.BreakVector` (* _output_get_2 _returnvalue_7)))
        (`InstancedStaticMeshComponent.AddInstance` _hism_md_ramp01 (`KismetMathLibrary.MakeTransform` (`KismetMathLibrary.MakeVector` 0.0 _returnvalue_y_10 _returnvalue_z_10)) false)
        (`SceneComponent.K2_SetRelativeLocation` _hism_end_ramp01 (0.0 0.0 0.0) false false)
        (`SceneComponent.K2_AddLocalTransform` _hism_end_ramp01 (`KismetMathLibrary.MakeTransform` (`KismetMathLibrary.MakeVector` 0.0 _returnvalue_y_7 _returnvalue_z_7)) false false)))
    (:`then_2`
      (`AddComponent|NODE_AddHierarchicalInstancedStaticMeshComponent-8` :`self` (`ActorComponent.GetOwner` (`self.HISM_SmallSteps`)) :`RelativeTransform` (`KismetMathLibrary.MakeTransform` (0.0 0.0 0.0) (struct) (1.0 1.0 1.0)))
      (`InstancedStaticMeshComponent.AddInstance` (`self.HISM_SmallSteps`) (`KismetMathLibrary.MakeTransform` (25.0 0.0 0.0) (struct) (0.0 1.0 1.0)) false)
      (for _index_3 (range (+ (+ 3 (* (`self.Number Steps`) 3)) 1))
        (bind _output_get_3 (set `self.FinalStep` _index_3))
        (bind (_returnvalue_x_12 _returnvalue_y_11 _returnvalue_z_11) (`KismetMathLibrary.BreakVector` (* _output_get_3 (/ (- (- _returnvalue_max _returnvalue_min) (0.0 99.97 31.74)) 3))))
        (`InstancedStaticMeshComponent.AddInstance` (`self.HISM_SmallSteps`) (`KismetMathLibrary.MakeTransform` (`KismetMathLibrary.MakeVector` 0.0 _returnvalue_y_11 _returnvalue_z_11) (struct) (`KismetMathLibrary.MakeVector` (`KismetMathLibrary.FClamp` (* (`self.Width`) 2.0) 0.0 20.0) 1.0 1.0)) false)))
    (:`then_3`
      (`SceneComponent.K2_AddLocalTransform` (`self.Spline`) (`KismetMathLibrary.MakeTransform` (0.0 0.0 0.0) (struct) (`KismetMathLibrary.MakeVector` (`self.Width`) 1.0 1.0)) false false)
      (`AddComponent|NODE_AddHierarchicalInstancedStaticMeshComponent-11` :`self` (`ActorComponent.GetOwner` (`self.HISM_St_Ramp02`)))
      (`InstancedStaticMeshComponent.AddInstance` (`self.HISM_St_Ramp02`) (`KismetMathLibrary.MakeTransform` (`KismetMathLibrary.MakeVector` _returnvalue_2)) false)
      (`AddComponent|NODE_AddHierarchicalInstancedStaticMeshComponent-12` :`self` (`ActorComponent.GetOwner` (`self.HISM_End_Ramp02`)))
      (`InstancedStaticMeshComponent.AddInstance` (`self.HISM_End_Ramp02`) (`KismetMathLibrary.MakeTransform` (0.0 -30.75 35.85)) false)
      (`AddComponent|NODE_AddHierarchicalInstancedStaticMeshComponent-10` :`self` (`ActorComponent.GetOwner` (`self.HISM_Md_Ramp02`)))
      (`SceneComponent.K2_AddLocalTransform` (`self.HISM_Md_Ramp02`) (`KismetMathLibrary.MakeTransform` (`KismetMathLibrary.MakeVector` _returnvalue_2 _returnvalue_y_2 _returnvalue_z_2)) false false)
      (for _index_4 (range (`self.Number Steps`))
        (bind _output_get_4 (set `self.FinalStep` _index_4))
        (bind (_returnvalue_x_13 _returnvalue_y_12 _returnvalue_z_12) (`KismetMathLibrary.BreakVector` (* _output_get_4 _returnvalue_4)))
        (`InstancedStaticMeshComponent.AddInstance` _hism_md_ramp02 (`KismetMathLibrary.MakeTransform` (`KismetMathLibrary.MakeVector` 0.0 _returnvalue_y_12 _returnvalue_z_12)) false)
        (`SceneComponent.K2_SetRelativeLocation` _hism_end_ramp02 (0.0 0.0 0.0) false false)
        (`SceneComponent.K2_AddLocalTransform` _hism_end_ramp02 (`KismetMathLibrary.MakeTransform` (`KismetMathLibrary.MakeVector` _returnvalue_2 _returnvalue_y_8 _returnvalue_z_8)) false false)))
    (:`then_4`
      (`AddComponent|NODE_AddHierarchicalInstancedStaticMeshComponent-17` :`self` (`ActorComponent.GetOwner` (`self.HISM_StartBorder`)))
      (`InstancedStaticMeshComponent.AddInstance` (`self.HISM_StartBorder`) (`KismetMathLibrary.MakeTransform` (`KismetMathLibrary.MakeVector` _returnvalue_3)) false)
      (`AddComponent|NODE_AddHierarchicalInstancedStaticMeshComponent-18` :`self` (`ActorComponent.GetOwner` (`self.HISM_EndBorder`)))
      (`InstancedStaticMeshComponent.AddInstance` (`self.HISM_EndBorder`) (`KismetMathLibrary.MakeTransform` (`KismetMathLibrary.MakeVector` _returnvalue_3 -30.75 35.87)) false)
      (`AddComponent|NODE_AddHierarchicalInstancedStaticMeshComponent-16` :`self` (`ActorComponent.GetOwner` (`self.HISM_MdBorder`)))
      (`SceneComponent.K2_AddLocalTransform` (`self.HISM_MdBorder`) (`KismetMathLibrary.MakeTransform` (`KismetMathLibrary.MakeVector` _returnvalue_3 _returnvalue_y_3 _returnvalue_z_3)) false false)
      (for _index_5 (range (`self.Number Steps`))
        (bind _output_get_5 (set `self.FinalStep` _index_5))
        (bind (_returnvalue_x_14 _returnvalue_y_13 _returnvalue_z_13) (`KismetMathLibrary.BreakVector` (* _output_get_5 _returnvalue_6)))
        (`InstancedStaticMeshComponent.AddInstance` _hism_mdborder (`KismetMathLibrary.MakeTransform` (`KismetMathLibrary.MakeVector` 0.0 _returnvalue_y_13 _returnvalue_z_13)) false)
        (`SceneComponent.K2_SetRelativeLocation` _hism_endborder (0.0 0.0 0.0) false false)
        (`SceneComponent.K2_AddLocalTransform` _hism_endborder (`KismetMathLibrary.MakeTransform` (`KismetMathLibrary.MakeVector` (/ _returnvalue_3 2.0) _returnvalue_y_6 _returnvalue_z_6)) false false)))))