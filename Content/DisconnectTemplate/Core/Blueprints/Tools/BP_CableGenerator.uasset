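; Cable generator tool that builds a cable along an editable spline in its construction script.
; For each segment between spline points it adds a spline mesh component using the cable mesh, uniform cross-section scale and the points' local positions and tangents.
; The sag option has no effect: its branch is empty, and experiments with subdivided sag and instanced meshes along the spline are left disconnected.
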(fn `UserConstructionScript`
  (locals (L_SplineMeshComp :type "SplineMeshComponent Object Reference") (L_StartLocation :type "Vector Structure" :default (0.0 0.0 0.0)) (L_EndLocation :type "Vector Structure" :default (0.0 0.0 0.0)) (L_Alpha :type Integer))
  (bind _meshscale (`self.MeshScale`))
  (bind _returnvalue (`KismetMathLibrary.MakeVector2D` _meshscale _meshscale))
  (for _index (range (+ (- (`SplineComponent.GetNumberOfSplinePoints` (`self.Spline`)) 2) 1))
    (bind _returnvalue_2 (`AddComponent|NODE_AddSplineMeshComponent-5`))
    (bind _output_get (set `local.L_SplineMeshComp` _returnvalue_2))
    (`StaticMeshComponent.SetStaticMesh` _output_get (`self.CableMesh`))
    (`SplineMeshComponent.SetStartScale` (`local.L_SplineMeshComp`) _returnvalue true)
    (`SplineMeshComponent.SetEndScale` (`local.L_SplineMeshComp`) _returnvalue true)
    (bind (_location _tangent) (`SplineComponent.GetLocationAndTangentAtSplinePoint` (`self.Spline`) _index "Local"))
    (set `local.L_StartLocation` _location)
    (bind (_location_2 _tangent_2) (`SplineComponent.GetLocationAndTangentAtSplinePoint` (`self.Spline`) (+ _index 1) "Local"))
    (set `local.L_EndLocation` _location_2)
    (`SplineMeshComponent.SetStartAndEnd` (`local.L_SplineMeshComp`) (`local.L_StartLocation`) _tangent (`local.L_EndLocation`) _tangent_2 true)
    (if (`self.b_Sag?`)
      _)))