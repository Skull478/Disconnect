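; BP_Ventilation is a configurable ventilation prop with case and fan blade meshes, optional Niagara steam and Wwise audio started on BeginPlay.
; The construction script adds both meshes as instanced static meshes.
; Blade rotation is material-driven through axis and speed parameters, with speed either manual or random from a stream.
; Steam visibility is only updated inside the rotation branch, so it depends on rotation being enabled.
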(event `self.ReceiveBeginPlay`
  (`AkGameObject.PostAssociatedAkEvent` :`self` (`self.Play_OBJ_Ventilation_Big`)))

(event `self.ReceiveTick`
  (params (DeltaSeconds :type "Float (single-precision)")))

(fn `F_RotationSpeed`
  (if (`self.b_UseRandomRotation?`)
    (`MeshComponent.SetScalarParameterValueOnMaterials` (`self.ISM_Ventilation_Palm`) "RotationSpeed" (`KismetMathLibrary.RandomFloatInRangeFromStream` (`self.RandomStream`) (`self.MinRotatingSpeed`) (`self.MaxRotatingSpeed`)))
    (else
      (`MeshComponent.SetScalarParameterValueOnMaterials` (`self.ISM_Ventilation_Palm`) "RotationSpeed" (`self.ManualSpeed`)))))

(fn `UserConstructionScript`
  (locals (L_RandomSpeed :type "Float (single-precision)" :default 0.0) (L_ChanceOfNiagara :type "Float (double-precision)" :default 0.35))
  (`InstancedStaticMeshComponent.AddInstance` (`self.ISM_Ventilation_Case`) (`KismetMathLibrary.MakeTransform` (0.0 0.0 0.0)) false)
  (`StaticMeshComponent.SetStaticMesh` (`self.ISM_Ventilation_Case`) (`self.SM_VentilationCase`))
  (`InstancedStaticMeshComponent.AddInstance` (`self.ISM_Ventilation_Palm`) (`KismetMathLibrary.MakeTransform` (0.0 0.0 0.0)) false)
  (`StaticMeshComponent.SetStaticMesh` (`self.ISM_Ventilation_Palm`) (`self.SM_VentilationPalm`))
  (if (`self.b_ActivateRotation?`)
    (`self.F_RotationSpeed`)
    (if (`|EnumEquality` (`self.AxisOfRotation`) "NewEnumerator0")
      (`MeshComponent.SetVectorParameterValueOnMaterials` (`self.ISM_Ventilation_Palm`) "LookAtVector" (1.0 0.0 0.0))
      (`SceneComponent.SetVisibility` (`self.NS_Steam`) (`self.b_ActivateNiagaraSystem?`) false :!label _label)
      (elif (`|EnumEquality` (`self.AxisOfRotation`) "NewEnumerator1")
        (`MeshComponent.SetVectorParameterValueOnMaterials` (`self.ISM_Ventilation_Palm`) "LookAtVector" (0.0 1.0 0.0))
        (goto _label)
        (elif (`|EnumEquality` (`self.AxisOfRotation`) "NewEnumerator2")
          (`MeshComponent.SetVectorParameterValueOnMaterials` (`self.ISM_Ventilation_Palm`) "LookAtVector" (0.0 0.0 1.0))
          (goto _label))))))