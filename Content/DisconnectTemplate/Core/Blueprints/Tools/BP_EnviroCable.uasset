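; BP_EnviroCable is an environment tool actor that strings hanging cables along an editable spline.
; Its construction script adds a cable component at each spline point but the last, ending it at the next point, with shared thickness, gravity scale and material.
; Cable length is the current point's spline distance minus the next's, so the segment span enters as a negative value, plus ExtratLength.
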(fn `UserConstructionScript`
  (locals (L_CableComp :type "CableComponent Object Reference") (L_Index :type Integer))
  (bind _returnvalue (`SplineComponent.GetNumberOfSplinePoints` (`self.Spline`)))
  (for _index (range (+ _returnvalue 1))
    (set `local.L_Index` _index)
    (bind _returnvalue_2 (+ _index 1))
    (if (< _returnvalue_2 _returnvalue)
      (bind (_returnvalue_inputkey _returnvalue_position) (break `SplinePoint` (`SplineComponent.GetSplinePointAt` (`self.Spline`) _index "Local")))
      (bind _returnvalue_3 (`AddComponent|NODE_AddCableComponent-0` :`RelativeTransform` (`KismetMathLibrary.Conv_VectorToTransform` _returnvalue_position)))
      (bind _output_get (set `local.L_CableComp` _returnvalue_3))
      (bind (_returnvalue_inputkey_2 _returnvalue_position_2) (break `SplinePoint` (`SplineComponent.GetSplinePointAt` (`self.Spline`) _returnvalue_2 "Local")))
      (set `CableComponent.EndLocation` _returnvalue_position_2 _output_get)
      (set `CableComponent.CableLength` (+ (- (`SplineComponent.GetDistanceAlongSplineAtSplinePoint` (`self.Spline`) (`local.L_Index`)) (`SplineComponent.GetDistanceAlongSplineAtSplinePoint` (`self.Spline`) _returnvalue_2)) (`self.Extrat_Length`)) (`local.L_CableComp`))
      (set `CableComponent.CableWidth` (`self.Cable_Thickness`) (`local.L_CableComp`))
      (set `CableComponent.CableGravityScale` (`self.Cable_GravityScale`) (`local.L_CableComp`))
      (`PrimitiveComponent.SetMaterial` (`local.L_CableComp`) 0 (`self.Cable_Material`))
      (`ActorComponent.SetComponentTickEnabled` (`self.Spline`) false))))