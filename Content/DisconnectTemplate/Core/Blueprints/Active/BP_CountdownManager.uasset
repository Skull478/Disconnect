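; BP_CountdownManager is a manager actor that prepares static mesh actors for what appears to be a countdown number display.
; When ApplyDMI is set, its construction script loops over RefAndIDs, pairs of actor references and material slot IDs.
; For each valid reference, it creates dynamic instances of MI_NumberNoBackground on those slots.
; BeginPlay only waits through two next-tick delays, with no countdown logic.
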(event `self.ReceiveBeginPlay`
  (`KismetSystemLibrary.DelayUntilNextTick`)
  (`KismetSystemLibrary.DelayUntilNextTick`))

(fn `UserConstructionScript`
  (if (`self.bApplyDMI?`)
    (for _array_element (`self.RefAndIDs`)
      (bind (_reference _materialids) (break `/Game/DisconnectTemplate/Core/Blueprints/Active/S_CountdownInformations` _array_element))
      (`/Engine/EditorBlueprintResources/StandardMacros.IsValid` _reference
        (:`Is Valid`
          (for _array_element_2 _materialids
            (`PrimitiveComponent.CreateDynamicMaterialInstance` (`StaticMeshActor.StaticMeshComponent` _reference) _array_element_2 "/Game/DisconnectTemplate/MaterialLibrary/Flip/Masked/MI_NumberNoBackground.MI_NumberNoBackground" "None")))))))