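; Timer manager actor that shows the match's remaining minutes on number-board materials of referenced static mesh actors.
; The construction script creates a dynamic MI_BoardNumber instance on material slot 2 of each mesh, with a default number.
; A looping one-second SRV event rounds the game mode's CurrentTimeLeft up to whole minutes, retrying the interface-message lookup if the reference is invalid.
; An MC event writes the clamped value to each material's "Numero" parameter.
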(event `self.ReceiveBeginPlay`
  (`self.GetGM_Ref`)
  (`KismetSystemLibrary.K2_SetTimerDelegate` (delegate `SRV_UpdateNumberInDMI`) 1.0 true))

(event `SRV_UpdateNumberInDMI`
  (`self.GM_Ref`
    (:`then`
      (`self.MC_Update` (`KismetMathLibrary.Conv_IntToDouble` (`KismetMathLibrary.FCeil` (/ (`/Game/DisconnectTemplate/Core/Blueprints/Character/Game/BP_DisconnectGame_GameMode.currentTimeLeft` (`self.GM_Ref`)) 60.0)))))
    (:`else`
      (`self.GetGM_Ref`))))

(event `MC_Update`
  (params (Value :type "Float (single-precision)"))
  (for _array_element (`self.DMI_Refs`)
    (`MaterialInstanceDynamic.SetScalarParameterValue` _array_element "Numero" (`KismetMathLibrary.FClamp` Value 0.0 10.0))))

(fn `GetGM_Ref`
  (bind _ref (message `/Game/DisconnectTemplate/Core/Library/BPI_Game_GameMode.GetGameModeRef` (`GameplayStatics.GetGameMode`)))
  (set `self.GM_Ref` _ref))

(fn `UserConstructionScript`
  (`KismetArrayLibrary.Array_Clear` (`self.DMI_Refs`))
  (for _array_element (`self.StaticMeshActorRefs`)
    (bind _returnvalue (`PrimitiveComponent.CreateDynamicMaterialInstance` (`StaticMeshActor.StaticMeshComponent` _array_element) 2 "/Game/DisconnectTemplate/MaterialLibrary/Flip/Masked/MI_BoardNumber.MI_BoardNumber" "None"))
    (`KismetArrayLibrary.Array_AddUnique` (`self.DMI_Refs`) _returnvalue))
  (for _array_element_2 (`self.DMI_Refs`)
    (`MaterialInstanceDynamic.SetScalarParameterValue` _array_element_2 "Numero" 5.0)))