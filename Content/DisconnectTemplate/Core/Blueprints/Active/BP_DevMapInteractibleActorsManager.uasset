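; Manager actor that tracks interactable actors for the dev map and whether each has been notified.
; Construction resets a parallel boolean array, which TSRV functions update as actors are added or change state.
; New actors can trigger MC_TriggerUIForDev, which adds a map message icon to the cached Dev character's HUD.
; UpdateDataActor also sets flags, decoding index and state from a float list.
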(event `self.ReceiveBeginPlay`
  (`KismetSystemLibrary.DelayUntilNextTick`)
  (`KismetSystemLibrary.DelayUntilNextTick`)
  (bind _returnvalue (`GameplayStatics.GetActorOfClass` "/Game/DisconnectTemplate/Core/Blueprints/Character/Game/Dev/BP_DisconnectDev_Character.BP_DisconnectDev_Character_C"))
  (set `self.RefDevChara` _returnvalue))

(event `/Game/DisconnectTemplate/Core/Library/BPI_UpdateData.UpdateDataActor`
  (params (DataList :type "/Game/DisconnectTemplate/Core/Library/S_BasicListOfData Structure"))
  (bind _listoffloat (break `/Game/DisconnectTemplate/Core/Library/S_BasicListOfData` DataList))
  ; Change State of the var in SRV
  (`KismetArrayLibrary.Array_Set` (`self.ActorsHaveBeenNotified?`) (`KismetMathLibrary.FFloor` (`|GetArrayItem` _listoffloat)) (== (`KismetMathLibrary.FFloor` (`|GetArrayItem` _listoffloat 1)) 1)))

(event `MC_TriggerUIForDev`
  (params (InteractActorRef :type "/Game/DisconnectTemplate/Core/Blueprints/InteractableObjects/BP_ParentInteractableObject Object Reference"))
  (bind _devhud_ref (`/Game/DisconnectTemplate/Core/Blueprints/Character/Game/Dev/BP_DisconnectDev_Character.DevHUD_Ref` (`self.RefDevChara`)))
  ; If Dev is it will work
  (`self.RefDevChara`
    (:`then`
      _)
    (:`else`
      (bind _returnvalue (`GameplayStatics.GetActorOfClass` "/Game/DisconnectTemplate/Core/Blueprints/Character/Game/Dev/BP_DisconnectDev_Character.BP_DisconnectDev_Character_C"))
      (set `self.RefDevChara` _returnvalue)))
  (`/Engine/EditorBlueprintResources/StandardMacros.IsValid` _devhud_ref
    (:`Is Valid`
      (message `/Game/DisconnectTemplate/Widgets/Data/BPI_DevHUD.AddIconToMap` _devhud_ref InteractActorRef))))

(fn `getMessages`
  (returns (Messages :type "Array of /Game/DisconnectTemplate/Widgets/Data/S_MessageProfile Structure"))
  (return))

(fn `getPlayerHUD`
  (returns (PlayerHUD :type "/Game/DisconnectTemplate/Widgets/Organismes/WBP_PlayerHUD Object Reference"))
  (return null))

(fn `TSRV_ActorChangeNotify`
  (params (RefInteract :type "/Game/DisconnectTemplate/Core/Blueprints/InteractableObjects/BP_ParentInteractableObject Object Reference (by ref)") (NotifyTo :type Boolean))
  (`KismetArrayLibrary.Array_Set` (`self.ActorsHaveBeenNotified?`) (`KismetArrayLibrary.Array_Find` (`self.ActorsInteractable`) RefInteract) NotifyTo))

(fn `TSRV_AddActor`
  (params (NewItem :type "/Game/DisconnectTemplate/Core/Blueprints/InteractableObjects/BP_ParentInteractableObject Object Reference (by ref)") (`refreshUI?` :type Boolean))
  (bind _actorsinteractable (`self.ActorsInteractable`))
  (bind _returnvalue (`KismetArrayLibrary.Array_AddUnique` _actorsinteractable NewItem))
  (`/Engine/EditorBlueprintResources/StandardMacros.IsValid` (`|GetArrayItem` _actorsinteractable _returnvalue)
    (:`Is Valid`
      (`KismetArrayLibrary.Array_Add` (`self.ActorsHaveBeenNotified?`) true)
      (if `refreshUI?`
        (`self.MC_TriggerUIForDev` (`local.NewItem`))))))

(fn `UserConstructionScript`
  (`KismetArrayLibrary.Array_Clear` (`self.ActorsHaveBeenNotified?`))
  (for _ (`self.ActorsInteractable`)
    (`KismetArrayLibrary.Array_Add` (`self.ActorsHaveBeenNotified?`))))