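; Valve-controlled oil jet that launches characters entering its box along the eject direction, with a fixed upward boost.
; UpdateAndCheckSystem stores the valve angle, whose RepNotify toggles the jet: off inside any paired min/max angle range, on otherwise.
; Toggling scales PivotBox to the throw range or zero and sets the Niagara spawn rate to match.
; The construction script sizes the box and previews this state.
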(event `self.ReceiveBeginPlay`
  (`AkGameObject.PostAssociatedAkEvent` :`self` (`self.Audio`)))

(event `UpdateAndCheckSystem`
  (params (VavleAngle :type "Float (double-precision)"))
  (set `self.ValveCurrentAngle` VavleAngle))

(event `self.Box.OnComponentBeginOverlap`
  (params (OverlappedComponent :type "PrimitiveComponent Object Reference") (OtherActor :type "Actor Object Reference") (OtherComp :type "PrimitiveComponent Object Reference") (OtherBodyIndex :type Integer) (bFromSweep :type Boolean) (SweepResult :type "HitResult Structure (by ref)"))
  ; If it's a character launch it
  (bind _ascharacter (cast `Character` OtherActor))
  (`Character.LaunchCharacter` _ascharacter (+ (* (`SceneComponent.GetForwardVector` (`self.EjectDirection`)) (`KismetSystemLibrary.MakeLiteralDouble` (`self.ThrowForce`))) (0.0 0.0 400.0)) true true))

(fn `checkIfThrowOil`
  (params (ValveAngle :type "Float (double-precision)"))
  (returns (`ThrowOil?` :type Boolean))
  (locals (L_Index :type Integer) (`L_ThrowOil?` :type Boolean))
  (set `local.L_ThrowOil?` true)
  (for _index (range (`KismetArrayLibrary.Array_Length` (`self.VavleAngleMin`)))
    (set `local.L_Index` _index)
    ; If inside this values don't throw oil
    (if (and (>= (`local.ValveAngle`) (`|GetArrayItem` (`self.VavleAngleMin`) (`local.L_Index`))) (<= (`local.ValveAngle`) (`|GetArrayItem` (`self.VavleAngleMax`) (`local.L_Index`))))
      (set `local.L_ThrowOil?` false)
      (break)))
  (return (`local.L_ThrowOil?`)))

(fn `OnRep_ValveCurrentAngle`
  (`self.ThrowOilSystem`))

(fn `setScale`
  (params (Scale :type "Float (double-precision)"))
  (`SceneComponent.SetRelativeScale3D` (`self.PivotBox`) (`KismetMathLibrary.MakeVector` Scale 1.0 1.0)))

(fn `ThrowOilSystem`
  (bind _throwoil_ (`self.checkIfThrowOil` (`self.ValveCurrentAngle`)))
  (if _throwoil_
    (`self.setScale` (/ (`self.OilDistanceThrowRange`) 100.0))
    (`FXSystemComponent.SetFloatParameter` (`self.NS_Oil`) "SpawnRate" 200.0)
    (else
      (`self.setScale` 0.0)
      (`FXSystemComponent.SetFloatParameter` (`self.NS_Oil`) "SpawnRate" 0.0))))

(fn `UserConstructionScript`
  (bind _boxdetectionscale (`self.BoxDetectionScale`))
  (`BoxComponent.SetBoxExtent` (`self.Box`) _boxdetectionscale true)
  (`SceneComponent.K2_SetRelativeLocation` (`self.Box`) (`KismetMathLibrary.MakeVector` (.x _boxdetectionscale)) false false)
  (`self.ThrowOilSystem`))