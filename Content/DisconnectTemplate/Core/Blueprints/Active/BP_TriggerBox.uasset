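; Configurable level trigger box whose type selects checkpoint setting, map travel, checkpoint respawn, floor change, glitch effect, dialogue, cinematic or timer change.
; Overlap sends an action code through the first player controller, returning as UpdateDataActor on the server to dispatch it.
; Respawn teleports the actor to the BP_CheckPointManager transform, spawning a manager if missing.
; Construction colors some types and can add a second box restoring the old floor.
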(event `self.ReceiveBeginPlay`
  (`/Engine/EditorBlueprintResources/ActorMacros.Switch Has Authority`
    (:`Authority`
      (switch `/Game/DisconnectTemplate/Core/Blueprints/Active/E_TypeOfTriggerBox` (`self.TypeOfTrigger`)
        (:`NewEnumerator4`
          (`self.RefManager`
            (:`then`)
            (:`else`
              (bind _returnvalue (`GameplayStatics.GetActorOfClass` "/Game/DisconnectTemplate/Core/Blueprints/Active/BP_CheckPointManager.BP_CheckPointManager_C"))
              (set `self.RefManager` _returnvalue))))))))

(event `self.Box.OnComponentBeginOverlap`
  (params (OverlappedComponent :type "PrimitiveComponent Object Reference") (OtherActor :type "Actor Object Reference") (OtherComp :type "PrimitiveComponent Object Reference") (OtherBodyIndex :type Integer) (bFromSweep :type Boolean) (SweepResult :type "HitResult Structure (by ref)"))
  (set `self.ActorHit` OtherActor)
  (switch `/Game/DisconnectTemplate/Core/Blueprints/Active/E_TypeOfTriggerBox` (`self.TypeOfTrigger`)
    (:`NewEnumerator4`
      (`self.TOWN_CallUpdate` 4.0))
    (:`NewEnumerator0`
      (`self.TOWN_CallUpdate` 0.0))
    (:`NewEnumerator1`
      (`self.TOWN_CallUpdate` 1.0))
    (:`NewEnumerator2`)
    (:`NewEnumerator3`
      (`self.TOWN_CallUpdate` 3.0 (`self.ActorHit`)))
    (:`NewEnumerator5`
      (`self.TOWN_CallUpdate` 5.0))
    (:`NewEnumerator6`
      (`self.TOWN_CallUpdate` 7.0))
    (:`NewEnumerator7`
      (`self.TOWN_CallUpdate` 8.0))
    (:`NewEnumerator8`
      (`self.TOWN_CallUpdate` 9.0))
    (:`NewEnumerator9`
      (`self.TOWN_CallUpdate` 10.0))))

(event `EnterVirusSpace`
  ; Update Data Actor (event triggered in SRV)
)

(event `/Game/DisconnectTemplate/Core/Library/BPI_UpdateData.UpdateDataActor`
  (params (DataList :type "/Game/DisconnectTemplate/Core/Library/S_BasicListOfData Structure"))
  (bind ((`ListOfFloat_3_018B9153488B47BE83268E87B9A7408B` _listoffloat) (`ActorRef_17_7615B6DF4A56B9F3E23F52A40E611D38` _actorref)) (break `/Game/DisconnectTemplate/Core/Library/S_BasicListOfData` DataList))
  ; Update Data Actor (event triggered in SRV)
  (switch `int` (`self.getXFromArrayOfFloat` _listoffloat)
    (:`0`
      (`AdvancedSessionsLibrary.ServerTravel` (`.RightS` (`KismetStringLibrary.Split` (`KismetSystemLibrary.Conv_SoftObjectReferenceToString` (`.WorldAsset` (break `SoftWorldReference` (`self.Map`)))) ".")) true :!label _label))
    (:`1`
      (goto _label))
    (:`3`
      (`self.TSRV_RespawnAtTriggerLoc` (`|GetArrayItem` _actorref)))
    (:`4`
      (bind _refmanager (`self.RefManager`)
        (:`then`
          (set `/Game/DisconnectTemplate/Core/Blueprints/Active/BP_CheckPointManager.CheckpointTransform` (`SceneComponent.K2_GetComponentToWorld` (`self.LookAt`)) _refmanager))
        (:`else`)))
    (:`5`
      (message `/Game/DisconnectTemplate/Core/Library/BPI_Game_GameMode.GM_UpdateFloor` (`GameplayStatics.GetGameMode`) (`self.UpdateToFloor`)))
    (:`6`
      (message `/Game/DisconnectTemplate/Core/Library/BPI_Game_GameMode.GM_UpdateFloor` (`GameplayStatics.GetGameMode`) (`self.OldFloor`)))
    (:`7`
      (`/Engine/EditorBlueprintResources/StandardMacros.DoOnce` false
        (:`Completed`
          (bind _ref (message `/Game/DisconnectTemplate/Core/Library/BPI_Game_GameMode.GetGameModeRef` (`GameplayStatics.GetGameMode`)))
          (`/Game/DisconnectTemplate/Core/Blueprints/Character/Game/BP_DisconnectGame_GameMode.GlitchEffect` _ref false 2.0 false))))
    (:`8`
      (message `/Game/DisconnectTemplate/Core/Library/BPI_Game_GameMode.TriggerDialogue` (`GameplayStatics.GetGameMode`) (`self.DialogueTag`)))
    (:`9`
      (`self.TSRV_Cinematique`))
    (:`10`
      (message `/Game/DisconnectTemplate/Core/Library/BPI_Game_GameMode.GM_SetTime` (`GameplayStatics.GetGameMode`) 300.0))))

(event `SRV_Tp`
  (params (ActorHit :type "Actor Object Reference"))
  ; TP
  (bind _output_get (set `self.ActorHit` ActorHit))
  (`self.K2_TeleportTo` _output_get (+ (`self.K2_GetActorLocation`) (`self.TP_TopLoc`)) (`self.RotationOnTP`)))

(event `TSRV_Cinematique`
  ; CINEMATIC
  (message `/Game/DisconnectTemplate/Core/Library/BPI_Game_GameMode.RemoveHUD` (`GameplayStatics.GetGameMode`))
  (`self.MC_Cinematic`))

(event `MC_Cinematic`
  ; CINEMATIC
  (`MovieSceneSequencePlayer.Play` (`LevelSequenceActor.SequencePlayer` (`self.Cinematic`))))

(event `TSRV_RespawnAtTriggerLoc`
  (params (Target :type "Actor Object Reference"))
  ; Respawn At Trigger Loc
  (`/Engine/EditorBlueprintResources/StandardMacros.IsValid` Target
    (:`Is Valid`
      (set `self.TargetRef` Target)
      (`self.TSR_RespawnEffect` false true)
      (bind _refmanager (`self.RefManager` :!label _label_2)
        (:`then`
          (bind _output_get (set `self.Location` (.location (`/Game/DisconnectTemplate/Core/Blueprints/Active/BP_CheckPointManager.CheckpointTransform` _refmanager))))
          (`self.K2_TeleportTo` (`self.TargetRef`) _output_get (.rotation (`/Game/DisconnectTemplate/Core/Blueprints/Active/BP_CheckPointManager.CheckpointTransform` _refmanager)))
          (message `/Game/DisconnectTemplate/Core/Library/BPI_Game_GameMode.GM_DevProgrammeTimeReduction` (`GameplayStatics.GetGameMode`) "NewEnumerator0"))
        (:`else`
          (bind _returnvalue (`GameplayStatics.GetActorOfClass` "/Game/DisconnectTemplate/Core/Blueprints/Active/BP_CheckPointManager.BP_CheckPointManager_C"))
          (bind _output_get_2 (set `self.RefManager` _returnvalue))
          (`/Engine/EditorBlueprintResources/StandardMacros.IsValid` _output_get_2
            (:`Is Valid`
              (goto _label_2))
            (:`Is Not Valid`
              (bind _returnvalue_2 (`|SpawnActorFromClass` "/Game/DisconnectTemplate/Core/Blueprints/Active/BP_CheckPointManager.BP_CheckPointManager_C" (`KismetMathLibrary.MakeTransform` (0.0 0.0 0.0)) "AlwaysSpawn" "MultiplyWithRoot" null null))
              (set `self.RefManager` _returnvalue_2)
              (goto _label_2))))))))

(event `TSR_RespawnEffect`
  (params (`IsReverse?` :type Boolean) (`BlockMovements?` :type Boolean))
  ; Respawn Effect
  (bind _ref (message `/Game/DisconnectTemplate/Core/Library/BPI_Game_GameMode.GetGameModeRef` (`GameplayStatics.GetGameMode`)))
  (`/Game/DisconnectTemplate/Core/Blueprints/Character/Game/BP_DisconnectGame_GameMode.GlitchEffect` _ref `IsReverse?` 0.2 `BlockMovements?`))

(event `OldFloorBoxOverlap`
  (params (OverlappedComponent :type "PrimitiveComponent Object Reference") (OtherActor :type "Actor Object Reference") (OtherComp :type "PrimitiveComponent Object Reference") (OtherBodyIndex :type Integer) (bFromSweep :type Boolean) (SweepResult :type "HitResult Structure (by ref)"))
  ; Box for changing floor
  (set `self.ActorHit` OtherActor)
  (switch `/Game/DisconnectTemplate/Core/Blueprints/Active/E_TypeOfTriggerBox` (`self.TypeOfTrigger`)
    (:`NewEnumerator5`
      (`self.TOWN_CallUpdate` 6.0))))

(fn `getCurrentFloor`
  (returns (PlayerCurrentFloor :type Integer))
  (return 0))

(fn `getMessages`
  (returns (Messages :type "Array of /Game/DisconnectTemplate/Widgets/Data/S_MessageProfile Structure"))
  (return))

(fn `getPC_KillPlayerCD`
  (returns (CD_KillPlayer :type "Float (double-precision)"))
  (return 0.0))

(fn `getPC_Role`
  (returns (`validPC?` :type Boolean) (PlayerRoles :type "/Game/DisconnectTemplate/Core/Blueprints/Character/Data/EPlayerRole Enum"))
  (return false "NewEnumerator0"))

(fn `getPlayerHUD`
  (returns (PlayerHUD :type "/Game/DisconnectTemplate/Widgets/Organismes/WBP_PlayerHUD Object Reference"))
  (return null))

(fn `getPlayerRotationFromDev_PC`
  (returns (Rotation :type "Rotator Structure"))
  (return))

(fn `getXFromArrayOfFloat`
  (params (Array :type "Array of Float (double-precision)") (Index :type Integer))
  (returns (ReturnValue :type Integer))
  (return (`KismetMathLibrary.FFloor` (`|GetArrayItem` Array Index))))

(fn `OnRep_Location`
  (`KismetMaterialLibrary.SetVectorParameterValue` "/Game/DisconnectTemplate/MaterialLibrary/AllTypeOfGlitchPP/Respawn/PC_WorldRespawn.PC_WorldRespawn" "Location" (`KismetMathLibrary.Conv_VectorToLinearColor` (`self.Location`))))

(fn `OnRep_PPAlpha`
  (`KismetMaterialLibrary.SetScalarParameterValue` "/Game/DisconnectTemplate/MaterialLibrary/AllTypeOfGlitchPP/Respawn/PC_WorldRespawn.PC_WorldRespawn" "Amount" (`self.PPAlpha`)))

(fn `PC_ReturnTimeLeftValueTo`
  (returns (TimeLeft :type "Float (double-precision)") (TimeMax :type "Float (double-precision)"))
  (return 0.0 0.0))

(fn `setShapeColor`
  (params (ShapeColor :type "Color Structure"))
  (set `ShapeComponent.ShapeColor` ShapeColor (`self.Box`)))

(fn `TOWN_CallUpdate`
  (params (float :type "Float (double-precision)") (actor :type "Actor Object Reference"))
  (message `/Game/DisconnectTemplate/Core/Library/BPI_UpdateData.CallUpdate` (`GameplayStatics.GetPlayerController` 0) self (make `/Game/DisconnectTemplate/Core/Library/S_BasicListOfData` :`ListOfFloat` (`|MakeArray` float) :`ActorRef` (`|MakeArray` actor))))

(fn `UserConstructionScript`
  (`BoxComponent.SetBoxExtent` (`self.Box`) (`self.BoxExtent`) true)
  (`SceneComponent.K2_SetRelativeRotation` (`self.LookAt`) (`self.RotationOnTP`) false false)
  (`SceneComponent.K2_SetRelativeLocation` (`self.LookAt`) (`self.TP_TopLoc`) false false)
  (switch `/Game/DisconnectTemplate/Core/Blueprints/Active/E_TypeOfTriggerBox` (`self.TypeOfTrigger`)
    (:`NewEnumerator4`
      (`self.setShapeColor` (`self.ColorNone`)))
    (:`NewEnumerator3`
      (`self.setShapeColor` (`self.ColorRespawAt`)))
    (:`NewEnumerator5`
      (`self.setShapeColor` (`self.ColorChangeFloor`))
      (if (not (`self.bOnlyOneBox?`))
        (bind _returnvalue (`AddComponent|NODE_AddBoxComponent-0`))
        (add `PrimitiveComponent.OnComponentBeginOverlap` _returnvalue (`|CreateDelegate` :!event `OldFloorBoxOverlap`))
        (`BoxComponent.SetBoxExtent` _returnvalue (`BoxComponent.GetScaledBoxExtent` (`self.Box`)) true)
        (`SceneComponent.K2_SetRelativeLocation` _returnvalue (`KismetMathLibrary.MakeVector` (.x (+ (select `bool` (`self.bUseBoxExtentDefaultOffset?`) :`true` (* (`SceneComponent.GetForwardVector` (`self.LookAt`)) (* -1.0 (.x (`BoxComponent.GetScaledBoxExtent` (`self.Box`))) 2.0))) (`self.AddOffsetForBox`))) (.y (+ (select `bool` (`self.bUseBoxExtentDefaultOffset?`) :`true` (* (`SceneComponent.GetForwardVector` (`self.LookAt`)) (* -1.0 (.x (`BoxComponent.GetScaledBoxExtent` (`self.Box`))) 2.0))) (`self.AddOffsetForBox`))) (.z (+ (select `bool` (`self.bUseBoxExtentDefaultOffset?`) :`true` (* (`SceneComponent.GetForwardVector` (`self.LookAt`)) (* -1.0 (.x (`BoxComponent.GetScaledBoxExtent` (`self.Box`))) 2.0))) (`self.AddOffsetForBox`)))) false false)))
    (:`NewEnumerator6`
      (`self.setShapeColor` (`self.ScriptedSpawnEffect`)))
    (:`NewEnumerator7`
      (`self.setShapeColor` (`self.DialogueSystemColor`)))))