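; BP_DevMapCreatorManager is a dev map-creation actor that sets up an orthographic scene capture of the level's floor.
; Two seconds after BeginPlay it scales the capture's ortho width by OrthoSizeMultiplicator.
; The authority then gathers static mesh actors tagged "Floor" and passes them through MC_SetSceneCapture, apparently a multicast, into the capture's show-only list.
; An unconnected player-character lookup never runs.
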(event `self.ReceiveBeginPlay`
  (`KismetSystemLibrary.Delay` 2.0)
  (set `SceneCaptureComponent2D.OrthoWidth` (* 1536.0 (`self.OrthoSizeMultiplicator`)) (`self.SceneCaptureComponent2D`))
  (`/Engine/EditorBlueprintResources/ActorMacros.Switch Has Authority`
    (:`Authority`
      (bind _outactors (`GameplayStatics.GetAllActorsOfClassWithTag` "/Script/Engine.StaticMeshActor" "Floor"))
      (`self.MC_SetSceneCapture` _outactors))))

(event `MC_SetSceneCapture`
  (params (`Show Only Actors` :type "Array of Actor Object Reference"))
  (set `SceneCaptureComponent.ShowOnlyActors` `Show Only Actors` (`self.SceneCaptureComponent2D`)))

(fn `UserConstructionScript`)