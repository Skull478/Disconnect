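; BP_TriggerUpdate is a one-shot sphere trigger that sends a tagged update message to the game mode.
; First overlap by any actor passes the trigger to player controller 0 via CallUpdateMessage; its separate UpdateDataActor event forwards TagTrigger to GameUpdateMessage.
; On authority, BeginPlay polls until it finds and caches BP_DisconnectDev_Character, though this graph never uses that reference.
; The construction script applies the configurable sphere radius.
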(event `self.ReceiveBeginPlay`
  (`KismetSystemLibrary.DelayUntilNextTick`)
  (`KismetSystemLibrary.DelayUntilNextTick`)
  (`/Engine/EditorBlueprintResources/ActorMacros.Switch Has Authority`
    (:`Authority`
      (bind _returnvalue (`GameplayStatics.GetActorOfClass` "/Game/DisconnectTemplate/Core/Blueprints/Character/Game/Dev/BP_DisconnectDev_Character.BP_DisconnectDev_Character_C" :!label _label))
      (`/Engine/EditorBlueprintResources/StandardMacros.IsValid` _returnvalue
        (:`Is Valid`
          (set `self.RefDevChara` _returnvalue))
        (:`Is Not Valid`
          (`KismetSystemLibrary.Delay` 1.0)
          (goto _label))))))

(event `self.Sphere.OnComponentBeginOverlap`
  (params (OverlappedComponent :type "PrimitiveComponent Object Reference") (OtherActor :type "Actor Object Reference") (OtherComp :type "PrimitiveComponent Object Reference") (OtherBodyIndex :type Integer) (bFromSweep :type Boolean) (SweepResult :type "HitResult Structure (by ref)"))
  (`/Engine/EditorBlueprintResources/StandardMacros.DoOnce` false
    (:`Completed`
      (message `/Game/DisconnectTemplate/Core/Library/BPI_UpdateData.CallUpdate` (`GameplayStatics.GetPlayerController` 0) self (struct)))))

(event `/Game/DisconnectTemplate/Core/Library/BPI_UpdateData.UpdateDataActor`
  (params (DataList :type "/Game/DisconnectTemplate/Core/Library/S_BasicListOfData Structure"))
  (message `/Game/DisconnectTemplate/Core/Library/BPI_Game_GameMode.GameUpdate` (`GameplayStatics.GetGameMode`) (`self.TagTrigger`)))

(fn `UserConstructionScript`
  (`SphereComponent.SetSphereRadius` (`self.Sphere`) (`self.InSphereRadius`) true))