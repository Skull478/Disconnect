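; Base Blueprint for interactable objects, providing a look-at outline and key prompt, with interaction events left empty.
; The construction script applies the icon texture, type tag, mesh height, and overlay, sphere and prompt setup.
; Looking at the object sets replicated ActivateOutline, whose OnRep toggles custom depth stencil and prompt visibility.
; A second OnRep applies an outline overlay material; overlap handlers do nothing, and InteractableObjectPutOverlay only prints debug names.
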(event `self.ReceiveBeginPlay`
  ; Setup to false the outline from start
  (`/Engine/EditorBlueprintResources/ActorMacros.Switch Has Authority`
    (:`Authority`
      (set `self.Activate Outline?` false))))

(event `/Game/DisconnectTemplate/Core/Blueprints/InteractableObjects/BPI_InteractableObject.DevInteract`
  (params (Ref :type "/Game/DisconnectTemplate/Core/Blueprints/Character/Game/Dev/BP_DisconnectDev_Character Object Reference")))

(event `/Game/DisconnectTemplate/Core/Blueprints/InteractableObjects/BPI_InteractableObject.PlayerInteract`
  (params (Ref :type "/Game/DisconnectTemplate/Core/Blueprints/Character/Game/Player/BP_DisconnectPlayer_Character Object Reference")))

(event `self.Sphere.OnComponentBeginOverlap`
  (params (OverlappedComponent :type "PrimitiveComponent Object Reference") (OtherActor :type "Actor Object Reference") (OtherComp :type "PrimitiveComponent Object Reference") (OtherBodyIndex :type Integer) (bFromSweep :type Boolean) (SweepResult :type "HitResult Structure (by ref)"))
  (bind _disconnectplayerref (message `/Game/DisconnectTemplate/Core/Blueprints/Character/Game/BPI_DisconnectCharacter.GetPlayerCharacter` OtherActor))
  (`/Engine/EditorBlueprintResources/StandardMacros.IsValid` _disconnectplayerref))

(event `self.Sphere.OnComponentEndOverlap`
  (params (OverlappedComponent :type "PrimitiveComponent Object Reference") (OtherActor :type "Actor Object Reference") (OtherComp :type "PrimitiveComponent Object Reference") (OtherBodyIndex :type Integer))
  (bind _disconnectplayerref (message `/Game/DisconnectTemplate/Core/Blueprints/Character/Game/BPI_DisconnectCharacter.GetPlayerCharacter` OtherActor))
  (`/Engine/EditorBlueprintResources/StandardMacros.IsValid` _disconnectplayerref))

(event `/Game/DisconnectTemplate/Core/Blueprints/InteractableObjects/BPI_InteractableObject.PlayerLookAtInteractableObject`
  (params (`LookAt?` :type Boolean))
  (set `self.Activate Outline?` `LookAt?`))

(fn `getCurrentFloor`
  (returns (PlayerCurrentFloor :type Integer))
  (return 0))

(fn `getMessages`
  (returns (Messages :type "Array of /Game/DisconnectTemplate/Widgets/Data/S_MessageProfile Structure"))
  (return))

(fn `getPC_KillPlayerCD`
  (returns (CD_KillPlayer :type "Float (double-precision)"))
  (return 0.0))

(fn `getPC_Role`
  (returns (`validPC?` :type Boolean) (PlayerRoles :type "/Game/DisconnectTemplate/Core/Blueprints/Character/Data/EPlayerRole Enum"))
  (return false "NewEnumerator0"))

(fn `getPlayerHUD`
  (returns (PlayerHUD :type "/Game/DisconnectTemplate/Widgets/Organismes/WBP_PlayerHUD Object Reference"))
  (return null))

(fn `getPlayerRotationFromDev_PC`
  (returns (Rotation :type "Rotator Structure"))
  (return))

(fn `InteractableObjectPutOverlay`
  (params (`PutAnOverlay?` :type Boolean))
  (returns (`ValidBPI?` :type Boolean))
  (bind _meshtooverlay (`self.MeshToOverlay`))
  (`self.MeshToOverlay`
    (:`then`
      (`KismetSystemLibrary.PrintString` (`KismetSystemLibrary.GetDisplayName` _meshtooverlay) true false (struct :`G` 0.66 :`B` 1.0 :`A` 1.0) 0.2)
      (`KismetSystemLibrary.PrintString` (`KismetSystemLibrary.GetDisplayName` (`MeshComponent.GetOverlayMaterial` _meshtooverlay)) true false (struct :`R` 0.98979 :`G` 0.015 :`B` 1.0 :`A` 1.0) 0.2)
      (return true))
    (:`else`
      (return false))))

(fn `IsInteractible?`
  (returns (IsInteractable :type Boolean))
  (return true))

(fn `OnRep_Activate Outline?`
  (bind _sm_overlaymesh (`self.SM_OverlayMesh`))
  (`PrimitiveComponent.SetRenderCustomDepth` _sm_overlaymesh (`self.Activate Outline?`))
  (`PrimitiveComponent.SetCustomDepthStencilValue` _sm_overlaymesh (`KismetMathLibrary.SelectInt` 2 0 (`self.Activate Outline?`)))
  (`SceneComponent.SetHiddenInGame` (`self.InputToPress`) (not (`self.Activate Outline?`)) false))

(fn `OnRep_Overlay?`
  (`MeshComponent.SetOverlayMaterial` (`self.MeshToOverlay`) (select `bool` (`self.bUseOverlayMesh?`) :`true` "/Game/DisconnectTemplate/MaterialLibrary/Outlines/V2/MI_OutlineV2.MI_OutlineV2" :!type "MaterialInterface Object Reference")))

(fn `PC_ReturnTimeLeftValueTo`
  (returns (TimeLeft :type "Float (double-precision)") (TimeMax :type "Float (double-precision)"))
  (return 0.0 0.0))

(fn `UserConstructionScript`
  (bind _returnvalue (not (`self.bUseOverlayMesh?`)))
  (`|ExecutionSequence`
    (:`then_0`
      (bind _returnvalue_2 (`PrimitiveComponent.CreateDynamicMaterialInstance` (`self.Plane`) 0 "/Game/DisconnectTemplate/Art/Material_GD/Icons/MI_IconTextureTest.MI_IconTextureTest" "None"))
      (`MaterialInstanceDynamic.SetTextureParameterValue` _returnvalue_2 "Texture" (`self.TextureForIcon`))
      ; Set Tags
      (set `self.Tags` (`|MakeArray` (`self.TypeOfInteractable`))))
    (:`then_1`
      (if (`self.bIsOffset?`)
        ; OFFSET ON Z
        (`SceneComponent.K2_SetWorldLocationAndRotation` (`self.SM_Mesh`) (+ (`self.K2_GetActorLocation`) (`KismetMathLibrary.MakeVector` 0.0 0.0 (`self.Z_Offset`))) (struct :`Yaw` 90.0) false false)
        (else
          ; Z ONLY
          (`SceneComponent.K2_SetWorldLocationAndRotation` (`self.SM_Mesh`) (+ (`KismetMathLibrary.MakeVector` (.x (`self.K2_GetActorLocation`)) (.y (`self.K2_GetActorLocation`))) (`KismetMathLibrary.MakeVector` 0.0 0.0 (`self.Z_Offset`))) (struct :`Yaw` 90.0) false false))))
    (:`then_2`
      (`|ExecutionSequence`
        (:`then_0`
          (if (`self.bUseOverlayMesh?`)
            (`PrimitiveComponent.SetCollisionEnabled` (`self.SM_OverlayMesh`) "QueryAndPhysics")
            (else
              (`PrimitiveComponent.SetCollisionEnabled` (`self.SM_OverlayMesh`) "NoCollision"))))
        (:`then_1`
          ; OVERLAY
          (`SceneComponent.SetHiddenInGame` (`self.SM_OverlayMesh`) _returnvalue _returnvalue)
          (set `PrimitiveComponent.bGenerateOverlapEvents` (`self.bUseOverlayMesh?`) (`self.Sphere`))
          (`SphereComponent.SetSphereRadius` (`self.Sphere`) (`self.SphereRadius`) true))
        (:`then_2`
          (if (not (`self.bUseOverlayMesh?`))
            (`SceneComponent.SetHiddenInGame` (`self.InputToPress`) true false))
          (`MaterialBillboardComponent.SetElements` (`self.InputToPress`) (`|MakeArray` (`self.KeyToPressMaterial`)))
          (`SceneComponent.K2_SetRelativeLocation` (`self.InputToPress`) (`self.keyToPressRelativeLocation`) false false))))))