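; Capsule generator actor that randomizes a set of capsules on the server and opens a capsule window on the developer's HUD when interacted with.
; On BeginPlay the authority polls until every capsule reports generated, then shuffles capsules and positions.
; It packs each capsule's colors, logo, numbers, letter and position into parallel arrays stored in CapsuleInfos.
; AttributeGoodCapsules randomly flags good capsules, allowing exactly one wherever a position repeats.
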(event `self.ReceiveBeginPlay`
  (`parent.ReceiveBeginPlay`)
  (`/Engine/EditorBlueprintResources/ActorMacros.Switch Has Authority`
    (:`Authority`
      (bind _l_cangenerate_ (`self.CheckAllCapsuleGenerated?` :!label _label))
      (if _l_cangenerate_
        (`self.TSRV_GenerateCapsule`)
        (else
          (`KismetSystemLibrary.Delay` 0.2)
          (goto _label))))))

(event `TSRV_GenerateCapsule`
  (`KismetArrayLibrary.Array_Clear` (`self.Colors`))
  (`KismetArrayLibrary.Array_Clear` (`self.Numbers1`))
  (`KismetArrayLibrary.Array_Clear` (`self.Numbers2`))
  (`KismetArrayLibrary.Array_Clear` (`self.Letters`))
  (`KismetArrayLibrary.Array_Clear` (`self.Logos`))
  (`KismetArrayLibrary.Array_Clear` (`self.Position`))
  (`KismetArrayLibrary.Array_Clear` (`self.GoodCapsule`))
  (`KismetArrayLibrary.Array_Shuffle` (`self.Capsules`))
  (`KismetArrayLibrary.Array_Shuffle` (`self.PositionArray`))
  (for (_array_element _array_index) (`self.Capsules`)
    (`KismetArrayLibrary.Array_Add` (`self.Colors`) (make `/Game/DisconnectTemplate/Widgets/Data/S_ArrayCapsuleColors` (`/Game/DisconnectTemplate/Core/Blueprints/InteractableObjects/PlayerSide/BP_Capsule.ColorsDisplayed` _array_element)))
    (`KismetArrayLibrary.Array_Add` (`self.Logos`) (`/Game/DisconnectTemplate/Core/Blueprints/InteractableObjects/PlayerSide/BP_Capsule.SymbolDisplayed` _array_element))
    (`KismetArrayLibrary.Array_Add` (`self.Numbers1`) (`/Game/DisconnectTemplate/Core/Blueprints/InteractableObjects/PlayerSide/BP_Capsule.NumberDisplayed1` _array_element))
    (`KismetArrayLibrary.Array_Add` (`self.Numbers2`) (`/Game/DisconnectTemplate/Core/Blueprints/InteractableObjects/PlayerSide/BP_Capsule.NumberDisplayed2` _array_element))
    (`KismetArrayLibrary.Array_Add` (`self.Letters`) (`/Game/DisconnectTemplate/Core/Library/BFL_Disconnect.getNumberToAlphabet` (`/Game/DisconnectTemplate/Core/Blueprints/InteractableObjects/PlayerSide/BP_Capsule.LetterDisplayed` _array_element)))
    (`KismetArrayLibrary.Array_Add` (`self.Position`) (`|GetArrayItem` (`self.PositionArray`) _array_index)))
  (`self.AttributeGoodCapsules`)
  (`KismetArrayLibrary.Array_Add` (`self.CapsuleInfos`) (make `/Game/DisconnectTemplate/Widgets/Data/S_ArrayCapsuleInfos` (`self.Letters`) (`self.Numbers1`) (`self.Numbers2`) (`self.Logos`) (`self.Colors`) (`self.Position`) (`self.GoodCapsule`))))

(event `/Game/DisconnectTemplate/Core/Blueprints/InteractableObjects/BPI_InteractableObject.DevInteract`
  (params (Ref :type "/Game/DisconnectTemplate/Core/Blueprints/Character/Game/Dev/BP_DisconnectDev_Character Object Reference"))
  (bind _devhud_ref (`/Game/DisconnectTemplate/Core/Blueprints/Character/Game/Dev/BP_DisconnectDev_Character.DevHUD_Ref` Ref))
  (set `self.DevControllerRef` (`Pawn.GetLocalViewingPlayerController` Ref))
  (`/Game/DisconnectTemplate/Widgets/Organismes/WBP_DevHUD.AddWindowCapsule` _devhud_ref self)
  (set `self.WBP_CapsuleRef` (`/Game/DisconnectTemplate/Widgets/Organismes/WBP_DevHUD.W_Capsule` _devhud_ref)))

(event `/Game/DisconnectTemplate/Core/Blueprints/InteractableObjects/BPI_InteractableObject.PlayerInteract`
  (params (Ref :type "/Game/DisconnectTemplate/Core/Blueprints/Character/Game/Player/BP_DisconnectPlayer_Character Object Reference"))
  (`/Engine/EditorBlueprintResources/StandardMacros.IsValid` (`/Game/DisconnectTemplate/Core/Blueprints/Character/Game/Player/BP_DisconnectPlayer_Character.InteractedObjectRef` Ref)))

(fn `AttributeGoodCapsules`
  (locals (L_PositionToGoodCapsuleAttributed :type "Array of Integer") (L_RandomBool :type Boolean) (L_CurrentPosition :type Integer) (L_PositionToFalseCapsuleAttributed :type "Array of Integer"))
  (`KismetArrayLibrary.Array_Clear` (`local.L_PositionToGoodCapsuleAttributed`))
  (`KismetArrayLibrary.Array_Clear` (`local.L_PositionToFalseCapsuleAttributed`))
  (for (_ _array_index) (`self.Capsules`)
    (bind _output (`|GetArrayItem` (`self.Position`) _array_index))
    (set `local.L_CurrentPosition` _output)
    (if (`KismetArrayLibrary.Array_Contains` (`local.L_PositionToGoodCapsuleAttributed`) _output)
      (`KismetArrayLibrary.Array_Add` (`self.GoodCapsule`))
      (`KismetArrayLibrary.Array_Add` (`local.L_PositionToFalseCapsuleAttributed`) (`local.L_CurrentPosition`))
      (else
        (set `local.L_RandomBool` (`KismetMathLibrary.RandomBool`))
        (if (`local.L_RandomBool`)
          (`KismetArrayLibrary.Array_Add` (`self.GoodCapsule`) (`local.L_RandomBool`))
          (`KismetArrayLibrary.Array_Add` (`local.L_PositionToGoodCapsuleAttributed`) (`local.L_CurrentPosition`))
          (elif (`KismetArrayLibrary.Array_Contains` (`local.L_PositionToFalseCapsuleAttributed`) (`local.L_CurrentPosition`))
            (`KismetArrayLibrary.Array_Add` (`self.GoodCapsule`) true)
            (`KismetArrayLibrary.Array_Add` (`local.L_PositionToGoodCapsuleAttributed`) (`local.L_CurrentPosition`))
            (else
              (`KismetArrayLibrary.Array_Add` (`self.GoodCapsule`))
              (`KismetArrayLibrary.Array_Add` (`local.L_PositionToFalseCapsuleAttributed`) (`local.L_CurrentPosition`)))))))))

(fn `CheckAllCapsuleGenerated?`
  (returns (`L_CanGenerate?` :type Boolean))
  (locals (`L_AllGenerated?` :type Boolean))
  (set `local.L_AllGenerated?` true)
  (for _array_element (`self.Capsules`)
    (if (not (`/Game/DisconnectTemplate/Core/Blueprints/InteractableObjects/PlayerSide/BP_Capsule.bGenerated?` _array_element))
      (set `local.L_AllGenerated?` false)))
  (return (`local.L_AllGenerated?`)))

(fn `UserConstructionScript`
  (`parent.UserConstructionScript`)
  (bind _returnvalue (`|GenericCreateObject` "/Game/DisconnectTemplate/Core/Blueprints/InteractableObjects/PlayerSide/BO_MapForCapsule.BO_MapForCapsule_C"))
  (set `self.BO_RefForMaps` _returnvalue))