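; Player-side interactable object that blends the player's view to itself on interaction.
; PlayerInteract runs only while no controller is cached: it stores the local controller, registers itself as the interacted object, shows the cursor and sets Game-and-UI input.
; PlayerDesinteract blends back to the player, clears that registration and hides the cursor, leaving the cached controller and input mode unchanged.
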(event `/Game/DisconnectTemplate/Core/Blueprints/InteractableObjects/BPI_InteractableObject.PlayerInteract`
  (params (Ref :type "/Game/DisconnectTemplate/Core/Blueprints/Character/Game/Player/BP_DisconnectPlayer_Character Object Reference"))
  (bind _returnvalue (`Pawn.GetLocalViewingPlayerController` Ref))
  (`self.PlayerControllerRef`
    (:`then`)
    (:`else`
      (set `self.PlayerControllerRef` _returnvalue)
      (`PlayerController.SetViewTargetWithBlend` _returnvalue self (`self.Blend Time`) "VTBlend_Linear" 2.0 false)
      (set `/Game/DisconnectTemplate/Core/Blueprints/Character/Game/Player/BP_DisconnectPlayer_Character.InteractedObjectRef` self Ref)
      (set `PlayerController.bShowMouseCursor` true (`self.PlayerControllerRef`))
      (`WidgetBlueprintLibrary.SetInputMode_GameAndUIEx` (`self.PlayerControllerRef`) null))))

(event `/Game/DisconnectTemplate/Core/Blueprints/InteractableObjects/BPI_InteractableObject.PlayerDesinteract`
  (params (Ref :type "/Game/DisconnectTemplate/Core/Blueprints/Character/Game/Player/BP_DisconnectPlayer_Character Object Reference"))
  (`PlayerController.SetViewTargetWithBlend` (`self.PlayerControllerRef`) Ref (`self.Blend Time`) "VTBlend_Linear" 2.0 false)
  (set `/Game/DisconnectTemplate/Core/Blueprints/Character/Game/Player/BP_DisconnectPlayer_Character.InteractedObjectRef` null Ref)
  (set `PlayerController.bShowMouseCursor` false (`self.PlayerControllerRef`)))

(fn `UserConstructionScript`
  (`parent.UserConstructionScript`))