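; Symbol puzzle actor where players click up to three of ten symbols to match those in the world and send lava into connected cables.
; The server picks three random symbols, and the MeshArray RepNotify builds dynamic icon materials and triggers assigning the picks to world symbol actors.
; Clicks toggle highlights; a correct trio routes through the player controller's update message to UpdateDataActor, which activates the cables.
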(event `self.ReceiveBeginPlay`
  ; Generate random symbols at the start
  (`parent.ReceiveBeginPlay`)
  (`/Engine/EditorBlueprintResources/ActorMacros.Switch Has Authority`
    (:`Authority`
      (`self.GenerateRandomSymbols`)
      (set `self.MeshArray` (`|MakeArray` (`self.Symbol1`) (`self.Symbol2`) (`self.Symbol3`) (`self.Symbol4`) (`self.Symbol5`) (`self.Symbol6`) (`self.Symbol7`) (`self.Symbol8`) (`self.Symbol9`) (`self.Symbol10`))))))

(event `TSRV_GenerateSymbols`
  ; Generate random symbols at the start
  (for (_array_element _array_index) (`self.SymbolsInWorld`)
    (bind _output_get (set `/Game/DisconnectTemplate/Core/Blueprints/InteractableObjects/PlayerSide/BP_WorldSymbol.Symbol` (`|GetArrayItem` (`self.RandomSymbols`) _array_index) _array_element))))

(event `TSRV_ActivateLavaCables`
  ; Send Lava into the cables when the puzzle is completed
  (for _array_element (`self.Lava Cable Connected`)
    (`/Game/DisconnectTemplate/Core/Blueprints/InteractableObjects/PlayerSide/BP_LavaCable.TSRV_PuzzleCompleted` _array_element)))

(event `self.Symbol1.OnClicked`
  (params (TouchedComponent :type "PrimitiveComponent Object Reference") (ButtonPressed :type "Key Structure"))
  ; Select symbols by clicking on them
  (`self.ClickOnSymbols` (`self.Symbol1`)))

(event `self.Symbol6.OnClicked`
  (params (TouchedComponent :type "PrimitiveComponent Object Reference") (ButtonPressed :type "Key Structure"))
  ; Select symbols by clicking on them
  (`self.ClickOnSymbols` (`self.Symbol6`) 5))

(event `self.Symbol2.OnClicked`
  (params (TouchedComponent :type "PrimitiveComponent Object Reference") (ButtonPressed :type "Key Structure"))
  ; Select symbols by clicking on them
  (`self.ClickOnSymbols` (`self.Symbol2`) 1))

(event `self.Symbol7.OnClicked`
  (params (TouchedComponent :type "PrimitiveComponent Object Reference") (ButtonPressed :type "Key Structure"))
  ; Select symbols by clicking on them
  (`self.ClickOnSymbols` (`self.Symbol7`) 6))

(event `/Game/DisconnectTemplate/Core/Library/BPI_UpdateData.UpdateDataActor`
  (params (DataList :type "/Game/DisconnectTemplate/Core/Library/S_BasicListOfData Structure"))
  ; Event update data actor
  (switch `int` (`KismetMathLibrary.FFloor` (`|GetArrayItem` (`.ListOfFloat_3_018B9153488B47BE83268E87B9A7408B` (break `/Game/DisconnectTemplate/Core/Library/S_BasicListOfData` DataList))))
    (:`0`
      (`self.TSRV_ActivateLavaCables`))))

(event `self.Symbol3.OnClicked`
  (params (TouchedComponent :type "PrimitiveComponent Object Reference") (ButtonPressed :type "Key Structure"))
  ; Select symbols by clicking on them
  (`self.ClickOnSymbols` (`self.Symbol3`) 2))

(event `self.Symbol8.OnClicked`
  (params (TouchedComponent :type "PrimitiveComponent Object Reference") (ButtonPressed :type "Key Structure"))
  ; Select symbols by clicking on them
  (`self.ClickOnSymbols` (`self.Symbol8`) 7))

(event `self.Symbol4.OnClicked`
  (params (TouchedComponent :type "PrimitiveComponent Object Reference") (ButtonPressed :type "Key Structure"))
  ; Select symbols by clicking on them
  (`self.ClickOnSymbols` (`self.Symbol4`) 3))

(event `self.Symbol9.OnClicked`
  (params (TouchedComponent :type "PrimitiveComponent Object Reference") (ButtonPressed :type "Key Structure"))
  ; Select symbols by clicking on them
  (`self.ClickOnSymbols` (`self.Symbol9`) 8))

(event `self.Symbol5.OnClicked`
  (params (TouchedComponent :type "PrimitiveComponent Object Reference") (ButtonPressed :type "Key Structure"))
  ; Select symbols by clicking on them
  (`self.ClickOnSymbols` (`self.Symbol5`) 4))

(event `self.Symbol10.OnClicked`
  (params (TouchedComponent :type "PrimitiveComponent Object Reference") (ButtonPressed :type "Key Structure"))
  ; Select symbols by clicking on them
  (`self.ClickOnSymbols` (`self.Symbol10`) 9))

(fn `AllCorrectSymbolsSelected?`
  (returns (`AllSymbolsCorrect?` :type Boolean))
  (locals (L_NumberOfSymbolsCorrect :type Integer))
  (set `local.L_NumberOfSymbolsCorrect` 0)
  (for _array_element (`self.SymbolsInWorld`)
    (if (`|GetArrayItem` (`self.ClickedSymbols`) (`BlueprintMapLibrary.Map_Find` (`self.AllSymbolsMap`) (`/Game/DisconnectTemplate/Core/Blueprints/InteractableObjects/PlayerSide/BP_WorldSymbol.Symbol` _array_element)))
      (`/Engine/EditorBlueprintResources/StandardMacros.IncrementInt` (`local.L_NumberOfSymbolsCorrect`))))
  (return (== (`local.L_NumberOfSymbolsCorrect`) 3)))

(fn `ClickOnSymbols`
  (params (SMClicked :type "StaticMeshComponent Object Reference (by ref)") (Index :type Integer))
  (if (`|GetArrayItem` (`self.ClickedSymbols`) Index)
    (`MaterialInstanceDynamic.SetVectorParameterValue` (`BlueprintMapLibrary.Map_Find` (`self.SM_DMI_Map`) (`local.SMClicked`)) "ColorNumber" (struct :`R` 1.0 :`G` 1.0 :`B` 1.0 :`A` 1.0))
    (`KismetArrayLibrary.Array_Set` (`self.ClickedSymbols`) (`local.Index`))
    (bind _allsymbolscorrect_ (`self.AllCorrectSymbolsSelected?` :!label _label))
    (if _allsymbolscorrect_
      (message `/Game/DisconnectTemplate/Core/Library/BPI_UpdateData.CallUpdate` (`GameplayStatics.GetPlayerController` 0) self (make `/Game/DisconnectTemplate/Core/Library/S_BasicListOfData` (`|MakeArray` 0.0))))
    (elif (< (`/Game/DisconnectTemplate/Core/Library/BFL_Disconnect.getNumberOfTrueAndFalse` (`self.ClickedSymbols`)) 3)
      (`MaterialInstanceDynamic.SetVectorParameterValue` (`BlueprintMapLibrary.Map_Find` (`self.SM_DMI_Map`) (`local.SMClicked`)) "ColorNumber" (struct :`R` 1.0 :`A` 1.0))
      (`KismetArrayLibrary.Array_Set` (`self.ClickedSymbols`) (`local.Index`) true)
      (goto _label))))

(fn `CreateDMI`
  (params (StaticMesh :type "StaticMeshComponent Object Reference (by ref)") (Number :type "Float (single-precision)") (Index :type Integer))
  (bind _index (`local.Index`))
  (bind _returnvalue (`PrimitiveComponent.CreateDynamicMaterialInstance` StaticMesh 0 "/Game/DisconnectTemplate/MaterialLibrary/Flip/MI_Icon.MI_Icon" "None"))
  (`BlueprintMapLibrary.Map_Add` (`self.SM_DMI_Map`) (`local.StaticMesh`) _returnvalue)
  (`MaterialInstanceDynamic.SetScalarParameterValue` _returnvalue "Numero" (`local.Number`))
  (`BlueprintMapLibrary.Map_Add` (`self.AllSymbolsMap`) (`|GetArrayItem` (`self.AllSymbols`) _index) _index))

(fn `GenerateRandomSymbols`
  (locals (L_IntArray :type "Array of Integer"))
  (`KismetArrayLibrary.Array_Clear` (`self.RandomSymbols`))
  (`KismetArrayLibrary.Array_Shuffle` (`local.L_IntArray`))
  (for _index (range 3)
    (`KismetArrayLibrary.Array_AddUnique` (`self.RandomSymbols`) (`|GetArrayItem` (`self.AllSymbols`) (`|GetArrayItem` (`local.L_IntArray`) _index))))
  (set `self.RandomSymbols` (`self.RandomSymbols`)))

(fn `OnRep_MeshArray`
  (for (_array_element _array_index) (`self.MeshArray`)
    (`self.CreateDMI` _array_element (`|GetArrayItem` (`self.IndexToNumber`) _array_index) _array_index))
  (`self.TSRV_GenerateSymbols`))

(fn `UserConstructionScript`
  (locals (IndexToNumber :type "Array of Float (double-precision)"))
  (`parent.UserConstructionScript`))