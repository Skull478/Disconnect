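; Co-op generator puzzle where the player plugs five colored cables into sockets while the Dev's widget shows the correct color order.
; The server randomizes colors and order, with RepNotifies tinting cables and pre-plugging one.
; A looping timer drags cable ends along the deprojected mouse position; each plug-in checks all pairings.
; Controller update messages relay results to the Dev widget and activate the generator, allowing a multicast sequence to open the garage.
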(event `MC_CableColors`
  (params (Target :type "PrimitiveComponent Object Reference") (Value :type "LinearColor Structure"))
  (bind _returnvalue (`PrimitiveComponent.CreateDynamicMaterialInstance` Target 0 "/Game/DisconnectTemplate/Core/Blueprints/InteractableObjects/PlayerSide/CableMaterial/MI_Cable.MI_Cable" "None"))
  (`MaterialInstanceDynamic.SetVectorParameterValue` _returnvalue "ColorAdjustment" Value))

(event `self.ReceiveBeginPlay`
  ; Begin Play
  (`parent.ReceiveBeginPlay`)
  (`KismetSystemLibrary.Delay` 2.5)
  (`/Engine/EditorBlueprintResources/ActorMacros.Switch Has Authority`
    (:`Authority`
      (`self.GenerateCablesV2`)
      (`KismetArrayLibrary.Array_Add` (`self.EndCableLocation`) (`SceneComponent.RelativeLocation` (`self.End1`)))
      (`KismetArrayLibrary.Array_Add` (`self.EndCableLocation`) (`SceneComponent.RelativeLocation` (`self.End2`)))
      (`KismetArrayLibrary.Array_Add` (`self.EndCableLocation`) (`SceneComponent.RelativeLocation` (`self.End3`)))
      (`KismetArrayLibrary.Array_Add` (`self.EndCableLocation`) (`SceneComponent.RelativeLocation` (`self.End4`)))
      (`KismetArrayLibrary.Array_Add` (`self.EndCableLocation`) (`SceneComponent.RelativeLocation` (`self.End5`)))
      (`KismetSystemLibrary.DelayUntilNextTick`)
      (set `self.RandomCableToConnect` (`KismetMathLibrary.RandomIntegerInRange` 0 4)))))

(event `TOWN_CheckCable`
  (params (Index :type Integer) (CubeEnd :type "SceneComponent Object Reference (by ref)"))
  (bind _returnvalue (`SceneComponent.K2_GetComponentLocation` CubeEnd))
  ; Check Cable
  (`KismetSystemLibrary.K2_ClearTimer` null "UpdateCableLoc")
  (`/Engine/EditorBlueprintResources/StandardMacros.IsValid` (`self.EndRef`)
    (:`Is Valid`
      (bind _allcableareconnected (`self.CheckIfCableIsConnected` Index CubeEnd))
      (`SceneComponent.K2_SetWorldLocation` (`self.EndRef`) _returnvalue false false)
      (`NiagaraFunctionLibrary.SpawnSystemAtLocation` "/Game/DisconnectTemplate/VFX/Riddles/NS_SparkleElevator.NS_SparkleElevator" _returnvalue (struct) (0.3 0.3 0.3))
      (`AkGameplayStatics.PostEvent` "/Game/WwiseAudio/Events/Default_Work_Unit/Play_INT_Cable_Plug.Play_INT_Cable_Plug")
      (set `self.EndRef` null)
      (`|ExecutionSequence`
        (:`then_0`
          (if _allcableareconnected
            (message `/Game/DisconnectTemplate/Core/Library/BPI_UpdateData.CallUpdate` (`GameplayStatics.GetPlayerController` 0) self (make `/Game/DisconnectTemplate/Core/Library/S_BasicListOfData` :`ListOfFloat` (`|MakeArray` 1.0)))
            (set `self.AllCableAreGood` true)
            (`AkGameplayStatics.PostEvent` "/Game/WwiseAudio/Events/PlayerEvents/Play_INT_Gen_Success.Play_INT_Gen_Success")))
        (:`then_1`
          ; Call Update (for Dev UI)
          (message `/Game/DisconnectTemplate/Core/Library/BPI_UpdateData.CallUpdate` (`GameplayStatics.GetPlayerController` 0) self (make `/Game/DisconnectTemplate/Core/Library/S_BasicListOfData` :`ListOfFloat` (`|MakeArray` 2.0) :`ListOfInteger` (`|MakeArray` (`KismetMathLibrary.Conv_BoolToInt` _allcableareconnected)))))))))

(event `self.CubeStart1.OnClicked`
  (params (TouchedComponent :type "PrimitiveComponent Object Reference") (ButtonPressed :type "Key Structure"))
  ; Player Interact with wire and desinteract
  (`self.TriggerUpdateCable` (`self.End1`)))

(event `self.CubeEnd1.OnReleased`
  (params (TouchedComponent :type "PrimitiveComponent Object Reference") (ButtonReleased :type "Key Structure"))
  ; Player Interact with wire and desinteract
  (`self.TOWN_CheckCable` 0 (`self.CubeEnd1`)))

(event `self.CubeEnd1.OnClicked`
  (params (TouchedComponent :type "PrimitiveComponent Object Reference") (ButtonPressed :type "Key Structure"))
  ; Player Interact with wire and desinteract
  (`self.TriggerUpdateCable` (`|GetArrayItem` (`self.CableConnected`)) true (`self.CubeEnd1`)))

(event `self.SM_OverlayMesh.OnReleased`
  (params (TouchedComponent :type "PrimitiveComponent Object Reference") (ButtonReleased :type "Key Structure"))
  ; Comment
  (`self.RepositionCurrentCable`))

(event `self.CubeStart2.OnClicked`
  (params (TouchedComponent :type "PrimitiveComponent Object Reference") (ButtonPressed :type "Key Structure"))
  ; Player Interact with wire and desinteract
  (`self.TriggerUpdateCable` (`self.End2`)))

(event `self.CubeEnd2.OnReleased`
  (params (TouchedComponent :type "PrimitiveComponent Object Reference") (ButtonReleased :type "Key Structure"))
  ; Player Interact with wire and desinteract
  (`self.TOWN_CheckCable` 1 (`self.CubeEnd2`)))

(event `self.CubeEnd2.OnClicked`
  (params (TouchedComponent :type "PrimitiveComponent Object Reference") (ButtonPressed :type "Key Structure"))
  ; Player Interact with wire and desinteract
  (`self.TriggerUpdateCable` (`|GetArrayItem` (`self.CableConnected`) 1) true (`self.CubeEnd2`)))

(event `self.CubeStart3.OnClicked`
  (params (TouchedComponent :type "PrimitiveComponent Object Reference") (ButtonPressed :type "Key Structure"))
  ; Player Interact with wire and desinteract
  (`self.TriggerUpdateCable` (`self.End3`)))

(event `self.CubeEnd3.OnReleased`
  (params (TouchedComponent :type "PrimitiveComponent Object Reference") (ButtonReleased :type "Key Structure"))
  ; Player Interact with wire and desinteract
  (`self.TOWN_CheckCable` 2 (`self.CubeEnd3`)))

(event `self.CubeEnd3.OnClicked`
  (params (TouchedComponent :type "PrimitiveComponent Object Reference") (ButtonPressed :type "Key Structure"))
  ; Player Interact with wire and desinteract
  (`self.TriggerUpdateCable` (`|GetArrayItem` (`self.CableConnected`) 2) true (`self.CubeEnd3`)))

(event `self.CubeStart4.OnClicked`
  (params (TouchedComponent :type "PrimitiveComponent Object Reference") (ButtonPressed :type "Key Structure"))
  ; Player Interact with wire and desinteract
  (`self.TriggerUpdateCable` (`self.End4`)))

(event `self.CubeEnd4.OnReleased`
  (params (TouchedComponent :type "PrimitiveComponent Object Reference") (ButtonReleased :type "Key Structure"))
  ; Player Interact with wire and desinteract
  (`self.TOWN_CheckCable` 3 (`self.CubeEnd4`)))

(event `self.CubeEnd4.OnClicked`
  (params (TouchedComponent :type "PrimitiveComponent Object Reference") (ButtonPressed :type "Key Structure"))
  ; Player Interact with wire and desinteract
  (`self.TriggerUpdateCable` (`|GetArrayItem` (`self.CableConnected`) 3) true (`self.CubeEnd4`)))

(event `MC_Sequence`
  ; Sequence
  (bind _sequencerref (`self.SequencerRef`)
    (:`then`
      (`MovieSceneSequencePlayer.Play` (`LevelSequenceActor.SequencePlayer` _sequencerref)))
    (:`else`)))

(event `/Game/DisconnectTemplate/Core/Library/BPI_UpdateData.UpdateDataActor`
  (params (DataList :type "/Game/DisconnectTemplate/Core/Library/S_BasicListOfData Structure"))
  (bind (_listoffloat _command _listofinteger) (break `/Game/DisconnectTemplate/Core/Library/S_BasicListOfData` DataList))
  ; 0 is for open the garage
  (switch `int` (`KismetMathLibrary.FFloor` (`|GetArrayItem` _listoffloat))
    (:`0`
      (if (`self.bGeneratorIsActivated?`)
        (`self.MC_Sequence`)))
    (:`1`
      ;; Set this ref in serv
      (set `self.bGeneratorIsActivated?` true))
    (:`2`
      (`self.MC_ValidateDevGeneratorWidgetRef` (`KismetMathLibrary.Conv_IntToBool` (`|GetArrayItem` _listofinteger))))))

(event `self.CubeStart5.OnClicked`
  (params (TouchedComponent :type "PrimitiveComponent Object Reference") (ButtonPressed :type "Key Structure"))
  ; Player Interact with wire and desinteract
  (`self.TriggerUpdateCable` (`self.End5`)))

(event `self.CubeEnd5.OnReleased`
  (params (TouchedComponent :type "PrimitiveComponent Object Reference") (ButtonReleased :type "Key Structure"))
  ; Player Interact with wire and desinteract
  (`self.TOWN_CheckCable` 4 (`self.CubeEnd5`)))

(event `self.CubeEnd5.OnClicked`
  (params (TouchedComponent :type "PrimitiveComponent Object Reference") (ButtonPressed :type "Key Structure"))
  ; Player Interact with wire and desinteract
  (`self.TriggerUpdateCable` (`|GetArrayItem` (`self.CableConnected`) 4) true (`self.CubeEnd5`)))

(event `MC_ValidateDevGeneratorWidgetRef`
  (params (InputPin :type Boolean))
  ;[0.7 0.1 0 0.5] Ajout d'Alexandre
  (bind _generatorwidget_ref (`self.GeneratorWidget_Ref`)
    (:`then`
      (`/Game/DisconnectTemplate/Widgets/Molecules/Dev/Riddles/WBP_DevGenerator.OnTriggerButton` _generatorwidget_ref InputPin))
    (:`else`)))

(event `/Game/DisconnectTemplate/Core/Blueprints/InteractableObjects/BPI_InteractableObject.DevInteract`
  (params (Ref :type "/Game/DisconnectTemplate/Core/Blueprints/Character/Game/Dev/BP_DisconnectDev_Character Object Reference"))
  (bind _devhud_ref (`/Game/DisconnectTemplate/Core/Blueprints/Character/Game/Dev/BP_DisconnectDev_Character.DevHUD_Ref` Ref))
  (bind _w_generator (`/Game/DisconnectTemplate/Widgets/Organismes/WBP_DevHUD.W_Generator` _devhud_ref))
  ; Dev Interact
  (set `self.DevControllerRef` (`Pawn.GetLocalViewingPlayerController` Ref))
  (message `/Game/DisconnectTemplate/Widgets/Data/BPI_DevHUD.AddWidgetGenerator` _devhud_ref self)
  (`/Engine/EditorBlueprintResources/StandardMacros.IsValid` _w_generator :!label _label
    (:`Is Valid`
      (set `self.GeneratorWidget_Ref` _w_generator)
      (bind _colors (`self.createMapColorsOrder`))
      (`/Game/DisconnectTemplate/Widgets/Molecules/Dev/Riddles/WBP_DevGenerator.ChangeColors` _w_generator _colors)
      (`UserWidget.AddToViewport` _w_generator 0))
    (:`Is Not Valid`
      (`KismetSystemLibrary.DelayUntilNextTick`)
      (goto _label))))

(event `self.DesinteractClear`
  ; Player Desinteract
  (`KismetSystemLibrary.K2_ClearTimer` null "UpdateCableLoc"))

(fn `CheckIfCableIsConnected`
  (params (Index :type Integer) (CubeEnd :type "SceneComponent Object Reference (by ref)"))
  (returns (AllCableAreConnected :type Boolean))
  (locals (L_NumberOfCableConnected :type Integer))
  (bind _output (`|GetArrayItem` (`self.CableConnected`) (`local.Index`)))
  (bind _returnvalue (`KismetStringLibrary.Conv_StringToInt` (`KismetStringLibrary.Conv_NameToString` (`|GetArrayItem` (`ActorComponent.ComponentTags` (`self.EndRef`))))))
  (set `local.L_NumberOfCableConnected` 0)
  (`/Engine/EditorBlueprintResources/StandardMacros.IsValid` _output
    (:`Is Valid`
      (`SceneComponent.K2_SetRelativeLocation` _output (`|GetArrayItem` (`self.EndCableLocation`) (- (`BlueprintMapLibrary.Map_Find` (`self.CableConnectedToEnd`) CubeEnd) 1)) false false)
      (`KismetArrayLibrary.Array_Set` (`self.CableConnected`) (`KismetArrayLibrary.Array_Find` (`self.CableConnected`) (`self.EndRef`)) null true))
    (:`Is Not Valid`
      _))
  (`KismetArrayLibrary.Array_Set` (`self.CableConnected`) (`local.Index`) (`self.EndRef`) true)
  (`BlueprintMapLibrary.Map_Add` (`self.CableConnectedToEnd`) CubeEnd _returnvalue)
  (`BlueprintMapLibrary.Map_Add` (`self.CableConnectedToEndOther`) _returnvalue (`KismetStringLibrary.Conv_StringToInt` (`KismetStringLibrary.Conv_NameToString` (`|GetArrayItem` (`ActorComponent.ComponentTags` CubeEnd)))))
  ; Check if the right cables are connected to the right colors
  (for _index (range 5)
    (if (== (`|GetArrayItem` (`self.ColorsOrder2`) _index) (`BlueprintMapLibrary.Map_Find` (`self.CableConnectedToEndOther`) (`|GetArrayItem` (`self.CableColors2`) (`KismetArrayLibrary.Array_Find` (`self.CableColors1`) (`|GetArrayItem` (`self.ColorsOrder1`) _index)))))
      (set `local.L_NumberOfCableConnected` (+ (`local.L_NumberOfCableConnected`) 1))))
  (return (>= (`local.L_NumberOfCableConnected`) 5)))

(fn `CreateDMIColor`
  (params (Ref :type "PrimitiveComponent Object Reference") (Color :type "LinearColor Structure"))
  (set `self.CurrentRef` Ref))

(fn `createMapCableColors`
  (returns (Colors :type "Map of LinearColor Structure to Integer"))
  (locals (L_Colors :type "Map of LinearColor Structure to Integer") (L_Index :type Integer))
  (for _index (range (`KismetArrayLibrary.Array_Length` (`self.CableColors1`)))
    (set `local.L_Index` _index)
    (`BlueprintMapLibrary.Map_Add` (`local.L_Colors`) (`|GetArrayItem` (`self.CableColors1`) (`local.L_Index`)) (`|GetArrayItem` (`self.CableColors2`) (`local.L_Index`))))
  (return (`local.L_Colors`)))

(fn `createMapColorsOrder`
  (returns (Colors :type "Map of LinearColor Structure to Integer"))
  (locals (L_Colors :type "Map of LinearColor Structure to Integer") (L_Index :type Integer))
  (for _index (range (`KismetArrayLibrary.Array_Length` (`self.ColorsOrder1`)))
    (set `local.L_Index` _index)
    (`BlueprintMapLibrary.Map_Add` (`local.L_Colors`) (`|GetArrayItem` (`self.ColorsOrder1`) (`local.L_Index`)) (`|GetArrayItem` (`self.ColorsOrder2`) (`local.L_Index`))))
  (return (`local.L_Colors`)))

(fn `DisconnectCableConnectedToEnd`
  (params (Index :type Integer) (CubeEnd :type "SceneComponent Object Reference (by ref)"))
  (bind _cableconnected (`self.CableConnected`))
  (bind _output (`|GetArrayItem` (`self.CableConnected`) (`local.Index`)))
  (if (not (`KismetSystemLibrary.K2_IsTimerActive` null "UpdateCableLoc"))
    (`/Engine/EditorBlueprintResources/StandardMacros.IsValid` _output
      (:`Is Valid`
        (`SceneComponent.K2_SetRelativeLocation` _output (`|GetArrayItem` (`self.EndCableLocation`) (- (`BlueprintMapLibrary.Map_Find` (`self.CableConnectedToEnd`) CubeEnd) 1)) false false)
        (`KismetArrayLibrary.Array_Set` _cableconnected (`KismetArrayLibrary.Array_Find` _cableconnected _output))))))

(fn `distance`
  (params (A :type "Float (double-precision)") (B :type "Float (double-precision)"))
  (returns (ReturnValue :type "Float (double-precision)"))
  (return (`KismetMathLibrary.Abs` (- A B))))

(fn `GenerateCables`
  (locals (L_Cable :type "Array of PrimitiveComponent Object Reference") (L_Colors :type "Array of LinearColor Structure") (L_Index :type Integer))
  (bind _l_colors (`local.L_Colors`))
  (bind _l_colors_2 (`local.L_Colors`))
  (bind _output (`|GetArrayItem` _l_colors_2 (`local.L_Index`)))
  (`BlueprintMapLibrary.Map_Clear` (`self.CableColors`))
  (set `local.L_Cable` (`|MakeArray` (`self.Cable1`) (`self.Cable2`) (`self.Cable3`) (`self.Cable4`) (`self.Cable5`) :!type "PrimitiveComponent Object Reference"))
  (set `local.L_Colors` (`self.Colors`))
  (for _array_element (`local.L_Cable`)
    (set `local.L_Index` (`.OutIndex` (`KismetArrayLibrary.Array_RandomFromStream` _l_colors_2 (`self.Stream`))))
    (`self.CreateDMIColor` _array_element _output)
    (`BlueprintMapLibrary.Map_Add` (`self.CableColors`) _output (`KismetStringLibrary.Conv_StringToInt` (`.RightS` (`KismetStringLibrary.Split` (`KismetSystemLibrary.GetDisplayName` _array_element) "BP_Generator.Cable"))))
    (`KismetArrayLibrary.Array_Remove` (`local.L_Colors`) (`local.L_Index`)))
  (set `local.L_Colors` (`self.Colors`))
  (for _index (range 5)
    (set `local.L_Index` (`.OutIndex` (`KismetArrayLibrary.Array_Random` _l_colors)))
    (`BlueprintMapLibrary.Map_Add` (`self.Colors Order`) (`|GetArrayItem` _l_colors (`local.L_Index`)) (+ _index 1))
    (`KismetArrayLibrary.Array_Remove` (`local.L_Colors`) (`local.L_Index`))))

(fn `GenerateCablesV2`
  (locals (L_Cable :type "Array of PrimitiveComponent Object Reference") (L_Colors :type "Array of LinearColor Structure") (L_Index :type Integer))
  (bind _l_colors (`local.L_Colors`))
  (bind _l_colors_2 (`local.L_Colors`))
  (bind _output (`|GetArrayItem` _l_colors_2 (`local.L_Index`)))
  (`KismetArrayLibrary.Array_Clear` (`self.CableColors1`))
  (`KismetArrayLibrary.Array_Clear` (`self.CableColors2`))
  (set `local.L_Cable` (`|MakeArray` (`self.Cable1`) (`self.Cable2`) (`self.Cable3`) (`self.Cable4`) (`self.Cable5`) :!type "PrimitiveComponent Object Reference"))
  (set `local.L_Colors` (`self.Colors`))
  (for (_array_element _array_index) (`local.L_Cable`)
    (set `local.L_Index` (`.OutIndex` (`KismetArrayLibrary.Array_Random` _l_colors_2)))
    (`self.CreateDMIColor` _array_element _output)
    (`KismetArrayLibrary.Array_Set` (`self.CableColors1`) _array_index _output true)
    (`KismetArrayLibrary.Array_Set` (`self.CableColors2`) _array_index (`KismetStringLibrary.Conv_StringToInt` (`KismetStringLibrary.Conv_NameToString` (`|GetArrayItem` (`ActorComponent.ComponentTags` _array_element)))) true)
    (`KismetArrayLibrary.Array_Remove` (`local.L_Colors`) (`local.L_Index`)))
  (set `local.L_Colors` (`self.Colors`))
  (for _index (range 5)
    (set `local.L_Index` (`.OutIndex` (`KismetArrayLibrary.Array_Random` _l_colors)))
    (`KismetArrayLibrary.Array_Set` (`self.ColorsOrder1`) _index (`|GetArrayItem` _l_colors (`local.L_Index`)) true)
    (`KismetArrayLibrary.Array_Set` (`self.ColorsOrder2`) _index (+ _index 1) true)
    (`KismetArrayLibrary.Array_Remove` (`local.L_Colors`) (`local.L_Index`)))
  (set `self.CurrentColors` (`self.CableColors1`)))

(fn `OnRep_CurrentColors`
  (for (_array_element _array_index) (`|MakeArray` (`self.Cable1`) (`self.Cable2`) (`self.Cable3`) (`self.Cable4`) (`self.Cable5`))
    (bind _returnvalue (`PrimitiveComponent.CreateDynamicMaterialInstance` _array_element 0 "/Game/DisconnectTemplate/Core/Blueprints/InteractableObjects/PlayerSide/CableMaterial/MI_Cable.MI_Cable" "None"))
    (`MaterialInstanceDynamic.SetVectorParameterValue` _returnvalue "ColorAdjustment" (`|GetArrayItem` (`self.CurrentColors`) _array_index))))

(fn `OnRep_RandomCableToConnect`
  (bind _cubeend1 (`self.CubeEnd1`))
  (bind _end1 (`self.End1`))
  (bind _output (`|GetArrayItem` (`self.ColorsOrder2`) (`self.RandomCableToConnect`)))
  (set `self.EndRef` (select `int` (`|GetArrayItem` (`self.CableColors2`) (`KismetArrayLibrary.Array_Find` (`self.CableColors1`) (`|GetArrayItem` (`self.ColorsOrder1`) (`self.RandomCableToConnect`)))) :`0` _end1 :`1` _end1 :`2` (`self.End2`) :`3` (`self.End3`) :`4` (`self.End4`) :`5` (`self.End5`)))
  (`self.TOWN_CheckCable` (- _output 1) (select `int` _output :`0` _cubeend1 :`1` _cubeend1 :`2` (`self.CubeEnd2`) :`3` (`self.CubeEnd3`) :`4` (`self.CubeEnd4`) :`5` (`self.CubeEnd5`) :!type "SceneComponent Object Reference")))

(fn `RepositionCurrentCable`
  (`/Engine/EditorBlueprintResources/StandardMacros.IsValid` (`self.EndRef`)
    (:`Is Valid`
      (`SceneComponent.K2_SetRelativeLocation` (`self.EndRef`) (`|GetArrayItem` (`self.EndCableLocation`) (- (`KismetStringLibrary.Conv_StringToInt` (`KismetStringLibrary.Conv_NameToString` (`|GetArrayItem` (`ActorComponent.ComponentTags` (`self.EndRef`))))) 1)) false false)
      (set `self.EndRef` null))))

(fn `TriggerUpdateCable`
  (params (EndRef :type "SceneComponent Object Reference") (`Disconnect?` :type Boolean) (CubeEndRef :type "SceneComponent Object Reference"))
  (bind _cableconnected (`self.CableConnected`))
  (bind _endref (`self.EndRef`))
  (bind (_returnvalue_x _returnvalue_y _returnvalue_z) (`KismetMathLibrary.BreakVector` (`SceneComponent.K2_GetComponentLocation` _endref)))
  (bind (_relativelocation_x _relativelocation_y _relativelocation_z) (`KismetMathLibrary.BreakVector` (`SceneComponent.RelativeLocation` _endref)))
  (if (not (`self.AllCableAreGood`))
    (bind _output_get (set `self.EndRef` EndRef))
    (if `Disconnect?`
      (`KismetArrayLibrary.Array_Set` _cableconnected (`KismetArrayLibrary.Array_Find` _cableconnected _output_get))
      (`BlueprintMapLibrary.Map_Remove` (`self.CableConnectedToEndOther`) (`KismetStringLibrary.Conv_StringToInt` (`KismetStringLibrary.Conv_NameToString` (`|GetArrayItem` (`ActorComponent.ComponentTags` _output_get)))))
      (`BlueprintMapLibrary.Map_Remove` (`self.CableConnectedToEnd`) (`local.CubeEndRef`)))
    (set `self.ZOffset` (- _returnvalue_z _relativelocation_z))
    (set `self.YOffset` (- _returnvalue_y _relativelocation_y))
    (`KismetSystemLibrary.K2_SetTimer` null "UpdateCableLoc" 0.01 true true)
    (`AkGameplayStatics.PostEvent` "/Game/WwiseAudio/Events/Default_Work_Unit/Play_INT_Cable_Select.Play_INT_Cable_Select")))

(fn `UpdateCableLoc`
  (bind _endref (`self.EndRef`))
  (bind _endref_2 (`self.EndRef`))
  (bind (_worldlocation _worlddirection) (`PlayerController.DeprojectMousePositionToWorld` (`self.PlayerControllerRef`)))
  (bind (_returnvalue_x _returnvalue_y _returnvalue_z) (`KismetMathLibrary.BreakVector` (`SceneComponent.K2_GetComponentLocation` _endref)))
  (bind (_relativelocation_x _relativelocation_y _relativelocation_z) (`KismetMathLibrary.BreakVector` (`SceneComponent.RelativeLocation` _endref)))
  (bind _relativelocation_x_2 (`KismetMathLibrary.BreakVector` (`SceneComponent.RelativeLocation` _endref_2)))
  (`/Engine/EditorBlueprintResources/StandardMacros.IsValid` (`self.EndRef`)
    (:`Is Valid`
      (if (`PlayerController.IsInputKeyDown` (`self.PlayerControllerRef`) "LeftMouseButton")
        (set `self.ZOffset` (- _returnvalue_z _relativelocation_z))
        (set `self.YOffset` (- _returnvalue_y _relativelocation_y))
        (`SceneComponent.K2_SetRelativeLocation` _endref_2 (`KismetMathLibrary.MakeVector` _relativelocation_x_2 (- (.y (+ _worldlocation (* _worlddirection (`KismetSystemLibrary.MakeLiteralDouble` (`KismetMathLibrary.Vector_Distance` (`SceneComponent.K2_GetComponentLocation` (`self.EndRef`)) (`PlayerController.DeprojectMousePositionToWorld` (`self.PlayerControllerRef`))))))) (`self.YOffset`)) (- (.z (+ _worldlocation (* _worlddirection (`KismetSystemLibrary.MakeLiteralDouble` (`KismetMathLibrary.Vector_Distance` (`SceneComponent.K2_GetComponentLocation` (`self.EndRef`)) (`PlayerController.DeprojectMousePositionToWorld` (`self.PlayerControllerRef`))))))) (`self.ZOffset`))) false false)))))

(fn `UserConstructionScript`
  (locals (L_Colors :type "Array of LinearColor Structure") (L_Index :type Integer :default 0) (L_Cable :type "Array of PrimitiveComponent Object Reference"))
  (`parent.UserConstructionScript`))