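; BP_Elevator is an interactable elevator whose mesh travels along two splines, one for up/down and one for forward/backward.
; MC_MoveElevator maps a command, received directly or through UpdateDataActor, to playing, reversing or stopping two timelines that place the mesh along its spline.
; DevInteract adds an elevator message widget to the developer HUD.
; The construction script applies mesh, scale and material, then previews position from test alphas, combining both splines.
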(event `self.ReceiveBeginPlay`
  (`parent.ReceiveBeginPlay`)
  (`self.NewTime` (`self.SlpineForwardBackwardValueTest`)))

(event `MC_MoveElevator`
  (params (Selection :type String))
  (bind _splineforwardbackward (`self.SplineForwardBackward`))
  (bind _splineupdown (`self.SplineUpDown`))
  (set `self.Command` Selection)
  (switch `string` (`self.Command`)
    (:`Stop()`
      (`|ExecutionSequence`
        (:`then_0`
          (bind (_direction _newtrack_0) (`Timeline|MoveUpDown` :!via `Stop` :!label _label)
            (:`Update`
              (`SceneComponent.K2_SetWorldLocation` (`self.SM_Elevator`) (`SplineComponent.GetLocationAtDistanceAlongSpline` _splineupdown (`KismetMathLibrary.Lerp` 0.0 (`SplineComponent.GetSplineLength` _splineupdown) _newtrack_0) "World") false false))))
        (:`then_1`
          (bind (_direction_2 _newtrack_0_2) (`Timeline|MoveBackwardForward` :`NewTime` (* (stale `NewTime` NewTime) (`TimelineComponent.GetTimelineLength` (`self.MoveBackwardForward`))) :!via `Stop` :!label _label_2)
            (:`Update`
              (`SceneComponent.K2_SetWorldLocation` (`self.SM_Elevator`) (`SplineComponent.GetLocationAtDistanceAlongSpline` _splineforwardbackward (`KismetMathLibrary.Lerp` 0.0 (`SplineComponent.GetSplineLength` _splineforwardbackward) _newtrack_0_2) "World") false false))))))
    (:`MoveUp()`
      (goto _label))
    (:`MoveDown()`
      (goto _label :!via `Reverse`))
    (:`MoveForward()`
      (goto _label_2))
    (:`MoveBackward()`
      (goto _label_2 :!via `Reverse`))))

(event `NewTime`
  (params (NewTime :type "Float (single-precision)"))
  ; Set the time by the length and value of new time (0 <-> 1)
  (goto _label_2 :!via `SetNewTime`))

(event `/Game/DisconnectTemplate/Core/Library/BPI_UpdateData.UpdateDataActor`
  (params (DataList :type "/Game/DisconnectTemplate/Core/Library/S_BasicListOfData Structure"))
  (`self.MC_MoveElevator` (`|GetArrayItem` (`.Command_7_052874A84B17D8D0D0896993E62AD439` (break `/Game/DisconnectTemplate/Core/Library/S_BasicListOfData` DataList)))))

(event `/Game/DisconnectTemplate/Core/Blueprints/InteractableObjects/BPI_InteractableObject.DevInteract`
  (params (Ref :type "/Game/DisconnectTemplate/Core/Blueprints/Character/Game/Dev/BP_DisconnectDev_Character Object Reference"))
  (set `self.DevControllerRef` (`Pawn.GetLocalViewingPlayerController` Ref))
  (message `/Game/DisconnectTemplate/Widgets/Data/BPI_DevHUD.AddWidgetElevator` (`/Game/DisconnectTemplate/Core/Blueprints/Character/Game/Dev/BP_DisconnectDev_Character.DevHUD_Ref` Ref) self))

(fn `UserConstructionScript`
  (bind _splineforwardbackward (`self.SplineForwardBackward`))
  (bind _sm_elevator (`self.SM_Elevator`))
  (bind _splineupdown (`self.SplineUpDown`))
  (bind (_returnvalue_x _returnvalue_y) (`KismetMathLibrary.BreakVector` (`SplineComponent.GetLocationAtDistanceAlongSpline` _splineforwardbackward (`KismetMathLibrary.Lerp` 0.0 (`SplineComponent.GetSplineLength` _splineforwardbackward) (`self.SlpineForwardBackwardValueTest`)) "World")))
  (bind (_returnvalue_x_2 _returnvalue_y_2 _returnvalue_z) (`KismetMathLibrary.BreakVector` (`SplineComponent.GetLocationAtDistanceAlongSpline` _splineupdown (`KismetMathLibrary.Lerp` 0.0 (`SplineComponent.GetSplineLength` _splineupdown) (`self.SlpineUpDownValueTest`)) "World")))
  (`parent.UserConstructionScript`)
  (`|ExecutionSequence`
    (:`then_0`
      (`StaticMeshComponent.SetStaticMesh` _sm_elevator (`self.SM_ElevatorMesh`))
      (`SceneComponent.SetWorldScale3D` _sm_elevator (`self.SM_ElevatorScale`))
      (bind _elevatormaterial (`self.ElevatorMaterial`)
        (:`then`
          (`PrimitiveComponent.SetMaterial` (`self.SM_Elevator`) 0 _elevatormaterial))
        (:`else`)))
    (:`then_1`
      (`SceneComponent.K2_SetWorldLocation` (`self.SM_Elevator`) (`KismetMathLibrary.MakeVector` _returnvalue_x _returnvalue_y _returnvalue_z) false false))))