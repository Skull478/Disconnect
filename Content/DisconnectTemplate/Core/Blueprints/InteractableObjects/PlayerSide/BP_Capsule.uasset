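; BP_Capsule is a networked capsule that players pick up, inspect and drop, marked with a random symbol, two numbers, a letter and colors.
; The authority randomizes the markings on BeginPlay, and OnRep functions display them through dynamic material instances and visibility.
; Interaction attaches it to the player's item.
; Release sends the player's location for a downward trace whose replicated hit places it, and may insert it into a capsule generator.
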(event `self.ReceiveBeginPlay`
  (bind (_returnvalue_min _returnvalue_max) (break `Box` (`StaticMesh.GetBoundingBox` (`StaticMeshComponent.StaticMesh` (`self.Capsule`)))))
  (bind (_returnvalue_x _returnvalue_y _returnvalue_z) (`KismetMathLibrary.BreakVector` (- _returnvalue_max _returnvalue_min)))
  (`parent.ReceiveBeginPlay`)
  (`/Engine/EditorBlueprintResources/ActorMacros.Switch Has Authority`
    (:`Authority`
      (`self.GenerateCapsule`)
      (set `self.bGenerated?` true)
      (set `self.ZOffset` (/ _returnvalue_z 4.0)))))

(event `/Game/DisconnectTemplate/Core/Blueprints/InteractableObjects/BPI_InteractableObject.PlayerInteract`
  (params (Ref :type "/Game/DisconnectTemplate/Core/Blueprints/Character/Game/Player/BP_DisconnectPlayer_Character Object Reference"))
  (set `/Game/DisconnectTemplate/Core/Blueprints/Character/Game/Player/BP_DisconnectPlayer_Character.CanInspect?` true Ref)
  (set `/Game/DisconnectTemplate/Core/Blueprints/Character/Game/Player/BP_DisconnectPlayer_Character.InteractedObjectRef` self Ref)
  (`KismetSystemLibrary.K2_SetTimer` Ref "CollisionWhenObjectGrabbed" 0.033333 true true)
  (`PrimitiveComponent.SetCollisionEnabled` (`self.Capsule`) "NoCollision")
  (`self.K2_AttachToComponent` (`/Game/DisconnectTemplate/Core/Blueprints/Character/Game/BP_DisconnectCore_Character.Item` Ref) "None" "SnapToTarget" "SnapToTarget" "KeepWorld" false))

(event `/Game/DisconnectTemplate/Core/Blueprints/InteractableObjects/BPI_InteractableObject.PlayerDesinteract`
  (params (Ref :type "/Game/DisconnectTemplate/Core/Blueprints/Character/Game/Player/BP_DisconnectPlayer_Character Object Reference"))
  (bind (_returnvalue_x _returnvalue_y _returnvalue_z) (`KismetMathLibrary.BreakVector` (`self.K2_GetActorLocation` Ref)))
  (`KismetSystemLibrary.K2_ClearTimer` Ref "CollisionWhenObjectGrabbed")
  (set `/Game/DisconnectTemplate/Core/Blueprints/Character/Game/Player/BP_DisconnectPlayer_Character.CanInspect?` false Ref)
  (set `/Game/DisconnectTemplate/Core/Blueprints/Character/Game/Player/BP_DisconnectPlayer_Character.InteractedObjectRef` null Ref)
  (`self.K2_DetachFromActor` "KeepWorld" "KeepWorld" "KeepWorld")
  (`PrimitiveComponent.SetCollisionEnabled` (`self.Capsule`) "QueryAndPhysics")
  (message `/Game/DisconnectTemplate/Core/Library/BPI_UpdateData.CallUpdate` (`GameplayStatics.GetPlayerController` 0) self (make `/Game/DisconnectTemplate/Core/Library/S_BasicListOfData` (`|MakeArray` _returnvalue_x _returnvalue_y _returnvalue_z)))
  (`/Engine/EditorBlueprintResources/StandardMacros.IsValid` (`self.BoxCollisionRef`)
    (:`Is Valid`
      (`/Game/DisconnectTemplate/Core/Blueprints/InteractableObjects/PlayerSide/BP_CapsuleGenerator.PutCapsuleIn` (`self.CapsuleGeneratorRef`) self))))

(event `/Game/DisconnectTemplate/Core/Library/BPI_UpdateData.UpdateDataActor`
  (params (DataList :type "/Game/DisconnectTemplate/Core/Library/S_BasicListOfData Structure"))
  (bind _listoffloat (break `/Game/DisconnectTemplate/Core/Library/S_BasicListOfData` DataList))
  (bind _returnvalue (`KismetMathLibrary.MakeVector` (`|GetArrayItem` _listoffloat) (`|GetArrayItem` _listoffloat 1) (`|GetArrayItem` _listoffloat 2)))
  (bind _outhit (`KismetSystemLibrary.LineTraceSingleForObjects` _returnvalue (- _returnvalue (0.0 0.0 2000.0)) (`|MakeArray` "ObjectTypeQuery1" "ObjectTypeQuery2" :!type "EObjectTypeQuery Enum")))
  (set `self.LocationToPutObjectDown` (`.Location` (`GameplayStatics.BreakHitResult` _outhit))))

(fn `DefaultValues`
  (bind _returnvalue (`PrimitiveComponent.CreateDynamicMaterialInstance` (`self.DefaultLetter`) 1 "/Game/DisconnectTemplate/MaterialLibrary/Flip/MI_Alphabet.MI_Alphabet" "None"))
  (`MaterialInstanceDynamic.SetScalarParameterValue` _returnvalue "Numero" 2.0)
  (bind _returnvalue_2 (`PrimitiveComponent.CreateDynamicMaterialInstance` (`self.DefaultNumber2`) 1 "/Game/DisconnectTemplate/MaterialLibrary/Flip/MI_Numbers.MI_Numbers" "None"))
  (`MaterialInstanceDynamic.SetScalarParameterValue` _returnvalue_2 "Numero" 7.0)
  (bind _returnvalue_3 (`PrimitiveComponent.CreateDynamicMaterialInstance` (`self.DefaultNumber3`) 1 "/Game/DisconnectTemplate/MaterialLibrary/Flip/MI_Numbers.MI_Numbers" "None"))
  (`MaterialInstanceDynamic.SetScalarParameterValue` _returnvalue_3 "Numero" 0.0)
  (bind _returnvalue_4 (`PrimitiveComponent.CreateDynamicMaterialInstance` (`self.DefaultNumber4`) 1 "/Game/DisconnectTemplate/MaterialLibrary/Flip/MI_Numbers.MI_Numbers" "None"))
  (`MaterialInstanceDynamic.SetScalarParameterValue` _returnvalue_4 "Numero" 8.0)
  (bind _returnvalue_5 (`PrimitiveComponent.CreateDynamicMaterialInstance` (`self.DefaultNumber1`) 1 "/Game/DisconnectTemplate/MaterialLibrary/Flip/MI_Numbers.MI_Numbers" "None"))
  (`MaterialInstanceDynamic.SetScalarParameterValue` _returnvalue_5 "Numero" 0.0))

(fn `GenerateCapsule`
  (locals (L_Rnds :type "Array of Integer") (L_Symbols :type "Array of Texture2D Object Reference"))
  (`KismetArrayLibrary.Array_Shuffle` (`self.RndIntForColors`))
  (`KismetArrayLibrary.Array_Clear` (`self.ColorsDisplayed`))
  (`KismetArrayLibrary.Array_Shuffle` (`self.PossibleColors`))
  (set `self.RndIntSymbols` (`KismetMathLibrary.RandomIntegerInRange` 0 2))
  (set `self.SymbolDisplayed` (`|GetArrayItem` (`local.L_Symbols`) (`self.RndIntSymbols`)))
  (set `self.SM_ForColors` (`|MakeArray` (`self.Color1`) (`self.Color2`) (`self.Color3`)))
  (set `self.Numero1Ref` (`KismetMathLibrary.RandomIntegerInRange` 0 8))
  (set `self.NumberDisplayed1` (+ (`self.Numero1Ref`) 1))
  (set `self.Numero2Ref` (`KismetMathLibrary.RandomIntegerInRange` 0 8))
  (set `self.NumberDisplayed2` (+ (`self.Numero2Ref`) 1))
  (set `self.LetterRef` (`KismetMathLibrary.RandomIntegerInRange` 0 25))
  (set `self.LetterDisplayed` (`self.LetterRef`)))

(fn `GetCapsule`
  (returns (CapsuleRef :type "/Game/DisconnectTemplate/Core/Blueprints/InteractableObjects/PlayerSide/BP_Capsule Object Reference"))
  (return self))

(fn `OnRep_IndexLoopForColors`)

(fn `OnRep_LetterDisplayed`
  (bind _returnvalue (`PrimitiveComponent.CreateDynamicMaterialInstance` (`self.Number1`) 1 "/Game/DisconnectTemplate/MaterialLibrary/Flip/MI_Numbers.MI_Numbers" "None"))
  (`MaterialInstanceDynamic.SetScalarParameterValue` _returnvalue "Numero" (`KismetMathLibrary.Conv_IntToDouble` (`self.Numero1Ref`)))
  (bind _returnvalue_2 (`PrimitiveComponent.CreateDynamicMaterialInstance` (`self.Number2`) 1 "/Game/DisconnectTemplate/MaterialLibrary/Flip/MI_Numbers.MI_Numbers" "None"))
  (`MaterialInstanceDynamic.SetScalarParameterValue` _returnvalue_2 "Numero" (`KismetMathLibrary.Conv_IntToDouble` (`self.Numero2Ref`)))
  (bind _returnvalue_3 (`PrimitiveComponent.CreateDynamicMaterialInstance` (`self.Letter`) 1 "/Game/DisconnectTemplate/MaterialLibrary/Flip/MI_Alphabet.MI_Alphabet" "None"))
  (`MaterialInstanceDynamic.SetScalarParameterValue` _returnvalue_3 "Numero" (`KismetMathLibrary.Conv_IntToDouble` (`self.LetterRef`))))

(fn `OnRep_LocationToPutObjectDown`
  (bind (_locationtoputobjectdown_x _locationtoputobjectdown_y _locationtoputobjectdown_z) (`KismetMathLibrary.BreakVector` (`self.LocationToPutObjectDown`)))
  (`self.K2_SetActorLocationAndRotation` (`KismetMathLibrary.MakeVector` _locationtoputobjectdown_x _locationtoputobjectdown_y (+ _locationtoputobjectdown_z (`self.ZOffset`))))
  (`SceneComponent.K2_SetRelativeRotation` :`self` (`self.Capsule`)))

(fn `OnRep_SM_ForColors`
  (for (_array_element _array_index) (`self.SM_ForColors`)
    (set `self.currentTargetForDMI` _array_element)
    (set `self.IndexLoopForColors` _array_index)
    (bind _returnvalue (`PrimitiveComponent.CreateDynamicMaterialInstance` (`self.currentTargetForDMI`) 0 "/Game/DisconnectTemplate/MaterialLibrary/Master/M_BaseColor.M_BaseColor" "None"))
    (`MaterialInstanceDynamic.SetVectorParameterValue` _returnvalue "Color" (`|GetArrayItem` (`self.PossibleColors`) (`self.IndexLoopForColors`)))
    (if (== (`|GetArrayItem` (`self.RndIntForColors`) (`self.IndexLoopForColors`)) 0)
      (`SceneComponent.SetVisibility` (`self.currentTargetForDMI`) false false)
      (`KismetArrayLibrary.Array_Add` (`self.ColorsDisplayed`))
      (else
        (`KismetArrayLibrary.Array_Add` (`self.ColorsDisplayed`) (`|GetArrayItem` (`self.PossibleColors`) (`self.IndexLoopForColors`)))
        (`SceneComponent.SetVisibility` (`self.currentTargetForDMI`) true false)))))

(fn `OnRep_SymbolDisplayed`
  (bind _returnvalue (`PrimitiveComponent.CreateDynamicMaterialInstance` (`self.Symbol`) 1 "/Game/DisconnectTemplate/MaterialLibrary/Flip/MI_Symbol.MI_Symbol" "None"))
  (`MaterialInstanceDynamic.SetScalarParameterValue` _returnvalue "Numero" (`KismetMathLibrary.Conv_IntToDouble` (`self.RndIntSymbols`))))

(fn `UserConstructionScript`
  (`parent.UserConstructionScript`)
  (`self.DefaultValues`))