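; Base Blueprint for a player-side interactable capsule that animates between two states and tracks whether it is occupied.
; UpdateDataActor truncates the first float of incoming data into Anim, then calls MC_Anim, which plays the actor sequence forward or in reverse and sets IsOccupied to match.
; Anim's RepNotify repeats the sequence playback on replication but leaves IsOccupied untouched.
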(event `self.ReceiveBeginPlay`
  (`parent.ReceiveBeginPlay`))

(event `/Game/DisconnectTemplate/Core/Library/BPI_UpdateData.UpdateDataActor`
  (params (DataList :type "/Game/DisconnectTemplate/Core/Library/S_BasicListOfData Structure"))
  (set `self.Anim` (`KismetMathLibrary.FTrunc` (`|GetArrayItem` (`.ListOfFloat_3_018B9153488B47BE83268E87B9A7408B` (break `/Game/DisconnectTemplate/Core/Library/S_BasicListOfData` DataList)))))
  (`self.MC_Anim`))

(event `MC_Anim`
  (switch `int` (`self.Anim`)
    (:`0`
      (set `self.IsOccupied` true)
      (`MovieSceneSequencePlayer.Play` (`ActorSequenceComponent.SequencePlayer` (`self.ActorSequence`))))
    (:`1`
      (`MovieSceneSequencePlayer.PlayReverse` (`ActorSequenceComponent.SequencePlayer` (`self.ActorSequence`)))
      (set `self.IsOccupied` false))))

(fn `OnRep_Anim`
  (switch `int` (`self.Anim`)
    (:`0`
      (`MovieSceneSequencePlayer.Play` (`ActorSequenceComponent.SequencePlayer` (`self.ActorSequence`))))
    (:`1`
      (`MovieSceneSequencePlayer.PlayReverse` (`ActorSequenceComponent.SequencePlayer` (`self.ActorSequence`))))))

(fn `UserConstructionScript`
  (`parent.UserConstructionScript`))