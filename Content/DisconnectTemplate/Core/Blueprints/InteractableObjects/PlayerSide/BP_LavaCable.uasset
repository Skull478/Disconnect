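; Spline-based lava cable that visually fills with lava when its puzzle completes, then triggers the next linked cable.
; The construction script tiles a mesh along the spline as spline mesh segments, each with its own dynamic material.
; On completion, a timeline replays for each segment in turn, with rate set by a duration variable.
; Timeline progress goes to a RepNotify variable that drives the current material's Time parameter, replicating the fill.
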(event `self.ReceiveBeginPlay`)

(event `FilltheLava`
  (bind _output (`|GetArrayItem` (`self.DMI_Array`) (`self.Index`)))
  (`/Engine/EditorBlueprintResources/StandardMacros.IsValid` _output :!label _label
    (:`Is Valid`
      (set `self.MaterialToEdit` _output)
      (bind (_direction _newtrack_0) (`Timeline|T_LavaFill` :!via `PlayFromStart`)
        (:`Update`
          (set `self.New Track 0` _newtrack_0))
        (:`Finished`
          (set `self.Index` (+ (`self.Index`) 1))
          (`self.FilltheLava`))))
    (:`Is Not Valid`
      (`self.TSRV_PuzzleCompleted` (`self.NextCable`)))))

(event `TSRV_PuzzleCompleted`
  (`TimelineComponent.SetPlayRate` (`self.T_LavaFill`) (/ 1.0 (`self.TimelineDuration`)))
  (set `self.Index` 0)
  (goto _label))

(fn `OnRep_New Track 0`
  (`MaterialInstanceDynamic.SetScalarParameterValue` (`self.MaterialToEdit`) "Time" (`self.New Track 0`)))

(fn `UserConstructionScript`
  (bind _spline1 (`self.Spline1`))
  (bind _spline1_2 (`self.Spline1`))
  (bind (_returnvalue_min _returnvalue_max) (break `Box` (`StaticMesh.GetBoundingBox` (`self.Mesh`))))
  (bind (_returnvalue_x _returnvalue_y _returnvalue_z) (`KismetMathLibrary.BreakVector` (+ (`KismetMathLibrary.Vector_GetAbs` _returnvalue_min) (`KismetMathLibrary.Vector_GetAbs` _returnvalue_max))))
  (bind _output_get (set `self.Length` (select `ESplineMeshAxis` (`self.Axis`) :`X` _returnvalue_x :`Y` _returnvalue_y :`Z` _returnvalue_z)))
  (for _index (range (+ (`KismetMathLibrary.FTrunc` (/ (`SplineComponent.GetSplineLength` (`self.Spline1`)) _output_get)) 1))
    (bind _returnvalue (`AddComponent|NODE_AddSplineMeshComponent-1`))
    (`PrimitiveComponent.SetCollisionEnabled` _returnvalue "QueryAndPhysics")
    (`SplineMeshComponent.SetForwardAxis` _returnvalue (`self.Axis`) true)
    (`StaticMeshComponent.SetStaticMesh` _returnvalue (`self.Mesh`))
    (bind _returnvalue_2 (`PrimitiveComponent.CreateDynamicMaterialInstance` _returnvalue 0 (`self.Material`) "None"))
    (`KismetArrayLibrary.Array_Add` (`self.DMI_Array`) _returnvalue_2)
    (bind _returnvalue_3 (* _index (`self.Length`)))
    (bind _returnvalue_4 (* (+ _index 1) (`self.Length`)))
    (`SplineMeshComponent.SetStartAndEnd` _returnvalue (`SplineComponent.GetLocationAtDistanceAlongSpline` _spline1_2 _returnvalue_3 "Local") (`KismetMathLibrary.ClampVectorSize` (`SplineComponent.GetTangentAtDistanceAlongSpline` _spline1_2 _returnvalue_3 "Local") 0.0 (`self.Length`)) (`SplineComponent.GetLocationAtDistanceAlongSpline` _spline1 _returnvalue_4 "Local") (`KismetMathLibrary.ClampVectorSize` (`SplineComponent.GetTangentAtDistanceAlongSpline` _spline1 _returnvalue_4 "Local") 0.0 (`self.Length`)) true)))