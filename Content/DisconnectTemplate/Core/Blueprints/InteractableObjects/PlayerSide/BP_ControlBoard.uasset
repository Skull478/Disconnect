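; Clickable control board puzzle prop with number buttons, on/off toggles, exclusive left/right arrows, oil selectors with reset, a slider and a wheel.
; BeginPlay sets NumberMeshArray, whose OnRep builds a mesh-to-dynamic-material map for changing digits, symbols and colors.
; Clicks update state and materials, while oil picks color and raise up to three liquid meshes in turn.
; Slider and wheel follow the deprojected mouse via looping timers, snapping to the nearest preset on release.
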(event `self.ReceiveBeginPlay`
  (`parent.ReceiveBeginPlay`)
  (set `self.NumberMeshArray` (`|MakeArray` (`self.Button_Number1`) (`self.Button_Number2`))))

(event `self.Button_Number1.OnClicked`
  (params (TouchedComponent :type "PrimitiveComponent Object Reference") (ButtonPressed :type "Key Structure"))
  (`self.ChangeNumber` (`self.Button_Number1`)))

(event `self.ButtonOnOff1.OnClicked`
  (params (TouchedComponent :type "PrimitiveComponent Object Reference") (ButtonPressed :type "Key Structure"))
  (`self.ClickButtonOnOff` (`self.ButtonOnOff1`)))

(event `self.OilType1.OnClicked`
  (params (TouchedComponent :type "PrimitiveComponent Object Reference") (ButtonPressed :type "Key Structure"))
  (`self.AddLiquid` (struct :`R` 1.0 :`A` 1.0)))

(event `self.ButtonOnOff2.OnClicked`
  (params (TouchedComponent :type "PrimitiveComponent Object Reference") (ButtonPressed :type "Key Structure"))
  (`self.ClickButtonOnOff` (`self.ButtonOnOff2`) 1))

(event `self.Button_Number2.OnClicked`
  (params (TouchedComponent :type "PrimitiveComponent Object Reference") (ButtonPressed :type "Key Structure"))
  (`self.ChangeNumber` (`self.Button_Number2`) 1))

(event `self.OilType2.OnClicked`
  (params (TouchedComponent :type "PrimitiveComponent Object Reference") (ButtonPressed :type "Key Structure"))
  (`self.AddLiquid` (struct :`B` 1.0 :`A` 1.0)))

(event `self.ButtonOnOff3.OnClicked`
  (params (TouchedComponent :type "PrimitiveComponent Object Reference") (ButtonPressed :type "Key Structure"))
  (`self.ClickButtonOnOff` (`self.ButtonOnOff3`) 2))

(event `self.Button_ArrowL.OnClicked`
  (params (TouchedComponent :type "PrimitiveComponent Object Reference") (ButtonPressed :type "Key Structure"))
  (`self.ClickButtonRightLeft` (`self.Button_ArrowL`) false (`self.Button_ArrowR`)))

(event `self.OilType3.OnClicked`
  (params (TouchedComponent :type "PrimitiveComponent Object Reference") (ButtonPressed :type "Key Structure"))
  (`self.AddLiquid` (struct :`G` 1.0 :`A` 1.0)))

(event `self.ButtonOnOff4.OnClicked`
  (params (TouchedComponent :type "PrimitiveComponent Object Reference") (ButtonPressed :type "Key Structure"))
  (`self.ClickButtonOnOff` (`self.ButtonOnOff4`) 3))

(event `self.Button_ArrowR.OnClicked`
  (params (TouchedComponent :type "PrimitiveComponent Object Reference") (ButtonPressed :type "Key Structure"))
  (`self.ClickButtonRightLeft` (`self.Button_ArrowR`) true (`self.Button_ArrowL`)))

(event `self.Reset.OnClicked`
  (params (TouchedComponent :type "PrimitiveComponent Object Reference") (ButtonPressed :type "Key Structure"))
  (`self.ResetLiquid`))

(event `self.ButtonOnOff5.OnClicked`
  (params (TouchedComponent :type "PrimitiveComponent Object Reference") (ButtonPressed :type "Key Structure"))
  (`self.ClickButtonOnOff` (`self.ButtonOnOff5`) 4))

(event `self.Slider.OnClicked`
  (params (TouchedComponent :type "PrimitiveComponent Object Reference") (ButtonPressed :type "Key Structure"))
  (bind _slider (`self.Slider`))
  (bind (_returnvalue_x _returnvalue_y _returnvalue_z) (`KismetMathLibrary.BreakVector` (`SceneComponent.K2_GetComponentLocation` _slider)))
  (bind (_relativelocation_x _relativelocation_y _relativelocation_z) (`KismetMathLibrary.BreakVector` (`SceneComponent.RelativeLocation` _slider)))
  (set `self.ZOffset` (- _returnvalue_z _relativelocation_z))
  (`KismetSystemLibrary.K2_SetTimer` null "UpdateSliderLoc" 0.01 true true))

(event `self.Wheel.OnClicked`
  (params (TouchedComponent :type "PrimitiveComponent Object Reference") (ButtonPressed :type "Key Structure"))
  (`KismetSystemLibrary.K2_SetTimer` null "UpdateWheelRotation" 0.01 true true))

(fn `AddLiquid`
  (params (OilColor :type "LinearColor Structure"))
  (bind _numberofoiladded (`self.NumberOfOilAdded`))
  (`/Engine/EditorBlueprintResources/StandardMacros.IncrementInt` _numberofoiladded
    (:`  `
      (switch `int` _numberofoiladded
        (:`1`
          (`self.AddOilToCorrespondantPosition` (`self.Liquid1`) (`local.OilColor`)))
        (:`2`
          (`self.AddOilToCorrespondantPosition` (`self.Liquid2`) (`local.OilColor`)))
        (:`3`
          (`self.AddOilToCorrespondantPosition` (`self.Liquid3`) (`local.OilColor`)))))))

(fn `AddOilToCorrespondantPosition`
  (params (SM_ToMove :type "StaticMeshComponent Object Reference (by ref)") (OilColor :type "LinearColor Structure"))
  (bind (_relativelocation_x _relativelocation_y _relativelocation_z) (`KismetMathLibrary.BreakVector` (`SceneComponent.RelativeLocation` SM_ToMove)))
  (`MaterialInstanceDynamic.SetVectorParameterValue` (`BlueprintMapLibrary.Map_Find` (`self.SM DMI Map`) SM_ToMove) "Color" (`local.OilColor`))
  (`SceneComponent.K2_SetRelativeLocation` (`local.SM_ToMove`) (`KismetMathLibrary.MakeVector` _relativelocation_x _relativelocation_y (+ _relativelocation_z 15.0)) false false))

(fn `ChangeNumber`
  (params (SM_Clicked :type "StaticMeshComponent Object Reference") (Index :type Integer))
  (bind _value (`BlueprintMapLibrary.Map_Find` (`self.SM DMI Map`) (`local.SM_Clicked`)))
  (bind _returnvalue (`MaterialInstanceDynamic.K2_GetScalarParameterValue` _value "Numero"))
  (bind _returnvalue_2 (select `bool` (> _returnvalue 7.0) :`false` (+ _returnvalue 1.0) :!type "Float (single-precision)"))
  (`MaterialInstanceDynamic.SetScalarParameterValue` _value "Numero" _returnvalue_2)
  (`KismetArrayLibrary.Array_Set` (`self.Numbers`) (`local.Index`) (+ (`KismetMathLibrary.FTrunc` _returnvalue_2) 1)))

(fn `ClickButtonOnOff`
  (params (SM_Clicked :type "StaticMeshComponent Object Reference") (Index :type Integer))
  (bind _value (`BlueprintMapLibrary.Map_Find` (`self.SM DMI Map`) (`local.SM_Clicked`)))
  (bind _returnvalue (not (`|GetArrayItem` (`self.ButtonsOn?`) (`local.Index`))))
  (bind _returnvalue_2 (`MaterialInstanceDynamic.K2_GetVectorParameterValue` _value "Color"))
  (`MaterialInstanceDynamic.SetVectorParameterValue` _value "Color" (select `int` (`KismetMathLibrary.Conv_DoubleToInt64` (`.G` (`KismetMathLibrary.BreakColor` _returnvalue_2))) :`0` (struct :`G` 1.0 :`A` 1.0) :`1` (struct :`R` 1.0 :`A` 1.0) :!type "LinearColor Structure"))
  (`KismetSystemLibrary.PrintString` (`KismetStringLibrary.Conv_BoolToString` _returnvalue) true false (struct :`R` 1.0 :`G` 0.073719 :`B` 0.470803 :`A` 1.0) 10.0)
  (`KismetArrayLibrary.Array_Set` (`self.ButtonsOn?`) (`local.Index`) _returnvalue))

(fn `ClickButtonRightLeft`
  (params (SM_Clicked :type "StaticMeshComponent Object Reference") (RightClicked :type Boolean) (SM_NotClicked :type "StaticMeshComponent Object Reference"))
  (bind _value (`BlueprintMapLibrary.Map_Find` (`self.SM DMI Map`) (`local.SM_NotClicked`)))
  (bind _value_2 (`BlueprintMapLibrary.Map_Find` (`self.SM DMI Map`) (`local.SM_Clicked`)))
  (if (not (== RightClicked (`self.RightSelected`)))
    (bind _returnvalue (`MaterialInstanceDynamic.K2_GetVectorParameterValue` _value_2 "Color"))
    (`MaterialInstanceDynamic.SetVectorParameterValue` _value_2 "Color" (select `int` (`KismetMathLibrary.Conv_DoubleToInt64` (`.G` (`KismetMathLibrary.BreakColor` _returnvalue))) :`0` (struct :`R` 1.0 :`G` 1.0 :`B` 1.0 :`A` 1.0) :`1` (struct :`A` 1.0) :!type "LinearColor Structure"))
    (bind _returnvalue_2 (`MaterialInstanceDynamic.K2_GetVectorParameterValue` _value "Color"))
    (`MaterialInstanceDynamic.SetVectorParameterValue` _value "Color" (select `int` (`KismetMathLibrary.Conv_DoubleToInt64` (`.G` (`KismetMathLibrary.BreakColor` _returnvalue_2))) :`0` (struct :`R` 1.0 :`G` 1.0 :`B` 1.0 :`A` 1.0) :`1` (struct :`A` 1.0) :!type "LinearColor Structure"))
    (set `self.RightSelected` (`local.RightClicked`))))

(fn `CreateDMI`
  (params (StaticMesh :type "StaticMeshComponent Object Reference") (MaterialIndex :type Integer) (SourceMaterial :type "MaterialInterface Object Reference") (`ScalarParameter?` :type Boolean) (Color :type "LinearColor Structure") (Numero :type Integer))
  (bind _returnvalue (`PrimitiveComponent.CreateDynamicMaterialInstance` StaticMesh MaterialIndex SourceMaterial "None"))
  (`BlueprintMapLibrary.Map_Add` (`self.SM DMI Map`) (`local.StaticMesh`) _returnvalue)
  (if (`local.ScalarParameter?`)
    (`MaterialInstanceDynamic.SetScalarParameterValue` _returnvalue "Numero" (`KismetMathLibrary.Conv_IntToDouble` (- (`local.Numero`) 1)))
    (else
      (`MaterialInstanceDynamic.SetVectorParameterValue` _returnvalue "Color" (`local.Color`)))))

(fn `NearestSlider`
  (returns (LocToClamp :type "Float (double-precision)"))
  (locals (L_LowestDistance :type "Float (double-precision)") (L_LocToClamp :type "Float (double-precision)"))
  (bind (_relativelocation_x _relativelocation_y _relativelocation_z) (`KismetMathLibrary.BreakVector` (`SceneComponent.RelativeLocation` (`self.Slider`))))
  (set `local.L_LowestDistance` 1000.0)
  (for _array_element (`self.SliderLoc`)
    (bind _distance (`/Game/DisconnectTemplate/Core/Library/BFL_Disconnect.getFloatDistance` _relativelocation_z _array_element))
    (if (< _distance (`local.L_LowestDistance`))
      (set `local.L_LowestDistance` _distance)
      (set `local.L_LocToClamp` _array_element)))
  (return (`local.L_LocToClamp`)))

(fn `NearestWheelRotation`
  (returns (RotationToGo :type "Float (double-precision)"))
  (locals (L_LowestDifference :type "Float (double-precision)" :default 1000.0) (L_RotationToGo :type "Float (double-precision)"))
  (bind _relativerotation_roll (`KismetMathLibrary.BreakRotator` (`SceneComponent.RelativeRotation` (`self.Wheel`))))
  (for _array_element (`self.WheelRotation`)
    (bind _returnvalue (`KismetMathLibrary.Abs` (- _array_element (select `bool` (< _relativerotation_roll 0.0) :`false` _relativerotation_roll :`true` (+ _relativerotation_roll 360.0) :!type "Float (double-precision)"))))
    (if (< _returnvalue (`local.L_LowestDifference`))
      (set `local.L_LowestDifference` _returnvalue)
      (set `local.L_RotationToGo` _array_element)))
  (return (`local.L_RotationToGo`)))

(fn `OnRep_NumberMeshArray`
  (for _array_element (`self.NumberMeshArray`)
    (`self.CreateDMI` _array_element 1 "/Game/DisconnectTemplate/MaterialLibrary/Flip/MI_Numbers.MI_Numbers" true (struct) 1))
  (for _array_element_2 (`|MakeArray` (`self.ButtonOnOff1`) (`self.ButtonOnOff2`) (`self.ButtonOnOff3`) (`self.ButtonOnOff4`) (`self.ButtonOnOff5`))
    (`self.CreateDMI` _array_element_2 1 "/Game/DisconnectTemplate/MaterialLibrary/Instance/MI_BaseColor.MI_BaseColor" false (struct :`R` 1.0 :`A` 1.0)))
  (for (_array_element_3 _array_index) (`|MakeArray` (`self.SliderNumber1`) (`self.SliderNumber2`) (`self.SliderNumber3`) (`self.SliderNumber4`) (`self.SliderNumber5`) (`self.SliderNumber6`))
    (`self.CreateDMI` _array_element_3 1 "/Game/DisconnectTemplate/MaterialLibrary/Flip/MI_Numbers.MI_Numbers" true (struct :`A` 1.0) (+ _array_index 1)))
  (for (_array_element_4 _array_index_2) (`|MakeArray` (`self.OilType1`) (`self.OilType2`) (`self.OilType3`))
    (`self.CreateDMI` _array_element_4 1 "/Game/DisconnectTemplate/MaterialLibrary/Flip/MI_Symbol.MI_Symbol" true (struct :`A` 1.0) (+ _array_index_2 1)))
  (for _array_element_5 (`|MakeArray` (`self.Liquid1`) (`self.Liquid2`) (`self.Liquid3`))
    (`self.CreateDMI` _array_element_5 0 "/Game/DisconnectTemplate/MaterialLibrary/Instance/MI_BaseColor.MI_BaseColor"))
  (`self.CreateDMI` (`self.Button_ArrowR`) 1 "/Game/DisconnectTemplate/MaterialLibrary/Instance/MI_BaseColor.MI_BaseColor" false (struct :`A` 1.0))
  (set `self.RightSelected` true)
  (`self.CreateDMI` (`self.Button_ArrowL`) 1 "/Game/DisconnectTemplate/MaterialLibrary/Instance/MI_BaseColor.MI_BaseColor" false (struct :`R` 1.0 :`G` 1.0 :`B` 1.0 :`A` 1.0)))

(fn `ResetLiquid`
  (set `self.NumberOfOilAdded` 0)
  (for _array_element (`|MakeArray` (`self.Liquid1`) (`self.Liquid2`) (`self.Liquid3`))
    (bind (_relativelocation_x _relativelocation_y _relativelocation_z) (`KismetMathLibrary.BreakVector` (`SceneComponent.RelativeLocation` _array_element)))
    (`SceneComponent.K2_SetRelativeLocation` _array_element (`KismetMathLibrary.MakeVector` _relativelocation_x _relativelocation_y (- _relativelocation_z 15.0)) false false)))

(fn `UpdateSliderLoc`
  (bind (_worldlocation _worlddirection) (`PlayerController.DeprojectMousePositionToWorld` (`self.PlayerControllerRef`)))
  (bind (_relativelocation_x _relativelocation_y) (`KismetMathLibrary.BreakVector` (`SceneComponent.RelativeLocation` (`self.Slider`))))
  (bind (_relativelocation_x_2 _relativelocation_y_2) (`KismetMathLibrary.BreakVector` (`SceneComponent.RelativeLocation` (`self.Slider`))))
  (if (`PlayerController.IsInputKeyDown` (`self.PlayerControllerRef`) "LeftMouseButton")
    (`SceneComponent.K2_SetRelativeLocation` (`self.Slider`) (`KismetMathLibrary.MakeVector` _relativelocation_x _relativelocation_y (`KismetMathLibrary.FClamp` (- (.z (+ _worldlocation (* _worlddirection (`KismetSystemLibrary.MakeLiteralDouble` (`KismetMathLibrary.Vector_Distance` (`SceneComponent.K2_GetComponentLocation` (`self.Slider`)) (`PlayerController.DeprojectMousePositionToWorld` (`self.PlayerControllerRef`))))))) (`self.ZOffset`)) -36.0 34.0)) false false)
    (else
      (`KismetSystemLibrary.K2_ClearTimer` null "UpdateSliderLoc")
      (bind _loctoclamp (`self.NearestSlider`))
      (`SceneComponent.K2_SetRelativeLocation` (`self.Slider`) (`KismetMathLibrary.MakeVector` _relativelocation_x_2 _relativelocation_y_2 _loctoclamp) false false))))

(fn `UpdateWheelRotation`
  (bind (_worldlocation _worlddirection) (`PlayerController.DeprojectMousePositionToWorld` (`self.PlayerControllerRef`)))
  (bind _returnvalue (`SceneComponent.K2_GetComponentLocation` (`self.Wheel`)))
  (bind (_relativerotation_roll _relativerotation_pitch _relativerotation_yaw) (`KismetMathLibrary.BreakRotator` (`SceneComponent.RelativeRotation` (`self.Wheel`))))
  (bind (_relativerotation_roll_2 _relativerotation_pitch_2 _relativerotation_yaw_2) (`KismetMathLibrary.BreakRotator` (`SceneComponent.RelativeRotation` (`self.Wheel`))))
  (if (`PlayerController.IsInputKeyDown` (`self.PlayerControllerRef`) "LeftMouseButton")
    (`SceneComponent.K2_SetRelativeRotation` (`self.Wheel`) (`KismetMathLibrary.MakeRotator` (`KismetMathLibrary.DegAtan2` (.y (- (+ _worldlocation (* _worlddirection (`KismetMathLibrary.Vector_Distance` _worldlocation _returnvalue))) _returnvalue)) (.z (- (+ _worldlocation (* _worlddirection (`KismetMathLibrary.Vector_Distance` _worldlocation _returnvalue))) _returnvalue))) _relativerotation_pitch_2 _relativerotation_yaw_2) false false)
    (else
      (`KismetSystemLibrary.K2_ClearTimer` null "UpdateWheelRotation")
      (bind _rotationtogo (`self.NearestWheelRotation`))
      (`SceneComponent.K2_SetRelativeRotation` (`self.Wheel`) (`KismetMathLibrary.MakeRotator` _rotationtogo _relativerotation_pitch _relativerotation_yaw) false false))))

(fn `UserConstructionScript`
  (`parent.UserConstructionScript`))