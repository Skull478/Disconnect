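; Sliding-tile puzzle (taquin) actor with eight numbered cubes, where clicking a cube moves it into an adjacent free slot.
; On authority at BeginPlay, it picks a random preset from RandomTaquin as the goal layout, matched to cubes by component tag.
; Each move checks positions against that goal and only prints on completion.
; UpdateDataActor restores construction-time positions and rebuilds the goal; DevInteract opens a Taquin window on the dev HUD.
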(event `/Game/DisconnectTemplate/Core/Library/BPI_UpdateData.UpdateDataActor`
  (params (DataList :type "/Game/DisconnectTemplate/Core/Library/S_BasicListOfData Structure"))
  (`self.MC_ResetPositions`))

(event `MC_ResetPositions`
  (bind (_keypin _valuepin) (`|MapForEach` (`self.StartingPositions`))
    (:`then`
      (`SceneComponent.K2_SetRelativeLocation` _valuepin _keypin false false))
    (:`CompletedPin`
      (`self.SetUpRandomPositions`))))

(event `self.ReceiveBeginPlay`
  ; Set up positions of squares
  (`parent.ReceiveBeginPlay`)
  (`/Engine/EditorBlueprintResources/ActorMacros.Switch Has Authority`
    (:`Authority`
      (set `self.IndexStructure` (`.OutIndex` (`KismetArrayLibrary.Array_Random` (`self.RandomTaquin`))))
      (`self.SetUpRandomPositions`)
      (set `self.MeshToOverlay` (`self.SUPERCUBE`)))))

(event `self.Cube1.OnClicked`
  (params (TouchedComponent :type "PrimitiveComponent Object Reference") (ButtonPressed :type "Key Structure"))
  ; Interact with squares and move them
  (`self.MoveCube` TouchedComponent))

(event `self.Cube2.OnClicked`
  (params (TouchedComponent :type "PrimitiveComponent Object Reference") (ButtonPressed :type "Key Structure"))
  ; Interact with squares and move them
  (`self.MoveCube` TouchedComponent))

(event `self.Cube3.OnClicked`
  (params (TouchedComponent :type "PrimitiveComponent Object Reference") (ButtonPressed :type "Key Structure"))
  ; Interact with squares and move them
  (`self.MoveCube` TouchedComponent))

(event `self.Cube4.OnClicked`
  (params (TouchedComponent :type "PrimitiveComponent Object Reference") (ButtonPressed :type "Key Structure"))
  ; Interact with squares and move them
  (`self.MoveCube` TouchedComponent))

(event `self.Cube5.OnClicked`
  (params (TouchedComponent :type "PrimitiveComponent Object Reference") (ButtonPressed :type "Key Structure"))
  ; Interact with squares and move them
  (`self.MoveCube` TouchedComponent))

(event `self.Cube6.OnClicked`
  (params (TouchedComponent :type "PrimitiveComponent Object Reference") (ButtonPressed :type "Key Structure"))
  ; Interact with squares and move them
  (`self.MoveCube` TouchedComponent))

(event `self.Cube7.OnClicked`
  (params (TouchedComponent :type "PrimitiveComponent Object Reference") (ButtonPressed :type "Key Structure"))
  ; Interact with squares and move them
  (`self.MoveCube` TouchedComponent))

(event `self.Cube8.OnClicked`
  (params (TouchedComponent :type "PrimitiveComponent Object Reference") (ButtonPressed :type "Key Structure"))
  ; Interact with squares and move them
  (`self.MoveCube` TouchedComponent))

(event `/Game/DisconnectTemplate/Core/Blueprints/InteractableObjects/BPI_InteractableObject.DevInteract`
  (params (Ref :type "/Game/DisconnectTemplate/Core/Blueprints/Character/Game/Dev/BP_DisconnectDev_Character Object Reference"))
  (set `self.DevControllerRef` (`Pawn.GetLocalViewingPlayerController` Ref))
  (`/Game/DisconnectTemplate/Widgets/Organismes/WBP_DevHUD.AddWindowTaquin` (`/Game/DisconnectTemplate/Core/Blueprints/Character/Game/Dev/BP_DisconnectDev_Character.DevHUD_Ref` Ref) self))

(fn `CheckIfCubeAreInRightPositions`
  (returns (CorrectTaquin :type Boolean))
  (locals (L_CorrectSquares :type Integer))
  (set `local.L_CorrectSquares` 0)
  (for _array_element (`self.Squares`)
    (if (== (`SceneComponent.RelativeLocation` _array_element) (`|GetArrayItem` (`self.SquarePositionsGoal2`) (`KismetArrayLibrary.Array_Find` (`self.SquarePositionsGoal1`) (`|GetArrayItem` (`ActorComponent.ComponentTags` _array_element)))) :`ErrorTolerance` 5.0)
      (bind _output_get (set `local.L_CorrectSquares` (+ (`local.L_CorrectSquares`) 1)))
      (`KismetSystemLibrary.PrintString` (`KismetStringLibrary.Conv_IntToString` _output_get) true false (struct :`R` 0.585286 :`G` 0.142877 :`B` 1.0 :`A` 1.0))))
  (return (== (`local.L_CorrectSquares`) 8)))

(fn `GetArrayOfRandomTaquin`
  (returns (Array :type "Array of Integer"))
  (return (`.RandomTaquin_3_922D51DB4B691E8C1348CE906E618B3C` (break `/Game/DisconnectTemplate/Widgets/Data/S_ArrayTaquin` (`|GetArrayItem` (`self.RandomTaquin`) (`self.IndexStructure`))))))

(fn `MoveCube`
  (params (CubeInteracted :type "SceneComponent Object Reference"))
  (bind _output_get (set `self.SquareRef` CubeInteracted))
  (set `self.PositionToMove` (`SceneComponent.RelativeLocation` _output_get))
  (for _array_element (`self.PossibleMovement`)
    (bind _returnvalue (+ (`SceneComponent.RelativeLocation` (`self.SquareRef`)) _array_element))
    (if (`KismetArrayLibrary.Array_Contains` (`self.PositionOccupied`) _returnvalue)
      _
      (elif (`KismetArrayLibrary.Array_Contains` (`self.AllPositions`) _returnvalue)
        (set `self.PositionToMove` _returnvalue)
        (break))))
  (`KismetArrayLibrary.Array_RemoveItem` (`self.PositionOccupied`) (`SceneComponent.RelativeLocation` (`self.SquareRef`)))
  (`SceneComponent.K2_SetRelativeLocation` (`self.SquareRef`) (`self.PositionToMove`) false false)
  (`KismetArrayLibrary.Array_Add` (`self.PositionOccupied`) (`self.PositionToMove`))
  (set `self.SquareRef` null)
  (bind _correcttaquin (`self.CheckIfCubeAreInRightPositions`))
  (if _correcttaquin
    (`KismetSystemLibrary.PrintString` "TAQUIN FINISHED" true false (struct :`R` 0.585286 :`G` 0.142877 :`B` 1.0 :`A` 1.0) 10.0)))

(fn `SetUpRandomPositions`
  (locals (L_AllPositions :type "Array of Vector Structure") (L_Index :type Integer) (L_Index1 :type Integer))
  (`KismetArrayLibrary.Array_Clear` (`self.SquarePositionsGoal1`))
  (`KismetArrayLibrary.Array_Clear` (`self.SquarePositionsGoal2`))
  (`KismetArrayLibrary.Array_Clear` (`self.PositionOccupied`))
  (`BlueprintMapLibrary.Map_Clear` (`self.SquarePositions`))
  (set `local.L_AllPositions` (`self.AllPositions`))
  (set `self.Squares` (`|MakeArray` (`self.Cube1`) (`self.Cube2`) (`self.Cube3`) (`self.Cube4`) (`self.Cube5`) (`self.Cube6`) (`self.Cube7`) (`self.Cube8`) :!type "SceneComponent Object Reference"))
  (for _array_element (`self.Squares`)
    (bind _relativelocation (`SceneComponent.RelativeLocation` _array_element))
    (`KismetArrayLibrary.Array_Add` (`self.PositionOccupied`) _relativelocation)
    (`BlueprintMapLibrary.Map_Add` (`self.SquarePositions`) (`|GetArrayItem` (`ActorComponent.ComponentTags` _array_element)) _relativelocation))
  (for (_array_element_2 _array_index) (`self.GetArrayOfRandomTaquin`)
    (`KismetArrayLibrary.Array_Set` (`self.SquarePositionsGoal1`) _array_index (`KismetStringLibrary.Conv_StringToName` (`KismetStringLibrary.Conv_IntToString` _array_element_2)) true)
    (`KismetArrayLibrary.Array_Set` (`self.SquarePositionsGoal2`) _array_index (`|GetArrayItem` (`self.AllPositions`) _array_index) true)))

(fn `UserConstructionScript`
  (locals (L_Squares :type "Array of PrimitiveComponent Object Reference"))
  (`parent.UserConstructionScript`)
  (for _index (range 8)
    (bind _returnvalue (select `int` _index :`0` (`self.Cube1`) :`1` (`self.Cube2`) :`2` (`self.Cube3`) :`3` (`self.Cube4`) :`4` (`self.Cube5`) :`5` (`self.Cube6`) :`6` (`self.Cube7`) :`7` (`self.Cube8`)))
    (bind _returnvalue_2 (`PrimitiveComponent.CreateDynamicMaterialInstance` _returnvalue 0 "/Game/DisconnectTemplate/MaterialLibrary/Flip/MI_Numbers.MI_Numbers" "None"))
    (`MaterialInstanceDynamic.SetScalarParameterValue` _returnvalue_2 "Numero" (`KismetMathLibrary.Conv_IntToDouble` _index))
    (`BlueprintMapLibrary.Map_Add` (`self.StartingPositions`) (`SceneComponent.RelativeLocation` _returnvalue) _returnvalue)))