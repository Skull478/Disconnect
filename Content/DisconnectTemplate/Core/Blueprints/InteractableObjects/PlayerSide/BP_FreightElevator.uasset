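; Freight elevator that shuttles between the first two points of a spline, looping from BeginPlay with pauses at each end.
; Up and down timelines drive the movement, and MC_ events can start either leg.
; Each descent increments a fall counter; the down timeline toggles sparks and escalates smoke by that count, which the break event resets.
; The construction script applies mesh, scale and material, sets starting height and attaches the control board.
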(event `MC_FreightElevatorUp`
  (params (Index :type Integer))
  (bind _splineupdown (`self.SplineUpDown`))
  (bind _splineupdown_2 (`self.SplineUpDown`))
  (bind _ns_sparkleelevator1 (`self.NS_SparkleElevator1`))
  (bind _ns_sparkleelevator (`self.NS_SparkleElevator`))
  (bind _ns_smokeelevator (`self.NS_SmokeElevator`))
  (bind (_direction _newtrack_0) (`Timeline|T_Up` :!via `PlayFromStart` :!label _label)
    (:`Update`
      (`SceneComponent.K2_SetWorldLocation` (`self.SM_FreightElevator`) (`KismetMathLibrary.VLerp` (`.Position` (break `SplinePoint` (`SplineComponent.GetSplinePointAt` _splineupdown_2 (- 1 1) "World"))) (`.Position` (break `SplinePoint` (`SplineComponent.GetSplinePointAt` _splineupdown_2 1 "World"))) _newtrack_0) false false))
    (:`Finished`
      (`KismetSystemLibrary.Delay` 2.0)
      (set `self.NumberOfFall` (+ (`self.NumberOfFall`) 1) :!label _label_2)
      (bind (_direction_2 _elevatormovedown) (`Timeline|T_Down` :!via `PlayFromStart`)
        (:`Update`
          (`SceneComponent.K2_SetWorldLocation` (`self.SM_FreightElevator`) (`KismetMathLibrary.VLerp` (`.Position` (break `SplinePoint` (`SplineComponent.GetSplinePointAt` _splineupdown 1 "World"))) (`.Position` (break `SplinePoint` (`SplineComponent.GetSplinePointAt` _splineupdown (- 1 1) "World"))) _elevatormovedown) false false))
        (:`Finished`
          (`KismetSystemLibrary.Delay` 2.0)
          (goto _label :!via `PlayFromStart`))
        (:`SparkleTimer`
          (`/Engine/EditorBlueprintResources/StandardMacros.FlipFlop`
            (:`A`
              (`ActorComponent.Activate` _ns_sparkleelevator false)
              (`ActorComponent.Activate` _ns_sparkleelevator1 false)
              (switch `int` (`self.NumberOfFall`)
                (:`1`
                  (`ActorComponent.Activate` _ns_smokeelevator false))
                (:`2`
                  (`FXSystemComponent.SetColorParameter` _ns_smokeelevator "Color" (struct :`R` 0.166667 :`G` 0.166667 :`B` 0.166667 :`A` 1.0))
                  (`FXSystemComponent.SetFloatParameter` _ns_smokeelevator "None" 150.0))
                (:`3`
                  (`FXSystemComponent.SetColorParameter` _ns_smokeelevator "Color" (struct :`R` 0.078125 :`G` 0.078125 :`B` 0.078125 :`A` 1.0))
                  (`FXSystemComponent.SetFloatParameter` _ns_smokeelevator "None" 250.0))))
            (:`B`
              (`ActorComponent.Deactivate` _ns_sparkleelevator)
              (`ActorComponent.Deactivate` _ns_sparkleelevator1))))))))

(event `self.ReceiveBeginPlay`
  (goto _label :!via `PlayFromStart`))

(event `MC_FreightElevatorDown`
  (params (Index :type Integer))
  (goto _label_2))

(event `MC_FreightElevatorBreak`
  (set `self.NumberOfFall` 0))

(fn `UserConstructionScript`
  (bind _sm_freightelevator (`self.SM_FreightElevator`))
  (bind _splineupdown (`self.SplineUpDown`))
  (bind (_returnvalue_x _returnvalue_y) (`KismetMathLibrary.BreakVector` (`SceneComponent.K2_GetComponentLocation` (`self.SM_FreightElevator`))))
  (bind (_returnvalue_x_2 _returnvalue_y_2 _returnvalue_z) (`KismetMathLibrary.BreakVector` (`SplineComponent.GetLocationAtDistanceAlongSpline` _splineupdown (`KismetMathLibrary.Lerp` 0.0 (`SplineComponent.GetSplineLength` _splineupdown)) "World")))
  (`|ExecutionSequence`
    (:`then_0`
      (`StaticMeshComponent.SetStaticMesh` _sm_freightelevator (`self.SM_ElevatorMesh`))
      (`SceneComponent.SetWorldScale3D` _sm_freightelevator (`self.SM_ElevatorScale`))
      (bind _elevatormaterial (`self.ElevatorMaterial`)
        (:`then`
          (`PrimitiveComponent.SetMaterial` (`self.SM_FreightElevator`) 0 _elevatormaterial))
        (:`else`)))
    (:`then_1`
      (`SceneComponent.K2_SetWorldLocation` (`self.SM_FreightElevator`) (`KismetMathLibrary.MakeVector` _returnvalue_x _returnvalue_y _returnvalue_z) false false))
    (:`then_2`
      (bind _controlboardref (`self.ControlBoardRef`)
        (:`then`
          (`self.K2_AttachToComponent` _controlboardref (`self.ControlBoardPlacement`) "None" "SnapToTarget" "SnapToTarget" "SnapToTarget" true))
        (:`else`)))))