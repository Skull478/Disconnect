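; Freight rotation direction button that works as one of a linked pair, showing red or green for the selected direction.
; Interaction routes an update through the player controller, which toggles this button and its partner and reports the direction via OnMoved, intended for the control board.
; A multicast-style color event recolors both buttons' dynamic materials.
; A separate update type drives optional Niagara smoke in three levels of density and darkness.
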(event `self.ReceiveBeginPlay`
  (`parent.ReceiveBeginPlay`))

(event `/Game/DisconnectTemplate/Core/Library/BPI_UpdateData.UpdateDataActor`
  (params (DataList :type "/Game/DisconnectTemplate/Core/Library/S_BasicListOfData Structure"))
  (bind ((`ListOfFloat_3_018B9153488B47BE83268E87B9A7408B` _listoffloat) (`ListOfInteger_11_DAD0FA91461EA0E9D5ADCE8364933B65` _listofinteger)) (break `/Game/DisconnectTemplate/Core/Library/S_BasicListOfData` DataList))
  (bind _otherbuttonref (`self.OtherButtonRef`))
  (bind _ns_smoke (`self.NS_Smoke`))
  (bind _ns_smoke_2 (`self.NS_Smoke`))
  (bind _ns_smoke_3 (`self.NS_Smoke`))
  ; Select direction and communicate it to control board
  (switch `int` (`KismetMathLibrary.FFloor` (`|GetArrayItem` _listoffloat))
    (:`0`
      (bind _output_get (set `self.OnOff` (select `int` (`self.OnOff`) :`0` 1 :`1` 0)))
      (`self.MC_ChangeColor` _output_get)
      (set `/Game/DisconnectTemplate/Core/Blueprints/InteractableObjects/PlayerSide/Freight/BP_FE_RotationDirection.OnOff` (select `int` (`/Game/DisconnectTemplate/Core/Blueprints/InteractableObjects/PlayerSide/Freight/BP_FE_RotationDirection.OnOff` _otherbuttonref) :`0` 1 :`1` 0) _otherbuttonref)
      (`self.OnMoved` 0 (`self.OnOff`) (`self.Direction`)))
    (:`2`
      (if (`self.Smoke?`)
        (switch `int` (`|GetArrayItem` _listofinteger)
          (:`0`
            (`ActorComponent.Activate` _ns_smoke_2 false)
            (`FXSystemComponent.SetFloatParameter` _ns_smoke_2 "SpawnRate" 2.0))
          (:`1`
            (`FXSystemComponent.SetColorParameter` _ns_smoke "Color" (struct :`R` 0.197917 :`G` 0.197917 :`B` 0.197917 :`A` 0.75))
            (`FXSystemComponent.SetFloatParameter` _ns_smoke "SpawnRate" 8.0))
          (:`2`
            (`FXSystemComponent.SetColorParameter` _ns_smoke_3 "Color" (struct :`R` 0.078125 :`G` 0.078125 :`B` 0.078125 :`A` 1.0))
            (`FXSystemComponent.SetFloatParameter` _ns_smoke_3 "SpawnRate" 15.0)))))))

(event `MC_ChangeColor`
  (params (Index :type Integer))
  ; Change color corresponding to which direction is selected
  (`MaterialInstanceDynamic.SetVectorParameterValue` (`self.DMI_Ref`) "ColorAdjustment" (select `int` Index :`0` (struct :`R` 1.0 :`A` 1.0) :`1` (struct :`G` 1.0 :`A` 1.0) :!type "LinearColor Structure"))
  (`MaterialInstanceDynamic.SetVectorParameterValue` (`/Game/DisconnectTemplate/Core/Blueprints/InteractableObjects/PlayerSide/Freight/BP_FE_RotationDirection.DMI_Ref` (`self.OtherButtonRef`)) "ColorAdjustment" (select `int` Index :`0` (struct :`G` 1.0 :`A` 1.0) :`1` (struct :`R` 1.0 :`A` 1.0) :!type "LinearColor Structure")))

(fn `IsInteractible?`
  (returns (IsInteractable :type Boolean))
  (message `/Game/DisconnectTemplate/Core/Library/BPI_UpdateData.CallUpdate` (`GameplayStatics.GetPlayerController` 0) self (make `/Game/DisconnectTemplate/Core/Library/S_BasicListOfData` :`ListOfFloat` (`|MakeArray` 0.0)))
  (return false))

(fn `UserConstructionScript`
  (`parent.UserConstructionScript`)
  (bind _returnvalue (`PrimitiveComponent.CreateDynamicMaterialInstance` (`self.SM_Lingot_low`) 0 "/Game/DisconnectTemplate/MaterialLibrary/Instance/MI_Lingot.MI_Lingot" "None"))
  (bind _output_get (set `self.DMI_Ref` _returnvalue))
  (`MaterialInstanceDynamic.SetVectorParameterValue` _output_get "ColorAdjustment" (select `int` (`self.OnOff`) :`0` (struct :`R` 1.0 :`A` 1.0) :`1` (struct :`G` 1.0 :`A` 1.0) :!type "LinearColor Structure"))
  (set `self.PrimitiveComponentAsOverlayMesh` (`|MakeArray` (`self.SM_Lingot_low`) :!type "PrimitiveComponent Object Reference")))