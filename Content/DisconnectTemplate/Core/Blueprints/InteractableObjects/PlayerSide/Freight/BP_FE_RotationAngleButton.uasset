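; BP_FE_RotationAngleButton is an interactable freight-side button that nudges a referenced rotation angle actor in one of two directions.
; Its construction script tints a dynamic material on the ingot mesh according to the RightButton flag and registers that mesh for overlay.
; The IsInteractible check does the work itself: it sends a signed unit step through the player controller's CallUpdateMessage to RotationAngleRef, then always returns false.
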(fn `IsInteractible?`
  (returns (IsInteractable :type Boolean))
  (message `/Game/DisconnectTemplate/Core/Library/BPI_UpdateData.CallUpdate` (`GameplayStatics.GetPlayerController` 0) (`self.RotationAngleRef`) (make `/Game/DisconnectTemplate/Core/Library/S_BasicListOfData` :`ListOfFloat` (`|MakeArray` 0.0) :`ListOfInteger` (`|MakeArray` (`KismetMathLibrary.SelectInt` 1 -1 (`self.RightButton?`)))))
  (return false))

(fn `UserConstructionScript`
  (`parent.UserConstructionScript`)
  (bind _returnvalue (`PrimitiveComponent.CreateDynamicMaterialInstance` (`self.SM_Lingot_low`) 0 "/Game/DisconnectTemplate/MaterialLibrary/Instance/MI_Lingot.MI_Lingot" "None"))
  (bind _output_get (set `self.DMI_Ref` _returnvalue))
  (`MaterialInstanceDynamic.SetVectorParameterValue` _output_get "ColorAdjustment" (select `bool` (`self.RightButton?`) :`false` (struct :`R` 0.688715 :`G` 1.0 :`A` 1.0) :`true` (struct :`G` 0.26436 :`B` 1.0 :`A` 1.0) :!type "LinearColor Structure"))
  (set `self.PrimitiveComponentAsOverlayMesh` (`|MakeArray` (`self.SM_Lingot_low`) :!type "PrimitiveComponent Object Reference")))