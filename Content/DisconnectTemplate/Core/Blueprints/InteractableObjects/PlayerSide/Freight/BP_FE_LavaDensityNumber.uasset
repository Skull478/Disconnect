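; A keypad button actor, apparently for a lava density puzzle, that represents either a number or a clear (C) key.
; The construction script gives Numero1 a dynamic digit or letter material, offsets the digit parameter from Number, and registers Button as the overlay mesh.
; Its IsInteractible check doubles as the press handler, sending the clear flag and Number to ManagerRef through the player controller's update message, then returning false.
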(fn `IsInteractible?`
  (returns (IsInteractable :type Boolean))
  (message `/Game/DisconnectTemplate/Core/Library/BPI_UpdateData.CallUpdate` (`GameplayStatics.GetPlayerController` 0) (`self.ManagerRef`) (make `/Game/DisconnectTemplate/Core/Library/S_BasicListOfData` :`ListOfFloat` (`|MakeArray` (`KismetMathLibrary.Conv_IntToDouble` (`KismetMathLibrary.SelectInt` 1 0 (`self.ClearButton?`))) (`self.Number`))))
  (return false))

(fn `UserConstructionScript`
  (bind _clearbutton_ (`self.ClearButton?`))
  (`parent.UserConstructionScript`)
  (bind _returnvalue (`PrimitiveComponent.CreateDynamicMaterialInstance` (`self.Numero1`) 0 (select `bool` _clearbutton_ :`false` "/Game/DisconnectTemplate/MaterialLibrary/Flip/Masked/MI_Numbers.MI_Numbers" :`true` "/Game/DisconnectTemplate/MaterialLibrary/Flip/Masked/MI_LetterC.MI_LetterC" :!type "MaterialInterface Object Reference") "None"))
  (bind _output_get (set `self.DMI_Ref` _returnvalue))
  (`MaterialInstanceDynamic.SetScalarParameterValue` _output_get (select `bool` _clearbutton_ :`false` "Numero" :!type "Name") (- (`self.Number`) 1.0))
  (set `self.PrimitiveComponentAsOverlayMesh` (`|MakeArray` (`self.Button`) :!type "PrimitiveComponent Object Reference")))