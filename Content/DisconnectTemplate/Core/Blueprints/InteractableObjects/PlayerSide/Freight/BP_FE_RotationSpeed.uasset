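; Player-side Freight interactable: a rotation speed lever that steps through six positions, reversing direction at either end.
; IsInteractible routes an update through the player controller to UpdateDataActor, which sets a replicated rotation applied to the pivot in its OnRep, broadcasts the position via OnMoved and multicasts a sound.
; A separate server activation event multicasts smoke that grows denser and changes color over three successive failures.
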(event `self.ReceiveBeginPlay`
  (`parent.ReceiveBeginPlay`))

(event `/Game/DisconnectTemplate/Core/Blueprints/InteractableObjects/BPI_InteractableObject.PlayerInteract`
  (params (Ref :type "/Game/DisconnectTemplate/Core/Blueprints/Character/Game/Player/BP_DisconnectPlayer_Character Object Reference") (Location :type "Vector Structure"))
  ; Move the lever each time player interact
)

(event `/Game/DisconnectTemplate/Core/Library/BPI_UpdateData.UpdateDataActor`
  (params (DataList :type "/Game/DisconnectTemplate/Core/Library/S_BasicListOfData Structure"))
  (bind _inverted_ (`self.Inverted?`))
  ; Move the lever each time player interact
  (switch `int` (`KismetMathLibrary.FFloor` (`|GetArrayItem` (`.ListOfFloat_3_018B9153488B47BE83268E87B9A7408B` (break `/Game/DisconnectTemplate/Core/Library/S_BasicListOfData` DataList))))
    (:`0`
      (bind _output_get (set `self.Position` (`KismetMathLibrary.Clamp` (+ (`self.Position`) (`KismetMathLibrary.SelectInt` -1 1 (`self.Inverted?`))) 1 6)))
      (set `self.Inverted?` (select `bool` (or (== (`self.Position`) 6) (== (`self.Position`) 1)) :`false` _inverted_ :`true` (not _inverted_)))
      (set `self.Rotation` (`KismetMathLibrary.MakeRotator` 0.0 (`|GetArrayItem` (`self.RotationX`) (- _output_get 1)) 90.0))
      (`self.OnMoved` 3 (`self.Position`))
      (`self.MC_Sound`))))

(event `MC_Sound`
  ; Move the lever each time player interact
  (`AkGameObject.PostAssociatedAkEvent` :`self` (`self.Play_INT_RotationSpeed`)))

(event `/Game/DisconnectTemplate/Core/Library/BPI_UpdateData.TSRV_ActivateEvent`
  ; Activate smoke
  (`self.MC_ActivateSmoke`))

(event `MC_ActivateSmoke`
  (bind _ns_smoke (`self.NS_Smoke`))
  (bind _ns_smoke_2 (`self.NS_Smoke`))
  (bind _ns_smoke_3 (`self.NS_Smoke`))
  ; Activate smoke
  (bind _result (`/Engine/EditorBlueprintResources/StandardMacros.IncrementInt` (`self.NumberOfFails`))
    (:`  `
      (switch `int` _result
        (:`1`
          (`ActorComponent.Activate` _ns_smoke_2 false)
          (`FXSystemComponent.SetFloatParameter` _ns_smoke_2 "SpawnRate" 2.0))
        (:`2`
          (`FXSystemComponent.SetColorParameter` _ns_smoke "Color" (struct :`R` 0.197917 :`G` 0.197917 :`B` 0.197917 :`A` 0.75))
          (`FXSystemComponent.SetFloatParameter` _ns_smoke "SpawnRate" 8.0))
        (:`3`
          (`FXSystemComponent.SetColorParameter` _ns_smoke_3 "Color" (struct :`R` 0.078125 :`G` 0.078125 :`B` 0.078125 :`A` 1.0))
          (`FXSystemComponent.SetFloatParameter` _ns_smoke_3 "SpawnRate" 15.0))))))

(fn `IsInteractible?`
  (returns (IsInteractable :type Boolean))
  (message `/Game/DisconnectTemplate/Core/Library/BPI_UpdateData.CallUpdate` (`GameplayStatics.GetPlayerController` 0) self (make `/Game/DisconnectTemplate/Core/Library/S_BasicListOfData` :`ListOfFloat` (`|MakeArray` 0.0)))
  (return false))

(fn `OnRep_Rotation`
  (`SceneComponent.K2_SetRelativeRotation` (`self.ObjectToRotatePivot`) (`self.Rotation`) false false))

(fn `UserConstructionScript`
  (`parent.UserConstructionScript`)
  (set `self.PrimitiveComponentAsOverlayMesh` (`|MakeArray` (`self.SM_Reactor`) (`self.SM_Lever`) (`self.SM_Metal`) :!type "PrimitiveComponent Object Reference")))