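; Freight interactable wheel that players step through four rotation settings, raising or lowering a lava level indicator to match.
; Incoming data updates shift the clamped level and multicast a timeline turn, whose RepNotify rotation drives both wheel and lava mesh.
; When the turn finishes, it reports the quarter-turn index through CallOnMoved.
; Construction attaches referenced left/right buttons, and repeated failures escalate Niagara smoke in three stages.
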(event `/Game/DisconnectTemplate/Core/Library/BPI_UpdateData.UpdateDataActor`
  (params (DataList :type "/Game/DisconnectTemplate/Core/Library/S_BasicListOfData Structure"))
  (bind (_listoffloat _command _listofinteger) (break `/Game/DisconnectTemplate/Core/Library/S_BasicListOfData` DataList))
  ; Move the whell when player move and when player desinteract set the wheel to nearest rotation (every 90 degrees)
  (switch `int` (`KismetMathLibrary.FFloor` (`|GetArrayItem` _listoffloat))
    (:`0`
      (bind _output_get (set `self.CurrentLavaLevel` (`KismetMathLibrary.Clamp` (+ (`self.CurrentLavaLevel`) (`|GetArrayItem` _listofinteger)) 0 3)))
      (bind _output (`|GetArrayItem` (`self.RotationZ`) _output_get))
      (`self.MC_RotateGear` _output)
      (`KismetSystemLibrary.PrintString` (`KismetStringLibrary.Conv_DoubleToString` _output) true false (struct :`R` 1.0 :`G` 0.835938 :`A` 1.0) 5.0))))

(event `MC_RotateGear`
  (params (`Rotation to Go` :type "Float (double-precision)"))
  (bind (_rotationbefore_roll _rotationbefore_pitch) (`KismetMathLibrary.BreakRotator` (`self.RotationBefore`)))
  (bind (_relativerotation_roll _relativerotation_pitch _relativerotation_yaw) (`KismetMathLibrary.BreakRotator` (`SceneComponent.RelativeRotation` (`self.SM_OverlayMesh`))))
  ; Move the whell when player move and when player desinteract set the wheel to nearest rotation (every 90 degrees)
  (set `self.Rotation to Go` `Rotation to Go`)
  (set `self.RotationBefore` (`SceneComponent.RelativeRotation` (`self.SM_OverlayMesh`)))
  (bind (_direction _newtrack_0) (`Timeline|T_Wheel` :!via `PlayFromStart` :!label _label)
    (:`Update`
      (set `self.RotationAfterMovement` (`KismetMathLibrary.RLerp` (`self.RotationBefore`) (`KismetMathLibrary.MakeRotator` _rotationbefore_roll _rotationbefore_pitch (`self.Rotation to Go`)) _newtrack_0 true)))
    (:`Finished`
      (`self.OnMoved` 4 (`KismetMathLibrary.Round` (`KismetMathLibrary.Abs` (/ (select `bool` (< _relativerotation_yaw 0.0) :`false` _relativerotation_yaw :`true` (+ _relativerotation_yaw 360.0) :!type "Float (double-precision)") 90.0))))
      (set `self.AnimatedLavaLevel` (`self.getLavaLocFromRotation`)))))

(event `/Game/DisconnectTemplate/Core/Library/BPI_UpdateData.TSRV_ActivateEvent`
  ; Move the whell when player move and when player desinteract set the wheel to nearest rotation (every 90 degrees)
  (`self.MC_ActivateSmoke`))

(event `StopTimeline`
  ; Move the whell when player move and when player desinteract set the wheel to nearest rotation (every 90 degrees)
  (goto _label :!via `Stop`))

(event `MC_ActivateSmoke`
  (bind _ns_smoke (`self.NS_Smoke`))
  (bind _ns_smoke_2 (`self.NS_Smoke`))
  (bind _ns_smoke_3 (`self.NS_Smoke`))
  ; Activate Smoke
  (bind _result (`/Engine/EditorBlueprintResources/StandardMacros.IncrementInt` (`self.Number Of Fails`))
    (:`  `
      (switch `int` _result
        (:`1`
          (`ActorComponent.Activate` _ns_smoke_2 false)
          (`FXSystemComponent.SetFloatParameter` _ns_smoke_2 "SpawnRate" 2.0))
        (:`2`
          (`FXSystemComponent.SetColorParameter` _ns_smoke "Color" (struct :`R` 0.197917 :`G` 0.197917 :`B` 0.197917 :`A` 0.75))
          (`FXSystemComponent.SetFloatParameter` _ns_smoke "SpawnRate" 8.0))
        (:`3`
          (`FXSystemComponent.SetColorParameter` _ns_smoke_3 "Color" (struct :`R` 0.078125 :`G` 0.078125 :`B` 0.078125 :`A` 1.0))
          (`FXSystemComponent.SetFloatParameter` _ns_smoke_3 "SpawnRate" 15.0))))))

(fn `getLavaLocFromRotation`
  (returns (ReturnValue :type "Float (double-precision)"))
  (bind (_relativerotation_roll _relativerotation_pitch _relativerotation_yaw) (`KismetMathLibrary.BreakRotator` (`SceneComponent.RelativeRotation` (`self.SM_OverlayMesh`))))
  (return (`KismetMathLibrary.Lerp` -20.0 10.0 (/ (`KismetMathLibrary.Abs` (/ (select `bool` (< _relativerotation_yaw 0.0) :`false` _relativerotation_yaw :`true` (+ _relativerotation_yaw 360.0) :!type "Float (double-precision)") 90.0)) 4.0))))

(fn `IsInteractible?`
  (returns (IsInteractable :type Boolean))
  (return true))

(fn `OnRep_AnimatedLavaLevel`
  (bind _animatedlavalevel (`self.AnimatedLavaLevel`))
  (`SceneComponent.K2_SetRelativeLocation` (`self.SM_LavaLevel`) (`KismetMathLibrary.MakeVector` 0.0 0.0 _animatedlavalevel) false false)
  (`KismetSystemLibrary.PrintString` (`KismetStringLibrary.Conv_DoubleToString` _animatedlavalevel) true false))

(fn `OnRep_RotationAfterMovement`
  (`SceneComponent.K2_SetRelativeRotation` (`self.SM_OverlayMesh`) (`self.RotationAfterMovement`) false false)
  (`SceneComponent.K2_SetRelativeLocation` (`self.SM_LavaLevel`) (`KismetMathLibrary.MakeVector` 0.0 0.0 (`self.getLavaLocFromRotation`)) false false))

(fn `UserConstructionScript`
  (`parent.UserConstructionScript`)
  (for _array_element (`self.ButtonRef`)
    (`/Engine/EditorBlueprintResources/StandardMacros.IsValid` _array_element
      (:`Is Valid`
        (`self.K2_AttachToComponent` _array_element (select `bool` (`/Game/DisconnectTemplate/Core/Blueprints/InteractableObjects/PlayerSide/Freight/BP_FE_RotationAngleButton.RightButton?` _array_element) :`false` (`self.LeftButton`) :`true` (`self.RightButton`)) "None" "SnapToTarget" "KeepWorld" "KeepWorld" true)))))