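; Manager for a Freight lava density puzzle that collects a two-digit number from linked number actors and shows it on two displays.
; On BeginPlay it registers itself with each linked actor; UpdateDataActor then either stores a digit or resets the entry.
; MC events drive the "Numero" parameter on dynamic materials to update the displays.
; After the second digit, it concatenates both and sends the value through CallOnMoved.
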(event `self.ReceiveBeginPlay`
  (`parent.ReceiveBeginPlay`)
  (for _array_element (`self.NumberRef`)
    (set `/Game/DisconnectTemplate/Core/Blueprints/InteractableObjects/PlayerSide/Freight/BP_FE_LavaDensityNumber.ManagerRef` self _array_element)))

(event `/Game/DisconnectTemplate/Core/Library/BPI_UpdateData.UpdateDataActor`
  (params (DataList :type "/Game/DisconnectTemplate/Core/Library/S_BasicListOfData Structure"))
  (bind _listoffloat (break `/Game/DisconnectTemplate/Core/Library/S_BasicListOfData` DataList))
  (bind _output (`|GetArrayItem` _listoffloat 1))
  (bind _returnvalue (`KismetMathLibrary.FTrunc` _output))
  (switch `int` (`KismetMathLibrary.FFloor` (`|GetArrayItem` _listoffloat))
    (:`0`
      (if (< (`self.NumberOfNumbers`) 2)
        (`self.MC_ChangeNumber` _output)
        (bind _output_get (set `self.NumberOfNumbers` (+ (`self.NumberOfNumbers`) 1)))
        (if (== _output_get 1)
          (set `self.FirstNumber` _returnvalue)
          (else
            (set `self.SecondNumber` _returnvalue)))
        (if (== _output_get 2)
          (`self.OnMoved` 1 (`KismetStringLibrary.Conv_StringToInt` (`KismetStringLibrary.Concat_StrStr` (`KismetStringLibrary.Conv_IntToString` (`self.FirstNumber`)) (`KismetStringLibrary.Conv_IntToString` (`self.SecondNumber`))))))))
    (:`1`
      (set `self.NumberOfNumbers` 0)
      (`self.MC_ResetNumbers`))))

(event `MC_ChangeNumber`
  (params (Number :type "Float (double-precision)"))
  (`MaterialInstanceDynamic.SetScalarParameterValue` (select `int` (`self.NumberOfNumbers`) :`0` (`self.DMI_Number1`) :`1` (`self.DMI_Number2`)) "Numero" (- Number 1.0)))

(event `MC_ResetNumbers`
  (`MaterialInstanceDynamic.SetScalarParameterValue` (`self.DMI_Number1`) "Numero" 0.0)
  (`MaterialInstanceDynamic.SetScalarParameterValue` (`self.DMI_Number2`) "Numero" 0.0))

(fn `UserConstructionScript`
  (`parent.UserConstructionScript`)
  (bind _returnvalue (`PrimitiveComponent.CreateDynamicMaterialInstance` (`self.Number1`) 0 "/Game/DisconnectTemplate/MaterialLibrary/Flip/Masked/MI_NumberNoBackground.MI_NumberNoBackground" "None"))
  (set `self.DMI_Number1` _returnvalue)
  (bind _returnvalue_2 (`PrimitiveComponent.CreateDynamicMaterialInstance` (`self.Number2`) 0 "/Game/DisconnectTemplate/MaterialLibrary/Flip/Masked/MI_NumberNoBackground.MI_NumberNoBackground" "None"))
  (set `self.DMI_Number2` _returnvalue_2))