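; Replicated gear pressure animation actor that slides a gear mesh between start and end relative locations.
; TSRVMoveGear plays or reverses a timeline that lerps NewRelativeLocation, whose RepNotify moves the mesh.
; BeginPlay reassigns the duration to itself to fire its RepNotify, which sets the timeline play rate to the inverse of that duration.
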(event `self.ReceiveBeginPlay`
  ; Setup Anim Duration
  (set `self.GearPressureAnimDuration` (`self.GearPressureAnimDuration`)))

(event `/Game/DisconnectTemplate/Core/Blueprints/InteractableObjects/PlayerSide/Freight/GearPressureAnim/BPI_AnimatedActors.TSRV_MoveGear`
  (params (`GearON?` :type Boolean))
  ; Move Gear
  (if `GearON?`
    (bind (_direction _alpha) (`Timeline|GearPressureAnim` :!label _label)
      (:`Update`
        (set `self.NewRelativeLocation` (`KismetMathLibrary.VLerp` (`self.StartRelativeLocation`) (`self.EndRelativeLocation`) _alpha))))
    (else
      (goto _label :!via `Reverse`))))

(fn `OnRep_GearPressureAnimDuration`
  (`TimelineComponent.SetPlayRate` (`self.GearPressureAnim`) (/ 1.0 (`self.GearPressureAnimDuration`))))

(fn `OnRep_NewRelativeLocation`
  (`SceneComponent.K2_SetRelativeLocation` (`self.SM_GearsPressure`) (`self.NewRelativeLocation`) false false))

(fn `UserConstructionScript`)