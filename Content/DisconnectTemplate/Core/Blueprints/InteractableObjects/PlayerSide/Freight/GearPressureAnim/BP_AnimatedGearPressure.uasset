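; BP_AnimatedGearPressure is a freight-interactable actor that animates gear pressure mechanisms made of several child-actor gears.
; The TSRVChangeGearPressure event stores the gear index and on/off state, then selects one of five BPGearPressure child actors by that index.
; It forwards the state to the chosen actor through TSRVMoveGearMessage, with index 0 falling back to the first gear.
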(event `self.ReceiveBeginPlay`)

(event `/Game/DisconnectTemplate/Core/Blueprints/InteractableObjects/PlayerSide/Freight/GearPressureAnim/BPI_AnimatedActors.TSRV_ChangeGearPressure`
  (params (Gear :type Integer) (`On?` :type Boolean))
  (bind _childactor (`ChildActorComponent.ChildActor` (`self.BP_GearPressure1`)))
  (set `self.Pressure_ON?` `On?`)
  (bind _output_get (set `self.CurrentGear` Gear))
  (message `/Game/DisconnectTemplate/Core/Blueprints/InteractableObjects/PlayerSide/Freight/GearPressureAnim/BPI_AnimatedActors.TSRV_MoveGear` (select `int` _output_get :`0` _childactor :`1` _childactor :`2` (`ChildActorComponent.ChildActor` (`self.BP_GearPressure2`)) :`3` (`ChildActorComponent.ChildActor` (`self.BP_GearPressure3`)) :`4` (`ChildActorComponent.ChildActor` (`self.BP_GearPressure4`)) :`5` (`ChildActorComponent.ChildActor` (`self.BP_GearPressure5`)) :!type "Object Object Reference") (`self.Pressure_ON?`)))

(fn `UserConstructionScript`)