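; Six-position rotation speed lever on the player-side Freight interactables, with numbered labels set through dynamic material instances at construction.
; IsInteractible sends an update through the player controller and returns false, while PlayerInteract is empty.
; UpdateDataActor steps Position, reversing at either end, and fires OnMoved with ID 3 and the new position.
; The RepNotify Rotation, looked up from RotationX, turns the overlay mesh.
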(event `self.ReceiveBeginPlay`
  (`parent.ReceiveBeginPlay`))

(event `/Game/DisconnectTemplate/Core/Blueprints/InteractableObjects/BPI_InteractableObject.PlayerInteract`
  (params (Ref :type "/Game/DisconnectTemplate/Core/Blueprints/Character/Game/Player/BP_DisconnectPlayer_Character Object Reference"))
  ; Move the lever each time player interact
)

(event `/Game/DisconnectTemplate/Core/Library/BPI_UpdateData.UpdateDataActor`
  (params (DataList :type "/Game/DisconnectTemplate/Core/Library/S_BasicListOfData Structure"))
  (bind _inverted_ (`self.Inverted?`))
  ; Move the lever each time player interact
  (switch `int` (`KismetMathLibrary.FFloor` (`|GetArrayItem` (`.ListOfFloat_3_018B9153488B47BE83268E87B9A7408B` (break `/Game/DisconnectTemplate/Core/Library/S_BasicListOfData` DataList))))
    (:`0`
      (bind _output_get (set `self.Position` (`KismetMathLibrary.Clamp` (+ (`self.Position`) (`KismetMathLibrary.SelectInt` -1 1 (`self.Inverted?`))) 1 6)))
      (set `self.Inverted?` (select `bool` (or (== (`self.Position`) 6) (== (`self.Position`) 1)) :`false` _inverted_ :`true` (not _inverted_)))
      (set `self.Rotation` (`KismetMathLibrary.MakeRotator` (`|GetArrayItem` (`self.RotationX`) (- _output_get 1))))
      (`self.OnMoved` 3 (`self.Position`)))))

(fn `IsInteractible?`
  (returns (IsInteractable :type Boolean))
  (message `/Game/DisconnectTemplate/Core/Library/BPI_UpdateData.CallUpdate` (`GameplayStatics.GetPlayerController` 0) self (make `/Game/DisconnectTemplate/Core/Library/S_BasicListOfData` :`ListOfFloat` (`|MakeArray` 0.0)))
  (return false))

(fn `OnRep_Rotation`
  (`SceneComponent.K2_SetRelativeRotation` (`self.SM_OverlayMesh`) (`self.Rotation`) false false))

(fn `UserConstructionScript`
  (`parent.UserConstructionScript`)
  (bind _returnvalue (`PrimitiveComponent.CreateDynamicMaterialInstance` (`self.Number1`) 0 "/Game/DisconnectTemplate/MaterialLibrary/Flip/Masked/MI_NumberNoBackground.MI_NumberNoBackground" "None"))
  (`MaterialInstanceDynamic.SetScalarParameterValue` _returnvalue "Numero" 0.0)
  (bind _returnvalue_2 (`PrimitiveComponent.CreateDynamicMaterialInstance` (`self.Number2`) 0 "/Game/DisconnectTemplate/MaterialLibrary/Flip/Masked/MI_NumberNoBackground.MI_NumberNoBackground" "None"))
  (`MaterialInstanceDynamic.SetScalarParameterValue` _returnvalue_2 "Numero" 1.0)
  (bind _returnvalue_3 (`PrimitiveComponent.CreateDynamicMaterialInstance` (`self.Number3`) 0 "/Game/DisconnectTemplate/MaterialLibrary/Flip/Masked/MI_NumberNoBackground.MI_NumberNoBackground" "None"))
  (`MaterialInstanceDynamic.SetScalarParameterValue` _returnvalue_3 "Numero" 2.0)
  (bind _returnvalue_4 (`PrimitiveComponent.CreateDynamicMaterialInstance` (`self.Number4`) 0 "/Game/DisconnectTemplate/MaterialLibrary/Flip/Masked/MI_NumberNoBackground.MI_NumberNoBackground" "None"))
  (`MaterialInstanceDynamic.SetScalarParameterValue` _returnvalue_4 "Numero" 3.0)
  (bind _returnvalue_5 (`PrimitiveComponent.CreateDynamicMaterialInstance` (`self.Number5`) 0 "/Game/DisconnectTemplate/MaterialLibrary/Flip/Masked/MI_NumberNoBackground.MI_NumberNoBackground" "None"))
  (`MaterialInstanceDynamic.SetScalarParameterValue` _returnvalue_5 "Numero" 4.0)
  (bind _returnvalue_6 (`PrimitiveComponent.CreateDynamicMaterialInstance` (`self.Number6`) 0 "/Game/DisconnectTemplate/MaterialLibrary/Flip/Masked/MI_NumberNoBackground.MI_NumberNoBackground" "None"))
  (`MaterialInstanceDynamic.SetScalarParameterValue` _returnvalue_6 "Numero" 5.0))