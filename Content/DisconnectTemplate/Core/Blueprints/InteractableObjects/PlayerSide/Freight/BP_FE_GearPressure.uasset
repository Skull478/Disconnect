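; Interactable gear-pressure lever in the Freight set, labelled with a red number through a dynamic material.
; IsInteractible routes a message through the player controller to UpdateDataActor, which toggles Position, calls OnMoved and plays or reverses the MoveLever timeline.
; The timeline drives a RepNotify rotation on the lever pivot.
; On finish, it sends the gear number, parsed from LeverTag's name, and on/off state to RefAnimatedGearPressure.
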(event `/Game/DisconnectTemplate/Core/Library/BPI_UpdateData.UpdateDataActor`
  (params (DataList :type "/Game/DisconnectTemplate/Core/Library/S_BasicListOfData Structure"))
  (switch `int` (`KismetMathLibrary.FFloor` (`|GetArrayItem` (`.ListOfFloat_3_018B9153488B47BE83268E87B9A7408B` (break `/Game/DisconnectTemplate/Core/Library/S_BasicListOfData` DataList))))
    (:`0`
      (bind _output_get (set `self.Position` (select `int` (`self.Position`) :`0` 1 :`1` 0)))
      (`self.OnMoved` 2 (`self.Position`) (`self.LeverTag`))
      (switch `int` _output_get
        (:`0`
          (bind (_direction _alpha) (`Timeline|MoveLever` :!via `Reverse` :!label _label)
            (:`Update`
              (set `self.LeverRotation` (`KismetMathLibrary.MakeRotator` 0.0 (`KismetMathLibrary.Lerp` 0.0 60.0 _alpha))))
            (:`Finished`
              (message `/Game/DisconnectTemplate/Core/Blueprints/InteractableObjects/PlayerSide/Freight/GearPressureAnim/BPI_AnimatedActors.TSRV_ChangeGearPressure` (`self.RefAnimatedGearPressure`) (`KismetStringLibrary.Conv_StringToInt` (`.RightS` (`KismetStringLibrary.Split` (`KismetStringLibrary.Conv_NameToString` (`BlueprintGameplayTagLibrary.GetTagName` (`self.LeverTag`))) "Data.GearPressure."))) (== (`self.Position`) 1)))))
        (:`1`
          (goto _label))))))

(fn `IsInteractible?`
  (returns (IsInteractable :type Boolean))
  (message `/Game/DisconnectTemplate/Core/Library/BPI_UpdateData.CallUpdate` (`GameplayStatics.GetPlayerController` 0) self (make `/Game/DisconnectTemplate/Core/Library/S_BasicListOfData` :`ListOfFloat` (`|MakeArray` 0.0)))
  (return false))

(fn `OnRep_LeverRotation`
  (`SceneComponent.K2_SetRelativeRotation` (`self.LeverPivot`) (`self.LeverRotation`) false false))

(fn `UserConstructionScript`
  (`parent.UserConstructionScript`)
  (bind _returnvalue (`PrimitiveComponent.CreateDynamicMaterialInstance` (`self.Number`) 0 "/Game/DisconnectTemplate/MaterialLibrary/Flip/Masked/MI_NumberNoBackground.MI_NumberNoBackground" "None"))
  (`MaterialInstanceDynamic.SetScalarParameterValue` _returnvalue "Numero" (`self.LeverNumero`))
  (`MaterialInstanceDynamic.SetVectorParameterValue` _returnvalue "ColorNumber" (struct :`R` 1.0 :`A` 1.0))
  (set `self.PrimitiveComponentAsOverlayMesh` (`|MakeArray` (`self.SM_Manche`) (`self.SM_Lever`) (`self.StaticGear2`) (`self.SM_Gear`) :!type "PrimitiveComponent Object Reference")))