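; Interactable NPC camera that the Dev player views through, and that can be glitched once.
; DevInteract adds a HUD camera widget and routes updates through the player controller; the replicated flag toggles the scene capture render target, face glow and billboard.
; IsInteractible sends the glitch update, triggering dialogue and a time message, then OnRep reveals a capture-only effect and hides prompts.
; Construction sets up the flipbook face material; spline movement is stubbed out.
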(event `self.ReceiveBeginPlay`
  (`parent.ReceiveBeginPlay`)
  (`/Engine/EditorBlueprintResources/ActorMacros.Switch Has Authority`
    (:`Authority`
      (if (`self.bUseSpline?`)
        (`self.TSRV_RecallEvent`)))))

(event `RemoveComp`
  ; Remove CRT when leave cam
  (message `/Game/DisconnectTemplate/Core/Library/BPI_UpdateData.CallUpdate` (`GameplayStatics.GetPlayerController` 0) self (make `/Game/DisconnectTemplate/Core/Library/S_BasicListOfData` (`|MakeArray` 1.0))))

(event `/Game/DisconnectTemplate/Core/Blueprints/InteractableObjects/BPI_InteractableObject.DevInteract`
  (params (Ref :type "/Game/DisconnectTemplate/Core/Blueprints/Character/Game/Dev/BP_DisconnectDev_Character Object Reference"))
  (set `self.CharaRef` Ref)
  (`self.CameraReceiveOrder` self)
  ; Place camera component on srv
  (message `/Game/DisconnectTemplate/Core/Library/BPI_UpdateData.CallUpdate` (`GameplayStatics.GetPlayerController` 0) self (make `/Game/DisconnectTemplate/Core/Library/S_BasicListOfData` (`|MakeArray` 0.0)))
  ; Add Widget Camera
  (message `/Game/DisconnectTemplate/Widgets/Data/BPI_DevHUD.AddWidgetCamera` (`/Game/DisconnectTemplate/Core/Blueprints/Character/Game/Dev/BP_DisconnectDev_Character.DevHUD_Ref` (`self.CharaRef`)) (make `/Game/DisconnectTemplate/Core/Blueprints/InteractableObjects/DevSide/Camera/S_CameraProfile` (`.Name_4_317AABC94D86C8AE257648976E0B1A9A` (break `/Game/DisconnectTemplate/Core/Blueprints/InteractableObjects/DevSide/Camera/S_CameraProfile` (`self.CameraProfile`))) self)))

(event `/Game/DisconnectTemplate/Core/Library/BPI_UpdateData.UpdateDataActor`
  (params (DataList :type "/Game/DisconnectTemplate/Core/Library/S_BasicListOfData Structure"))
  (bind _output (`|GetArrayItem` (`.ListOfFloat_3_018B9153488B47BE83268E87B9A7408B` (break `/Game/DisconnectTemplate/Core/Library/S_BasicListOfData` DataList))))
  ; Add or remove on srv the camera component
  (if (== _output 2.0)
    ;; Add Dialogue Glitched
    (if (not (`self.PlayerMakeTheNPC_Glitch?`))
      (message `/Game/DisconnectTemplate/Core/Library/BPI_Game_GameMode.TriggerDialogue` (`GameplayStatics.GetGameMode`) (struct :`TagName` "Dialogues.Glitch.VarA"))
      (set `self.PlayerMakeTheNPC_Glitch?` true)
      (message `/Game/DisconnectTemplate/Core/Library/BPI_Game_GameMode.AddTime` (`GameplayStatics.GetGameMode`) (`self.TimeAdded`)))
    (else
      (set `self.TruggerCameraComponents` (== _output 0.0)))))

(event `TSRV_RecallEvent`
  ; Move character along spline
)

(fn `getCharaRef`
  (returns (SkeletalMesh :type "SkeletalMeshComponent Object Reference"))
  (return (`self.SkeletalMesh`)))

(fn `getDeltaSecModified`
  (returns (ReturnValue :type "Float (double-precision)"))
  (return (/ (`GameplayStatics.GetWorldDeltaSeconds`) 2.0)))

(fn `getTransformFromDistanceAlongSpline`
  (returns (ReturnValue :type "Transform Structure")))

(fn `IsInteractible?`
  (returns (IsInteractable :type Boolean))
  (message `/Game/DisconnectTemplate/Core/Library/BPI_UpdateData.CallUpdate` (`GameplayStatics.GetPlayerController` 0) self (make `/Game/DisconnectTemplate/Core/Library/S_BasicListOfData` (`|MakeArray` 2.0)))
  (return false))

(fn `lerpDistanceDependingOfSens`
  (params (Alpha :type "Float (double-precision)"))
  (returns (ReturnValue :type "Float (double-precision)")))

(fn `NPC_Faces_EmissiveColor`
  (params (Value :type "LinearColor Structure"))
  (`MaterialInstanceDynamic.SetVectorParameterValue` (`self.DMI_NPC_Faces`) "EmissiveColor" Value))

(fn `NPC_Faces_Face`
  (params (Value :type "Float (single-precision)"))
  (`MaterialInstanceDynamic.SetScalarParameterValue` (`self.DMI_NPC_Faces`) "Numero" (`KismetMathLibrary.FClamp` Value 0.0 9.0)))

(fn `NPC_Faces_FaceColor`
  (params (Value :type "LinearColor Structure"))
  (`MaterialInstanceDynamic.SetVectorParameterValue` (`self.DMI_NPC_Faces`) "ColorNumber" Value))

(fn `OnRep_CharaRef`)

(fn `OnRep_PlayerMakeTheNPC_Glitch?`
  (bind _skeletalmesh (`self.SkeletalMesh`))
  ; Can be reactivated
  (set `self.bUseOtherOverlayMesh?` false)
  ; Remove Outline
  (`PrimitiveComponent.SetRenderCustomDepth` _skeletalmesh true)
  (`PrimitiveComponent.SetCustomDepthStencilValue` _skeletalmesh 4)
  (`SceneComponent.SetHiddenInGame` (`self.GlitchEffect`) false false)
  (`PrimitiveComponent.SetVisibleInSceneCaptureOnly` (`self.GlitchEffect`) true)
  (`SceneComponent.SetVisibility` (`self.MaterialBillboard_0`) false false)
  (`SceneComponent.SetVisibility` (`self.InteractionKey`) false false))

(fn `OnRep_Transform`
  (`SceneComponent.K2_SetRelativeLocationAndRotation` (`self.getCharaRef`) (.location (`self.Transform`)) (`KismetMathLibrary.ComposeRotators` (.rotation (`self.Transform`)) (struct :`Yaw` -90.0)) false false))

(fn `OnRep_TruggerCameraComponents`
  (bind (_material _distancetoopacitycurve _bsizeisinscreenspace _basesizex _basesizey _distancetosizecurve) (break `MaterialSpriteElement` (`self.Item`)))
  (if (`self.TruggerCameraComponents`)
    (set `SceneCaptureComponent2D.TextureTarget` "/Game/DisconnectTemplate/Core/Blueprints/InteractableObjects/DevSide/CRT_Cameras.CRT_Cameras" (`self.SceneCaptureComponent2D`))
    (`self.NPC_Faces_EmissiveColor` (`self.DevConnected_NPC_FaceColor`))
    (`MaterialBillboardComponent.SetElements` (`self.MaterialBillboard_0`) (`|MakeArray` (make `MaterialSpriteElement` _material _distancetoopacitycurve _bsizeisinscreenspace 32.0 32.0 _distancetosizecurve)))
    (else
      (set `SceneCaptureComponent2D.TextureTarget` null (`self.SceneCaptureComponent2D`))
      (`self.NPC_Faces_EmissiveColor` (struct))
      (`MaterialBillboardComponent.SetElements` (`self.MaterialBillboard_0`) (`|MakeArray` (`self.Item`))))))

(fn `playAnimationData`
  (params (AnimationData :type "SingleAnimationPlayData Structure"))
  (bind _output_get (set `SkeletalMeshComponent.AnimationData` AnimationData (`self.getCharaRef`)))
  (bind (_animtoplay _bsavedlooping) (break `SingleAnimationPlayData` _output_get))
  (`SkeletalMeshComponent.PlayAnimation` (`self.getCharaRef`) _animtoplay _bsavedlooping))

(fn `UserConstructionScript`
  (`|ExecutionSequence`
    (:`then_0`
      (if (`self.bUseAnimationAsset?`)
        (`parent.UserConstructionScript`)))
    (:`then_1`
      (`KismetArrayLibrary.Array_Set` (`MaterialBillboardComponent.Elements` (`self.MaterialBillboard_0`)) 0 (`self.Item`)))
    (:`then_2`
      (bind _returnvalue (`PrimitiveComponent.CreateDynamicMaterialInstance` (`self.SM_Face`) 0 "/Game/DisconnectTemplate/MaterialLibrary/Flip/Alpha/MI_FlipbookAlphaNPC_Faces.MI_FlipbookAlphaNPC_Faces" "None"))
      (set `self.DMI_NPC_Faces` _returnvalue)
      (if (`self.bUseRndFace`)
        (`self.NPC_Faces_Face` (`KismetMathLibrary.RandomFloatInRange` 0.0 9.0))
        (else
          (`self.NPC_Faces_Face` (`self.FaceNbr`)))))
    (:`then_3`
      (set `self.PrimitiveComponentAsOverlayMesh` (`|MakeArray` (`self.SkeletalMesh`) :!type "PrimitiveComponent Object Reference")))))