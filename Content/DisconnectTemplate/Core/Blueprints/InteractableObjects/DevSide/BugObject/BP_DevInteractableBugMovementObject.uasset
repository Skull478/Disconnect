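; Dev-interactable "bug" object that jumps between preset positions, launching characters that overlap it and notifying the GameMode.
; The server cycles a replicated index from a random start after random delays, and its OnRep moves the mesh.
; DevInteract opens a bug message on the dev HUD, while UpdateDataActor temporarily overrides the delays to slow it, restored by a retriggerable delay.
; The construction script adds randomly tilted, scaled mesh pairs at each position.
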(event `self.ReceiveBeginPlay`
  (`parent.ReceiveBeginPlay`)
  (`/Engine/EditorBlueprintResources/ActorMacros.Switch Has Authority`
    (:`Authority`
      (set `self.RandomPos_Index` (`.OutIndex` (`KismetArrayLibrary.Array_Random` (`self.Positions`))))
      (`self.TSRV_TriggerTpObjectPos`)
      (set `self.MIN_DELAY` (`self.MinDelay`))
      (set `self.MAX_DELAY` (`self.MaxDelay`)))))

(event `TSRV_TriggerTpObjectPos`
  ; Trigger Tp Object Pos
  (`KismetSystemLibrary.Delay` (`KismetMathLibrary.RandomFloatInRange` (`self.MinDelay`) (`self.MaxDelay`)))
  (bind _output_get (set `self.RandomPos_Index` (+ (`self.RandomPos_Index`) 1)))
  (if (> _output_get (- (`KismetArrayLibrary.Array_Length` (`self.Positions`)) 1))
    (set `self.RandomPos_Index` 0)
    (else
      (set `self.RandomPos_Index` (`self.RandomPos_Index`))))
  (`self.TSRV_TriggerTpObjectPos`))

(event `self.Sphere.OnComponentBeginOverlap`
  (params (OverlappedComponent :type "PrimitiveComponent Object Reference") (OtherActor :type "Actor Object Reference") (OtherComp :type "PrimitiveComponent Object Reference") (OtherBodyIndex :type Integer) (bFromSweep :type Boolean) (SweepResult :type "HitResult Structure (by ref)"))
  ; Player Enter Collision
  (bind _ascharacter (cast `Character` OtherActor))
  (`Character.LaunchCharacter` _ascharacter (+ (* (`SceneComponent.GetForwardVector` (`self.ThrowDir`)) (`self.ProjectionForce`) 1.0) (0.0 0.0 400.0)) true true)
  (message `/Game/DisconnectTemplate/Core/Library/BPI_Game_GameMode.PlayerCollideBugObject` (`GameplayStatics.GetGameMode`)))

(event `/Game/DisconnectTemplate/Core/Blueprints/InteractableObjects/BPI_InteractableObject.DevInteract`
  (params (Ref :type "/Game/DisconnectTemplate/Core/Blueprints/Character/Game/Dev/BP_DisconnectDev_Character Object Reference"))
  ; DEV INTERRACT
  (set `self.DevCharaRef` Ref)
  (message `/Game/DisconnectTemplate/Widgets/Data/BPI_DevHUD.AddWidgetObjectBug` (`/Game/DisconnectTemplate/Core/Blueprints/Character/Game/Dev/BP_DisconnectDev_Character.DevHUD_Ref` (`self.DevCharaRef`)) self))

(event `/Game/DisconnectTemplate/Core/Library/BPI_UpdateData.UpdateDataActor`
  (params (DataList :type "/Game/DisconnectTemplate/Core/Library/S_BasicListOfData Structure"))
  ; Slow object
  (set `self.MinDelay` 1.5)
  (set `self.MaxDelay` 2.0)
  ; Min / Max Delay
  (`KismetSystemLibrary.RetriggerableDelay` 0.15)
  (set `self.MinDelay` (`self.MIN_DELAY`))
  (set `self.MaxDelay` (`self.MAX_DELAY`)))

(fn `OnRep_RandomPos_Index`
  (`SceneComponent.K2_SetRelativeLocation` (`self.SM_BugObject`) (`|GetArrayItem` (`self.Positions`) (`self.RandomPos_Index`)) false false))

(fn `UserConstructionScript`
  (locals (L_Rotation :type "Rotator Structure" :default (struct)))
  (bind _returnvalue (`KismetMathLibrary.Conv_DoubleToVector` (`KismetMathLibrary.RandomFloatInRange` 0.9 1.25)))
  (`parent.UserConstructionScript`)
  (`SphereComponent.SetSphereRadius` (`self.Sphere`) (`self.SphereRadius`) true)
  (`SceneComponent.SetWorldScale3D` (`self.SM_BugObject`) (`self.Scale`))
  (`SceneComponent.K2_SetRelativeRotation` (`self.ThrowDir`) (`self.ThrowDirRotation`) false false)
  (for _array_element (`self.Positions`)
    (bind _output_get (set `local.L_Rotation` (`KismetMathLibrary.ComposeRotators` (`self.RelativeTransformRotation`) (`KismetMathLibrary.MakeRotator` (`KismetMathLibrary.RandomFloatInRange` 0.0 (`self.XRandom`)) (`KismetMathLibrary.RandomFloatInRange` 0.0 (`self.YRandom`))))))
    (`AddComponent|NODE_AddStaticMeshComponent-0` :`RelativeTransform` (`KismetMathLibrary.MakeTransform` _array_element _output_get _returnvalue))
    (`AddComponent|NODE_AddStaticMeshComponent-2` :`RelativeTransform` (`KismetMathLibrary.MakeTransform` _array_element (`KismetMathLibrary.ComposeRotators` (`local.L_Rotation`) (struct :`Yaw` 180.0)) _returnvalue))))