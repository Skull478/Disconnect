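; Dev-side interactable oil valve that lets the dev character adjust the angle driving linked oil throwers.
; On interaction it stores the dev character and adds a valve message widget to that character's HUD, passing itself.
; Data updates pass the first float, the valve angle, to every referenced oil thrower through its update-and-check call.
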(event `self.ReceiveBeginPlay`
  (`parent.ReceiveBeginPlay`))

(event `/Game/DisconnectTemplate/Core/Blueprints/InteractableObjects/BPI_InteractableObject.DevInteract`
  (params (Ref :type "/Game/DisconnectTemplate/Core/Blueprints/Character/Game/Dev/BP_DisconnectDev_Character Object Reference"))
  ; Add Valvle
  (set `self.DevCharaRef` Ref)
  (message `/Game/DisconnectTemplate/Widgets/Data/BPI_DevHUD.AddWidgetValve` (`/Game/DisconnectTemplate/Core/Blueprints/Character/Game/Dev/BP_DisconnectDev_Character.DevHUD_Ref` (`self.DevCharaRef`)) self))

(event `/Game/DisconnectTemplate/Core/Library/BPI_UpdateData.UpdateDataActor`
  (params (DataList :type "/Game/DisconnectTemplate/Core/Library/S_BasicListOfData Structure"))
  ; Update Oil Thrower
  (for _array_element (`self.RefMeshOilThrowers`)
    (`/Game/DisconnectTemplate/Core/Blueprints/Active/BP_OilThrower.UpdateAndCheckSystem` _array_element (`|GetArrayItem` (`.ListOfFloat_3_018B9153488B47BE83268E87B9A7408B` (break `/Game/DisconnectTemplate/Core/Library/S_BasicListOfData` DataList))))))

(fn `UserConstructionScript`
  (`parent.UserConstructionScript`))