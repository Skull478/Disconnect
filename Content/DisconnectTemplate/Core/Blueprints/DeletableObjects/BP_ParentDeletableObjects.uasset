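; Base actor for deletable objects, with a configurable mesh, player detection sphere, delete flag and goal tag.
; The construction script applies mesh, material and radius, and computes target coordinates from the actor location, optionally offset.
; UpdateDataActor re-registers ReactivatesObjects with the interactable manager, then multicasts a swap to TrueMesh, or destruction if none is set.
; Good and wrong delete functions both simply destroy the actor.
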(event `self.ReceiveBeginPlay`)

(event `/Game/DisconnectTemplate/Core/Library/BPI_UpdateData.UpdateDataActor`
  (params (DataList :type "/Game/DisconnectTemplate/Core/Library/S_BasicListOfData Structure"))
  ; Trigger by Icon the WBP deleteable object
  (if (>= (`KismetArrayLibrary.Array_Length` (`.ListOfFloat_3_018B9153488B47BE83268E87B9A7408B` (break `/Game/DisconnectTemplate/Core/Library/S_BasicListOfData` DataList))) 0)
    (for _array_element (`self.ReactivatesObjects`)
      (`/Game/DisconnectTemplate/Core/Blueprints/Active/BP_DevMapInteractibleActorsManager.TSRV_AddActor` (`self.RefManagerInteractble`) _array_element true)))
  (`self.MC_DestroyActor`))

(event `MC_DestroyActor`
  (bind _mesh (`self.Mesh`))
  ; Destroy Actor or replace it
  (`self.TrueMesh`
    (:`then`
      (`StaticMeshComponent.SetStaticMesh` _mesh (`self.TrueMesh`))
      (bind _truematerial (`self.TrueMaterial`)
        (:`then`
          (`PrimitiveComponent.SetMaterial` _mesh 0 _truematerial))
        (:`else`)))
    (:`else`
      (`self.K2_DestroyActor`))))

(fn `F_Destroy`
  (`self.K2_DestroyActor`))

(fn `F_DestroyGoodActor`
  (`self.F_Destroy`))

(fn `F_DestroyWrongActor`
  (`self.F_Destroy`))

(fn `F_TryDelete`
  (returns (`bIsObjToDelete?` :type Boolean) (ObjectTagGoal :type "GameplayTag Structure"))
  (return (`self.bIsObjToDelete?`) (`self.ObjectTagGoal`)))

(fn `getMessages`
  (returns (Messages :type "Array of /Game/DisconnectTemplate/Widgets/Data/S_MessageProfile Structure"))
  (return))

(fn `getPlayerHUD`
  (returns (PlayerHUD :type "/Game/DisconnectTemplate/Widgets/Organismes/WBP_PlayerHUD Object Reference"))
  (return null))

(fn `UserConstructionScript`
  (bind _returnvalue (`self.K2_GetActorLocation`))
  (bind _mesh (`self.Mesh`))
  (`SphereComponent.SetSphereRadius` (`self.PlayerDetection`) (`self.DetectionRadius`) true)
  (`|ExecutionSequence`
    (:`then_0`
      (if (`self.bUseTrueCoordinates?`)
        (set `self.Coordinates` _returnvalue)
        (else
          (set `self.Coordinates` (+ (`self.MoveToCoordinates`) _returnvalue)))))
    (:`then_1`
      (`StaticMeshComponent.SetStaticMesh` _mesh (`self.SM_Mesh`))
      (`PrimitiveComponent.SetMaterial` _mesh 0 (`self.Material`)))))