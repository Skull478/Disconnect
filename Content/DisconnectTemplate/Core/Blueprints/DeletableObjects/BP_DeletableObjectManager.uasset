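; BP_DeletableObjectManager tracks deletable BP_ObjectsPart2 actors near the player and resolves coordinates to one of them.
; One tick after BeginPlay, to spread load, it gathers all such actors and binds their player detect and undetect events.
; Those events maintain an in-range list.
; FindObjetToCoordinates searches only that list, returning the closest object whose coordinates match the input within half its detection radius.
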(event `self.ReceiveBeginPlay`
  ; Begin Play Setup
  ;; NOT LOAD EVERYTHING ON THE FIRST TICK
  (`KismetSystemLibrary.DelayUntilNextTick`)
  (bind _outactors (`GameplayStatics.GetAllActorsOfClass` "/Game/DisconnectTemplate/Core/Blueprints/DeletableObjects/Part2/BP_ObjectsPart2.BP_ObjectsPart2_C"))
  (bind _output_get (set `self.ActorsRef` _outactors))
  (add `/Game/DisconnectTemplate/Core/Blueprints/DeletableObjects/Part2/BP_ObjectsPart2.DetectPlayer` _output_get (`|CreateDelegate` :!event `DetectPlayer_Event`))
  (add `/Game/DisconnectTemplate/Core/Blueprints/DeletableObjects/Part2/BP_ObjectsPart2.UnDetectPlayer` _output_get (`|CreateDelegate` :!event `UndetectPlayer_Event`)))

(event `DetectPlayer_Event`
  (params (Actor :type "/Game/DisconnectTemplate/Core/Blueprints/DeletableObjects/Part2/BP_ObjectsPart2 Object Reference"))
  ; When player is in range
  (`KismetArrayLibrary.Array_AddUnique` (`self.ActorsInRangeRef`) Actor))

(event `UndetectPlayer_Event`
  (params (ActorRef :type "/Game/DisconnectTemplate/Core/Blueprints/DeletableObjects/Part2/BP_ObjectsPart2 Object Reference"))
  ; When player is out of range
  (`KismetArrayLibrary.Array_RemoveItem` (`self.ActorsInRangeRef`) ActorRef))

(fn `FindObjetToCoordinates`
  (params (Coordinates :type "Vector Structure"))
  (returns (Actor :type "/Game/DisconnectTemplate/Core/Blueprints/DeletableObjects/Part2/BP_ObjectsPart2 Object Reference"))
  (locals (L_Distance :type "Float (double-precision)" :default 0.0) (L_ClosestObject :type "/Game/DisconnectTemplate/Core/Blueprints/DeletableObjects/Part2/BP_ObjectsPart2 Object Reference"))
  (bind _coordinates (`local.Coordinates`))
  (set `local.L_Distance` 500000.0)
  (for _array_element (`self.ActorsInRangeRef`)
    (bind _coordinates_2 (`/Game/DisconnectTemplate/Core/Blueprints/DeletableObjects/BP_ParentDeletableObjects.Coordinates` _array_element))
    (bind _returnvalue (`KismetMathLibrary.Vector_Distance` _coordinates_2 _coordinates))
    (if (and (== _coordinates_2 _coordinates :`ErrorTolerance` (/ (`/Game/DisconnectTemplate/Core/Blueprints/DeletableObjects/BP_ParentDeletableObjects.DetectionRadius` _array_element) 2.0)) (< _returnvalue (`local.L_Distance`)))
      (set `local.L_Distance` _returnvalue)
      (set `local.L_ClosestObject` _array_element)))
  (return (`local.L_ClosestObject`)))

(fn `UserConstructionScript`)