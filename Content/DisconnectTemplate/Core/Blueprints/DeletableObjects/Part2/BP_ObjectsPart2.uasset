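; Deletable object Blueprint with a second mesh that extends a parent class and signals when a Character enters or leaves its detection volume.
; PlayerDetection overlaps route through SRV events, named as server calls, to fire DetectPlayer and UnDetectPlayer with itself.
; Construction copies Mesh's first material onto Mesh1 and disables Mesh1's custom depth if the object is not deletable.
; SetMeshGlitchEffect drives the glitch look through custom depth and stencil on Mesh only.
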(event `self.ReceiveBeginPlay`)

(event `self.PlayerDetection.OnComponentBeginOverlap`
  (params (OverlappedComponent :type "PrimitiveComponent Object Reference") (OtherActor :type "Actor Object Reference") (OtherComp :type "PrimitiveComponent Object Reference") (OtherBodyIndex :type Integer) (bFromSweep :type Boolean) (SweepResult :type "HitResult Structure (by ref)"))
  ; DETECT and End Overlap Call
  (cast `Character` OtherActor)
  (`self.SRV_DetectPlayer`))

(event `SRV_DetectPlayer`
  ; DETECT and End Overlap Call
  (`self.DetectPlayer` self))

(event `self.PlayerDetection.OnComponentEndOverlap`
  (params (OverlappedComponent :type "PrimitiveComponent Object Reference") (OtherActor :type "Actor Object Reference") (OtherComp :type "PrimitiveComponent Object Reference") (OtherBodyIndex :type Integer))
  ; DETECT and End Overlap Call
  (cast `Character` OtherActor)
  (`self.SRV_Undetect`))

(event `SRV_Undetect`
  ; DETECT and End Overlap Call
  (`self.UnDetectPlayer` self))

(fn `setMeshGlitchEffect`
  (params (bValue :type Boolean :default true) (Value :type Integer :default 1))
  (bind _mesh (`self.Mesh`))
  (`PrimitiveComponent.SetRenderCustomDepth` _mesh bValue)
  (`PrimitiveComponent.SetCustomDepthStencilValue` _mesh Value))

(fn `UserConstructionScript`
  (`parent.UserConstructionScript`)
  (`PrimitiveComponent.SetMaterial` (`self.Mesh1`) 0 (`PrimitiveComponent.GetMaterial` (`self.Mesh`) 0))
  (if (not (`self.bIsObjToDelete?`))
    (`PrimitiveComponent.SetRenderCustomDepth` (`self.Mesh1`) false)))