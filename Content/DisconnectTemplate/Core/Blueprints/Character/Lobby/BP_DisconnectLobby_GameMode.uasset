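; Lobby GameMode that tracks joined player controllers, handles exclusive Player/Dev role selection and launches the match.
; Role selection opens at two players; each pick updates PlayerState and a gameplay tag container, then refreshes every client's button locks.
; The all-roles-set flag only checks for the Dev tag.
; With that flag set and everyone ready, it saves roles by index to the GameInstance and ServerTravels to the map.
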(event `self.ReceiveBeginPlay`
  (`KismetSystemLibrary.PrintString` "BP_DisconnectLobbyGameMode // BEGIN PLAY" true false (struct :`G` 0.66 :`B` 1.0 :`A` 1.0) 5.0))

(event `self.K2_PostLogin`
  (params (NewPlayer :type "PlayerController Object Reference"))
  ; When someone Log In
  (bind _output_get (set `self.PC_Ref` NewPlayer))
  (bind _asbp_lobby_player_controller (cast `/Game/DisconnectTemplate/Core/Blueprints/Character/Lobby/BP_Lobby_PlayerController` _output_get))
  (`KismetArrayLibrary.Array_AddUnique` (`self.LobbyPlayerControllerRefs`) _asbp_lobby_player_controller)
  (`BlueprintMapLibrary.Map_Add` (`self.LobbyPlayerControllerAndRoles`) _asbp_lobby_player_controller "NewEnumerator0")
  (`KismetSystemLibrary.PrintString` "BP_DisconnectLobbyGameMode" true false (struct :`G` 0.66 :`B` 1.0 :`A` 1.0) 5.0)
  (if (>= (`KismetArrayLibrary.Array_Length` (`self.LobbyPlayerControllerRefs`)) 2)
    (for _array_element (`self.LobbyPlayerControllerRefs`)
      (`/Game/DisconnectTemplate/Core/Blueprints/Character/Lobby/BP_Lobby_PlayerController.OWN_EnableRoleSelection` _array_element true))))

(event `self.K2_OnLogout`
  (params (ExitingController :type "Controller Object Reference"))
  ; When someone log out
  (bind _asbp_lobby_player_controller (cast `/Game/DisconnectTemplate/Core/Blueprints/Character/Lobby/BP_Lobby_PlayerController` ExitingController))
  (`KismetArrayLibrary.Array_RemoveItem` (`self.LobbyPlayerControllerRefs`) _asbp_lobby_player_controller)
  (`DestroySessionCallbackProxy.DestroySession` _asbp_lobby_player_controller
    (:`OnSuccess`
      (`self.CheckPlayerLeft`))))

(event `TSRV_RequestRole`
  (params (PlayerRole :type "/Game/DisconnectTemplate/Core/Blueprints/Character/Data/EPlayerRole Enum" :default "NewEnumerator0") (PlayerController :type "/Game/DisconnectTemplate/Core/Blueprints/Character/Lobby/BP_Lobby_PlayerController Object Reference"))
  ; Request Role
  (bind _allroleareset_ (`self.RoleSystem` PlayerRole PlayerController))
  (set `self.bAllRoleAreSet?` _allroleareset_))

(event `TSRV_RequestStart`
  (params (`bReady?` :type Boolean))
  (bind _nbrplayersready (`self.NbrPlayersReady`))
  ; Request Start
  (if `bReady?`
    (`/Engine/EditorBlueprintResources/StandardMacros.IncrementInt` _nbrplayersready
      (:`  `
        _))
    (else
      (`/Engine/EditorBlueprintResources/StandardMacros.DecrementInt` _nbrplayersready
        (:`  `
          _))))
  (for _array_element (`self.LobbyPlayerControllerRefs`)
    (`/Game/DisconnectTemplate/Core/Blueprints/Character/Lobby/BP_Lobby_PlayerController.TOWN_NbrOfPeopleReady` _array_element (`self.NbrPlayersReady`)))
  (if (`self.getConditionToStart`)
    (for (_array_element_2 _array_index) (`self.LobbyPlayerControllerRefs`)
      (`self.SetRoleDependingOfGI` _array_index (`BlueprintMapLibrary.Map_Find` (`self.LobbyPlayerControllerAndRoles`) _array_element_2)))
    (`KismetSystemLibrary.PrintString` "BP_DisconnectLobbyGameMode // START GAME" true false)
    (`AdvancedSessionsLibrary.ServerTravel` (`.RightS` (`KismetStringLibrary.Split` (`KismetSystemLibrary.Conv_SoftObjectReferenceToString` (`.WorldAsset` (break `SoftWorldReference` (`self.Map`)))) "." "IgnoreCase" "FromEnd")) true)))

(fn `CheckPlayerLeft`
  (if (not (>= (`KismetArrayLibrary.Array_Length` (`self.LobbyPlayerControllerRefs`)) 2))
    (for _array_element (`self.LobbyPlayerControllerRefs`)
      (`/Game/DisconnectTemplate/Core/Blueprints/Character/Lobby/BP_Lobby_PlayerController.OWN_EnableRoleSelection` _array_element false))))

(fn `getConditionToStart`
  (returns (ReturnValue :type Boolean))
  (return (and (`self.bAllRoleAreSet?`) (>= (`self.NbrPlayersReady`) (`KismetArrayLibrary.Array_Length` (`self.LobbyPlayerControllerRefs`))))))

(fn `RoleSystem`
  (params (PlayerRole :type "/Game/DisconnectTemplate/Core/Blueprints/Character/Data/EPlayerRole Enum" :default "NewEnumerator0") (PlayerController :type "/Game/DisconnectTemplate/Core/Blueprints/Character/Lobby/BP_Lobby_PlayerController Object Reference"))
  (returns (`AllRoleAreSet?` :type Boolean))
  (locals (`L_AllRoleSet?` :type Boolean :default false) (`L_RoleChanged?` :type Boolean :default false) (L_OldRole :type "/Game/DisconnectTemplate/Core/Blueprints/Character/Data/EPlayerRole Enum" :default "NewEnumerator0") (L_FirstLoopPC :type "/Game/DisconnectTemplate/Core/Blueprints/Character/Lobby/BP_Lobby_PlayerController Object Reference") (L_FirstLoopRole :type "/Game/DisconnectTemplate/Core/Blueprints/Character/Data/EPlayerRole Enum" :default "NewEnumerator0") (L_SecondLoopPC_Ref :type "/Game/DisconnectTemplate/Core/Blueprints/Character/Lobby/BP_Lobby_PlayerController Object Reference") (L_RoleSecondLoop :type "/Game/DisconnectTemplate/Core/Blueprints/Character/Data/EPlayerRole Enum") (L_ArrayOfRoles :type "Array of /Game/DisconnectTemplate/Core/Blueprints/Character/Data/EPlayerRole Enum"))
  (`BlueprintMapLibrary.Map_Add` (`self.LobbyPlayerControllerAndRoles`) (`local.PlayerController`) (`local.PlayerRole`))
  (bind _ballroleset_ (`self.TSRV_UpdateRole` (`local.PlayerRole`) (`Controller.PlayerState` PlayerController)))
  (set `local.L_AllRoleSet?` _ballroleset_)
  ; IMPOSSIBLE TO CLICK ON LAUNCH BUTTON (UPDATE) and Attribute Button For Self
  (bind (_keypin _valuepin) (`|MapForEach` (`self.LobbyPlayerControllerAndRoles`))
    (:`then`
      (bind _output_get (set `local.L_FirstLoopPC` _keypin))
      (`/Game/DisconnectTemplate/Core/Blueprints/Character/Lobby/BP_Lobby_PlayerController.OWN_ButtonLaunchGameIsEnable` _output_get (`local.L_AllRoleSet?`))
      (set `local.L_FirstLoopRole` _valuepin)
      (if (`|EnumEquality` (`local.L_FirstLoopRole`) "NewEnumerator0")
        ; Make all roles selectable
        (for _array_element (`local.L_ArrayOfRoles`)
          (if (`|EnumInequality` _array_element (`local.L_FirstLoopRole`))
            (`/Game/DisconnectTemplate/Core/Blueprints/Character/Lobby/BP_Lobby_PlayerController.TSRV_LobbyState` (`local.L_FirstLoopPC`) _array_element "NewEnumerator0")))
        ; If someone have already take this role make it locked for you
        (bind (_keypin_2 _valuepin_2) (`|MapForEach` (`self.LobbyPlayerControllerAndRoles`))
          (:`then`
            (set `local.L_SecondLoopPC_Ref` _keypin_2)
            (set `local.L_RoleSecondLoop` _valuepin_2)
            (if (`|EnumInequality` (`local.L_RoleSecondLoop`) "NewEnumerator0")
              (`/Game/DisconnectTemplate/Core/Blueprints/Character/Lobby/BP_Lobby_PlayerController.TSRV_LobbyState` (`local.L_FirstLoopPC`) (`local.L_RoleSecondLoop`) "NewEnumerator2"))))
        (else
          ; Lock role for other player
          (bind (_keypin_3 _valuepin_3) (`|MapForEach` (`self.LobbyPlayerControllerAndRoles`))
            (:`then`
              (set `local.L_SecondLoopPC_Ref` _keypin_3)
              (set `local.L_RoleSecondLoop` _valuepin_3)
              (if (!= (`local.L_SecondLoopPC_Ref`) (`local.L_FirstLoopPC`))
                (`/Game/DisconnectTemplate/Core/Blueprints/Character/Lobby/BP_Lobby_PlayerController.TSRV_LobbyState` (`local.L_SecondLoopPC_Ref`) (`local.L_FirstLoopRole`) "NewEnumerator2")
                (else
                  (`/Game/DisconnectTemplate/Core/Blueprints/Character/Lobby/BP_Lobby_PlayerController.TSRV_LobbyState` (`local.L_SecondLoopPC_Ref`) (`local.L_FirstLoopRole`) "NewEnumerator1")
                  ; Need to lock the other role only for you
                  (for _array_element_2 (`local.L_ArrayOfRoles`)
                    (if (`|EnumInequality` _array_element_2 (`local.L_FirstLoopRole`))
                      (`/Game/DisconnectTemplate/Core/Blueprints/Character/Lobby/BP_Lobby_PlayerController.TSRV_LobbyState` (`local.L_SecondLoopPC_Ref`) _array_element_2 "NewEnumerator2"))))))))))
    (:`CompletedPin`
      (return (`local.L_AllRoleSet?`)))))

(fn `SetRoleDependingOfGI`
  (params (ID :type "Integer (by ref)") (Role :type "/Game/DisconnectTemplate/Core/Blueprints/Character/Data/EPlayerRole Enum (by ref)"))
  (bind _disconnectgi (`/Game/DisconnectTemplate/Core/Library/BFL_Disconnect.getProjectGI`))
  (bind _advanceddisconnectgi (`/Game/DisconnectTemplate/Core/Library/BFL_Disconnect.getProjectAdvancedGI`))
  (`/Engine/EditorBlueprintResources/StandardMacros.IsValid` _advanceddisconnectgi
    (:`Is Valid`
      (`/Game/DisconnectTemplate/Core/Library/BP_AdvancedDisconnectGI.setPCRole` _advanceddisconnectgi (`local.ID`) (`local.Role`)))
    (:`Is Not Valid`
      (`/Engine/EditorBlueprintResources/StandardMacros.IsValid` _disconnectgi
        (:`Is Valid`
          (`/Game/DisconnectTemplate/Core/Library/BP_DisonnectGI.setPCRole` _disconnectgi (`local.ID`) (`local.Role`)))))))

(fn `TSRV_UpdateRole`
  (params (PlayerRole :type "/Game/DisconnectTemplate/Core/Blueprints/Character/Data/EPlayerRole Enum" :default "NewEnumerator0") (PlayerState :type "PlayerState Object Reference"))
  (returns (`bAllRoleSet?` :type Boolean))
  (locals (L_PlayerPlayerState :type "/Game/DisconnectTemplate/Core/Blueprints/Character/BP_DisconnectCorePlayerState Object Reference"))
  (bind _asbp_disconnect_core_player_state (cast `/Game/DisconnectTemplate/Core/Blueprints/Character/BP_DisconnectCorePlayerState` PlayerState)
    (:`then`
      (set `local.L_PlayerPlayerState` _asbp_disconnect_core_player_state)
      ; REMOVE TAG (can't select none so don't remove it)
      (switch `/Game/DisconnectTemplate/Core/Blueprints/Character/Data/EPlayerRole` (`/Game/DisconnectTemplate/Core/Blueprints/Character/BP_DisconnectCorePlayerState.PlayerRole` (`local.L_PlayerPlayerState`))
        (:`NewEnumerator0`
          _)
        (:`NewEnumerator1`
          (`BlueprintGameplayTagLibrary.RemoveGameplayTag` (`self.TagContainer`) (select `/Game/DisconnectTemplate/Core/Blueprints/Character/Data/EPlayerRole` (`/Game/DisconnectTemplate/Core/Blueprints/Character/BP_DisconnectCorePlayerState.PlayerRole` (`local.L_PlayerPlayerState`)) :`NewEnumerator0` (struct :`TagName` "Role.None") :`NewEnumerator1` (struct :`TagName` "Role.Player") :`NewEnumerator2` (struct :`TagName` "Role.Dev") :!type "GameplayTag Structure") :!label _label))
        (:`NewEnumerator2`
          (goto _label)))
      (switch `/Game/DisconnectTemplate/Core/Blueprints/Character/Data/EPlayerRole` (`local.PlayerRole`)
        (:`NewEnumerator0`
          _)
        (:`NewEnumerator1`
          (`BlueprintGameplayTagLibrary.AddGameplayTag` (`self.TagContainer`) (select `/Game/DisconnectTemplate/Core/Blueprints/Character/Data/EPlayerRole` (`local.PlayerRole`) :`NewEnumerator0` (struct :`TagName` "Role.None") :`NewEnumerator1` (struct :`TagName` "Role.Player") :`NewEnumerator2` (struct :`TagName` "Role.Dev") :!type "GameplayTag Structure") :!label _label_2))
        (:`NewEnumerator2`
          (goto _label_2)))
      ; Set Player role
      (`/Game/DisconnectTemplate/Core/Blueprints/Character/BP_DisconnectCorePlayerState.setPlayerRole` (`local.L_PlayerPlayerState`) (`local.PlayerRole`))
      (return (`BlueprintGameplayTagLibrary.HasAllTags` (`self.TagContainer`) (`BlueprintGameplayTagLibrary.MakeLiteralGameplayTagContainer` (struct :`GameplayTags` (struct :`(TagName` "Role.Dev") :`(TagName` "Role.Player")))) true)))
    (:`CastFailed`
      (return false))))

(fn `UserConstructionScript`)