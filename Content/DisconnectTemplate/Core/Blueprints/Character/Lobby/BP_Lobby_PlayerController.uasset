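; Lobby player controller that gives each local player the lobby UI for picking a role and readying up.
; On BeginPlay it creates the lobby widget with UI-only input, and on authority caches the lobby game mode.
; Prefixed relay events pass role and ready requests to the game mode, and push role states, ready counts and launch-button availability back to the widget.
; The Steam friends list widget creation is left unconnected.
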(event `self.ReceiveBeginPlay`
  (`|ExecutionSequence`
    (:`then_0`
      ; Only add widgets to local players
      (if (`self.IsLocalPlayerController`)
        ; LOBBY UI
        (bind _returnvalue (`|CreateWidget` "/Game/DisconnectTemplate/Widgets/Organismes/WBP_Lobby.WBP_Lobby_C" self self))
        (bind _output_get (set `self.LobbyWidgetRef` _returnvalue))
        (`UserWidget.AddToViewport` _output_get 0)
        ; UI interaction setup
        (`WidgetBlueprintLibrary.SetInputMode_UIOnlyEx` self (`self.LobbyWidgetRef`))
        (set `self.bShowMouseCursor` true)
        (`/Game/DisconnectTemplate/Widgets/Organismes/WBP_Lobby.UpdateReadyState` (`self.LobbyWidgetRef`) 0)))
    (:`then_1`
      (`/Engine/EditorBlueprintResources/ActorMacros.Switch Has Authority`
        (:`Authority`
          ; Get Ref Lobby Game Mode
          (bind _asbp_disconnect_lobby_game_mode (cast `/Game/DisconnectTemplate/Core/Blueprints/Character/Lobby/BP_DisconnectLobby_GameMode` (`GameplayStatics.GetGameMode`)))
          (set `self.LobbyGameModeRef` _asbp_disconnect_lobby_game_mode))))))

(event `TOWN_NewRole`
  (params (Role :type "/Game/DisconnectTemplate/Core/Blueprints/Character/Data/EPlayerRole Enum" :default "NewEnumerator0"))
  ; Set the new role
  (`self.SRV_NewRole` Role self))

(event `SRV_NewRole`
  (params (Role :type "/Game/DisconnectTemplate/Core/Blueprints/Character/Data/EPlayerRole Enum" :default "NewEnumerator0") (PlayerController :type "/Game/DisconnectTemplate/Core/Blueprints/Character/Lobby/BP_Lobby_PlayerController Object Reference"))
  ; Set the new role
  (`/Game/DisconnectTemplate/Core/Blueprints/Character/Lobby/BP_DisconnectLobby_GameMode.TSRV_RequestRole` (`self.LobbyGameModeRef`) Role PlayerController))

(event `TSRV_LobbyState`
  (params (Role :type "/Game/DisconnectTemplate/Core/Blueprints/Character/Data/EPlayerRole Enum" :default "NewEnumerator0") (ButtonSelectionType :type "/Game/DisconnectTemplate/Widgets/Data/EButtonSelectionType Enum" :default "NewEnumerator0"))
  ; Set Button Role State
  (`self.OWN_LobbyState` Role ButtonSelectionType))

(event `OWN_LobbyState`
  (params (Role :type "/Game/DisconnectTemplate/Core/Blueprints/Character/Data/EPlayerRole Enum" :default "NewEnumerator0") (ButtonSelectionType :type "/Game/DisconnectTemplate/Widgets/Data/EButtonSelectionType Enum" :default "NewEnumerator0"))
  ; Set Button Role State
  (`/Game/DisconnectTemplate/Widgets/Organismes/WBP_Lobby.WidgetRoleStateChange` (`self.LobbyWidgetRef`) Role ButtonSelectionType))

(event `OWN_ButtonLaunchGameIsEnable`
  (params (bInIsEnabled :type Boolean))
  ; GM trigger Button Launch is in enabled
  (`/Game/DisconnectTemplate/Widgets/Organismes/WBP_Lobby.UpdateStartButton` (`self.LobbyWidgetRef`) bInIsEnabled))

(event `OWN_PlayersReady`
  (params (NbrOfPlayerReady :type Integer))
  ; Players ready (trigger by GM)
  (`/Game/DisconnectTemplate/Widgets/Organismes/WBP_Lobby.UpdateReadyState` (`self.LobbyWidgetRef`) NbrOfPlayerReady))

(event `TOWN_PlayerReadyState`
  (params (`Ready?` :type Boolean))
  ; ReadyState
  (`self.SRV_PlayerReadyState` `Ready?`))

(event `SRV_PlayerReadyState`
  (params (`Ready?` :type Boolean))
  ; ReadyState
  (`/Game/DisconnectTemplate/Core/Blueprints/Character/Lobby/BP_DisconnectLobby_GameMode.SRV_RequestStart` (`self.LobbyGameModeRef`) `Ready?`))

(event `TOWN_NbrOfPeopleReady`
  (params (NbrOfPlayerReady :type Integer))
  ; Update UI for Nbr Of People Ready
  (`/Game/DisconnectTemplate/Widgets/Organismes/WBP_Lobby.UpdateReadyState` (`self.LobbyWidgetRef`) NbrOfPlayerReady))

(fn `UserConstructionScript`)