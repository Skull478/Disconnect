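; First-person multiplayer player character for the Disconnect template, handling interaction, object inspection, pause menu and compass.
; Interactions sphere-trace from the camera on the owner, are re-traced by the server, then return to the owner to message the target.
; Sphere traces also send look-at messages, while inspection locks movement and look to rotate objects.
; Replicated values drive the respawn effect's material parameter collection, alongside timed control inversion, dev QTE input swapping and looping camera shake.
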(event `self.ReceiveBeginPlay`
  (`KismetSystemLibrary.Delay` 5.0 :!label _label)
  (`GameplayStatics.PlayWorldCameraShake` "/Game/DisconnectTemplate/Core/Blueprints/CameraShake/BP_FreightElevatorCameraShake.BP_FreightElevatorCameraShake_C" (`self.K2_GetActorLocation`) 1000.0 1000.0)
  (goto _label))

(event `OWN_CameraOrientation`
  (bind _returnvalue (`SceneComponent.K2_GetComponentLocation` (`self.FirstPersonCamera`)))
  ; OVERLAY SYSTEM
  (`self.SphereTraceWithData` _returnvalue (+ _returnvalue (* (`self.GetActorForwardVector` (`GameplayStatics.GetPlayerCameraManager` 0)) 300.0))))

(event `TSRV_RespawnEffect`
  (params (`IsReverse?` :type Boolean))
  ; PP Respawn Effect
  (`self.srv_newSpeed` true (struct :`TagName` "Inputs.Movements.Disable"))
  (if (not `IsReverse?`)
    (set `self.PPAlpha` 0.0)
    (bind (_direction _alpha) (`Timeline|RespawnEffect` :!via `PlayFromStart` :!label _label_2)
      (:`Update`
        (set `self.PPAlpha` _alpha))
      (:`Finished`
        (`self.srv_newSpeed` false (struct :`TagName` "Inputs.Movements.Disable"))))
    (else
      (set `self.PPAlpha` 5.0)
      (goto _label_2 :!via `ReverseFromEnd`))))

(event `SphereTraceWithData`
  (params (Start :type "Vector Structure") (End :type "Vector Structure"))
  ; OVERLAY SYSTEM
  (bind _outhit (`KismetSystemLibrary.SphereTraceSingle` :`Start` Start :`End` End :`Radius` 10.0 :`TraceChannel` "TraceTypeQuery1" :`DrawDebugType` "ForOneFrame"))
  (bind (_bblockinghit _binitialoverlap _time _distance _location _impactpoint _normal _impactnormal _physmat _hitactor) (`GameplayStatics.BreakHitResult` _outhit))
  (`/Engine/EditorBlueprintResources/StandardMacros.IsValid` _hitactor
    (:`Is Valid`
      (bind _actorlookedat (`self.ActorLookedAt`)
        (:`then`
          (if (!= _actorlookedat _hitactor)
            (message `/Game/DisconnectTemplate/Core/Blueprints/InteractableObjects/BPI_InteractableObject.PlayerLookAtInteractableObject` (`self.ActorLookedAt`) false)
            (bind _output_get (set `self.ActorLookedAt` _hitactor))
            (message `/Game/DisconnectTemplate/Core/Blueprints/InteractableObjects/BPI_InteractableObject.PlayerLookAtInteractableObject` _output_get true)))
        (:`else`
          (bind _output_get_2 (set `self.ActorLookedAt` _hitactor))
          (message `/Game/DisconnectTemplate/Core/Blueprints/InteractableObjects/BPI_InteractableObject.PlayerLookAtInteractableObject` _output_get_2 true))))
    (:`Is Not Valid`
      (`self.ActorLookedAt`
        (:`then`
          (message `/Game/DisconnectTemplate/Core/Blueprints/InteractableObjects/BPI_InteractableObject.PlayerLookAtInteractableObject` (`self.ActorLookedAt`) false))
        (:`else`)))))

(event `SRV_DetectGameplayObject`
  ; OVERLAY SYSTEM
  (`self.OWN_CameraOrientation`))

(event `self.ReceivePossessed`
  (params (NewController :type "Controller Object Reference"))
  ; Activate Effect On Possess
  (`TimelineComponent.SetPlayRate` (`self.RespawnEffect`) (/ 1.0 (`self.EffectRespawnDuration`)))
  (set `self.PPAlpha` 5.0)
  (set `self.Location` (`self.K2_GetActorLocation`))
  (`self.TSRV_RespawnEffect` true)
  (`KismetSystemLibrary.K2_SetTimerDelegate` (`|CreateDelegate` :!event `SRV_DetectGameplayObject`) 0.05 true true))

(event `self.RotateCompass`
  (params (Float :type "Float (double-precision)"))
  ; Rotate Compass
  (bind _wbpcompassref (`self.WBPCompassRef`)
    (:`then`
      (`/Game/DisconnectTemplate/Widgets/Molecules/Player/WBP_Compass.RotateCompass` _wbpcompassref Float))
    (:`else`)))

(event `/Game/DisconnectTemplate/Core/Blueprints/Character/Game/BPI_DisconnectCharacter.OnPossess`
  ; Possess Event
  (`self.OWN_Possess`))

(event `EnhancedInput|/Game/DisconnectTemplate/Core/Inputs/Actions/IA_D_InteractObject`
  (params (ActionValue :type Boolean) (ElapsedSeconds :type "Float (double-precision)") (TriggeredSeconds :type "Float (double-precision)") (InputAction :type "InputAction Object Reference" :default "/Game/DisconnectTemplate/Core/Inputs/Actions/IA_D_InteractObject.IA_D_InteractObject"))
  (bind _returnvalue (`self.GetController`))
  (bind _returnvalue_2 (`self.GetController`))
  ; Inspect and rotate object
  (:`Started`
    (if (`self.CanInspect?`)
      (set `self.CanRotateObject?` true)
      (`Controller.SetIgnoreLookInput` _returnvalue_2 true)
      (`Controller.SetIgnoreMoveInput` _returnvalue_2 true)))
  (:`Completed`
    (if (`self.CanInspect?`)
      (set `self.CanRotateObject?` false)
      (`Controller.ResetIgnoreMoveInput` _returnvalue)
      (`Controller.ResetIgnoreLookInput` _returnvalue))))

(event `OWN_Possess`
  ; Possess Event
  (bind _playerhud (message `/Game/DisconnectTemplate/Core/Library/BPI_UpdateData.getPlayerHUD` (`GameplayStatics.GetPlayerController` 0) :!label _label_3))
  (`/Engine/EditorBlueprintResources/StandardMacros.IsValid` _playerhud
    (:`Is Valid`
      (set `self.WBPCompassRef` (`/Game/DisconnectTemplate/Widgets/Organismes/WBP_PlayerHUD.RefCompass` _playerhud)))
    (:`Is Not Valid`
      (`KismetSystemLibrary.Delay` 0.2)
      (goto _label_3))))

(event `self.RotateObject`
  (params (X :type "Float (double-precision)") (Y :type "Float (double-precision)"))
  ; Inspect and rotate object
  (if (`self.CanRotateObject?`)
    (`SceneComponent.K2_AddLocalRotation` (`Actor.RootComponent` (`self.InteractedObjectRef`)) (`KismetMathLibrary.MakeRotator` (* X (`self.ObjectRotationSpeed`)) (* Y (* (`self.ObjectRotationSpeed`) -1.0))) false false)))

(event `/Game/DisconnectTemplate/Core/Blueprints/InteractableObjects/BPI_InteractableObject.DevInteract`
  (params (Ref :type "/Game/DisconnectTemplate/Core/Blueprints/Character/Game/Dev/BP_DisconnectDev_Character Object Reference"))
  ; WHEN DEV INTERACT WITH ICON (Virus Only)
  (bind _output_get (set `self.DevCharaRef` Ref))
  (set `/Game/DisconnectTemplate/Core/Blueprints/Character/Game/Dev/BP_DisconnectDev_Character.PlayerCharaRef` self _output_get)
  (bind _output_get_2 (set `self.OldDevPC` (`self.GetLocalViewingPlayerController` (`self.DevCharaRef`))))
  (bind _returnvalue (pcsubsystem `EnhancedInputLocalPlayerSubsystem` _output_get_2))
  ; REMOVE camera movement and add QTE inputs
  (`EnhancedInputSubsystemInterface.RemoveMappingContext` _returnvalue "/Game/DisconnectTemplate/Core/Inputs/IMC_Dev.IMC_Dev" (struct))
  (`EnhancedInputSubsystemInterface.AddMappingContext` _returnvalue "/Game/DisconnectTemplate/Core/Inputs/IMC_QTE.IMC_QTE" 0 (struct)))

(event `SRV_ItemLocation`
  (params (Location :type "Vector Structure"))
  ; Item Location
  (`SceneComponent.K2_SetWorldLocation` (`self.Item`) Location false false))

(event `OWN_SendInputToHUD`
  (params (Input :type Name))
  ; HUD is only owning so need to change in a owner event
  (bind _hudref (`self.HudRef`)
    (:`then`
      (`/Game/DisconnectTemplate/Widgets/Organismes/WBP_PlayerHUD.TOWN_InputName` _hudref Input))
    (:`else`)))

(event `EnhancedInput|/Game/DisconnectTemplate/Core/Inputs/Actions/IA_D_Interact`
  (params (ActionValue :type Boolean) (ElapsedSeconds :type "Float (double-precision)") (TriggeredSeconds :type "Float (double-precision)") (InputAction :type "InputAction Object Reference" :default "/Game/DisconnectTemplate/Core/Inputs/Actions/IA_D_Interact.IA_D_Interact"))
  ; Interactions
  (:`Triggered`
    (if (`self.CanInspect?`)
      (bind _outhit (`self.OWN_SphereTraceForObj` 400.0 20.0 "None" (`|MakeArray` (`self.InteractedObjectRef`) :!type "Actor Object Reference") "ObjectTypeQuery2"))
      (`self.TraceForInserting` _outhit)))
  (:`Canceled`
    (if (`self.Interacting?`)
      (`self.SRV_Desinteract`)
      (else
        (bind (_outhit_2 _worldlocation _worlddirection) (`self.OWN_SphereTraceForObj` 400.0 50.0))
        (`self.SRV_Interact` _outhit_2 _worldlocation _worlddirection)
        (bind (_bblockinghit _binitialoverlap _time _distance _location _impactpoint _normal _impactnormal _physmat _hitactor) (`GameplayStatics.BreakHitResult` _outhit_2))
        (`/Engine/EditorBlueprintResources/StandardMacros.IsValid` _hitactor
          (:`Is Valid`
            (bind _isinteractable (message `/Game/DisconnectTemplate/Core/Blueprints/InteractableObjects/BPI_InteractableObject.IsInteractible?` _hitactor))
            (set `self.Interacting?` _isinteractable)))))))

(event `EnhancedInput|/Game/DisconnectTemplate/Core/Inputs/Actions/IA_D_Pause`
  (params (ActionValue :type Boolean) (ElapsedSeconds :type "Float (double-precision)") (TriggeredSeconds :type "Float (double-precision)") (InputAction :type "InputAction Object Reference" :default "/Game/DisconnectTemplate/Core/Inputs/Actions/IA_D_Pause.IA_D_Pause"))
  (bind _hudref (`self.HudRef`))
  ; Pause
  (:`Triggered`
    (`self.HudRef`
      (:`then`
        _)
      (:`else`
        (bind _playerhud (message `/Game/DisconnectTemplate/Core/Library/BPI_UpdateData.getPlayerHUD` (`GameplayStatics.GetPlayerController` 0)))
        (set `self.HudRef` _playerhud)))
    (`/Engine/EditorBlueprintResources/StandardMacros.IsValid` (`/Game/DisconnectTemplate/Widgets/Organismes/WBP_PlayerHUD.W_PauseMenuRef` _hudref)
      (:`Is Valid`
        (`/Game/DisconnectTemplate/Widgets/Organismes/WBP_PlayerHUD.RemovePause` _hudref))
      (:`Is Not Valid`
        (`/Game/DisconnectTemplate/Widgets/Organismes/WBP_PlayerHUD.AddPauseMenu` (`self.HudRef`))))))

(event `SRV_Interact`
  (params (HitResult :type "HitResult Structure") (WorldLoc :type "Vector Structure") (Direction :type "Vector Structure"))
  ; Interactions
  (bind _bcaninteract_ (`self.SRV_SphereTraceForObj` 400.0 50.0 "None" HitResult WorldLoc Direction))
  (if _bcaninteract_
    (bind _output_get (set `self.LastInteractedObject` (`.HitActor` (`GameplayStatics.BreakHitResult` HitResult))))
    (`self.OWN_InteractFB` _output_get)))

(event `TraceForInserting`
  (params (Hit :type "HitResult Structure (by ref)"))
  (bind (_bblockinghit _binitialoverlap _time _distance _location _impactpoint _normal _impactnormal _physmat _hitactor) (`GameplayStatics.BreakHitResult` Hit))
  ; Interactions
  (message `/Game/DisconnectTemplate/Core/Blueprints/InteractableObjects/BPI_InteractableObject.PlayerInteractWithObject` _hitactor self _location))

(event `TOWN_InverseControls`
  ; Inverse Sens when collide bug object
  (set `self.SensInputs` -1.0)
  (`KismetSystemLibrary.RetriggerableDelay` 10.0)
  (set `self.SensInputs` 1.0))

(event `OWN_InteractFB`
  (params (Target :type "Object Object Reference"))
  ; Interactions
  (message `/Game/DisconnectTemplate/Core/Blueprints/InteractableObjects/BPI_InteractableObject.PlayerInteract` Target self))

(event `EnhancedInput|/Game/DisconnectTemplate/Core/Inputs/Actions/IA_D_Desinteract`
  (params (ActionValue :type Boolean) (ElapsedSeconds :type "Float (double-precision)") (TriggeredSeconds :type "Float (double-precision)") (InputAction :type "InputAction Object Reference" :default "/Game/DisconnectTemplate/Core/Inputs/Actions/IA_D_Desinteract.IA_D_Desinteract"))
  ; Interactions
  (:`Triggered`
    (`self.SRV_Desinteract`)))

(event `SRV_Desinteract`
  ; Interactions
  (bind _lastinteractedobject (`self.LastInteractedObject`)
    (:`then`
      (`self.OWN_Desinteract` _lastinteractedobject))
    (:`else`)))

(event `OWN_Desinteract`
  (params (Target :type "Object Object Reference"))
  ; Interactions
  (message `/Game/DisconnectTemplate/Core/Blueprints/InteractableObjects/BPI_InteractableObject.PlayerDesinteract` Target self)
  (set `self.Interacting?` false))

(event `EnhancedInput|/Game/DisconnectTemplate/Core/Inputs/Actions/IA_Messagerie`
  (params (ActionValue :type Boolean) (ElapsedSeconds :type "Float (double-precision)") (TriggeredSeconds :type "Float (double-precision)") (InputAction :type "InputAction Object Reference" :default "/Game/DisconnectTemplate/Core/Inputs/Actions/IA_Messagerie.IA_Messagerie"))
  (bind _returnvalue (`GameplayStatics.GetPlayerController` 0))
  (bind _returnvalue_2 (`GameplayStatics.GetPlayerController` 0))
  ; Switch Mode Message
  (:`Triggered`
    (bind _isa (`/Engine/EditorBlueprintResources/StandardMacros.FlipFlop`)
      (:`A`
        (set `PlayerController.bShowMouseCursor` _isa _returnvalue_2)
        (`WidgetBlueprintLibrary.SetInputMode_GameAndUIEx` _returnvalue_2 null "DoNotLock" false))
      (:`B`
        (set `PlayerController.bShowMouseCursor` _isa _returnvalue)
        (`WidgetBlueprintLibrary.SetInputMode_GameOnly` _returnvalue)))))

(fn `CollisionWhenObjectGrabbed`
  (bind _firstpersoncamera (`self.FirstPersonCamera`))
  (bind _returnvalue (`SceneComponent.K2_GetComponentLocation` _firstpersoncamera))
  (bind (_outhit _returnvalue_2) (`KismetSystemLibrary.LineTraceSingle` _returnvalue (+ _returnvalue (* (`SceneComponent.GetForwardVector` _firstpersoncamera) 70.0)) "TraceTypeQuery1" false (`|MakeArray` (`self.InteractedObjectRef`) :!type "Actor Object Reference")))
  (if _returnvalue_2
    (bind (_bblockinghit _binitialoverlap _time _distance _location _impactpoint _normal _impactnormal _physmat _hitactor _hitcomponent _hitbonename _bonename _hititem _elementindex _faceindex _tracestart _traceend) (`GameplayStatics.BreakHitResult` _outhit))
    (`SceneComponent.K2_SetWorldLocation` (`self.Item`) _location false false)
    (`self.SRV_ItemLocation` _location)
    (else
      (`SceneComponent.K2_SetWorldLocation` (`self.Item`) _traceend false false)
      (`self.SRV_ItemLocation` _traceend))))

(fn `getMessages`
  (returns (Messages :type "Array of /Game/DisconnectTemplate/Widgets/Data/S_MessageProfile Structure"))
  (return))

(fn `GetPlayerCharacter`
  (returns (DisconnectPlayerRef :type "/Game/DisconnectTemplate/Core/Blueprints/Character/Game/Player/BP_DisconnectPlayer_Character Object Reference"))
  (return self))

(fn `getPlayerHUD`
  (returns (PlayerHUD :type "/Game/DisconnectTemplate/Widgets/Organismes/WBP_PlayerHUD Object Reference"))
  (return null))

(fn `InteractableObjectPutOverlay`
  (params (`PutAnOverlay?` :type Boolean))
  (returns (`ValidBPI?` :type Boolean))
  (return false))

(fn `IsInteractible?`
  (returns (IsInteractable :type Boolean))
  (return false))

(fn `OnRep_Location`
  (`KismetMaterialLibrary.SetVectorParameterValue` "/Game/DisconnectTemplate/MaterialLibrary/AllTypeOfGlitchPP/Respawn/PC_WorldRespawn.PC_WorldRespawn" "Location" (`KismetMathLibrary.Conv_VectorToLinearColor` (`self.Location`))))

(fn `OnRep_newWalkSpeed`
  (set `CharacterMovementComponent.MaxWalkSpeed` (`self.newWalkSpeed`) (`self.CharacterMovement`)))

(fn `OnRep_PPAlpha`
  (`KismetMaterialLibrary.SetScalarParameterValue` "/Game/DisconnectTemplate/MaterialLibrary/AllTypeOfGlitchPP/Respawn/PC_WorldRespawn.PC_WorldRespawn" "Amount" (`self.PPAlpha`)))

(fn `OWN_SphereTraceForObj`
  (params (Distance :type "Float (double-precision)") (Radius :type "Float (single-precision)") (DrawDebugType :type "EDrawDebugTrace Enum" :default "None") (ActorsToIgnore :type "Array of Actor Object Reference (by ref)") (ObjectType :type "EObjectTypeQuery Enum" :default "ObjectTypeQuery1"))
  (returns (OutHit :type "HitResult Structure") (WorldLocation :type "Vector Structure") (WorldDirection :type "Vector Structure"))
  (bind _firstpersoncamera (`self.FirstPersonCamera`))
  (bind _firstpersoncamera_2 (`self.FirstPersonCamera`))
  (bind _returnvalue (`SceneComponent.K2_GetComponentLocation` _firstpersoncamera_2))
  (bind _outhit (`KismetSystemLibrary.SphereTraceSingleForObjects` _returnvalue (+ _returnvalue (* (`SceneComponent.GetForwardVector` _firstpersoncamera_2) (`KismetSystemLibrary.MakeLiteralDouble` (`local.Distance`)))) (`local.Radius`) (`|MakeArray` ObjectType) false (`local.ActorsToIgnore`) (`local.DrawDebugType`)))
  (return _outhit (`SceneComponent.K2_GetComponentLocation` _firstpersoncamera) (`SceneComponent.GetForwardVector` _firstpersoncamera)))

(fn `PlayerIconHidden?`
  (params (NewHidden :type Boolean))
  (`SceneComponent.SetHiddenInGame` (`self.PlayerIconForDev`) true true))

(fn `srv_newSpeed`
  (params (`add?` :type Boolean) (tag :type "GameplayTag Structure"))
  (if `add?`
    (`BlueprintGameplayTagLibrary.AddGameplayTag` (`self.DisabledInputsTags`) (`local.tag`))
    (else
      (`BlueprintGameplayTagLibrary.RemoveGameplayTag` (`self.DisabledInputsTags`) (`local.tag`)))))

(fn `SRV_SphereTraceForObj`
  (params (Distance :type "Float (double-precision)") (Radius :type "Float (single-precision)") (DrawDebugType :type "EDrawDebugTrace Enum" :default "None") (HitResult :type "HitResult Structure") (WorldLoc :type "Vector Structure") (Direction :type "Vector Structure"))
  (returns (`bCanInteract?` :type Boolean))
  (bind _worldloc (`local.WorldLoc`))
  (bind (_outhit _returnvalue) (`KismetSystemLibrary.SphereTraceSingleForObjects` :`Start` _worldloc :`End` (+ _worldloc (* (`local.Direction`) (`KismetSystemLibrary.MakeLiteralDouble` (`local.Distance`)))) :`Radius` (`local.Radius`) :`ObjectTypes` (`|MakeArray` "ObjectTypeQuery1" :!type "EObjectTypeQuery Enum") :`DrawDebugType` (`local.DrawDebugType`)))
  (if (and _returnvalue (== (`.HitActor` (`GameplayStatics.BreakHitResult` _outhit)) (`.HitActor` (`GameplayStatics.BreakHitResult` (`local.HitResult`)))))
    (return true)
    (else
      (return false))))

(fn `UserConstructionScript`
  (bind _playericonfordev (`self.PlayerIconForDev`))
  (`SceneComponent.K2_SetRelativeLocation` _playericonfordev (`KismetMathLibrary.InverseTransformLocation` (`self.GetTransform`) (`KismetMathLibrary.MakeVector` (.x (`self.K2_GetActorLocation`)) (.y (`self.K2_GetActorLocation`)) 1500.0)) false false)
  (`SceneComponent.K2_SetWorldRotation` _playericonfordev (struct :`Yaw` 90.0) false false)
  (bind _returnvalue (`PrimitiveComponent.CreateDynamicMaterialInstance` (`self.Plane`) 0 "/Game/DisconnectTemplate/Art/Material_GD/Icons/MI_IconTextureTest.MI_IconTextureTest" "None"))
  (`MaterialInstanceDynamic.SetTextureParameterValue` _returnvalue "Texture" "/Game/DisconnectTemplate/Art/Textures/Icons/T_Player.T_Player")
  (`self.PlayerIconHidden?` true))