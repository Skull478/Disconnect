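; BP_AfterImageSkeleton is a short-lived afterimage actor that freezes a copy of a skeletal mesh's pose.
; On BeginPlay the authority assigns ComponentToCopy to RepPos, whose RepNotify copies the pose onto a PoseableMesh and creates a Manny-based dynamic material stored as Fade.
; The authority also plays a slowed T_Fade timeline and destroys the actor when it finishes, though no timeline update drives the material here.
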(event `self.ReceiveBeginPlay`
  (`/Engine/EditorBlueprintResources/ActorMacros.Switch Has Authority`
    (:`Authority`
      (bind _componenttocopy (`self.ComponentToCopy`)
        (:`then`
          (set `self.RepPos` _componenttocopy)
          (`TimelineComponent.SetPlayRate` (`self.T_Fade`) (/ 1.0 2.0))
          (`Timeline|T_Fade` :!via `PlayFromStart`
            (:`Finished`
              (`self.K2_DestroyActor`))))
        (:`else`)))))

(fn `OnRep_RepPos`
  (`PoseableMeshComponent.CopyPoseFromSkeletalComponent` (`self.PoseableMesh`) (`self.RepPos`))
  (bind _returnvalue (`PrimitiveComponent.CreateDynamicMaterialInstance` (`self.PoseableMesh`) 0 "/Game/FP_Content/Characters/Mannequins/Materials/Manny/MI_Manny_01_New.MI_Manny_01_New" "None"))
  (set `self.Fade` _returnvalue))

(fn `UserConstructionScript`)