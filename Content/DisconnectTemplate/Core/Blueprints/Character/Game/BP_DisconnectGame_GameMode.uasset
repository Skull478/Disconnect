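; Game mode for Disconnect's asymmetric two-player session, pairing a Player with a Dev.
; Registers joining controllers, then assigns roles from the game instance, falling back to random, or shows a role picker for solo testing.
; Routes virus, messaging, floor, warning and game-update events to the relevant controllers, seeding messages from a data table.
; Game over teleports the Player to the checkpoint or PlayerStart and resets it; logout destroys sessions.
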(event `self.K2_OnLogout`
  (params (ExitingController :type "Controller Object Reference"))
  ; LOG OUT
  (bind (_keypin _valuepin) (`|MapForEach` (`self.PlayerControllers`))
    (:`then`
      (`DestroySessionCallbackProxy.DestroySession` _valuepin))))

(event `self.ReceiveBeginPlay`
  (`KismetSystemLibrary.PrintString` "BP_DisconnectGameGameMode // BEGIN PLAY" true false (struct :`G` 0.66 :`B` 1.0 :`A` 1.0) 20.0)
  ; Get Messages
  (bind _outrownames (`DataTableFunctionLibrary.GetDataTableRowNames` "/Game/DisconnectTemplate/Widgets/Data/DataTable/Messages/DT_MessagesDevToPlayer.DT_MessagesDevToPlayer"))
  (for _array_element _outrownames
    (bind _returnvalue (`|GetDataTableRow` "/Game/DisconnectTemplate/Widgets/Data/DataTable/Messages/DT_MessagesDevToPlayer.DT_MessagesDevToPlayer" _array_element)
      (:`then`
        (`KismetArrayLibrary.Array_Add` (`self.MessagesPlayerToDev`) _returnvalue)))))

(event `/Game/DisconnectTemplate/Core/Library/BPI_Game_GameMode.LevelIsLoaded`
  ; LEVELS READY ?
  (set `self.LevelsReady?` true)
  (`KismetSystemLibrary.PrintString` "LEVELS READY")
  ; Handle Players
  (if (and (>= (`BlueprintMapLibrary.Map_Length` (`self.PlayerControllers`)) 2) (`self.LevelsReady?`)) :!label _label
    (`/Engine/EditorBlueprintResources/StandardMacros.DoOnce` false :!label _label_2
      (:`Completed`
        (if (`self.bUseSoloTest?`)
          (`KismetSystemLibrary.PrintString` "BP_DisconnectGameGameMode // FOR SOLO TEST" true false (struct :`G` 0.66 :`B` 1.0 :`A` 1.0) 5.0 :!label _label_3)
          (bind _returnvalue (`|SpawnActorFromClass` "/Game/DisconnectTemplate/Core/Blueprints/Character/Game/BP_PawnSpectator.BP_PawnSpectator_C" (`KismetMathLibrary.MakeTransform` (0.0 0.0 0.0)) "Undefined" "MultiplyWithRoot" null null))
          (`Controller.Possess` (`BlueprintMapLibrary.Map_Find` (`self.PlayerControllers`)) _returnvalue)
          (bind _returnvalue_2 (`|CreateWidget` "/Game/DisconnectTemplate/Widgets/Molecules/WBP_SelectionCharaIfSolo.WBP_SelectionCharaIfSolo_C" (`BlueprintMapLibrary.Map_Find` (`self.PlayerControllers`))))
          (bind _output_get (set `self.SoloHUD_Ref` _returnvalue_2))
          (`UserWidget.AddToViewport` _output_get 0)
          (else
            (set `self.bNoRole?` false)
            (bind _keypin (`|MapForEach` (`self.PlayerControllers`) :!label _label_4)
              (:`then`
                (bind _role (`self.ValidPC` _keypin))
                (switch `/Game/DisconnectTemplate/Core/Blueprints/Character/Data/EPlayerRole` _role
                  (:`NewEnumerator0`
                    (set `self.bNoRole?` true)
                    (goto _label_4 :!via `BreakPin`))
                  (:`NewEnumerator1`
                    (`self.InitPlayerSide` _keypin)
                    (`KismetSystemLibrary.PrintString` "BP_DisconnectGameGameMode // INIT PLAYER" true false (struct :`G` 0.66 :`B` 1.0 :`A` 1.0) 5.0))
                  (:`NewEnumerator2`
                    (`self.InitDevSide` _keypin)
                    (`KismetSystemLibrary.PrintString` "BP_DisconnectGameGameMode // INIT DEV" true false (struct :`G` 0.66 :`B` 1.0 :`A` 1.0) 5.0))))
              (:`CompletedPin`
                (if (`self.bNoRole?`)
                  (`KismetSystemLibrary.PrintString` "BP_DisconnectGame_GameMode // FAILED TO GIVE ROLE" true false (struct :`R` 1.0 :`B` 0.01437 :`A` 1.0) 10.0)
                  (`self.GiveRndRoles`))))))))
    (else
      (`/Engine/EditorBlueprintResources/StandardMacros.DoOnce` false :!label _label_5
        (:`Completed`
          (if (`self.bUseSoloTest?`)
            (goto _label_3)))))))

(event `self.K2_PostLogin`
  (params (NewPlayer :type "PlayerController Object Reference"))
  ;[1 0 0.01437] Not Working after Server Travel
  (`KismetSystemLibrary.PrintString` "BP_DisconnectGameGameMode // POST LOG IN" true false (struct :`R` 1.0 :`A` 1.0) 5.0))

(event `self.HandleStartingNewPlayer`
  (params (NewPlayer :type "PlayerController Object Reference"))
  ; Handle Players
  (bind _output_get (set `self.PC_Ref` NewPlayer))
  (bind _asbp_disconnect_game_player_controller (cast `/Game/DisconnectTemplate/Core/Blueprints/Character/Game/BP_DisconnectGamePlayerController` _output_get)
    (:`then`
      (`BlueprintMapLibrary.Map_Add` (`self.PlayerControllers`) (`BlueprintMapLibrary.Map_Length` (`self.PlayerControllers`)) _asbp_disconnect_game_player_controller)
      (`|ExecutionSequence`
        (:`then_0`
          (goto _label))
        (:`then_1`
          (`KismetSystemLibrary.Delay` 5.0) ; TEST AGAIN AFTER DELAY (the do once will stop the event to trigger twice)
          (if (>= (`BlueprintMapLibrary.Map_Length` (`self.PlayerControllers`)) 2)
            (goto _label_2)
            (else
              (goto _label_5))))))
    (:`CastFailed`
      (`KismetSystemLibrary.PrintString` "Game Game Mode Failed Player Controller Cast To" true false (struct :`R` 1.0 :`A` 1.0) 5.0))))

(event `InitPlayerSide`
  (params (PlayerID :type Integer))
  ; INIT both Role and PC
  (bind _output_get (set `self.PlayerID` PlayerID))
  (bind _value (`BlueprintMapLibrary.Map_Find` (`self.PlayerControllers`) _output_get))
  (`/Game/DisconnectTemplate/Core/Blueprints/Character/Game/BP_DisconnectGamePlayerController.OWN_InitPlayerControllerToRole` _value "NewEnumerator1")
  (`/Game/DisconnectTemplate/Core/Blueprints/Character/Game/BP_DisconnectGamePlayerController.OWN_SetupVarMessages` _value (`self.MessagesPlayerToDev`)))

(event `InitDevSide`
  (params (DevID :type Integer))
  ; INIT both Role and PC
  (bind _output_get (set `self.DevID` DevID))
  (bind _value (`BlueprintMapLibrary.Map_Find` (`self.PlayerControllers`) _output_get))
  (`/Game/DisconnectTemplate/Core/Blueprints/Character/Game/BP_DisconnectGamePlayerController.OWN_SetupVarMessages` _value (`self.MessagesPlayerToDev`))
  (`/Game/DisconnectTemplate/Core/Blueprints/Character/Game/BP_DisconnectGamePlayerController.OWN_InitPlayerControllerToRole` _value "NewEnumerator2"))

(event `TSRV_TriggerVirusGame`
  ; Trigger Virus
  (bind (_keypin _valuepin) (`|MapForEach` (`self.PlayerControllers`))
    (:`then`
      (`/Game/DisconnectTemplate/Core/Blueprints/Character/Game/BP_DisconnectGamePlayerController.OWN_TriggerVirus` _valuepin))))

(event `/Game/DisconnectTemplate/Core/Library/BPI_Game_GameMode.ClearVirus`
  ; Clear Virus
  (bind (_keypin _valuepin) (`|MapForEach` (`self.PlayerControllers`))
    (:`then`
      (`/Game/DisconnectTemplate/Core/Blueprints/Character/Game/BP_DisconnectGamePlayerController.OWN_ClearVirus` _valuepin)
      (`KismetSystemLibrary.PrintString` "GAME MODE // TRIGGER OWN CLEAR VIRUS" true false (struct :`R` 1.0 :`G` 0.071405 :`A` 1.0) 10.0))))

(event `/Game/DisconnectTemplate/Core/Library/BPI_Game_GameMode.GameOver`
  (bind _playercharacterref (`/Game/DisconnectTemplate/Core/Blueprints/Character/Game/BP_DisconnectGamePlayerController.PlayerCharacterRef` (`BlueprintMapLibrary.Map_Find` (`self.PlayerControllers`) (`self.PlayerID`))))
  ; MAKE GAME OVER
  (`self.CheckPointManagerRef`
    (:`then`
      (`self.K2_TeleportTo` _playercharacterref (.location (`/Game/DisconnectTemplate/Core/Blueprints/Active/BP_CheckPointManager.CheckpointTransform` (`self.CheckPointManagerRef`))) (.rotation (`/Game/DisconnectTemplate/Core/Blueprints/Active/BP_CheckPointManager.CheckpointTransform` (`self.CheckPointManagerRef`))) :!label _label_6)
      (`/Game/DisconnectTemplate/Core/Blueprints/Character/Game/BP_DisconnectCore_Character.TSRV_GameOverResetVariables` _playercharacterref))
    (:`else`
      (bind _returnvalue (`GameplayStatics.GetActorOfClass` "/Game/DisconnectTemplate/Core/Blueprints/Active/BP_CheckPointManager.BP_CheckPointManager_C"))
      (bind _output_get (set `self.CheckPointManagerRef` _returnvalue))
      (`/Engine/EditorBlueprintResources/StandardMacros.IsValid` _output_get
        (:`Is Valid`
          (goto _label_6))
        (:`Is Not Valid`
          (bind _returnvalue_2 (`GameplayStatics.GetActorOfClass` "/Script/Engine.PlayerStart"))
          (`self.K2_TeleportTo` :`self` _playercharacterref :`DestLocation` (`self.K2_GetActorLocation` _returnvalue_2))
          (`/Game/DisconnectTemplate/Core/Blueprints/Character/Game/BP_DisconnectCore_Character.TSRV_GameOverResetVariables` _playercharacterref))))))

(event `/Game/DisconnectTemplate/Core/Library/BPI_Game_GameMode.SoloGM_TakeRole`
  (params (Role :type "/Game/DisconnectTemplate/Core/Blueprints/Character/Data/EPlayerRole Enum" :default "NewEnumerator0"))
  ; SoloGM_TakeRole
  (switch `/Game/DisconnectTemplate/Core/Blueprints/Character/Data/EPlayerRole` Role
    (:`NewEnumerator1`
      (`self.InitPlayerSide` 0))
    (:`NewEnumerator2`
      (`self.InitDevSide` 0)))
  (`Widget.RemoveFromParent` (`self.SoloHUD_Ref`)))

(event `/Game/DisconnectTemplate/Core/Library/BPI_Game_GameMode.GiveVirus`
  ; Give Virus
  (`self.TSRV_TriggerVirusGame`))

(event `/Game/DisconnectTemplate/Core/Library/BPI_Game_GameMode.GameUpdate`
  (params (EventTag :type "GameplayTag Structure") (DevDeleteableObj :type "/Game/DisconnectTemplate/Core/Blueprints/InteractableObjects/DevSide/BP_DevDeleteableInteractObject Object Reference"))
  ; Game Update
  (`/Game/DisconnectTemplate/Core/Blueprints/Character/Game/BP_DisconnectGamePlayerController.OWN_UpdateGame` (`BlueprintMapLibrary.Map_Find` (`self.PlayerControllers`) (`self.DevID`)) EventTag DevDeleteableObj))

(event `/Game/DisconnectTemplate/Core/Library/BPI_Game_GameMode.GM_SendMessage`
  (params (Message :type "/Game/DisconnectTemplate/Widgets/Data/S_MessageProfile Structure"))
  ; Message (update var in all pc) and update ui for the other
  (`KismetArrayLibrary.Array_Add` (`self.MessagesPlayerToDev`) Message)
  (bind (_keypin _valuepin) (`|MapForEach` (`self.PlayerControllers`))
    (:`then`
      (`/Game/DisconnectTemplate/Core/Blueprints/Character/Game/BP_DisconnectGamePlayerController.OWN_SetupVarMessages` _valuepin (`self.MessagesPlayerToDev`)))
    (:`CompletedPin`
      (`/Game/DisconnectTemplate/Core/Blueprints/Character/Game/BP_DisconnectGamePlayerController.OWN_Message` (`BlueprintMapLibrary.Map_Find` (`self.PlayerControllers`) (select `/Game/DisconnectTemplate/Widgets/Data/E_WhoBubble` (`.Who_4_C80EF01349568D5C607D8B9268229E7A` (break `/Game/DisconnectTemplate/Widgets/Data/S_MessageProfile` Message)) :`NewEnumerator0` (`self.DevID`) :`NewEnumerator1` (`self.PlayerID`))) Message))))

(event `/Game/DisconnectTemplate/Core/Library/BPI_Game_GameMode.VirusInfoFixTest`
  (params (Code :type Text))
  ; Info Virus send text
  (`/Game/DisconnectTemplate/Core/Blueprints/Character/Game/BP_DisconnectGamePlayerController.OWN_InfoVirus` (`BlueprintMapLibrary.Map_Find` (`self.PlayerControllers`) (`self.PlayerID`)) Code))

(event `/Game/DisconnectTemplate/Core/Library/BPI_Game_GameMode.GM_UpdateFloor`
  (params (Floor :type Integer))
  ; Update Floor (use only dev)
  (bind _output_get (set `self.PlayerCurrentFloor` Floor))
  (`/Game/DisconnectTemplate/Core/Blueprints/Character/Game/BP_DisconnectGamePlayerController.OWN_UpdateFloor` (`BlueprintMapLibrary.Map_Find` (`self.PlayerControllers`) (`self.DevID`)) _output_get))

(event `/Game/DisconnectTemplate/Core/Library/BPI_Game_GameMode.PlayerCollideBugObject`
  ; Collide bug object
  (bind (_keypin _valuepin) (`|MapForEach` (`self.PlayerControllers`))
    (:`then`
      (`/Game/DisconnectTemplate/Core/Blueprints/Character/Game/BP_DisconnectGamePlayerController.OWN_CollideBugObject` _valuepin))))

(event `/Game/DisconnectTemplate/Core/Library/BPI_Game_GameMode.StartWarning`
  (params (`bIsEndWarning?` :type Boolean) (Location :type "Vector Structure"))
  ; Start Warning
  (`/Game/DisconnectTemplate/Core/Blueprints/Character/Game/BP_DisconnectGamePlayerController.OWN_StartWarning` (`BlueprintMapLibrary.Map_Find` (`self.PlayerControllers`) (`self.DevID`)) `bIsEndWarning?` Location))

(fn `GetPlayerControllerFromRole`
  (params (Role :type "/Game/DisconnectTemplate/Core/Blueprints/Character/Data/EPlayerRole Enum" :default "NewEnumerator0"))
  (returns (PC_Ref :type "PlayerController Object Reference"))
  (return (select `/Game/DisconnectTemplate/Core/Blueprints/Character/Data/EPlayerRole` Role :`NewEnumerator1` (`BlueprintMapLibrary.Map_Find` (`self.PlayerControllers`) (`self.PlayerID`)) :`NewEnumerator2` (`BlueprintMapLibrary.Map_Find` (`self.PlayerControllers`) (`self.DevID`)) :!type "PlayerController Object Reference")))

(fn `getPlayerControllersMapNbrIndex`
  (returns (ReturnValue :type Integer))
  (return (- (`BlueprintMapLibrary.Map_Length` (`self.PlayerControllers`)) 1)))

(fn `GiveRndRoles`
  (locals (L_Roles :type "Array of /Game/DisconnectTemplate/Core/Blueprints/Character/Data/EPlayerRole Enum") (L_RoleIndex :type Integer :default 0) (L_RolePC :type "/Game/DisconnectTemplate/Core/Blueprints/Character/Data/EPlayerRole Enum" :default "NewEnumerator0"))
  (set `local.L_Roles` (`|MakeArray` "NewEnumerator1" "NewEnumerator2" :!type "/Game/DisconnectTemplate/Core/Blueprints/Character/Data/EPlayerRole Enum"))
  (if (>= (`BlueprintMapLibrary.Map_Length` (`self.PlayerControllers`)) 2)
    (if (`KismetMathLibrary.RandomBool`)
      (`self.InitPlayerSide` 1)
      (`self.InitDevSide` 0)
      (else
        (`self.InitPlayerSide` 0)
        (`self.InitDevSide` 1)))
    (else
      (return))))

(fn `setPC_Role`
  (params (ID :type "Integer (by ref)") (Role :type "/Game/DisconnectTemplate/Core/Blueprints/Character/Data/EPlayerRole Enum (by ref)"))
  (bind _disconnectgi (`/Game/DisconnectTemplate/Core/Library/BFL_Disconnect.getProjectGI`))
  (`/Engine/EditorBlueprintResources/StandardMacros.IsValid` _disconnectgi
    (:`Is Valid`
      (`/Game/DisconnectTemplate/Core/Library/BP_DisonnectGI.setPCRole` _disconnectgi (`local.ID`) (`local.Role`)))
    (:`Is Not Valid`
      (`/Game/DisconnectTemplate/Core/Library/BP_AdvancedDisconnectGI.setPCRole` (`/Game/DisconnectTemplate/Core/Library/BFL_Disconnect.getProjectAdvancedGI`) (`local.ID`) (`local.Role`)))))

(fn `UserConstructionScript`)

(fn `ValidPC`
  (params (Index :type "Integer (by ref)"))
  (returns (Role :type "/Game/DisconnectTemplate/Core/Blueprints/Character/Data/EPlayerRole Enum"))
  (bind _advanceddisconnectgi (`/Game/DisconnectTemplate/Core/Library/BFL_Disconnect.getProjectAdvancedGI`))
  (bind _disconnectgi (`/Game/DisconnectTemplate/Core/Library/BFL_Disconnect.getProjectGI`))
  (`/Engine/EditorBlueprintResources/StandardMacros.IsValid` _advanceddisconnectgi
    (:`Is Valid`
      (return (`/Game/DisconnectTemplate/Core/Library/BP_AdvancedDisconnectGI.getPCRole` _advanceddisconnectgi (`local.Index`))))
    (:`Is Not Valid`
      (`/Engine/EditorBlueprintResources/StandardMacros.IsValid` _disconnectgi
        (:`Is Valid`
          (return (`/Game/DisconnectTemplate/Core/Library/BP_DisonnectGI.getPCRole` _disconnectgi (`local.Index`))))
        (:`Is Not Valid`
          (return "NewEnumerator0"))))))