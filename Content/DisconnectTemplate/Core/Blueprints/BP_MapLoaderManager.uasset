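; BP_MapLoaderManager streams in a set of levels chosen by player role, Player or Dev.
; The TOWN_LoadStreamingLevel event loops over that role's soft-referenced level list, issuing non-blocking loads with visibility off.
; It then finds each streaming level by a name parsed from its soft path and, if valid, flags it to be visible.
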(event `TOWN_LoadStreamingLevel`
  (params (PlayerRole :type "/Game/DisconnectTemplate/Core/Blueprints/Character/Data/EPlayerRole Enum" :default "NewEnumerator0"))
  (switch `/Game/DisconnectTemplate/Core/Blueprints/Character/Data/EPlayerRole` PlayerRole
    (:`NewEnumerator1`
      (for _array_element (`self.LevelsPlayerToLoad`)
        (`GameplayStatics.LoadStreamLevelBySoftObjectPtr` _array_element)
        (bind _returnvalue (`GameplayStatics.GetStreamingLevel` (`self.WorldSoftToLevelName` _array_element)))
        (`/Engine/EditorBlueprintResources/StandardMacros.IsValid` _returnvalue
          (:`Is Valid`
            (set `LevelStreaming.bShouldBeVisible` true _returnvalue)))))
    (:`NewEnumerator2`
      (for _array_element_2 (`self.LevelsDevToLoad`)
        (`GameplayStatics.LoadStreamLevelBySoftObjectPtr` _array_element_2)
        (bind _returnvalue_2 (`GameplayStatics.GetStreamingLevel` (`self.WorldSoftToLevelName` _array_element_2)))
        (`/Engine/EditorBlueprintResources/StandardMacros.IsValid` _returnvalue_2
          (:`Is Valid`
            (set `LevelStreaming.bShouldBeVisible` true _returnvalue_2)))))))

(fn `UserConstructionScript`)

(fn `WorldSoftToLevelName`
  (params (SoftObjectReference :type "Object Soft Object Reference"))
  (returns (MapName :type Name))
  (return (`KismetStringLibrary.Conv_StringToName` (`.RightS` (`KismetStringLibrary.Split` (`KismetSystemLibrary.BreakSoftObjectPath` (`KismetSystemLibrary.Conv_SoftObjRefToSoftObjPath` SoftObjectReference)) "." "CaseSensitive" "FromEnd")))))