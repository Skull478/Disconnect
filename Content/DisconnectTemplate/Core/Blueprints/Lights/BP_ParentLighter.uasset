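; Parent actor that places street lamp or garage light meshes along a spline at construction, optionally with light components.
; Each spline point adds an instanced mesh by lamp type and, when active, a spot or rect light at the SM_LightPosition socket.
; LightParameter functions configure intensity, color, shadows and IES profiles.
; Light functions are assigned by seeded random chance, with spot lights also randomizing MPC_Flickering parameters.
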(event `self.ReceiveBeginPlay`)

(fn `UserConstructionScript`
  (locals (L_SpotLightComp :type "SpotLightComponent Object Reference") (L_NumOfSplinePoint :type Integer) (L_RecLightComp :type "RectLightComponent Object Reference") (NumberOfSpotLightPlaced :type Integer :default 0) (NumberOfRecLight :type Integer :default 0))
  (bind _b_usetemperature_ (`self.b_UseTemperature?`))
  (bind _b_usetemperature__2 (`self.b_UseTemperature?`))
  (for _index (range (`SplineComponent.GetNumberOfSplinePoints` (`self.Spline`)))
    (set `local.L_NumOfSplinePoint` _index)
    (set `self.SplinePoint_Location` (.location (`SplineComponent.GetTransformAtSplinePoint` (`self.Spline`) _index "World" false)))
    (set `self.SplinePoint_RotationZ` (+ (.yaw (.rotation (`SplineComponent.GetTransformAtSplinePoint` (`self.Spline`) _index "World" false))) (`self.MeshRotation`)))
    (set `self.SplinePoint_Scale` (.scale (`SplineComponent.GetTransformAtSplinePoint` (`self.Spline`) _index "World" false)))
    (`|ExecutionSequence`
      (:`then_0`
        (if (`|EnumEquality` (`.TypeOfLigth_2_939C1ECD4B0A2153740119AC34A7F802` (break `/Game/DisconnectTemplate/Core/Blueprints/Lights/S_LightParameter` (`self.LightParam`))) "NewEnumerator1")
          (`InstancedStaticMeshComponent.AddInstance` (`self.ISM_StreetLamp`) (`KismetMathLibrary.MakeTransform` (`self.SplinePoint_Location`) (`KismetMathLibrary.MakeRotator` 0.0 0.0 (`self.SplinePoint_RotationZ`)) (`self.SplinePoint_Scale`)) true)
          (`StaticMeshComponent.SetStaticMesh` (`self.ISM_StreetLamp`) (`self.SM_StreetLamp`))
          (if (`self.b_LightIsActive?`)
            (if (`|EnumEquality` (`.LightForm_5_05E2574D41C6295FD24B8C82B2FC0AE7` (break `/Game/DisconnectTemplate/Core/Blueprints/Lights/S_LightParameter` (`self.LightParam`))) "NewEnumerator0")
              (bind _returnvalue (`AddComponent|NODE_AddSpotLightComponent-0` :`bManualAttachment` true :`RelativeTransform` (`KismetMathLibrary.MakeTransform` (`KismetMathLibrary.TransformLocation` (`SplineComponent.GetTransformAtSplinePoint` (`self.Spline`) (`local.L_NumOfSplinePoint`) "World" false) (`StaticMeshSocket.RelativeLocation` (`StaticMesh.FindSocket` (`self.SM_StreetLamp`) "SM_LightPosition"))) (`KismetMathLibrary.MakeRotator` 0.0 (`self.Relative Transform Rotation Y (Pitch)`) (`self.SplinePoint_RotationZ`)) (`self.SplinePoint_Scale`))))
              (bind _output_get (set `local.L_SpotLightComp` _returnvalue))
              (set `local.NumberOfSpotLightPlaced` (`KismetArrayLibrary.Array_Length` (`|MakeArray` _output_get)))
              (`LocalLightComponent.SetIntensityUnits` _output_get (`self.LightIntensityUnit`))
              (`LightComponent.SetIntensity` (`local.L_SpotLightComp`) (`self.LightIntensity`))
              (`LightComponent.SetLightColor` (`local.L_SpotLightComp`) (`self.LightColor`) true)
              (`LocalLightComponent.SetAttenuationRadius` (`local.L_SpotLightComp`) (`self.LightAttenuationRadius`))
              (`SpotLightComponent.SetInnerConeAngle` (`local.L_SpotLightComp`) (`self.LightInnerConeAngle`))
              (`SpotLightComponent.SetOuterConeAngle` (`local.L_SpotLightComp`) (`self.LightOuterConeAngle`))
              (`PointLightComponent.SetSourceRadius` (`local.L_SpotLightComp`) (`self.LightSourceRadius`))
              (`PointLightComponent.SetSoftSourceRadius` (`local.L_SpotLightComp`) (`self.LightSoftSourceRadius`))
              (`PointLightComponent.SetSourceLength` (`local.L_SpotLightComp`) (`self.LightSourceLength`))
              (`|ExecutionSequence`
                (:`then_0`
                  (`LightComponent.SetUseTemperature` (`local.L_SpotLightComp`) _b_usetemperature__2)
                  (if _b_usetemperature__2
                    (`LightComponent.SetTemperature` (`local.L_SpotLightComp`) (`self.LightTemperature`))))
                (:`then_1`
                  (`LightComponentBase.SetCastShadows` (`local.L_SpotLightComp`) (`self.b_CastShadow?`))
                  (`LightComponent.SetIndirectLightingIntensity` (`local.L_SpotLightComp`) (`self.IndirectLightingIntensity`))
                  (`LightComponent.SetVolumetricScatteringIntensity` (`local.L_SpotLightComp`) (`self.VolumetricScatteringIntensity`)))
                (:`then_2`
                  (`PointLightComponent.SetInverseExposureBlend` (`local.L_SpotLightComp`) (`self.InverseExposureBlend`))
                  (`LightComponent.SetSpecularScale` (`local.L_SpotLightComp`) (`self.SpecularScale`))
                  (`LightComponent.SetDiffuseScale` (`local.L_SpotLightComp`) (`self.DiffuseScale`))
                  (`LightComponent.SetShadowBias` (`local.L_SpotLightComp`) (`self.ShadowBias`))
                  (`LightComponent.SetShadowSlopeBias` (`local.L_SpotLightComp`) (`self.ShadowSlopeBias`))
                  (set `LightComponent.ContactShadowLength` (`self.Contact Shadow Length`) (`local.L_SpotLightComp`)))
                (:`then_3`
                  (if (`self.b_LightFunction?`)
                    (if (`LightComponent.bAllowMegaLights` (`local.L_SpotLightComp`))
                      _
                      (else
                        _))
                    (for _index_2 (range (+ (`local.NumberOfSpotLightPlaced`) 1))
                      (if (<= (`KismetMathLibrary.RandomFloatInRangeFromStream` (`self.Stream`) 0.0 1.0) (* (`self.ChanceLightFunction`) _index_2))
                        (`LightComponent.SetLightFunctionMaterial` (`local.L_SpotLightComp`) (`self.LightFunctionMaterial`))
                        (`KismetMaterialLibrary.SetScalarParameterValue` "/Game/DisconnectTemplate/MaterialLibrary/MaterialParameterCollection/MPC_Flickering.MPC_Flickering" "Speed" (`KismetMathLibrary.RandomFloatInRangeFromStream` (`self.Stream`) 10.0 20.0))
                        (`KismetMaterialLibrary.SetScalarParameterValue` "/Game/DisconnectTemplate/MaterialLibrary/MaterialParameterCollection/MPC_Flickering.MPC_Flickering" "Min" (`KismetMathLibrary.RandomFloatInRangeFromStream` (`self.Stream`) -0.1 0.1))
                        (`KismetMaterialLibrary.SetScalarParameterValue` "/Game/DisconnectTemplate/MaterialLibrary/MaterialParameterCollection/MPC_Flickering.MPC_Flickering" "Max" (`KismetMathLibrary.RandomFloatInRangeFromStream` (`self.Stream`) 0.8 1.0))
                        (`LightComponent.SetLightFunctionScale` (`local.L_SpotLightComp`) (`self.LightFunctionScale`))
                        (`LightComponent.SetLightFunctionFadeDistance` (`local.L_SpotLightComp`) (`self.LightFunctionFadeDistance`))
                        (`LightComponent.SetLightFunctionDisabledBrightness` (`local.L_SpotLightComp`) (`self.LightFunctionDisabledBrightness`))))))
                (:`then_4`
                  (if (`self.b_IESProfile?`)
                    (`LightComponent.SetIESTexture` (`local.L_SpotLightComp`) (`self.IESTexture`))
                    (`LightComponent.SetUseIESBrightness` (`local.L_SpotLightComp`) (`self.b_UseIESIntesity?`))
                    (`LightComponent.SetIESBrightnessScale` (`local.L_SpotLightComp`) (`self.IESIntensityScale`)))))))))
      (:`then_1`
        (if (`|EnumEquality` (`.TypeOfLigth_2_939C1ECD4B0A2153740119AC34A7F802` (break `/Game/DisconnectTemplate/Core/Blueprints/Lights/S_LightParameter` (`self.LightParam`))) "NewEnumerator0")
          (`InstancedStaticMeshComponent.AddInstance` (`self.ISM_GarageLight`) (`KismetMathLibrary.MakeTransform` (`self.SplinePoint_Location`) (`KismetMathLibrary.MakeRotator` 0.0 0.0 (`self.SplinePoint_RotationZ`)) (`self.SplinePoint_Scale`)) true)
          (`StaticMeshComponent.SetStaticMesh` (`self.ISM_GarageLight`) (`self.SM_GarageLamp`))
          (if (`self.b_LightIsActive?`)
            (if (`|EnumEquality` (`.LightForm_5_05E2574D41C6295FD24B8C82B2FC0AE7` (break `/Game/DisconnectTemplate/Core/Blueprints/Lights/S_LightParameter` (`self.LightParam`))) "NewEnumerator1")
              (bind _returnvalue_2 (`AddComponent|NODE_AddRectLightComponent-0` :`bManualAttachment` true :`RelativeTransform` (`KismetMathLibrary.MakeTransform` (`KismetMathLibrary.TransformLocation` (`SplineComponent.GetTransformAtSplinePoint` (`self.Spline`) (`local.L_NumOfSplinePoint`) "World" false) (`StaticMeshSocket.RelativeLocation` (`StaticMesh.FindSocket` (`self.SM_GarageLamp`) "SM_LightPosition"))) (`KismetMathLibrary.MakeRotator` (`self.Relative Transform Rotation X (Roll)`) (`self.Relative Transform Rotation Y (Pitch)`) (`self.Relative Transform Rotation Z (Yaw)`)) (`self.SplinePoint_Scale`))))
              (bind _output_get_2 (set `local.L_RecLightComp` _returnvalue_2))
              (set `local.NumberOfRecLight` (`KismetArrayLibrary.Array_Length` (`|MakeArray` _output_get_2)))
              (`LocalLightComponent.SetIntensityUnits` _output_get_2 (`self.LightIntensityUnit`))
              (`LightComponent.SetIntensity` (`local.L_RecLightComp`) (`self.LightIntensity`))
              (`LightComponent.SetLightColor` (`local.L_RecLightComp`) (`self.LightColor`) true)
              (`LocalLightComponent.SetAttenuationRadius` (`local.L_RecLightComp`) (`self.LightAttenuationRadius`))
              (`RectLightComponent.SetSourceWidth` (`local.L_RecLightComp`) (`self.LightSourceWidth`))
              (`RectLightComponent.SetSourceHeight` (`local.L_RecLightComp`) (`self.LightSourceHeight`))
              (`RectLightComponent.SetBarnDoorAngle` (`local.L_RecLightComp`) (`self.LightSourceBarnDoorAngle`))
              (`RectLightComponent.SetBarnDoorLength` (`local.L_RecLightComp`) (`self.LightSourceBarnDoorLength`))
              (`RectLightComponent.SetSourceTexture` (`local.L_RecLightComp`) (`self.LightSourceTexture`))
              (`|ExecutionSequence`
                (:`then_0`
                  (`LightComponent.SetUseTemperature` (`local.L_RecLightComp`) _b_usetemperature_)
                  (if _b_usetemperature_
                    (`LightComponent.SetTemperature` (`local.L_RecLightComp`) (`self.LightTemperature`))))
                (:`then_1`
                  (`LightComponentBase.SetCastShadows` (`local.L_RecLightComp`) (`self.b_CastShadow?`))
                  (`LightComponent.SetIndirectLightingIntensity` (`local.L_RecLightComp`) (`self.IndirectLightingIntensity`))
                  (`LightComponent.SetVolumetricScatteringIntensity` (`local.L_RecLightComp`) (`self.VolumetricScatteringIntensity`)))
                (:`then_2`
                  (`LightComponent.SetSpecularScale` (`local.L_RecLightComp`) (`self.SpecularScale`))
                  (`LightComponent.SetDiffuseScale` (`local.L_RecLightComp`) (`self.DiffuseScale`))
                  (`LightComponent.SetShadowBias` (`local.L_RecLightComp`) (`self.ShadowBias`))
                  (`LightComponent.SetShadowSlopeBias` (`local.L_RecLightComp`) (`self.ShadowSlopeBias`))
                  (set `LightComponent.ContactShadowLength` (`self.Contact Shadow Length`) (`local.L_RecLightComp`)))
                (:`then_3`
                  (if (`self.b_LightFunction?`)
                    (if (`LightComponent.bAllowMegaLights` (`local.L_RecLightComp`))
                      _
                      (else
                        _))
                    (for _index_3 (range (+ (`local.NumberOfRecLight`) 1))
                      (if (<= (`KismetMathLibrary.RandomFloatInRangeFromStream` (`self.Stream`) 0.0 1.0) (* (`self.ChanceLightFunction`) _index_3))
                        (`LightComponent.SetLightFunctionMaterial` (`local.L_RecLightComp`) (`self.LightFunctionMaterial`))
                        (`LightComponent.SetLightFunctionScale` (`local.L_RecLightComp`) (`self.LightFunctionScale`))
                        (`LightComponent.SetLightFunctionFadeDistance` (`local.L_RecLightComp`) (`self.LightFunctionFadeDistance`))
                        (`LightComponent.SetLightFunctionDisabledBrightness` (`local.L_RecLightComp`) (`self.LightFunctionDisabledBrightness`))))))
                (:`then_4`
                  (if (`self.b_IESProfile?`)
                    (`LightComponent.SetIESTexture` (`local.L_RecLightComp`) (`self.IESTexture`))
                    (`LightComponent.SetUseIESBrightness` (`local.L_RecLightComp`) (`self.b_UseIESIntesity?`))
                    (`LightComponent.SetIESBrightnessScale` (`local.L_RecLightComp`) (`self.IESIntensityScale`))))))))))))