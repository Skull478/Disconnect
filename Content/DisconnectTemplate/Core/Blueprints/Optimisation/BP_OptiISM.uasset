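; BP_OptiISM is an optimisation actor that builds instanced static mesh components from the level's StaticMeshActors at runtime.
; Two seconds after BeginPlay, it adds each actor's mesh as a world-space instance, leaving the original actors untouched.
; FindOrCreateISM caches one component per mesh and slot-0 material pair in a map, ignoring other material slots.
; It then prints the map's size on screen.
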(event `self.ReceiveBeginPlay`
  (`KismetSystemLibrary.Delay` 2.0)
  (bind _outactors (`GameplayStatics.GetAllActorsOfClass` "/Script/Engine.StaticMeshActor"))
  (bind _output_get (set `self.LevelStaticMesh` _outactors))
  (for _array_element _output_get
    (bind _staticmeshcomponent (`StaticMeshActor.StaticMeshComponent` _array_element))
    (bind _ism (`self.FindOrCreateISM` (make `/Game/DisconnectTemplate/Core/Blueprints/Optimisation/FMeshAndMat` (`StaticMeshComponent.StaticMesh` _staticmeshcomponent) (`PrimitiveComponent.GetMaterial` _staticmeshcomponent 0))))
    (`InstancedStaticMeshComponent.AddInstance` _ism (`SceneComponent.K2_GetComponentToWorld` _staticmeshcomponent) true))
  (`KismetSystemLibrary.PrintString` (`KismetStringLibrary.Conv_IntToString` (`BlueprintMapLibrary.Map_Length` (`self.StaticMeshCreatedAndISM`))) true true (struct :`G` 0.66 :`B` 1.0 :`A` 1.0) 10.0))

(fn `FindOrCreateISM`
  (params (Struct :type "/Game/DisconnectTemplate/Core/Blueprints/Optimisation/FMeshAndMat Structure (by ref)"))
  (returns (ISM :type "InstancedStaticMeshComponent Object Reference"))
  (bind _struct (`local.Struct`))
  (bind (_mesh _material) (break `/Game/DisconnectTemplate/Core/Blueprints/Optimisation/FMeshAndMat` _struct))
  (bind _value (`BlueprintMapLibrary.Map_Find` (`self.StaticMeshCreatedAndISM`) Struct))
  (`/Engine/EditorBlueprintResources/StandardMacros.IsValid` _value
    (:`Is Valid`
      (return _value))
    (:`Is Not Valid`
      (bind _returnvalue (`AddComponent|NODE_AddInstancedStaticMeshComponent-0`))
      (`BlueprintMapLibrary.Map_Add` (`self.StaticMeshCreatedAndISM`) _struct _returnvalue)
      (`StaticMeshComponent.SetStaticMesh` _returnvalue _mesh)
      (`PrimitiveComponent.SetMaterial` _returnvalue 0 _material)
      (return _returnvalue))))

(fn `UserConstructionScript`)