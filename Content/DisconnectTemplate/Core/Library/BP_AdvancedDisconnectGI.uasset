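; Game instance for the Disconnect template that handles online session events and keeps a map of player roles by ID.
; Accepting an invite destroys the current session, then joins the invited one whether or not that succeeds; shutdown also destroys the session.
; Invite-received and login-status events are re-broadcast, with the previous status passed as the new one.
; Network and travel errors only print red debug messages; other login and talking events are empty.
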(event `self.ReceiveInit`)

(event `self.HandleNetworkError`
  (params (FailureType :type "ENetworkFailure Enum" :default "NetDriverAlreadyExists") (bIsServer :type Boolean))
  ; NETWORK ERROR
  (`KismetSystemLibrary.PrintString` (`KismetStringLibrary.Concat_StrStr` "(BP_AdvancedDisconnectGI) // ERROR - NETWORK ERROR TYPE : " (`|GetEnumeratorNameAsString` FailureType)) true true (struct :`R` 1.0 :`A` 1.0) 10.0))

(event `self.OnPlayerLoginChanged`
  (params (PlayerNum :type Integer))
  ; PLAY NUM LOGIN CHENGED
)

(event `self.OnPlayerLoginStatusChanged`
  (params (PlayerNum :type Integer) (PreviousStatus :type "EBPLoginStatus Enum" :default "NotLoggedIn") (NewStatus :type "EBPLoginStatus Enum" :default "NotLoggedIn") (NewPlayerUniqueNetID :type "BPUniqueNetId Structure"))
  ; LOGIN Status Changed
  (`self.PlayerLoginStatusChanged` PreviousStatus NewPlayerUniqueNetID))

(event `self.OnPlayerTalkingStateChanged`
  (params (PlayerId :type "BPUniqueNetId Structure") (bIsTalking :type Boolean))
  ; TALK
)

(event `self.OnSessionInviteAccepted`
  (params (LocalPlayerNum :type Integer) (PersonInvited :type "BPUniqueNetId Structure") (SessionToJoin :type "BlueprintSessionResult Structure (by ref)"))
  (bind _returnvalue (`GameplayStatics.GetPlayerController` 0))
  ; Session Invite Accepted
  (`DestroySessionCallbackProxy.DestroySession` _returnvalue
    (:`OnSuccess`
      _)
    (:`OnFailure`
      _))
  (`JoinSessionCallbackProxy.JoinSession` _returnvalue SessionToJoin))

(event `self.OnSessionInviteReceived`
  (params (LocalPlayerNum :type Integer) (PersonInviting :type "BPUniqueNetId Structure") (AppId :type String) (SessionToJoin :type "BlueprintSessionResult Structure (by ref)"))
  ; Session Invite Received
  (`self.SessionInviteReceived` LocalPlayerNum PersonInviting AppId SessionToJoin))

(event `self.ReceiveShutdown`
  ; Shutdown
  (`DestroySessionCallbackProxy.DestroySession` (`GameplayStatics.GetPlayerController` 0)))

(event `self.HandleTravelError`
  (params (FailureType :type "ETravelFailure Enum" :default "NoLevel"))
  ; TRAVEL ERROR
  (`KismetSystemLibrary.PrintString` (`KismetStringLibrary.Concat_StrStr` "(BP_AdvancedDisconnectGI) // ERROR - TRAVEL ERROR TYPE : " (`|GetEnumeratorNameAsString` FailureType)) true true (struct :`R` 1.0 :`A` 1.0) 10.0))

(fn `getPCRole`
  (params (Index :type "Integer (by ref)"))
  (returns (Role :type "/Game/DisconnectTemplate/Core/Blueprints/Character/Data/EPlayerRole Enum"))
  (return (`BlueprintMapLibrary.Map_Find` (`self.PlayerIDForRole`) Index)))

(fn `setPCRole`
  (params (ID :type "Integer (by ref)") (Role :type "/Game/DisconnectTemplate/Core/Blueprints/Character/Data/EPlayerRole Enum (by ref)"))
  (`BlueprintMapLibrary.Map_Add` (`self.PlayerIDForRole`) ID Role))