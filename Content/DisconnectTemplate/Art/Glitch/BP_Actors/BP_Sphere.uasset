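; BP_Sphere is a glitch-art actor that publishes its Sphere component's transform to the PC_Data_Box material parameter collection.
; The construction script writes world location, world scale (as Bounds) and forward, right and up axes as vector parameters, exposing an oriented volume to materials reading that collection.
; The event graph is empty, so values update only when construction reruns, with no per-frame tracking.
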(fn `UserConstructionScript`
  (bind _sphere (`self.Sphere`))
  (`KismetMaterialLibrary.SetVectorParameterValue` "/Game/DisconnectTemplate/Art/Glitch/PC/PC_Data_Box.PC_Data_Box" "Location" (`KismetMathLibrary.Conv_VectorToLinearColor` (`SceneComponent.K2_GetComponentLocation` _sphere)))
  (`KismetMaterialLibrary.SetVectorParameterValue` "/Game/DisconnectTemplate/Art/Glitch/PC/PC_Data_Box.PC_Data_Box" "Bounds" (`KismetMathLibrary.Conv_VectorToLinearColor` (`SceneComponent.K2_GetComponentScale` _sphere)))
  (`KismetMaterialLibrary.SetVectorParameterValue` "/Game/DisconnectTemplate/Art/Glitch/PC/PC_Data_Box.PC_Data_Box" "X" (`KismetMathLibrary.Conv_VectorToLinearColor` (`SceneComponent.GetForwardVector` _sphere)))
  (`KismetMaterialLibrary.SetVectorParameterValue` "/Game/DisconnectTemplate/Art/Glitch/PC/PC_Data_Box.PC_Data_Box" "Y" (`KismetMathLibrary.Conv_VectorToLinearColor` (`SceneComponent.GetRightVector` _sphere)))
  (`KismetMaterialLibrary.SetVectorParameterValue` "/Game/DisconnectTemplate/Art/Glitch/PC/PC_Data_Box.PC_Data_Box" "Z" (`KismetMathLibrary.Conv_VectorToLinearColor` (`SceneComponent.GetUpVector` _sphere))))