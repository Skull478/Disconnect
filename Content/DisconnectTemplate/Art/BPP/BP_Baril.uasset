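; BP_Baril is a barrel prop actor with a Wwise fire-barrel sound and an optional point light.
; The construction script assigns the chosen mesh to a hierarchical instanced mesh component and adds one instance.
; If AddLight is set, it spawns a point light component at a set location and Light_Param applies the exposed color, intensity, shadow and scattering settings.
; BeginPlay posts the associated Ak audio event.
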(event `self.ReceiveBeginPlay`
  (`AkGameObject.PostAssociatedAkEvent` :`self` (`self.Play_OBJ_FireBarell`)))

(fn `UserConstructionScript`
  (locals (L_PointLightComp :type "PointLightComponent Object Reference"))
  (`StaticMeshComponent.SetStaticMesh` (`self.HISM_Baril`) (`self.StaticMesh`))
  (`InstancedStaticMeshComponent.AddInstance` (`self.HISM_Baril`) (`KismetMathLibrary.MakeTransform` (0.0 0.0 0.0)) false)
  (if (`self.Add_Light?`)
    (bind _returnvalue (`AddComponent|NODE_AddPointLightComponent-0` :`RelativeTransform` (`KismetMathLibrary.MakeTransform` (`self.PointLight_Location`))))
    (bind _output_get (set `local.L_PointLightComp` _returnvalue))
    (`LightComponent.SetIntensity` _output_get (`self.PointLight_Intensity`))
    (`LocalLightComponent.SetIntensityUnits` (`local.L_PointLightComp`) (`self.PointLight_IntensityUnit`))
    (`LightComponent.SetLightColor` (`local.L_PointLightComp`) (`self.PointLight_Color`) true)
    (`LocalLightComponent.SetAttenuationRadius` (`local.L_PointLightComp`) (`self.PointLight_AttenuationRadius`))
    (`PointLightComponent.SetSourceRadius` (`local.L_PointLightComp`) (`self.PointLight_SourceRadius`))
    (`LightComponent.SetUseTemperature` (`local.L_PointLightComp`) (`self.PointLight_UseTemperature?`))
    (`LightComponent.SetTemperature` (`local.L_PointLightComp`) (`self.PointLight_Temperature`))
    (`LightComponentBase.SetCastShadows` (`local.L_PointLightComp`) (`self.PointLight_CastShadow?`))
    (`LightComponent.SetIndirectLightingIntensity` (`local.L_PointLightComp`) (`self.PointLight_IndirectLightingIntensity`))
    (`LightComponent.SetVolumetricScatteringIntensity` (`local.L_PointLightComp`) (`self.PointLight_VolumetricScatteringIntensity`))))