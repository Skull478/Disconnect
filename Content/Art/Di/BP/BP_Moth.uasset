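; Moth actor that flutters in an irregular orbit around the location its CenterActor has at BeginPlay.
; BeginPlay randomizes the start angle, speed scale and sine phases so each instance moves differently.
; Tick layers sine waves to vary angular speed, flip orbit direction, and wobble radius and height, then sets the location directly.
; It turns to face its frame-to-frame movement when that exceeds a small threshold.
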(event `self.ReceiveBeginPlay`
  (set `self.CenterLocation` (`self.K2_GetActorLocation` (`self.CenterActor`)))
  (set `self.Angle` (`KismetMathLibrary.RandomFloatInRange` 0.0 6.28))
  (set `self.OrbitSpeedScale` (`KismetMathLibrary.RandomFloatInRange` 0.6 1.4))
  (set `self.RadiusNoisePhase` (`KismetMathLibrary.RandomFloatInRange` 0.0 6.28))
  (set `self.VerticalPhase` (`KismetMathLibrary.RandomFloatInRange` 0.0 6.28))
  (set `self.SpeedPhase` (`KismetMathLibrary.RandomFloatInRange` 0.0 6.28))
  (set `self.DirPhase` (`KismetMathLibrary.RandomFloatInRange` 0.0 6.28)))

(event `self.ReceiveTick`
  (params (DeltaSeconds :type "Float (single-precision)"))
  (bind _speedminfactor (`self.SpeedMinFactor`))
  (bind _returnvalue (+ (`self.OrbitRadiusBase`) (* (`self.OrbitRadiusNoiseAmp`) (`KismetMathLibrary.Sin` (+ (* (`self.RunningTimeBP`) 0.8) (`self.RadiusNoisePhase`))))))
  (set `self.RunningTimeBP` (+ (`self.RunningTimeBP`) DeltaSeconds))
  (set `self.OrbitDirectionSign` (`KismetMathLibrary.SelectFloat` 1.0 -1.0 (>= (`KismetMathLibrary.Sin` (+ (* (`self.RunningTimeBP`) (`self.DirChangeSpeed`)) (`self.DirPhase`))) 0.0)))
  (set `self.Angle` (+ (`self.Angle`) (* DeltaSeconds (* (* (* (`self.OrbitSpeedBase`) (`self.OrbitSpeedScale`)) (+ _speedminfactor (* (* (+ (`KismetMathLibrary.Sin` (+ (* (`self.RunningTimeBP`) (`self.SpeedChangeSpeed`)) (`self.SpeedPhase`))) 1.0) 0.5) (- (`self.SpeedMaxFactor`) _speedminfactor)))) (`self.OrbitDirectionSign`)))))
  (bind _output_get (set `self.VerticalOffset` (* (`KismetMathLibrary.Sin` (+ (* (`self.RunningTimeBP`) 1.3) (`self.VerticalPhase`))) (`self.VerticalAmplitude`))))
  (bind _returnvalue_2 (+ (`self.CenterLocation`) (`KismetMathLibrary.MakeVector` (* (`KismetMathLibrary.Cos` (`self.Angle`)) _returnvalue) (* (`KismetMathLibrary.Sin` (`self.Angle`)) _returnvalue) _output_get)))
  (`self.K2_SetActorLocation` _returnvalue_2)
  (bind _returnvalue_3 (- _returnvalue_2 (`self.PreviousLocation`)))
  (if (> (`KismetMathLibrary.VSize` _returnvalue_3) 1.0)
    (`self.K2_SetActorRotation` (`KismetMathLibrary.MakeRotFromX` (`KismetMathLibrary.Normal` _returnvalue_3))))
  (set `self.PreviousLocation` _returnvalue_2))

(fn `UserConstructionScript`)